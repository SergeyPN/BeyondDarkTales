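; BPC_ActivateTrisignOwner is an actor component that turns its TriSign owner into a clickable collectible for a tutorial.
; The owner's collision is off until StartInteractive binds touch input, re-enables collision and spawns a screen-space WB_ArrowTutorial widget above it, tagged Tutorial.
; On touch it unbinds, hides that widget and calls UpdateCountCollectedTrisign on the BPC_CollectingTrisignTutorial component of BP_QuestManager.
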(event Custom|TriSignWasClicked
  (params (FingerIndex :type ETouchIndex%20Enum :default "Touch1") (TouchedActor :type Actor%20Object%20Reference))
  (EventDispatchers|UnbindEventfromOnInputTouchBegin (Components|GetOwner) (delegate Custom|TriSignWasClicked))
  (Development|SetHiddeninGame (Utilities|Array|Get(acopy) (Actor|GetComponentsbyTag (Components|GetOwner) "/Script/UMG.WidgetComponent" "Tutorial")) true false)
  (bind _returnvalue (Actor|GetActorOfClass "/Game/Blueprints/QuestSystem/BP_QuestManager.BP_QuestManager_C"))
  (Default|UpdateCountCollectedTrisign (Actor|GetComponentbyClass _returnvalue "/Game/Blueprints/QuestSystem/CavesLvlTasks/Secondary/BPC_CollectingTrisignTutorial.BPC_CollectingTrisignTutorial_C")))

(event EventBeginPlay
  (Collision|SetActorEnableCollision (Components|GetOwner) false))

(event EventStartInteractive
  (EventDispatchers|BindEventtoOnInputTouchBegin (Components|GetOwner) (delegate Custom|TriSignWasClicked))
  (CallFunction|Init))

(fn Init
  (bind _returnvalue (Game|AddComponentbyClass (Components|GetOwner) "/Script/UMG.WidgetComponent" false))
  (bind _output_get (LocalVariables|SetL_WidgetComponent _returnvalue))
  (Class|WidgetComponent|SetWidgetSpace _output_get "Screen")
  (Transformation|SetWorldRotation (LocalVariables|GetL_WidgetComponent) "0, 0, 0" false false)
  (Transformation|SetWorldLocation (LocalVariables|GetL_WidgetComponent) (+ (Transformation|GetActorLocation (Components|GetOwner)) (* (Math|Vector|GetUpVector (LocalVariables|GetL_WidgetComponent)) 8e+01)) false false)
  (Class|WidgetComponent|SetDrawSize (LocalVariables|GetL_WidgetComponent) "(X=250.000000,Y=250.000000)")
  (Utilities|Array|Add (Variables|/Script/Engine.ActorComponent|GetComponentTags (LocalVariables|GetL_WidgetComponent)) "Tutorial")
  (bind _returnvalue_2 (UserInterface|CreateWidget "/Game/Widgets/New/WB_ArrowTutorial.WB_ArrowTutorial_C" (Game|GetPlayerController 0)))
  (UserInterface|SetWidget (LocalVariables|GetL_WidgetComponent) _returnvalue_2)
  (Collision|SetActorEnableCollision (Components|GetOwner) true))