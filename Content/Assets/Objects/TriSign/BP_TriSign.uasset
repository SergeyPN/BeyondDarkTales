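; Touch-collectible TriSign pickup that adds to the player's per-level count and saves the best result for the current act.
; A touch by a living player fires once: counter increment, sound, particles, hidden mesh, count animation on its widget, and a BP_TrisignManager update.
; When the animation finishes, it writes the count to GameInstance and SaveGame if higher, then destroys itself.
; The construction script tints a dynamic material with two colors.
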(event Custom|FinishShowTriSign
  (bind _trisignwidget (Variables|Default|GetTriSignWidget))
  (Class|UserWidget|UnbindfromAnimationFinished _trisignwidget (Variables|/Game/Widgets/Trisign/WBP_LeftTriSignCollected.WBP_LeftTriSignCollected_C|GetShowCountTriSign _trisignwidget) (delegate Custom|FinishShowTriSign))
  (CallFunction|SaveTrisigns)
  (Actor|DestroyActor))

(event EventBeginPlay
  (bind _aswbp_left_tri_sign_collected (Utilities|Casting|CastToWBP_LeftTriSignCollected (UserInterface|GetUserWidgetObject (Variables|Default|GetWidget))))
  (Variables|Default|SetTriSignWidget _aswbp_left_tri_sign_collected))

(event EventActorOnInputTouchBegin
  (params (FingerIndex :type ETouchIndex%20Enum :default "Touch1"))
  (bind _trisignwidget (Variables|Default|GetTriSignWidget))
  (bind _trisignwidget_2 (Variables|Default|GetTriSignWidget))
  (if (not (Variables|/Game/Blueprints/CameraControl/Camera_PC_test.Camera_PC_test_C|GetbPlayer%20is%20dead? (.AsCamera%20PC%20Test (Utilities|Casting|CastToCamera_PC_test (Game|GetPlayerCharacter 0)))))
    (Utilities|FlowControl|DoOnce false
      (:Completed
        (bind _returnvalue (Actor|GetActorOfClass "/Game/Blueprints/New/Managers/LevelCameraAndDoorManager.LevelCameraAndDoorManager_C"))
        (Rendering|Components|TextRender|SetText (Variables|/Game/Widgets/Trisign/WBP_LeftTriSignCollected.WBP_LeftTriSignCollected_C|GetTextBlockAllCount (Variables|Default|GetTriSignWidget)) (Utilities|Text|ToText(String) (Utilities|String|Append " / " (Utilities|String|ToString(Integer) (Variables|/Game/Blueprints/New/Managers/LevelCameraAndDoorManager.LevelCameraAndDoorManager_C|GetAllCountTriSignsOnLvl _returnvalue)))))
        (bind _result (Math|Integer|IncrementInt (Variables|/Game/Blueprints/New/Main/01CaveMain/BDT_PlayerState.BDT_PlayerState_C|GetCurrentCountCollectStars (.AsBDT%20Player%20State (Utilities|Casting|CastToBDT_PlayerState (Variables|/Script/Engine.Pawn|GetPlayerState (Game|Player|GetPlayerPawn 0))))))
          (:%20%20
            (Rendering|Components|TextRender|SetText (Variables|/Game/Widgets/Trisign/WBP_LeftTriSignCollected.WBP_LeftTriSignCollected_C|GetTextBlockCurrentTriSign (Variables|Default|GetTriSignWidget)) (Utilities|Text|ToText(Integer) _result))
            (Audio|PlaySound2D "/Game/Audio/NEW_SOUNDS/SFX/fx_take_star.fx_take_star" 1.0 1.0 0.0 0 0)
            (Effects|SpawnEmitteratLocation "/Game/Assets/Particles/P_HO.P_HO" (Transformation|GetWorldLocation (Variables|Default|GetTriSign)))
            (Development|SetHiddeninGame (Variables|Default|GetTriSign) true false)
            (UserInterface|Animation|PlayAnimation _trisignwidget_2 (Variables|/Game/Widgets/Trisign/WBP_LeftTriSignCollected.WBP_LeftTriSignCollected_C|GetShowCountTriSign _trisignwidget_2) 0.0 1 "Forward" 1.0 false)
            (bind _returnvalue_2 (Actor|GetActorOfClass "/Game/Blueprints/New/InteractiveBPs/BP_Doors.BP_Doors_C"))
            (bind _returnvalue_3 (Actor|GetActorOfClass "/Game/Blueprints/Trisign/BP_TrisignManager.BP_TrisignManager_C"))
            (Default|UpdateCountCollectedTrisigns _returnvalue_3 (Utilities|String|StringToName (Utilities|GetDisplayName (Utilities|GetOuterObject (Utilities|GetOuterObject _returnvalue_2)))))
            (Class|UserWidget|BindtoAnimationFinished _trisignwidget (Variables|/Game/Widgets/Trisign/WBP_LeftTriSignCollected.WBP_LeftTriSignCollected_C|GetShowCountTriSign _trisignwidget) (delegate Custom|FinishShowTriSign))))))))

(fn ConstructionScript
  (Utilities|FlowControl|Sequence
    (:then_0
      (bind _returnvalue (Rendering|Material|CreateDynamicMaterialInstance (Variables|Default|GetTriSign) 0 "/Game/Assets/Objects/TriSign/Mats/MI_TriSign.MI_TriSign" "None" :!class /Script/Engine.PrimitiveComponent))
      (bind _output_get (Variables|Default|SetMI_TriSign _returnvalue))
      (Rendering|Material|SetVectorParameterValue _output_get "Color1" (Variables|Default|GetColor1) :!class /Script/Engine.MaterialInstanceDynamic)
      (Rendering|Material|SetVectorParameterValue _output_get "Color2" (Variables|Default|GetColor2) :!class /Script/Engine.MaterialInstanceDynamic))))

(fn SaveTrisigns
  (bind _mygameinstance (CallFunction|GetMyGameInstance))
  (bind _mygameinstance_2 (CallFunction|GetMyGameInstance))
  (bind _mygameinstance_3 (CallFunction|GetMyGameInstance))
  (if (> (Variables|/Game/Blueprints/New/Main/01CaveMain/BDT_PlayerState.BDT_PlayerState_C|GetCurrentCountCollectStars (.AsBDT%20Player%20State (Utilities|Casting|CastToBDT_PlayerState (Variables|/Script/Engine.Pawn|GetPlayerState (Game|Player|GetPlayerPawn 0))))) (.CountCollectedTriSigns (Utilities|Struct|BreakStruct_Act (Utilities|Array|Get(acopy) (.Acts (Utilities|Struct|BreakStruct_Season (Utilities|Array|Get(acopy) (Variables|/Game/Blueprints/SaveGame/BP_SaveGame.BP_SaveGame_C|GetSeason (Variables|/Game/Blueprints/GI/BP_GI.BP_GI_C|GetSaveGame _mygameinstance_2)) (Variables|/Game/Blueprints/GI/BP_GI.BP_GI_C|GetCurrentNumSeason _mygameinstance_2)))) (Variables|/Game/Blueprints/GI/BP_GI.BP_GI_C|GetCurrentNumAct _mygameinstance_2)))))
    (Utilities|Struct|SetmembersinStruct_Act (Utilities|Array|Get(acopy) (.Acts (Utilities|Struct|BreakStruct_Season (Utilities|Array|Get(acopy) (Variables|/Game/Blueprints/GI/BP_GI.BP_GI_C|GetSeason _mygameinstance) (Variables|/Game/Blueprints/GI/BP_GI.BP_GI_C|GetCurrentNumSeason _mygameinstance)))) (Variables|/Game/Blueprints/GI/BP_GI.BP_GI_C|GetCurrentNumAct _mygameinstance)) (Variables|/Game/Blueprints/New/Main/01CaveMain/BDT_PlayerState.BDT_PlayerState_C|GetCurrentCountCollectStars (.AsBDT%20Player%20State (Utilities|Casting|CastToBDT_PlayerState (Variables|/Script/Engine.Pawn|GetPlayerState (Game|Player|GetPlayerPawn 0))))))
    (Utilities|Struct|SetmembersinStruct_Act (Utilities|Array|Get(acopy) (.Acts (Utilities|Struct|BreakStruct_Season (Utilities|Array|Get(acopy) (Variables|/Game/Blueprints/SaveGame/BP_SaveGame.BP_SaveGame_C|GetSeason (Variables|/Game/Blueprints/GI/BP_GI.BP_GI_C|GetSaveGame _mygameinstance_3)) (Variables|/Game/Blueprints/GI/BP_GI.BP_GI_C|GetCurrentNumSeason _mygameinstance_3)))) (Variables|/Game/Blueprints/GI/BP_GI.BP_GI_C|GetCurrentNumAct _mygameinstance_3)) (Variables|/Game/Blueprints/New/Main/01CaveMain/BDT_PlayerState.BDT_PlayerState_C|GetCurrentCountCollectStars (.AsBDT%20Player%20State (Utilities|Casting|CastToBDT_PlayerState (Variables|/Script/Engine.Pawn|GetPlayerState (Game|Player|GetPlayerPawn 0))))))
    (SaveGame|SaveGametoSlot (Variables|/Game/Blueprints/GI/BP_GI.BP_GI_C|GetSaveGame (CallFunction|GetMyGameInstance)) "1")))