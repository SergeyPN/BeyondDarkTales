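; Lens flare actor that configures its particle component, PLensFlare, from color, initial size and alpha variables.
; On BeginPlay it creates a dynamic instance of MI_LensFlare on the component and passes those variables in as particle parameters.
; The alpha value also drives the material's Opacity_Contrast scalar.
; Setup runs once at play start, as the construction script is empty.
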(event EventBeginPlay
  (bind _p_lensflare (Variables|Default|GetP_LensFlare))
  (bind _alphaparticle (Variables|Default|GetAlphaParticle))
  (bind _returnvalue (Rendering|Material|CreateDynamicMaterialInstance _p_lensflare 0 "/Game/Assets/Particles/Materials/MI_LensFlare.MI_LensFlare" "None" :!class /Script/Engine.PrimitiveComponent))
  (Variables|Default|SetDynMat _returnvalue)
  (Effects|Components|ParticleSystem|SetColorParameter _p_lensflare "Color" (Variables|Default|GetColor))
  (Effects|Components|ParticleSystem|SetVectorParameter _p_lensflare "InitialSize" (Variables|Default|GetInitialSizeParticle))
  (Rendering|Material|SetScalarParameterValue (Variables|Default|GetDynMat) "Opacity_Contrast" _alphaparticle :!class /Script/Engine.MaterialInstanceDynamic)
  (Effects|Components|ParticleSystem|SetFloatParameter _p_lensflare "Alpha" _alphaparticle))

(fn ConstructionScript)