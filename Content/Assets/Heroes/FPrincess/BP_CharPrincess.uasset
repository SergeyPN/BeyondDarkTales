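; Princess character that materializes and vanishes with a glow effect and can walk to a destination.
; Looping timers interpolate dynamic material emissive parameters for both transitions; disappearing ends with a particle burst, hiding the mesh and teleporting to a fixed location.
; InteractwithObject waits, switches to the animation blueprint and issues an AI move.
; Tick fades the plane's blob-shadow opacity out while falling or flying and back in otherwise.
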(event Custom|BlueMat
  (bind _returnvalue (Rendering|Material|GetScalarParameterValue (Variables|Default|GetDynamicMaterial) "ExpEmiss" :!class /Script/Engine.MaterialInstanceDynamic))
  (Rendering|Material|SetScalarParameterValue (Variables|Default|GetDynamicMaterial) "ExpEmiss" (Math|Interpolation|FInterpTo _returnvalue 1e+01 (Utilities|Time|GetWorldDeltaSeconds) 3.0) :!class /Script/Engine.MaterialInstanceDynamic)
  (bind _returnvalue_2 (Rendering|Material|GetScalarParameterValue (Variables|Default|GetDynamicMaterial) "EmissVisibility" :!class /Script/Engine.MaterialInstanceDynamic))
  (Rendering|Material|SetScalarParameterValue (Variables|Default|GetDynamicMaterial) "EmissVisibility" (Math|Interpolation|FInterpTo _returnvalue_2 0.0 (Utilities|Time|GetWorldDeltaSeconds) 3.0) :!class /Script/Engine.MaterialInstanceDynamic)
  (if (and (== (Math|Interpolation|FInterpTo _returnvalue_2 0.0 (Utilities|Time|GetWorldDeltaSeconds) 3.0) 0.0) (== _returnvalue 1e+01))
    (Utilities|Time|ClearandInvalidateTimerbyHandle (Variables|Default|GetTimerAppear))))

(event Custom|AppearFPrincess
  (Rendering|Material|SetScalarParameterValue (Variables|Default|GetDynamicMaterial) "ExpEmiss" 0.0 :!class /Script/Engine.MaterialInstanceDynamic)
  (Rendering|Material|SetScalarParameterValue (Variables|Default|GetDynamicMaterial) "EmissVisibility" 1.0 :!class /Script/Engine.MaterialInstanceDynamic)
  (bind _returnvalue (Utilities|Time|SetTimerbyEvent (delegate Custom|BlueMat) 0.016 true))
  (Variables|Default|SetTimerAppear _returnvalue))

(event Custom|DissappearFPrincess
  (Development|SetHiddeninGame (Variables|Default|GetParticleSystem) false false)
  (bind _returnvalue (Utilities|Time|SetTimerbyEvent (delegate Custom|FromBlueInWhite) 0.016 true))
  (Variables|Default|SetTimerAppear _returnvalue))

(event Custom|FromBlueInWhite
  (bind _returnvalue (Rendering|Material|GetScalarParameterValue (Variables|Default|GetDynamicMaterial) "ExpEmiss" :!class /Script/Engine.MaterialInstanceDynamic))
  (Rendering|Material|SetScalarParameterValue (Variables|Default|GetDynamicMaterial) "ExpEmiss" (Math|Interpolation|FInterpTo _returnvalue 0.0 (Utilities|Time|GetWorldDeltaSeconds) 3e+01) :!class /Script/Engine.MaterialInstanceDynamic)
  (bind _returnvalue_2 (Rendering|Material|GetScalarParameterValue (Variables|Default|GetDynamicMaterial) "EmissVisibility" :!class /Script/Engine.MaterialInstanceDynamic))
  (Rendering|Material|SetScalarParameterValue (Variables|Default|GetDynamicMaterial) "EmissVisibility" (Math|Interpolation|FInterpTo _returnvalue_2 1.0 (Utilities|Time|GetWorldDeltaSeconds) 3e+01) :!class /Script/Engine.MaterialInstanceDynamic)
  (if (and (== (Math|Interpolation|FInterpTo _returnvalue_2 1.0 (Utilities|Time|GetWorldDeltaSeconds) 3e+01) 1.0) (== _returnvalue 0.0))
    (Utilities|Time|ClearandInvalidateTimerbyHandle (Variables|Default|GetTimerAppear))
    (Components|Activation|Activate (Variables|Default|GetParticleSystem) true)
    (Utilities|FlowControl|Delay 0.05)
    (Development|SetHiddeninGame (Variables|Character|GetMesh) true false)
    (Utilities|FlowControl|Delay 1.0)
    (Transformation|SetActorLocation "30.000000,140.000000,-860.000000" false false)
    (Rendering|Material|SetScalarParameterValue (Variables|Default|GetDynamicMaterial) "EmissVisibility" 0.0 :!class /Script/Engine.MaterialInstanceDynamic)
    (Rendering|Material|SetScalarParameterValue (Variables|Default|GetDynamicMaterial) "ExpEmiss" 1e+01 :!class /Script/Engine.MaterialInstanceDynamic)))

(event EventBeginPlay
  (bind _returnvalue (Rendering|Material|CreateDynamicMaterialInstance (Variables|Character|GetMesh) 0 "/Game/Assets/Heroes/FPrincess/Mats/MI_FPrincess.MI_FPrincess" "None" :!class /Script/Engine.PrimitiveComponent))
  (Variables|Default|SetDynamicMaterial _returnvalue))

(event EventTick
  (params (DeltaSeconds :type Float%20%28single-precision%29))
  (bind _shadowmat (Variables|Default|GetShadowMat))
  (bind _shadowmat_2 (Variables|Default|GetShadowMat))
  (if (or (AI|Components|NavMovement|IsFalling (Variables|Character|GetCharacterMovement)) (Utilities|Enum|Equal(Enum) (Variables|/Script/Engine.CharacterMovementComponent|GetMovementMode (Variables|Character|GetCharacterMovement)) "MOVE_Flying"))
    (bind _returnvalue (Rendering|Material|GetScalarParameterValue _shadowmat_2 "OpacityParameter" :!class /Script/Engine.MaterialInstanceDynamic))
    (if (not (Math|Float|NearlyEqual(Float) _returnvalue 0.0 0.01))
      (Rendering|Material|SetScalarParameterValue _shadowmat_2 "OpacityParameter" (Math|Interpolation|FInterpTo _returnvalue 0.0 (Utilities|Time|GetWorldDeltaSeconds) 3.0) :!class /Script/Engine.MaterialInstanceDynamic))
    (else
      (bind _returnvalue_2 (Rendering|Material|GetScalarParameterValue _shadowmat "OpacityParameter" :!class /Script/Engine.MaterialInstanceDynamic))
      (if (not (Math|Float|NearlyEqual(Float) _returnvalue_2 0.65 0.01))
        (Rendering|Material|SetScalarParameterValue _shadowmat "OpacityParameter" (Math|Interpolation|FInterpTo _returnvalue_2 0.65 (Utilities|Time|GetWorldDeltaSeconds) 1e+01) :!class /Script/Engine.MaterialInstanceDynamic)))))

(event EventInteractwithObject
  (params (DialogToStart :type Array%20of%20Integers) (MoveTo :type Vector :default "0, 0, 0"))
  (if (not (Math|Vector|Equal(Vector) MoveTo "0, 0, 0" 0.0001))
    (Utilities|FlowControl|Delay 2.0)
    (Components|Animation|SetAnimationMode (Variables|Character|GetMesh) "AnimationBlueprint")
    (AI|AIMoveTo self MoveTo 0 5.0 false)))

(fn ConstructionScript
  (bind _returnvalue (Rendering|Material|CreateDynamicMaterialInstance (Variables|Default|GetPlane) 0 0 "None" :!class /Script/Engine.PrimitiveComponent))
  (Variables|Default|SetShadowMat _returnvalue)
  (Variables|/Script/Engine.ParticleSystemComponent|SetAutoAttachSocketName (Variables|Default|GetParticleSystem) "Base-HumanRibcageSocket"))