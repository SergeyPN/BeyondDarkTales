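; BP_CharMax is the playable Max character, moved to target points by AI navigation and turned by timelines with left/right turn montages.
; MovePLayer rotates toward the path, runs AIMoveTo, then starts ladder climbs on looping timers or drag actions.
; Other events handle push/pull montages, parkour jumps, walk-speed switching and item pickup/drop with HUD popup.
; Tick fades a dynamic-material shadow plane while airborne; BeginPlay moves the audio listener to the character.
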(event Custom|Close
  (bind _charactermovement (Variables|Character|GetCharacterMovement))
  (if (not (Variables|Default|GetHide?))
    (bind _speed (Timeline|Timeline_0 PlayFromStart)
      (:Update
        (Variables|/Script/Engine.CharacterMovementComponent|SetMaxWalkSpeed _charactermovement _speed))
      (:Finished
        (Variables|/Script/Engine.CharacterMovementComponent|SetMaxWalkSpeed _charactermovement (Variables|Default|GetRun))))))

(event Custom|ChangeWS
  (bind _charactermovement (Variables|Character|GetCharacterMovement))
  (bind _result (Math|Integer|IncrementInt (Variables|Default|GetSwitch))
    (:%20%20
      (if (== _result 2)
        (Variables|Default|SetSwitch 0))
      (switch int (Variables|Default|GetSwitch)
        (:0
          (Variables|Default|SetHide? false)
          (Variables|/Script/Engine.CharacterMovementComponent|SetMaxWalkSpeed _charactermovement (Variables|Default|GetRun)))
        (:1
          (Variables|Default|SetHide? true)
          (Variables|/Script/Engine.CharacterMovementComponent|SetMaxWalkSpeed _charactermovement (Variables|Default|GetHide)))))))

(event Custom|JumpDownStart
  (params (Condition :type Boolean) (ParkourTypeEnum :type ParkourTypes%20Enum :default "NewEnumerator6") (Condition2 :type Boolean))
  (if Condition
    (Pawn|Components|CharacterMovement|SetMovementMode (Variables|Character|GetCharacterMovement) "MOVE_Flying" 0)
    (Variables|Default|SetParkourTypeEnum ParkourTypeEnum)
    (else
      (if Condition2
        (Character|LaunchCharacter "0, 0,-100.000000" false false))
      (Pawn|Components|CharacterMovement|SetMovementMode (Variables|Character|GetCharacterMovement) "MOVE_Walking" 0)
      (Variables|Default|SetParkourTypeEnum ParkourTypeEnum)
      (Variables|Default|SetOnParcour false))))

(event Custom|PickItem
  (params (ActorSender :type BP%20Pickable%20Simple%20Object%20Reference) (Target :type Actor%20Object%20Reference))
  (bind _returnvalue (Game|GetPlayerController 0))
  (bind _hud (Variables|Default|GetHUD))
  (bind _hud_2 (Variables|Default|GetHUD))
  (bind _playerpawn (Variables|Default|GetPlayerPawn))
  (bind _playerpawn_2 (Variables|Default|GetPlayerPawn))
  (bind _currentplayercontroller (Variables|/Game/Blueprints/CameraControl/Camera_PC_test.Camera_PC_test_C|GetCurrentPlayerController _playerpawn_2))
  (bind _currentplayercontroller_2 (Variables|/Game/Blueprints/CameraControl/Camera_PC_test.Camera_PC_test_C|GetCurrentPlayerController _playerpawn))
  (bind _getitemwidget (Variables|/Game/Blueprints/New/Main/MainMenu/BP_MainMenuHUD.BP_MainMenuHUD_C|GetGetItemWidget _hud))
  (bind _getitemwidget_2 (Variables|/Game/Blueprints/New/Main/MainMenu/BP_MainMenuHUD.BP_MainMenuHUD_C|GetGetItemWidget _hud_2))
  (bind _maininterface_w (Variables|/Game/Blueprints/New/Main/01CaveMain/01CM_PC.01CM_PC_C|GetMainInterface_W _currentplayercontroller))
  (bind _maininterface_w_2 (Variables|/Game/Blueprints/New/Main/01CaveMain/01CM_PC.01CM_PC_C|GetMainInterface_W _currentplayercontroller_2))
  ;[1 1 1] Pick Item
  (Variables|PickableItem|SetPickUpItem ActorSender)
  (CallFunction|StopMovement)
  (Input|DisableInput (Pawn|GetControlledPawn _returnvalue) _returnvalue)
  (if (Utilities|Name|NotEqual(Name) (.RowName (Utilities|Struct|BreakDataTableRowHandle (Variables|/Game/Blueprints/New/InteractiveBPs/BP_ActorMain.BP_ActorMain_C|GetWithSequence? (Variables|PickableItem|GetPickUpItem)))) "Before")
    (Variables|Default|SetLocBeforeMove (Transformation|GetActorForwardVector))
    (bind _newtrack_0 (Timeline|Timeline_2 PlayFromStart)
      (:Update
        (Transformation|SetActorRotation (Math|Rotator|MakeRotator 0.0 0.0 (.yaw (Math|Rotator|Lerp(Rotator) (Transformation|GetActorRotation) (Math|Rotator|FindLookatRotation (Transformation|GetActorLocation) (Transformation|GetActorLocation Target)) _newtrack_0 true))))
        (if (Variables|Default|GetBool1)
          (if (> (Math|Vector|DotProduct (Transformation|GetActorRightVector) (Variables|Default|GetLocBeforeMove)) 0.0)
            (Variables|Default|SetBool1 false)
            (Development|PrintString "left")
            (Animation|Montage|PlayMontage (Variables|Character|GetMesh) "/Game/Assets/Heroes/Max/Anim/RotateL_Montage.RotateL_Montage"
              (:then
                _))
            (elif (< (Math|Vector|DotProduct (Transformation|GetActorRightVector) (Variables|Default|GetLocBeforeMove)) 0.0)
              (Variables|Default|SetBool1 false)
              (Development|PrintString "right")
              (Animation|Montage|PlayMontage (Variables|Character|GetMesh) "/Game/Assets/Heroes/Max/Anim/RotateR_Montage.RotateR_Montage"
                (:then
                  _))
              (else
                (Development|PrintString "straigh"))))
          (Variables|Default|SetLocBeforeMove (Transformation|GetActorForwardVector))))
      (:Finished
        (Animation|Montage|PlayMontage (Variables|Character|GetMesh) "/Game/Assets/Heroes/Max/Anim/Take_Montage.Take_Montage"
          (:then
            (Utilities|FlowControl|Delay 0.1)
            (Default|DestroyActoronPicked (Variables|PickableItem|GetPickUpItem)))
          (:OnCompleted
            (UserInterface|Viewport|AddtoViewport (Variables|/Game/Blueprints/New/Main/MainMenu/BP_MainMenuHUD.BP_MainMenuHUD_C|GetGetItemWidget (Variables|Default|GetHUD)) 1)
            (Widget|SetVisibility (Variables|/Game/Widgets/Inventory/WB_GetItem.WB_GetItem_C|GetBorderGetItem (Variables|/Game/Blueprints/New/Main/MainMenu/BP_MainMenuHUD.BP_MainMenuHUD_C|GetGetItemWidget (Variables|Default|GetHUD))) "Visible")
            (Variables|/Game/Widgets/Inventory/WB_GetItem.WB_GetItem_C|SetActorMain (Variables|/Game/Blueprints/New/Main/MainMenu/BP_MainMenuHUD.BP_MainMenuHUD_C|GetGetItemWidget (Variables|Default|GetHUD)) (Variables|PickableItem|GetPickUpItem))
            (if (== (.a (Variables|/Script/UMG.Button|GetBackgroundColor (Variables|/Game/Widgets/New/MainInterface_W.MainInterface_W_C|GetButtonPause (Variables|/Game/Blueprints/New/Main/01CaveMain/01CM_PC.01CM_PC_C|GetMainInterface_W (Variables|/Game/Blueprints/CameraControl/Camera_PC_test.Camera_PC_test_C|GetCurrentPlayerController (Variables|Default|GetPlayerPawn)))))) 0.0)
              _
              (else
                (UserInterface|Animation|PlayAnimation _maininterface_w_2 (Variables|/Game/Widgets/New/MainInterface_W.MainInterface_W_C|GetShowPauseButton _maininterface_w_2) 0.0 1 "Reverse" 4.0 false)))
            (UserInterface|Animation|PlayAnimation _getitemwidget (Variables|/Game/Widgets/Inventory/WB_GetItem.WB_GetItem_C|GetAnimGetItem _getitemwidget) 0.0 1 "Forward" 2.0 false)))))
    (else
      (Default|DestroyActoronPicked (Variables|PickableItem|GetPickUpItem))
      (UserInterface|Viewport|AddtoViewport (Variables|/Game/Blueprints/New/Main/MainMenu/BP_MainMenuHUD.BP_MainMenuHUD_C|GetGetItemWidget (Variables|Default|GetHUD)) 1)
      (Widget|SetVisibility (Variables|/Game/Widgets/Inventory/WB_GetItem.WB_GetItem_C|GetBorderGetItem (Variables|/Game/Blueprints/New/Main/MainMenu/BP_MainMenuHUD.BP_MainMenuHUD_C|GetGetItemWidget (Variables|Default|GetHUD))) "Visible")
      (Variables|/Game/Widgets/Inventory/WB_GetItem.WB_GetItem_C|SetActorMain (Variables|/Game/Blueprints/New/Main/MainMenu/BP_MainMenuHUD.BP_MainMenuHUD_C|GetGetItemWidget (Variables|Default|GetHUD)) (Variables|PickableItem|GetPickUpItem))
      (if (== (.a (Variables|/Script/UMG.Button|GetBackgroundColor (Variables|/Game/Widgets/New/MainInterface_W.MainInterface_W_C|GetButtonPause (Variables|/Game/Blueprints/New/Main/01CaveMain/01CM_PC.01CM_PC_C|GetMainInterface_W (Variables|/Game/Blueprints/CameraControl/Camera_PC_test.Camera_PC_test_C|GetCurrentPlayerController (Variables|Default|GetPlayerPawn)))))) 0.0)
        _
        (else
          (UserInterface|Animation|PlayAnimation _maininterface_w (Variables|/Game/Widgets/New/MainInterface_W.MainInterface_W_C|GetShowPauseButton _maininterface_w) 0.0 1 "Reverse" 4.0 false)))
      (UserInterface|Animation|PlayAnimation _getitemwidget_2 (Variables|/Game/Widgets/Inventory/WB_GetItem.WB_GetItem_C|GetAnimGetItem _getitemwidget_2) 0.0 1 "Forward" 2.0 false)
      (Audio|PlaySound2D "/Game/Audio/NEW_SOUNDS/SFX/fx_new_item.fx_new_item" 1.0 1.0 0.0 0 0))))

(event Custom|IncreasePowerJump
  (Timeline|TimelineJump PlayFromStart
    (:Update
      (Class|Actor|AddActorWorldTransform (Math|Transform|MakeTransform (* (Math|Vector|GetForwardVector (Transformation|GetActorRotation)) (Variables|Interact|GetPowerOfJumpForward)) "0, 0, 0" "1,1,1") false false))))

(event Custom|Move
  (params (Indx :type Integer))
  (bind _mesh (Variables|Character|GetMesh))
  (bind _mesh_2 (Variables|Character|GetMesh))
  (bind _returnvalue (Components|SkeletalMesh|GetAnimInstance _mesh_2))
  (bind _returnvalue_2 (Components|SkeletalMesh|GetAnimInstance _mesh))
  ;[1 1 1] PushAnimation
  (switch int Indx
    (:0
      (Animation|Montage|MontagePlay _returnvalue_2 "/Game/Assets/Heroes/Max/Anim/PushL_Montage.PushL_Montage" 1.0 "MontageLength" 0.0 true))
    (:1
      (Animation|Montage|MontagePlay _returnvalue_2 "/Game/Assets/Heroes/Max/Anim/PushR_Montage.PushR_Montage" 1.0 "MontageLength" 0.0 true))
    (:2
      (Animation|Montage|MontagePlay _returnvalue "/Game/Assets/Heroes/Max/Anim/Push_Montage.Push_Montage" 1.0 "MontageLength" 0.0 true))
    (:3
      (Animation|Montage|MontagePlay _returnvalue "/Game/Assets/Heroes/Max/Anim/Pull_Montage.Pull_Montage" 1.0 "MontageLength" 0.0 true))))

(event Custom|1234
  (bind _randomlocation (Class|NavigationSystemV1|GetRandomLocationinNavigableRadius (Transformation|GetActorLocation) 1.5e+03 0 0))
  (bind _movementresult (AI|AIMoveTo self _randomlocation 0 5.0 false)
    (:OnSuccess
      (CallFunction|1234))
    (:OnFail
      (Development|PrintString (Utilities|String|EnumtoString _movementresult)))))

(event Custom|DropItem
  (params (ActorSender :type BP%20Actor%20Main%20Object%20Reference) (Target :type Actor%20Object%20Reference))
  (bind _returnvalue (Game|GetPlayerController 0))
  (bind _returnvalue_2 (Game|GetPlayerController 0))
  ;[1 1 1] Drop Item
  (CallFunction|StopMovement)
  (Input|DisableInput (Pawn|GetControlledPawn _returnvalue_2) _returnvalue_2)
  (Variables|Default|SetLocBeforeMove (Transformation|GetActorForwardVector))
  (bind _newtrack_0 (Timeline|Timeline_8 PlayFromStart)
    (:Update
      (Transformation|SetActorRotation (Math|Rotator|MakeRotator 0.0 0.0 (.yaw (Math|Rotator|Lerp(Rotator) (Transformation|GetActorRotation) (Math|Rotator|FindLookatRotation (Transformation|GetActorLocation) (Transformation|GetActorLocation Target)) _newtrack_0 true))))
      (if (Variables|Default|GetBool1)
        (if (> (Math|Vector|DotProduct (Transformation|GetActorRightVector) (Variables|Default|GetLocBeforeMove)) 0.0)
          (Variables|Default|SetBool1 false)
          (Development|PrintString "left")
          (Animation|Montage|PlayMontage (Variables|Character|GetMesh) "/Game/Assets/Heroes/Max/Anim/RotateL_Montage.RotateL_Montage"
            (:then
              _))
          (elif (< (Math|Vector|DotProduct (Transformation|GetActorRightVector) (Variables|Default|GetLocBeforeMove)) 0.0)
            (Variables|Default|SetBool1 false)
            (Development|PrintString "right")
            (Animation|Montage|PlayMontage (Variables|Character|GetMesh) "/Game/Assets/Heroes/Max/Anim/RotateR_Montage.RotateR_Montage"
              (:then
                _))
            (else
              (Development|PrintString "straigh"))))
        (Variables|Default|SetLocBeforeMove (Transformation|GetActorForwardVector))))
    (:Finished
      (Animation|Montage|PlayMontage (Variables|Character|GetMesh) "/Game/Assets/Heroes/Max/Anim/Take_Montage.Take_Montage"
        (:then
          (Utilities|FlowControl|Delay 0.1)
          (Default|DropActorSimple ActorSender))
        (:OnCompleted
          (Input|EnableInput (Pawn|GetControlledPawn _returnvalue) _returnvalue)
          (Variables|Default|SetAbleToPickItem true))))))

(event Custom|JumpDownChange
  (Variables|Default|SetVet2 (Transformation|GetActorLocation))
  (bind _newtrack_0 (Timeline|Timeline_7 PlayFromStart)
    (:Update
      (Transformation|SetActorLocation (Math|Vector|Lerp(Vector) (Variables|Default|GetVet2) (+ (* (Transformation|GetActorForwardVector) 5e+01) (Variables|Default|GetVet2)) (* _newtrack_0 2.0)) false false))
    (:Finished
      (Pawn|Components|CharacterMovement|SetMovementMode (Variables|Character|GetCharacterMovement) "MOVE_Walking" 0))))

(event Custom|MovePLayer
  (params (MousePoint :type Target%20Actor%20Object%20Reference) (LocToGo :type Vector) (StaticAction :type Boolean) (NewParam3 :type Rotator) (NewParam4 :type ParkourTypes%20Enum :default "NewEnumerator0") (LadderEndLoopLoc :type Vector) (DragArrow :type Arrow%20Component%20Object%20Reference) (DragAction :type Boolean) (DragACtor :type BP%20Drag%20Actor%20Object%20Reference) (JumpFallAction :type Boolean))
  (Variables|Default|SetDragACtor DragACtor)
  (if (Variables|Default|GetOnMove)
    (Variables|Default|SetLocToGo LocToGo :!label _label)
    (Variables|Default|SetMiusePoint\ MousePoint)
    (bind _returnvalue (Class|NavigationSystemV1|FindPathtoLocationSynchronously (Transformation|GetActorLocation) LocToGo 0 0))
    (Variables|Default|SetLocBeforeMove (Transformation|GetActorForwardVector))
    (CallFunction|StartActorRotate (Utilities|Array|Get(acopy) (Variables|/Script/NavigationSystem.NavigationPath|GetPathPoints _returnvalue) 1))
    (else
      (Utilities|FlowControl|Sequence
        (:then_0
          (CallFunction|StopMovement)
          (CallFunction|StopActorRotate))
        (:then_1
          (goto _label))))))

(event Custom|StartActorRotate
  (params (Target :type Vector%20%28by%20ref%29))
  (if (not (Math|Float|NearlyEqual(Float) (.yaw (Transformation|GetActorRotation)) (.yaw (Math|Rotator|FindLookatRotation (Transformation|GetActorLocation) Target)) 8.0))
    (bind _newtrack_0 (Timeline|Timeline_1 PlayFromStart)
      (:Update
        (Transformation|SetActorRotation (Math|Rotator|MakeRotator 0.0 0.0 (.yaw (Math|Rotator|Lerp(Rotator) (Transformation|GetActorRotation) (Math|Rotator|FindLookatRotation (Transformation|GetActorLocation) Target) _newtrack_0 true))))
        (if (Variables|Default|GetBool1)
          (if (> (Math|Vector|DotProduct (Transformation|GetActorRightVector) (Variables|Default|GetLocBeforeMove)) 0.0)
            (Variables|Default|SetBool1 false)
            (Development|PrintString "left")
            (Animation|Montage|PlayMontage (Variables|Character|GetMesh) "/Game/Assets/Heroes/Max/Anim/RotateL_Montage.RotateL_Montage"
              (:then
                _))
            (elif (< (Math|Vector|DotProduct (Transformation|GetActorRightVector) (Variables|Default|GetLocBeforeMove)) 0.0)
              (Variables|Default|SetBool1 false)
              (Development|PrintString "right")
              (Animation|Montage|PlayMontage (Variables|Character|GetMesh) "/Game/Assets/Heroes/Max/Anim/RotateR_Montage.RotateR_Montage"
                (:then
                  _))
              (else
                (Development|PrintString "straigh"))))
          (Variables|Default|SetLocBeforeMove (Transformation|GetActorForwardVector))))
      (:Finished
        (Variables|Default|SetOnMove false :!label _label)
        (Variables|Default|SetBool1 true)
        (AI|AIMoveTo self (Variables|Default|GetLocToGo) 0 15.0 false
          (:OnSuccess
            (CallFunction|StopMovement)
            (if (stale Custom|MovePLayer StaticAction)
              (bind _newtrack_0_2 (Timeline|Timeline_3 PlayFromStart)
                (:Update
                  (Transformation|SetActorRotation (Math|Rotator|MakeRotator 0.0 0.0 (.yaw (Math|Rotator|Lerp(Rotator) (Transformation|GetActorRotation) (stale Custom|MovePLayer NewParam3) _newtrack_0_2 true))))
                  (if (Variables|Default|GetBool1)
                    (if (> (Math|Vector|DotProduct (Transformation|GetActorRightVector) (Variables|Default|GetLocBeforeMove)) 0.0)
                      (Variables|Default|SetBool1 false)
                      (Development|PrintString "left")
                      (Animation|Montage|PlayMontage (Variables|Character|GetMesh) "/Game/Assets/Heroes/Max/Anim/RotateL_Montage.RotateL_Montage"
                        (:then
                          _))
                      (elif (< (Math|Vector|DotProduct (Transformation|GetActorRightVector) (Variables|Default|GetLocBeforeMove)) 0.0)
                        (Variables|Default|SetBool1 false)
                        (Development|PrintString "right")
                        (Animation|Montage|PlayMontage (Variables|Character|GetMesh) "/Game/Assets/Heroes/Max/Anim/RotateR_Montage.RotateR_Montage"
                          (:then
                            _))
                        (else
                          (Development|PrintString "straigh"))))
                    (Variables|Default|SetLocBeforeMove (Transformation|GetActorForwardVector))))
                (:Finished
                  (Variables|Default|SetBool1 true)
                  (switch Utilities|FlowControl|Switch|SwitchonParkourTypes (stale Custom|MovePLayer NewParam4)
                    (:NewEnumerator2
                      (Pawn|Components|CharacterMovement|SetMovementMode (Variables|Character|GetCharacterMovement) "MOVE_Flying" 0)
                      (Animation|Montage|PlayMontage (Variables|Character|GetMesh) (Variables|Default|GetMont2)
                        (:OnBlendOut
                          (Animation|Montage|PlayMontage (Variables|Character|GetMesh) "/Game/Assets/Heroes/Max/Anim/LadderLoop_Montage.LadderLoop_Montage"
                            (:then
                              (bind _returnvalue (Utilities|Time|SetTimerbyFunctionName 0 "MoveUpLadder" 0.01 true))
                              (Variables|Default|SetLadUpTim _returnvalue))))))
                    (:NewEnumerator3
                      (Pawn|Components|CharacterMovement|SetMovementMode (Variables|Character|GetCharacterMovement) "MOVE_Flying" 0)
                      (Animation|Montage|PlayMontage (Variables|Character|GetMesh) (Variables|Default|GetMont1)
                        (:OnBlendOut
                          (Animation|Montage|PlayMontage (Variables|Character|GetMesh) "/Game/Assets/Heroes/Max/Anim/LadderLoop1_Montage.LadderLoop1_Montage"
                            (:then
                              (bind _returnvalue_2 (Utilities|Time|SetTimerbyFunctionName 0 "MoveDownLadder" 0.01 true))
                              (Variables|Default|SetLadDownTim _returnvalue_2)))))))))
              (elif (stale Custom|MovePLayer DragAction)
                (bind _newtrack_0_3 (Timeline|Timeline_5 PlayFromStart)
                  (:Update
                    (Transformation|SetActorRotation (Math|Rotator|MakeRotator 0.0 0.0 (.yaw (Math|Rotator|Lerp(Rotator) (Transformation|GetActorRotation) (Transformation|GetWorldRotation (stale Custom|MovePLayer DragArrow)) _newtrack_0_3 true))))
                    (if (Variables|Default|GetBool1)
                      (if (> (Math|Vector|DotProduct (Transformation|GetActorRightVector) (Variables|Default|GetLocBeforeMove)) 0.0)
                        (Variables|Default|SetBool1 false)
                        (Development|PrintString "left")
                        (Animation|Montage|PlayMontage (Variables|Character|GetMesh) "/Game/Assets/Heroes/Max/Anim/RotateL_Montage.RotateL_Montage"
                          (:then
                            _))
                        (elif (< (Math|Vector|DotProduct (Transformation|GetActorRightVector) (Variables|Default|GetLocBeforeMove)) 0.0)
                          (Variables|Default|SetBool1 false)
                          (Development|PrintString "right")
                          (Animation|Montage|PlayMontage (Variables|Character|GetMesh) "/Game/Assets/Heroes/Max/Anim/RotateR_Montage.RotateR_Montage"
                            (:then
                              _))
                          (else
                            (Development|PrintString "straigh"))))
                      (Variables|Default|SetLocBeforeMove (Transformation|GetActorForwardVector))))
                  (:Finished
                    (Variables|Default|SetBool1 true)
                    (Variables|PushItem|SetPushItem? true)
                    (Default|DragWon (Variables|Default|GetDragACtor))))))))))
    (else
      (Audio|Components|Audio|Stop (Variables|Default|GetTimeline_1))
      (goto _label))))

(event Custom|StopActorRotate
  (bind _newtrack_0 (Timeline|Timeline_1 Stop)
    (:Update
      (Transformation|SetActorRotation (Math|Rotator|MakeRotator 0.0 0.0 (.yaw (Math|Rotator|Lerp(Rotator) (Transformation|GetActorRotation) (Math|Rotator|FindLookatRotation (Transformation|GetActorLocation) (stale Custom|StartActorRotate Target)) _newtrack_0 true))))
      (if (Variables|Default|GetBool1)
        (if (> (Math|Vector|DotProduct (Transformation|GetActorRightVector) (Variables|Default|GetLocBeforeMove)) 0.0)
          (Variables|Default|SetBool1 false)
          (Development|PrintString "left")
          (Animation|Montage|PlayMontage (Variables|Character|GetMesh) "/Game/Assets/Heroes/Max/Anim/RotateL_Montage.RotateL_Montage"
            (:then
              _))
          (elif (< (Math|Vector|DotProduct (Transformation|GetActorRightVector) (Variables|Default|GetLocBeforeMove)) 0.0)
            (Variables|Default|SetBool1 false)
            (Development|PrintString "right")
            (Animation|Montage|PlayMontage (Variables|Character|GetMesh) "/Game/Assets/Heroes/Max/Anim/RotateR_Montage.RotateR_Montage"
              (:then
                _))
            (else
              (Development|PrintString "straigh"))))
        (Variables|Default|SetLocBeforeMove (Transformation|GetActorForwardVector))))
    (:Finished
      (Variables|Default|SetOnMove false)
      (Variables|Default|SetBool1 true)
      (AI|AIMoveTo self (Variables|Default|GetLocToGo) 0 15.0 false
        (:OnSuccess
          (CallFunction|StopMovement)
          (if (stale Custom|MovePLayer StaticAction)
            (bind _newtrack_0_2 (Timeline|Timeline_3 PlayFromStart)
              (:Update
                (Transformation|SetActorRotation (Math|Rotator|MakeRotator 0.0 0.0 (.yaw (Math|Rotator|Lerp(Rotator) (Transformation|GetActorRotation) (stale Custom|MovePLayer NewParam3) _newtrack_0_2 true))))
                (if (Variables|Default|GetBool1)
                  (if (> (Math|Vector|DotProduct (Transformation|GetActorRightVector) (Variables|Default|GetLocBeforeMove)) 0.0)
                    (Variables|Default|SetBool1 false)
                    (Development|PrintString "left")
                    (Animation|Montage|PlayMontage (Variables|Character|GetMesh) "/Game/Assets/Heroes/Max/Anim/RotateL_Montage.RotateL_Montage"
                      (:then
                        _))
                    (elif (< (Math|Vector|DotProduct (Transformation|GetActorRightVector) (Variables|Default|GetLocBeforeMove)) 0.0)
                      (Variables|Default|SetBool1 false)
                      (Development|PrintString "right")
                      (Animation|Montage|PlayMontage (Variables|Character|GetMesh) "/Game/Assets/Heroes/Max/Anim/RotateR_Montage.RotateR_Montage"
                        (:then
                          _))
                      (else
                        (Development|PrintString "straigh"))))
                  (Variables|Default|SetLocBeforeMove (Transformation|GetActorForwardVector))))
              (:Finished
                (Variables|Default|SetBool1 true)
                (switch Utilities|FlowControl|Switch|SwitchonParkourTypes (stale Custom|MovePLayer NewParam4)
                  (:NewEnumerator2
                    (Pawn|Components|CharacterMovement|SetMovementMode (Variables|Character|GetCharacterMovement) "MOVE_Flying" 0)
                    (Animation|Montage|PlayMontage (Variables|Character|GetMesh) (Variables|Default|GetMont2)
                      (:OnBlendOut
                        (Animation|Montage|PlayMontage (Variables|Character|GetMesh) "/Game/Assets/Heroes/Max/Anim/LadderLoop_Montage.LadderLoop_Montage"
                          (:then
                            (bind _returnvalue (Utilities|Time|SetTimerbyFunctionName 0 "MoveUpLadder" 0.01 true))
                            (Variables|Default|SetLadUpTim _returnvalue))))))
                  (:NewEnumerator3
                    (Pawn|Components|CharacterMovement|SetMovementMode (Variables|Character|GetCharacterMovement) "MOVE_Flying" 0)
                    (Animation|Montage|PlayMontage (Variables|Character|GetMesh) (Variables|Default|GetMont1)
                      (:OnBlendOut
                        (Animation|Montage|PlayMontage (Variables|Character|GetMesh) "/Game/Assets/Heroes/Max/Anim/LadderLoop1_Montage.LadderLoop1_Montage"
                          (:then
                            (bind _returnvalue_2 (Utilities|Time|SetTimerbyFunctionName 0 "MoveDownLadder" 0.01 true))
                            (Variables|Default|SetLadDownTim _returnvalue_2)))))))))
            (elif (stale Custom|MovePLayer DragAction)
              (bind _newtrack_0_3 (Timeline|Timeline_5 PlayFromStart)
                (:Update
                  (Transformation|SetActorRotation (Math|Rotator|MakeRotator 0.0 0.0 (.yaw (Math|Rotator|Lerp(Rotator) (Transformation|GetActorRotation) (Transformation|GetWorldRotation (stale Custom|MovePLayer DragArrow)) _newtrack_0_3 true))))
                  (if (Variables|Default|GetBool1)
                    (if (> (Math|Vector|DotProduct (Transformation|GetActorRightVector) (Variables|Default|GetLocBeforeMove)) 0.0)
                      (Variables|Default|SetBool1 false)
                      (Development|PrintString "left")
                      (Animation|Montage|PlayMontage (Variables|Character|GetMesh) "/Game/Assets/Heroes/Max/Anim/RotateL_Montage.RotateL_Montage"
                        (:then
                          _))
                      (elif (< (Math|Vector|DotProduct (Transformation|GetActorRightVector) (Variables|Default|GetLocBeforeMove)) 0.0)
                        (Variables|Default|SetBool1 false)
                        (Development|PrintString "right")
                        (Animation|Montage|PlayMontage (Variables|Character|GetMesh) "/Game/Assets/Heroes/Max/Anim/RotateR_Montage.RotateR_Montage"
                          (:then
                            _))
                        (else
                          (Development|PrintString "straigh"))))
                    (Variables|Default|SetLocBeforeMove (Transformation|GetActorForwardVector))))
                (:Finished
                  (Variables|Default|SetBool1 true)
                  (Variables|PushItem|SetPushItem? true)
                  (Default|DragWon (Variables|Default|GetDragACtor)))))))))))

(event EventBeginPlay
  (Class|PlayerController|SetAudioListenerOverride (Game|GetPlayerController 0) (Variables|Default|GetSceneAudioListener) "0, 0, 0" (Math|Rotator|FindLookatRotation (Transformation|GetWorldLocation (Variables|Default|GetSceneAudioListener)) (Camera|GetCameraLocation (Game|GetPlayerCameraManager 0))))
  (bind _asbp_main_menu_hud (Utilities|Casting|CastToBP_MainMenuHUD (HUD|GetHUD (Game|GetPlayerController 0))))
  (Variables|Default|SetHUD _asbp_main_menu_hud)
  (bind _ascamera_pc_test (Utilities|Casting|CastToCamera_PC_test (Game|Player|GetPlayerPawn 0)))
  (Variables|Default|SetPlayerPawn _ascamera_pc_test))

(event EventTick
  (params (DeltaSeconds :type Float%20%28single-precision%29))
  (bind _shadowmat (Variables|Default|GetShadowMat))
  (bind _shadowmat_2 (Variables|Default|GetShadowMat))
  (Variables|Default|SetDeltaSeconds DeltaSeconds)
  (if (or (AI|Components|NavMovement|IsFalling (Variables|Character|GetCharacterMovement)) (Utilities|Enum|Equal(Enum) (Variables|/Script/Engine.CharacterMovementComponent|GetMovementMode (Variables|Character|GetCharacterMovement)) "MOVE_Flying"))
    (bind _returnvalue (Rendering|Material|GetScalarParameterValue _shadowmat_2 "OpacityParameter" :!class /Script/Engine.MaterialInstanceDynamic))
    (if (not (Math|Float|NearlyEqual(Float) _returnvalue 0.0 0.01))
      (Rendering|Material|SetScalarParameterValue _shadowmat_2 "OpacityParameter" (Math|Interpolation|FInterpTo _returnvalue 0.0 (Utilities|Time|GetWorldDeltaSeconds) 3.0) :!class /Script/Engine.MaterialInstanceDynamic))
    (else
      (bind _returnvalue_2 (Rendering|Material|GetScalarParameterValue _shadowmat "OpacityParameter" :!class /Script/Engine.MaterialInstanceDynamic))
      (if (not (Math|Float|NearlyEqual(Float) _returnvalue_2 0.65 0.01))
        (Rendering|Material|SetScalarParameterValue _shadowmat "OpacityParameter" (Math|Interpolation|FInterpTo _returnvalue_2 0.65 (Utilities|Time|GetWorldDeltaSeconds) 1e+01) :!class /Script/Engine.MaterialInstanceDynamic)))))

(event Collision|EventActorBeginOverlap
  (params (OtherActor :type Actor%20Object%20Reference)))

(fn ConstructionScript
  (bind _returnvalue (Rendering|Material|CreateDynamicMaterialInstance (Variables|Default|GetPlane) 0 0 "None" :!class /Script/Engine.PrimitiveComponent))
  (Variables|Default|SetShadowMat _returnvalue)
  (Transformation|AttachComponentToComponent (Variables|Default|GetBackPack) (Variables|Character|GetMesh) "HumanRibcageSocket" "SnapToTarget" "SnapToTarget" "SnapToTarget" true)
  (Variables|/Script/Engine.ParticleSystemComponent|SetAutoAttachSocketName (Variables|Default|GetParticleSystem) "Base-HumanRibcageSocket"))

(fn OnRepNewVar1
  (Animation|PlayAnimMontage "/Game/Assets/Heroes/Max/Anim/JumpUp_Montage.JumpUp_Montage" 1.0 "None"))

(fn StopMovement
  (bind _miusepoint_ (Variables|Default|GetMiusePoint\))
  (Class|NavMovementComponent|StopActiveMovement (Variables|Character|GetCharacterMovement))
  (Variables|Default|SetOnMove true)
  (Utilities|IsValid _miusepoint_
    (:Is%20Valid
      (Actor|DestroyActor _miusepoint_))))

(fn MoveUpLadder
  (Transformation|AddActorWorldOffset (Math|Vector|MakeVector 0.0 0.0 1.0) false true))

(fn MoveDownLadder
  (Transformation|AddActorWorldOffset (Math|Vector|MakeVector 0.0 0.0 -1.0) false true))

(fn JumpUpCheck
  (bind _returnvalue (Transformation|GetActorLocation))
  (bind (_x _y _z) (Math|Vector|BreakVector _returnvalue))
  (Transformation|SetActorLocation (Math|Vector|MakeVector _x _y (+ _z (Variables|Interact|GetJumpHeight))) false false)
  (Variables|Interact|SetJumpHeight 0.0))

(fn JumpDownCheck
  (Character|LaunchCharacter (+ (* (Transformation|GetActorForwardVector) 5e+01) "0, 0,50.000000") false false))