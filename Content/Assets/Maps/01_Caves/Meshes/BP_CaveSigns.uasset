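; BP_CaveSigns is a cave sign actor that can be powered on, animating the opacity of its sign material.
; The construction script applies the selected mesh to SignMesh, so one Blueprint serves several sign variants.
; BeginPlay creates a dynamic instance of MI_CaveSigns on that mesh.
; The PowerOnCaveSign event plays a timeline from the start, feeding its alpha into the SignOpacity parameter.
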(event Custom|PowerOnCaveSign
  (bind _alpha (Timeline|TimelinePowerOn PlayFromStart)
    (:Update
      (Rendering|Material|SetScalarParameterValue (Variables|Default|GetDynMat) "SignOpacity" _alpha :!class /Script/Engine.MaterialInstanceDynamic))))

(event EventBeginPlay
  (bind _returnvalue (Rendering|Material|CreateDynamicMaterialInstance (Variables|Default|GetSignMesh) 0 "/Game/Assets/Maps/01_Caves/Mats/MI_CaveSigns.MI_CaveSigns" "SignOpacity" :!class /Script/Engine.PrimitiveComponent))
  (Variables|Default|SetDynMat _returnvalue))

(fn ConstructionScript
  (Components|StaticMesh|SetStaticMesh (Variables|Default|GetSignMesh) (Variables|Default|GetSelectSignMesh)))