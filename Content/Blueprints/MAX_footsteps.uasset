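; Animation notify that plays surface-dependent footstep sounds for the MAX character.
; On notify, it traces a short distance straight down from the mesh's location and spawns the footstep Sound Cue there.
; The hit physical material's display name is looked up in the Materials array, and its index sets the cue's "Materials" integer parameter to select the surface sound.
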(fn ReceivedNotify
  (params (MeshComp :type Skeletal%20Mesh%20Component%20Object%20Reference) (Animation :type Anim%20Sequence%20Base%20Object%20Reference))
  (bind _returnvalue (Transformation|GetWorldLocation MeshComp))
  (bind _outhit (Collision|LineTraceByChannel _returnvalue (- _returnvalue "0, 0,50.000000") "TraceTypeQuery1" false 0 "None"))
  (bind _returnvalue_2 (Audio|SpawnSoundatLocation "/Game/Audio/NEW_SOUNDS/CUES/CuesFX/fs_max_footsteps_CUE.fs_max_footsteps_CUE" _returnvalue "0, 0, 0" 1.0 1.0 0.0 "/Game/Audio/NEW_SOUNDS/ATTENUATIONS/SA_max_footsteps.SA_max_footsteps" 0))
  (Utilities|IsValid _returnvalue_2
    (:Is%20Valid
      (Effects|Components|ParticleSystem|SetIntParameter _returnvalue_2 "Materials" (Utilities|Array|FindItem (LocalVariables|GetMaterials) (Utilities|GetDisplayName (.PhysMat (Collision|BreakHitResult _outhit)))))
      (return false))))