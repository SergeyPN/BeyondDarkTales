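; Quest component that tracks completion of a primary quest's secondary tasks.
; Each update event increments a completed-task counter and looks up BP_QuestManager in the level to fetch the primary quest by its QuestTag.
; When the counter equals the number of that quest's secondary quests, the component destroys itself.
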(event Custom|UpdateCountCompleteSecondaryTasks
  (Math|Integer|IncrementInt (Variables|Default|GetCurrentCountCompletedSecondaryTasks)
    (:%20%20
      (bind _returnvalue (Actor|GetActorOfClass "/Game/Blueprints/QuestSystem/BP_QuestManager.BP_QuestManager_C"))
      (if (== (Utilities|Map|Length (.SecondaryQuests (Utilities|Struct|BreakS_SetPrimaryQuests (Default|GetPrimaryQuest _returnvalue (Variables|Default|GetQuestTag))))) (Variables|Default|GetCurrentCountCompletedSecondaryTasks))
        (Components|DestroyComponent)))))