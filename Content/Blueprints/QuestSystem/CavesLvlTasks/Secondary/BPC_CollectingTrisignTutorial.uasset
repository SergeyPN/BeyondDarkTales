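; Quest component for the caves level's secondary tutorial task of collecting TriSigns.
; On BeginPlay it counts all BP_TriSign actors in the level as the target total.
; An update event increments the collected count and, when it matches that total, enables the first BP_Static actor tagged "Freska", then destroys the component.
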(event Custom|UpdateCountCollectedTrisign
  (bind _result (Math|Integer|IncrementInt (Variables|Default|GetCurrentCountCollectedTrisign))
    (:%20%20
      (if (== _result (Variables|Default|GetCountTutorialTrisign))
        (bind _outactors (Actor|GetAllActorsOfClasswithTag "/Game/Blueprints/New/InteractiveBPs/BP_Static.BP_Static_C" "Freska"))
        (Default|Enable/DisableActor (Utilities|Array|Get(acopy) _outactors) true)
        (Components|DestroyComponent)))))

(event EventBeginPlay
  (|CallParentFunction)
  (bind _outactors (Actor|GetAllActorsOfClass "/Game/Assets/Objects/TriSign/BP_TriSign.BP_TriSign_C"))
  (Variables|Default|SetCountTutorialTrisign (Utilities|Array|Length _outactors)))