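; BPC_QuestBase is a quest base component that ties a quest's state to the component's lifetime.
; On BeginPlay it finds BP_QuestManager in the level and sets the state for its QuestTag.
; EndPlay passes its reason to DestroyHandler, which sets a second state on the manager only when the reason is Destroyed, ignoring other end reasons.
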(event EventBeginPlay
  (bind _returnvalue (Actor|GetActorOfClass "/Game/Blueprints/QuestSystem/BP_QuestManager.BP_QuestManager_C"))
  (Default|SetStateQuest _returnvalue (Variables|Default|GetQuestTag) "NewEnumerator1"))

(event EventEndPlay
  (params (EndPlayReason :type EEndPlayReason%20Enum :default "Destroyed"))
  (CallFunction|DestroyHandler EndPlayReason))

(fn DestroyHandler
  (params (TypeEnd :type EEndPlayReason%20Enum :default "Destroyed"))
  (if (Utilities|Enum|Equal(Enum) TypeEnd "Destroyed")
    (bind _returnvalue (Actor|GetActorOfClass "/Game/Blueprints/QuestSystem/BP_QuestManager.BP_QuestManager_C"))
    (Default|SetStateQuest _returnvalue (Variables|Default|GetQuestTag) "NewEnumerator2")
    (return _returnvalue)))