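; Actor component that ends a quest when the actor it is attached to ends play.
; On BeginPlay it binds to the owner's OnEndPlay, without filtering on the end reason.
; When that fires, it finds the BP_QuestManager actor, calls DestroySelf on the first BPC_QuestBase component with a matching QuestTag, then destroys itself.
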(event Custom|EndPlayOwner
  (params (Actor :type Actor%20Object%20Reference) (EndPlayReason :type EEndPlayReason%20Enum :default "Destroyed"))
  (bind _returnvalue (Actor|GetActorOfClass "/Game/Blueprints/QuestSystem/BP_QuestManager.BP_QuestManager_C"))
  (bind _array_element (Utilities|Array|ForEachLoopwithBreak (Actor|GetComponentsByClass _returnvalue "/Game/Blueprints/QuestSystem/BPC_QuestBase.BPC_QuestBase_C") :!label _label)
    (:LoopBody
      (if (== (Variables|/Game/Blueprints/QuestSystem/BPC_QuestBase.BPC_QuestBase_C|GetQuestTag _array_element) (Variables|Default|GetQuestTag))
        (Default|DestroySelf _array_element)
        (goto _label Break)))
    (:Completed
      (Components|DestroyComponent))))

(event EventBeginPlay
  (Game|BindEventtoOnEndPlay (Components|GetOwner) (delegate Custom|EndPlayOwner)))