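; Actor component that starts a set of quests once the owning interactive actor's dialog ends.
; On BeginPlay it binds to the owner BP_InteractiveActor's dialog-end dispatcher, then on firing unbinds, activates the quests and destroys itself.
; Each QuestKey tag with fewer than two dot-separated parts is shown as a primary quest through MainInterface_W; deeper tags are activated through BP_QuestManager.
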(event Custom|DialogEndDispatcher_Event
  (bind _asbp_interactive_actor (Utilities|Casting|CastToBP_InteractiveActor (Components|GetOwner)))
  (EventDispatchers|UnbindEventfromDialogEndDispatcher _asbp_interactive_actor (delegate Custom|DialogEndDispatcher_Event))
  (CallFunction|ActivateQuests)
  (Components|DestroyComponent))

(event EventBeginPlay
  (bind _asbp_interactive_actor (Utilities|Casting|CastToBP_InteractiveActor (Components|GetOwner)))
  (EventDispatchers|BindEventtoDialogEndDispatcher _asbp_interactive_actor (delegate Custom|DialogEndDispatcher_Event)))

(fn ActivateQuests
  (bind _returnvalue (Actor|GetActorOfClass "/Game/Blueprints/QuestSystem/BP_QuestManager.BP_QuestManager_C"))
  (LocalVariables|SetL_QuestManager _returnvalue)
  (for _array_element (Variables|Default|GetQuest%20Key)
    (LocalVariables|SetL_QuestTag _array_element)
    (if (< (Utilities|Array|Length (Utilities|String|ParseIntoArray (Utilities|String|ToString(Name) (GameplayTags|GetTagName _array_element)) ".")) 2)
      (bind _foundwidgets (Widget|GetAllWidgetsOfClass "/Game/Widgets/New/MainInterface_W.MainInterface_W_C" true))
      (Default|ShowPrimaryQuest (Utilities|Array|Get(acopy) _foundwidgets) (LocalVariables|GetL_QuestTag))
      (else
        (Default|ActivateQuest (LocalVariables|GetL_QuestManager) (LocalVariables|GetL_QuestTag)))))
  (return))