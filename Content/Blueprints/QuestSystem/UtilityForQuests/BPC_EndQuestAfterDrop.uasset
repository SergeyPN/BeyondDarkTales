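; Actor component that ends a tagged quest when the drop it is attached to finishes.
; On BeginPlay it casts its owner to BP_DropMain and binds FinishQuest to the drop-end dispatcher.
; FinishQuest searches the BP_QuestManager's BPC_QuestBase components, calls DestroySelf on the first with a matching QuestTag, then destroys this component.
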(event Custom|FinishQuest
  (bind _returnvalue (Actor|GetActorOfClass "/Game/Blueprints/QuestSystem/BP_QuestManager.BP_QuestManager_C"))
  (bind _array_element (Utilities|Array|ForEachLoopwithBreak (Actor|GetComponentsByClass _returnvalue "/Game/Blueprints/QuestSystem/BPC_QuestBase.BPC_QuestBase_C") :!label _label)
    (:LoopBody
      (if (== (Variables|/Game/Blueprints/QuestSystem/BPC_QuestBase.BPC_QuestBase_C|GetQuestTag _array_element) (Variables|Default|GetQuestTag))
        (Default|DestroySelf _array_element)
        (goto _label Break)))
    (:Completed
      (Components|DestroyComponent))))

(event EventBeginPlay
  (bind _asbp_drop_main (Utilities|Casting|CastToBP_DropMain (Components|GetOwner)))
  (EventDispatchers|BindEventtoDropEndDispatcher _asbp_drop_main (delegate Custom|FinishQuest)))