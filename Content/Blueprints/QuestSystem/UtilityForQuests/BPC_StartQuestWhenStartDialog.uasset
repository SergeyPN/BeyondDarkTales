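; Actor component that activates a configured quest when dialog starts on its owning BP_InteractiveActor.
; On BeginPlay it binds to the owner's dialog-start dispatcher, though the handler is named for dialog end.
; When fired, it unbinds, finds BP_QuestManager in the level, calls ActivateQuest with QuestKey, and destroys itself, making it a one-shot trigger.
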(event Custom|DialogEndDispatcher_Event
  (bind _asbp_interactive_actor (Utilities|Casting|CastToBP_InteractiveActor (Components|GetOwner)))
  (EventDispatchers|UnbindEventfromDialogStartDispatcher _asbp_interactive_actor (delegate Custom|DialogEndDispatcher_Event))
  (bind _returnvalue (Actor|GetActorOfClass "/Game/Blueprints/QuestSystem/BP_QuestManager.BP_QuestManager_C"))
  (Default|ActivateQuest _returnvalue (Variables|Default|GetQuest%20Key))
  (Components|DestroyComponent))

(event EventBeginPlay
  (bind _asbp_interactive_actor (Utilities|Casting|CastToBP_InteractiveActor (Components|GetOwner)))
  (EventDispatchers|BindEventtoDialogStartDispatcher _asbp_interactive_actor (delegate Custom|DialogEndDispatcher_Event)))