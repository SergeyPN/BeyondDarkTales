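; Actor component that ends a specific quest once the dialog of its owning BP_InteractiveActor finishes.
; On BeginPlay it binds to the owner's dialog-end dispatcher.
; When that fires, it unbinds, searches BP_QuestManager's BPC_QuestBase components for the first matching QuestTag and calls DestroySelf on it.
; It then destroys itself, so it acts as a one-shot trigger.
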(event Custom|FinishQuest
  (bind _asbp_interactive_actor (Utilities|Casting|CastToBP_InteractiveActor (Components|GetOwner)))
  (EventDispatchers|UnbindEventfromDialogEndDispatcher _asbp_interactive_actor (delegate Custom|FinishQuest))
  (bind _returnvalue (Actor|GetActorOfClass "/Game/Blueprints/QuestSystem/BP_QuestManager.BP_QuestManager_C"))
  (bind _array_element (Utilities|Array|ForEachLoopwithBreak (Actor|GetComponentsByClass _returnvalue "/Game/Blueprints/QuestSystem/BPC_QuestBase.BPC_QuestBase_C") :!label _label)
    (:LoopBody
      (if (== (Variables|/Game/Blueprints/QuestSystem/BPC_QuestBase.BPC_QuestBase_C|GetQuestTag _array_element) (Variables|Default|GetQuestTag))
        (Default|DestroySelf _array_element)
        (goto _label Break)))
    (:Completed
      (Components|DestroyComponent))))

(event EventBeginPlay
  (bind _asbp_interactive_actor (Utilities|Casting|CastToBP_InteractiveActor (Components|GetOwner)))
  (EventDispatchers|BindEventtoDialogEndDispatcher _asbp_interactive_actor (delegate Custom|FinishQuest)))