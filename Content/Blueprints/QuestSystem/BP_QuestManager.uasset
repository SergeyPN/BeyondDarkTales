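; Quest manager Blueprint that holds the current level's quests, activates them and tracks their states.
; On BeginPlay it copies the quest map from the DT_Quests row named after the level.
; Gameplay tags split on dots address a primary quest or its nested secondary quest for lookup, activation and state writes.
; Activation adds the quest's component class to the manager, async-loading the soft class if needed.
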(event Custom|CreateQuest
  (params (AssetClass :type Object%20Soft%20Class%20Reference))
  (bind _output (Utilities|ResolveSoftReference AssetClass))
  (if (Utilities|IsValidClass _output)
    _
    (else
      (Utilities|AsyncLoadClassAsset AssetClass
        (:Completed
          _))))
  (bind _asactor_component (Utilities|Casting|CastToActorComponentClass _output))
  (Game|AddComponentbyClass _asactor_component))

(event EventBeginPlay
  (bind _returnvalue (Game|GetCurrentLevelName true))
  (bind _returnvalue_2 (Utilities|GetDataTableRow "/Game/Blueprints/QuestSystem/DT_Quests.DT_Quests" (Utilities|String|StringToName _returnvalue))
    (:then
      (Variables|Default|SetQuests (Utilities|Struct|BreakS_SetQuests _returnvalue_2)))))

(fn ConstructionScript)

(fn GetPrimaryQuest
  (params (TagPrimaryQuest :type Gameplay%20Tag%20Structure))
  (return (.Value (Utilities|Map|Find (Variables|Default|GetQuests) (GameplayTags|GetTagName TagPrimaryQuest)))))

(fn GetSecondaryQuest
  (params (SecondaryQuestTag :type Gameplay%20Tag%20Structure))
  (LocalVariables|SetL_TagsQuests (Utilities|String|ParseIntoArray (Utilities|String|ToString(Name) (GameplayTags|GetTagName SecondaryQuestTag)) "."))
  (return (.Value (Utilities|Map|Find (.SecondaryQuests (Utilities|Struct|BreakS_SetPrimaryQuests (.Value (Utilities|Map|Find (Variables|Default|GetQuests) (Utilities|String|StringToName (Utilities|Array|Get(acopy) (LocalVariables|GetL_TagsQuests))))))) (Utilities|String|StringToName (Utilities|Array|Get(acopy) (LocalVariables|GetL_TagsQuests) 1))))))

(fn ActivateQuest
  (params (QuestKey :type Gameplay%20Tag%20Structure))
  (LocalVariables|SetL_QuestsTags (Utilities|String|ParseIntoArray (Utilities|String|ToString(Name) (GameplayTags|GetTagName QuestKey)) "."))
  (LocalVariables|SetL_QuestClass (.PrimaryQuestComponent (Utilities|Struct|BreakS_SetPrimaryQuests (.Value (Utilities|Map|Find (Variables|Default|GetQuests) (Utilities|String|StringToName (Utilities|Array|Get(acopy) (LocalVariables|GetL_QuestsTags))))))))
  (if (Utilities|Array|IsValidIndex (LocalVariables|GetL_QuestsTags) 1)
    (bind _output_get (LocalVariables|SetL_QuestClass (.QuestComponent (Utilities|Struct|BreakS_SecondaryQuest (.Value (Utilities|Map|Find (.SecondaryQuests (Utilities|Struct|BreakS_SetPrimaryQuests (.Value (Utilities|Map|Find (Variables|Default|GetQuests) (Utilities|String|StringToName (Utilities|Array|Get(acopy) (LocalVariables|GetL_QuestsTags))))))) (Utilities|String|StringToName (Utilities|Array|Get(acopy) (LocalVariables|GetL_QuestsTags) 1))))))))
    (CallFunction|CreateQuest _output_get)
    (else
      (CallFunction|CreateQuest (LocalVariables|GetL_QuestClass)))))

(fn SetStateQuest
  (params (QuestTag :type Gameplay%20Tag%20Structure) (StateQuest :type E_StateQuest%20Enum :default "NewEnumerator0"))
  (bind _output_get (LocalVariables|SetL_QuestsTags (Utilities|String|ParseIntoArray (Utilities|String|ToString(Name) (GameplayTags|GetTagName QuestTag)) ".")))
  (switch int (Utilities|Array|Length _output_get)
    (:1
      ;[1 1 1] PrimaryTask
      (bind _structout (Utilities|Struct|SetmembersinS_SetPrimaryQuests (.Value (Utilities|Map|Find (Variables|Default|GetQuests) (Utilities|String|StringToName (Utilities|Array|Get(acopy) (LocalVariables|GetL_QuestsTags))))) StateQuest))
      (Utilities|Map|Add (Variables|Default|GetQuests) (Utilities|String|StringToName (Utilities|Array|Get(acopy) (LocalVariables|GetL_QuestsTags))) _structout))
    (:2
      ;[1 1 1] SecondaryTask
      (bind _output_get_2 (LocalVariables|SetL_SecondaryTasks (.SecondaryQuests (Utilities|Struct|BreakS_SetPrimaryQuests (.Value (Utilities|Map|Find (Variables|Default|GetQuests) (Utilities|String|StringToName (Utilities|Array|Get(acopy) (LocalVariables|GetL_QuestsTags)))))))))
      (bind _structout_2 (Utilities|Struct|SetmembersinS_SecondaryQuest (.Value (Utilities|Map|Find _output_get_2 (Utilities|String|StringToName (Utilities|Array|Get(acopy) (LocalVariables|GetL_QuestsTags) 1)))) StateQuest))
      (Utilities|Map|Add (LocalVariables|GetL_SecondaryTasks) (Utilities|String|StringToName (Utilities|Array|Get(acopy) (LocalVariables|GetL_QuestsTags) 1)) _structout_2)
      (bind _structout_3 (Utilities|Struct|SetmembersinS_SetPrimaryQuests (.Value (Utilities|Map|Find (Variables|Default|GetQuests) (Utilities|String|StringToName (Utilities|Array|Get(acopy) (LocalVariables|GetL_QuestsTags))))) (LocalVariables|GetL_SecondaryTasks)))
      (Utilities|Map|Add (Variables|Default|GetQuests) (Utilities|String|StringToName (Utilities|Array|Get(acopy) (LocalVariables|GetL_QuestsTags))) _structout_3))))