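; Test camera and input Blueprint that drives BP_CharMax and LevelCamera, applying a skin from MyGameInstance at startup.
; Axis and joystick input move the character relative to camera yaw, while Tick offsets the camera by character velocity or push direction.
; Mouse wheel zooms, middle-drag pans with sweeps, and touches feed CameraManager, with taps pressing widgets and showing an effect.
; Tap-to-move via traced, navmesh-projected TargetActor markers remains but is disconnected.
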(event Custom|SingleTap
  (params (PositionTouch :type Vector))
  (bind _charactermax (Variables|Default|GetCharacterMax))
  ;[1 1 1] PlayerController
  (Development|PrintString "!!" true true "(R=1.000000,G=0.000000,B=0.067656,A=1.000000)")
  (if (not (Variables|Default|GetPuzzle))
    (Class|WidgetInteractionComponent|PressPointerKey (Variables|Default|GetWidgetInteraction) "Touch1")
    (Utilities|IsValid _charactermax
      (:Is%20Valid
        (if (not (Variables|/Game/Assets/Heroes/Max/BP_CharMax.BP_CharMax_C|GetOnParcour _charactermax))
          (if (not (Variables|/Game/Assets/Heroes/Max/BP_CharMax.BP_CharMax_C|GetPushItem? (Variables|Default|GetCharacterMax)))
            (CallFunction|TouchEffect PositionTouch)))))))

(event Custom|MoveFromJoystick
  (params (Direction :type Vector%202D%20Structure))
  (bind _levelcamera (Variables|Default|GetLevelCamera))
  (bind _returnvalue (Transformation|GetActorRotation _levelcamera))
  (bind _yaw (Math|Rotator|BreakRotator _returnvalue))
  (bind _returnvalue_2 (Math|Rotator|MakeRotator 0.0 0.0 _yaw))
  ;[0.1767 1 0.04638] New moving character
  (Pawn|Input|AddMovementInput (Variables|Default|GetCharacterMax) (Math|Vector|GetForwardVector _returnvalue_2) (.x Direction) false)
  (Pawn|Input|AddMovementInput (Variables|Default|GetCharacterMax) (Math|Vector|GetRightVector _returnvalue_2) (.y Direction) false))

(event EventBeginPlay
  ;[1 1 1] BP
  (bind _outactors (Actor|GetAllActorsOfClass "/Game/Assets/Heroes/Max/BP_CharMax.BP_CharMax_C"))
  (Variables|Default|SetCharacterMax (Utilities|Array|Get(acopy) _outactors))
  (Utilities|FlowControl|Delay 0.5)
  (bind _asmy_game_instance (Utilities|Casting|CastToMyGameInstance (Game|GetGameInstance)))
  (bind _array_element (Utilities|Array|ForEachLoopwithBreak (Variables|/Game/Blueprints/MyGameInstance.MyGameInstance_C|GetSkins _asmy_game_instance) :!label _label)
    (:LoopBody
      (if (Utilities|Enum|Equal(Enum) (.StatusSkin (Utilities|Struct|BreakStruct_Skins _array_element)) "NewEnumerator0")
        (Class|SkinnedMeshComponent|SetSkeletalMesh (Variables|/Script/Engine.Character|GetMesh (Variables|Default|GetCharacterMax)) (.Mesh (Utilities|Struct|BreakStruct_Skins _array_element)) true)
        (goto _label Break)))
    (:Completed
      (bind _as01cm_pc (Utilities|Casting|CastTo01CM_PC (Game|GetPlayerController 0)))
      (Variables|Default|SetCurrentPlayerController _as01cm_pc))))

(event EventTick
  (params (DeltaSeconds :type Float%20%28single-precision%29))
  (bind _charactermax (Variables|Default|GetCharacterMax))
  (bind _charactermax_2 (Variables|Default|GetCharacterMax))
  (bind _returnvalue (Transformation|GetActorLocation _charactermax_2))
  (bind _charactermovement (Variables|/Script/Engine.Character|GetCharacterMovement _charactermax))
  ;[1 1 1] Tracking camera
  (Utilities|IsValid (Variables|Default|GetLevelCamera)
    (:Is%20Valid
      (if (Variables|/Game/Assets/Heroes/Max/BP_CharMax.BP_CharMax_C|GetPushItem? (Variables|Default|GetCharacterMax))
        (Transformation|AddActorWorldOffset (Variables|Default|GetLevelCamera) (Variables|/Game/Assets/Heroes/Max/BP_CharMax.BP_CharMax_C|GetDirectionDragObject (Variables|Default|GetCharacterMax)))
        (elif (AI|Components|NavMovement|IsFalling (Variables|/Script/Engine.Character|GetCharacterMovement (Variables|Default|GetCharacterMax)))
          (bind _outhit (Collision|LineTraceByChannel _returnvalue (+ _returnvalue (Math|Vector|MakeVector 0.0 0.0 (+ (.z (Transformation|GetActorLocation (Variables|Default|GetCharacterMax))) -1e+03))) "TraceTypeQuery1" false 0 "None"))
          (if (.bBlockingHit (Collision|BreakHitResult _outhit))
            (Transformation|AddActorWorldOffset (Variables|Default|GetLevelCamera) (* (/ (Variables|/Script/Engine.MovementComponent|GetVelocity _charactermovement) (Variables|/Script/Engine.CharacterMovementComponent|GetMaxWalkSpeed _charactermovement)) (* (Utilities|Time|GetWorldDeltaSeconds) 3.2e+02)) :!label _label))
          (else
            (goto _label)))))))

(event Input|AxisEvents|InputAxisMoveForward
  (params (AxisValue :type Float%20%28single-precision%29))
  ;[0.1767 1 0.04638] New moving character
  (Pawn|Input|AddMovementInput (Variables|Default|GetCharacterMax) (Math|Vector|GetForwardVector (Math|Rotator|MakeRotator 0.0 0.0 (.Yaw (Math|Rotator|BreakRotator (Transformation|GetActorRotation (Variables|Default|GetLevelCamera)))))) AxisValue false))

(event Input|AxisEvents|InputAxisMoveRight
  (params (AxisValue :type Float%20%28single-precision%29))
  ;[0.1767 1 0.04638] New moving character
  (Pawn|Input|AddMovementInput (Variables|Default|GetCharacterMax) (Math|Vector|GetRightVector (Math|Rotator|MakeRotator 0.0 0.0 (.Yaw (Math|Rotator|BreakRotator (Transformation|GetActorRotation (Variables|Default|GetLevelCamera)))))) AxisValue false))

(event Input|AxisEvents|InputAxisTurnDown
  (params (AxisValue :type Float%20%28single-precision%29))
  (bind _returnvalue (* AxisValue -1e+02))
  ;[1 1 1] Mouse control
  (if (!= (Class|Widget|GetRenderOpacity (Variables|/Game/Widgets/New/TouchInterface/WBP_TouchInterface.WBP_TouchInterface_C|GetBack (Variables|/Game/Widgets/New/MainInterface_W.MainInterface_W_C|GetWBP_TouchInterface (CallFunction|GetMainInterfaceWidget)))) 0.2)
    (if (Variables|MouseControl|GetMiddleMouseButton)
      (Math|Float|CompareFloat _returnvalue 0.0
        (:>
          (Variables|MouseControl|SetStateCameraMoving "NewEnumerator0")
          (if (not (Utilities|Enum|Equal(Enum) (Variables|MouseControl|GetStopCameraMoving) "NewEnumerator0"))
            (bind _sweephitresult (Transformation|AddLocalOffset (Variables|/Script/Engine.Actor|GetRootComponent (Variables|Default|GetLevelCamera)) (Math|Vector|MakeVector 0.0 0.0 _returnvalue) true false :!label _label))
            (if (.bBlockingHit (Collision|BreakHitResult _sweephitresult))
              (if (Utilities|Enum|Equal(Enum) (Variables|MouseControl|GetStateCameraMoving) "NewEnumerator0")
                (Variables|MouseControl|SetStopCameraMoving "NewEnumerator0")
                (else
                  (Variables|MouseControl|SetStopCameraMoving "NewEnumerator1")))
              (else
                (Variables|MouseControl|SetStopCameraMoving "NewEnumerator4")))))
        (:<
          (Variables|MouseControl|SetStateCameraMoving "NewEnumerator1")
          (if (not (Utilities|Enum|Equal(Enum) (Variables|MouseControl|GetStopCameraMoving) "NewEnumerator1"))
            (goto _label)))))))

(event Input|AxisEvents|InputAxisTurnRight
  (params (AxisValue :type Float%20%28single-precision%29))
  (bind _returnvalue (* AxisValue -1e+02))
  ;[1 1 1] Mouse control
  (if (!= (Class|Widget|GetRenderOpacity (Variables|/Game/Widgets/New/TouchInterface/WBP_TouchInterface.WBP_TouchInterface_C|GetBack (Variables|/Game/Widgets/New/MainInterface_W.MainInterface_W_C|GetWBP_TouchInterface (CallFunction|GetMainInterfaceWidget)))) 0.2)
    (if (Variables|MouseControl|GetMiddleMouseButton)
      (Math|Float|CompareFloat _returnvalue 0.0
        (:>
          (Variables|MouseControl|SetStateCameraMoving "NewEnumerator3")
          (if (not (Utilities|Enum|Equal(Enum) (Variables|MouseControl|GetStopCameraMoving) "NewEnumerator3"))
            (bind _sweephitresult (Transformation|AddLocalOffset (Variables|/Script/Engine.Actor|GetRootComponent (Variables|Default|GetLevelCamera)) (Math|Vector|MakeVector 0.0 _returnvalue 0.0) true false :!label _label))))
        (:<
          (Variables|MouseControl|SetStateCameraMoving "NewEnumerator2")
          (if (not (Utilities|Enum|Equal(Enum) (Variables|MouseControl|GetStopCameraMoving) "NewEnumerator2"))
            (goto _label)))))))

(event Input|MouseEvents|MouseWheelAxis
  (params (AxisValue :type Float%20%28single-precision%29))
  (bind _levelcamera (Variables|Default|GetLevelCamera))
  (bind _levelcamera_2 (Variables|Default|GetLevelCamera))
  (bind _springarm (Variables|/Game/Blueprints/New/LevelCamera.LevelCamera_C|GetSpringArm _levelcamera))
  (bind _cinecamera (Variables|/Game/Blueprints/New/LevelCamera.LevelCamera_C|GetCineCamera _levelcamera))
  (bind _cinecamera_2 (Variables|/Game/Blueprints/New/LevelCamera.LevelCamera_C|GetCineCamera _levelcamera_2))
  (bind _returnvalue (Transformation|GetWorldLocation _cinecamera_2))
  (bind _returnvalue_2 (Transformation|GetWorldLocation _springarm))
  (bind _returnvalue_3 (Transformation|GetWorldLocation _cinecamera))
  (bind _returnvalue_4 (Math|Vector|Distance(Vector) _returnvalue_2 _returnvalue_3))
  (bind _returnvalue_5 (+ _returnvalue_4 -3e+01))
  ;[1 1 1] Mouse control
  (if (!= (Class|Widget|GetRenderOpacity (Variables|/Game/Widgets/New/TouchInterface/WBP_TouchInterface.WBP_TouchInterface_C|GetBack (Variables|/Game/Widgets/New/MainInterface_W.MainInterface_W_C|GetWBP_TouchInterface (CallFunction|GetMainInterfaceWidget)))) 0.2)
    (Math|Float|CompareFloat AxisValue 0.0
      (:>
        _)
      (:<
        _))
    (bind _returnvalue_6 (Collision|LineTraceForObjects _returnvalue (+ _returnvalue (* (Math|Vector|GetForwardVector (Variables|/Game/Blueprints/New/LevelCamera.LevelCamera_C|GetCineCamera (Variables|Default|GetLevelCamera))) -3000)) (Utilities|Array|MakeArray "ObjectTypeQuery8") false 0 "None"))
    (if _returnvalue_6
      (if (<= (Variables|/Game/Blueprints/New/LevelCamera.LevelCamera_C|GetMultiplyMovingCamera (Variables|Default|GetLevelCamera)) 0.0)
        (Variables|/Game/Blueprints/New/LevelCamera.LevelCamera_C|SetMultiplyMovingCamera (Variables|Default|GetLevelCamera) 0.0)
        (else
          (Variables|/Game/Blueprints/New/LevelCamera.LevelCamera_C|SetMultiplyMovingCamera (Variables|Default|GetLevelCamera) (- (Variables|/Game/Blueprints/New/LevelCamera.LevelCamera_C|GetMultiplyMovingCamera (Variables|Default|GetLevelCamera)) 0.01))))
      (elif (>= (Variables|/Game/Blueprints/New/LevelCamera.LevelCamera_C|GetMultiplyMovingCamera (Variables|Default|GetLevelCamera)) 1.0)
        (Variables|/Game/Blueprints/New/LevelCamera.LevelCamera_C|SetMultiplyMovingCamera (Variables|Default|GetLevelCamera) 1.0)
        (else
          (Variables|/Game/Blueprints/New/LevelCamera.LevelCamera_C|SetMultiplyMovingCamera (Variables|Default|GetLevelCamera) (+ (Variables|/Game/Blueprints/New/LevelCamera.LevelCamera_C|GetMultiplyMovingCamera (Variables|Default|GetLevelCamera)) 0.01)))))
    (Variables|/Script/Engine.SpringArmComponent|SetTargetArmLength (Variables|/Game/Blueprints/New/LevelCamera.LevelCamera_C|GetSpringArm (Variables|Default|GetLevelCamera)) (+ (Variables|/Script/Engine.SpringArmComponent|GetTargetArmLength (Variables|/Game/Blueprints/New/LevelCamera.LevelCamera_C|GetSpringArm (Variables|Default|GetLevelCamera))) (* (* AxisValue -3e+01) (Variables|/Game/Blueprints/New/LevelCamera.LevelCamera_C|GetMultiplyMovingCamera (Variables|Default|GetLevelCamera)))))
    (if (> AxisValue 0.0)
      (if (> (Variables|/Script/Engine.SpringArmComponent|GetTargetArmLength (Variables|/Game/Blueprints/New/LevelCamera.LevelCamera_C|GetSpringArm (Variables|Default|GetLevelCamera))) _returnvalue_5)
        (Variables|/Script/Engine.SpringArmComponent|SetTargetArmLength (Variables|/Game/Blueprints/New/LevelCamera.LevelCamera_C|GetSpringArm (Variables|Default|GetLevelCamera)) _returnvalue_5)))))

(event Input|KeyboardEvents|SpaceBar
  (params (Key :type Key%20Structure)))

(event Input|MouseEvents|MiddleMouseButton
  (params (Key :type Key%20Structure))
  ;[1 1 1] Mouse control
  (:Pressed
    (Variables|MouseControl|SetMiddleMouseButton true))
  (:Released
    (Variables|MouseControl|SetMiddleMouseButton false)))

(event Input|KeyboardEvents|Q
  (params (Key :type Key%20Structure))
  ;[1 1 1] SwitchWS
  (:Pressed
    (Default|ChangeWS (Variables|Default|GetCharacterMax))))

(event Input|TouchEvents|InputTouch
  (params (Location :type Vector) (FingerIndex :type ETouchIndex%20Enum))
  (bind _returnvalue (Game|GetPlayerController 0))
  (bind (_x _y) (Math|Vector|BreakVector Location))
  (bind _array (Utilities|Array|MakeArray "ObjectTypeQuery1"))
  (bind _levelcamera (Variables|Default|GetLevelCamera))
  (bind _levelcamera_2 (Variables|Default|GetLevelCamera))
  (bind _hitresult (Class|PlayerController|GetHitResultUnderCursorforObjects _returnvalue _array true))
  (bind _cameramanager (Variables|/Game/Blueprints/New/LevelCamera.LevelCamera_C|GetCameraManager _levelcamera))
  (bind _cameramanager_2 (Variables|/Game/Blueprints/New/LevelCamera.LevelCamera_C|GetCameraManager _levelcamera_2))
  (bind _hitactor (Collision|BreakHitResult _hitresult))
  (bind _startlocationfirst (Variables|/Game/Blueprints/CameraControl/CameraManager.CameraManager_C|GetStartLocationFirst _cameramanager))
  (bind _returnvalue_2 (Utilities|GetClass _hitactor))
  (:Pressed
    (Default|Pressed _cameramanager_2 Location FingerIndex)
    (if (== _returnvalue_2 "/Game/Assets/Objects/TriSign/BP_TriSign.BP_TriSign_C")
      (Variables|Default|SetTriSign _returnvalue_2)
      (else
        (Variables|Default|SetTriSign 0))))
  (:Released
    (Default|Released _cameramanager_2 FingerIndex)
    (if (Math|Vector|Equal(Vector) (Math|Vector2D|MakeVector2D (.x _startlocationfirst) (.y _startlocationfirst)) (Math|Vector2D|MakeVector2D _x _y) 1.5)
      (Default|ClearFirstLocation (Variables|/Game/Blueprints/New/LevelCamera.LevelCamera_C|GetCameraManager (Variables|Default|GetLevelCamera)))
      (if (not (Variables|/Game/Blueprints/CameraControl/CameraManager.CameraManager_C|GetSecondFinger? (Variables|/Game/Blueprints/New/LevelCamera.LevelCamera_C|GetCameraManager (Variables|Default|GetLevelCamera))))
        (CallFunction|SingleTap Location))
      (else
        (Default|ClearFirstLocation (Variables|/Game/Blueprints/New/LevelCamera.LevelCamera_C|GetCameraManager (Variables|Default|GetLevelCamera))))))
  (:Moved
    (Default|Moved _cameramanager_2 Location FingerIndex)))

(fn ConstructionScript)

(fn LineTrace
  (bind (_startlocation _endlocation) (CallFunction|GetTouchLocation))
  (bind (_startlocation_2 _endlocation_2) (CallFunction|GetTouchLocation))
  (bind (_startlocation_3 _endlocation_3) (CallFunction|GetTouchLocation))
  (bind (_outhit _returnvalue) (Collision|LineTraceByChannel _startlocation_2 _endlocation_2 "TraceTypeQuery4" false 0 "None" false))
  (if _returnvalue
    (bind (_outhit_2 _returnvalue_2) (Collision|LineTraceByChannel _startlocation _endlocation "TraceTypeQuery3" false 0 "None" false))
    (if _returnvalue_2
      (if (< (.Distance (Collision|BreakHitResult _outhit_2)) (.Distance (Collision|BreakHitResult _outhit)))
        (bind _returnvalue_3 (Game|SpawnActorfromClass "/Game/Blueprints/CameraControl/TargetActor.TargetActor_C" (Math|Transform|MakeTransform (.ProjectedLocation (AI|Navigation|ProjectPointtoNavigation (.Location (Collision|BreakHitResult _outhit_2)) 0 0 "0, 0, 0"))) "AlwaysSpawn" 0 0))
        (Variables|Default|SetTargetMoto _returnvalue_3)
        (Audio|PlaySound2D "/Game/Audio/Snd/FX/LocationMark.LocationMark" 1.0 1.0 0.0 0 0 :!label _label)
        (bind _outactors (Actor|GetAllActorsOfClass "/Game/Blueprints/CameraControl/TargetActor.TargetActor_C"))
        (if (> (Utilities|Array|Length _outactors) 1)
          (Actor|DestroyActor (Utilities|Array|Get(acopy) _outactors)))
        (return (Variables|Default|GetTargetMoto) true))
      (else
        (bind _output_get (Variables|Default|SetTargetMoto 0))
        (return _output_get false)))
    (else
      (bind (_outhit_3 _returnvalue_4) (Collision|LineTraceByChannel _startlocation_3 _endlocation_3 "TraceTypeQuery3" false 0 "None" false))
      (if _returnvalue_4
        (bind _returnvalue_5 (Game|SpawnActorfromClass "/Game/Blueprints/CameraControl/TargetActor.TargetActor_C" (Math|Transform|MakeTransform (.ProjectedLocation (AI|Navigation|ProjectPointtoNavigation (.Location (Collision|BreakHitResult _outhit_3)) 0 0 "0, 0, 0"))) "AlwaysSpawn" 0 0))
        (Variables|Default|SetTargetMoto _returnvalue_5)
        (goto _label)))))

(fn 3Touch
  (bind _returnvalue (Game|GetPlayerController 0))
  (bind (_locationx _locationy) (Class|PlayerController|GetInputTouchState _returnvalue "Touch3"))
  (return (Math|Vector2D|MakeVector2D _locationx _locationy)))

(fn TouchEffect
  (params (PositionTouch :type Vector))
  (bind (_x _y) (Math|Vector|BreakVector PositionTouch))
  (bind _returnvalue (Viewport|GetViewportSize))
  (bind _currentplayercontroller (Variables|Default|GetCurrentPlayerController))
  (bind _currentplayercontroller_2 (Variables|Default|GetCurrentPlayerController))
  (bind _maininterface_w (Variables|/Game/Blueprints/New/Main/01CaveMain/01CM_PC.01CM_PC_C|GetMainInterface_W _currentplayercontroller_2))
  (bind _maininterface_w_2 (Variables|/Game/Blueprints/New/Main/01CaveMain/01CM_PC.01CM_PC_C|GetMainInterface_W _currentplayercontroller))
  (bind _canvaspanelmain (Variables|/Game/Widgets/New/MainInterface_W.MainInterface_W_C|GetCanvasPanelMain _maininterface_w_2))
  (bind _returnvalue_2 (Class|Widget|GetCachedGeometry _canvaspanelmain))
  (bind _returnvalue_3 (Class|SlateBlueprintLibrary|GetLocalSize _returnvalue_2))
  (Class|CanvasPanelSlot|SetPosition (Class|WidgetLayoutLibrary|SlotasCanvasSlot (Variables|/Game/Widgets/New/MainInterface_W.MainInterface_W_C|GetImageTouchEffect (Variables|/Game/Blueprints/New/Main/01CaveMain/01CM_PC.01CM_PC_C|GetMainInterface_W (Variables|Default|GetCurrentPlayerController)))) (Math|Vector2D|MakeVector2D (+ (* _x (/ (.x _returnvalue_3) (.x _returnvalue))) -2e+01) (+ (* _y (/ (.y _returnvalue_3) (.y _returnvalue))) -2e+01)))
  (UserInterface|Animation|PlayAnimation _maininterface_w (Variables|/Game/Widgets/New/MainInterface_W.MainInterface_W_C|GetTouchEffectAnim _maininterface_w) 0.0 1 "Forward" 3.0 false))

(fn ReturnControl
  (Input|EnableInput (Game|Player|GetPlayerPawn 0) (Game|GetPlayerController 0))
  (Utilities|Time|ClearandInvalidateTimerbyHandle (Variables|Default|GetTimerReturnControl)))

(fn GetTouchLocation
  (bind _returnvalue (Game|GetPlayerController 0))
  (bind _returnvalue_2 (Game|GetPlayerController 0))
  (bind (_locationx _locationy) (Class|PlayerController|GetInputTouchState _returnvalue "Touch1"))
  (bind (_worldlocation _worlddirection) (Class|PlayerController|DeprojectScreenPositiontoWorld _returnvalue_2 _locationx _locationy))
  (return _worldlocation (+ _worldlocation (* _worlddirection 1e+04))))