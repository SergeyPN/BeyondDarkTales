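; Touch camera controller for the LevelCamera actor: one finger rotates, two parallel fingers pan, other two-finger gestures zoom the spring arm.
; Speeds load from the BP_GI save game; touch handlers store finger positions, which Tick processes depending on touch-interface Back opacity.
; Start points chase current touches for inertia.
; Rotation has pitch and optional yaw limits, panning sweeps for collision, and backward line traces damp rotation and zoom near obstacles.
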(event EventTick
  (params (DeltaSeconds :type Float%20%28single-precision%29))
  (if (!= (Class|Widget|GetRenderOpacity (Variables|/Game/Widgets/New/TouchInterface/WBP_TouchInterface.WBP_TouchInterface_C|GetBack (Variables|/Game/Widgets/New/MainInterface_W.MainInterface_W_C|GetWBP_TouchInterface (CallFunction|GetMainInterfaceWidget)))) 0.2)
    (CallFunction|Calculate)
    (if (Variables|Default|GetSecondFinger?)
      (if (Math|Vector|Equal(Vector) (Math|Vector|Normalize (Math|Vector|GetUnitDirection(Vector) (Variables|Other|GetLocationFirst) (Variables|Other|GetStartLocationFirst))) (Math|Vector|Normalize (Math|Vector|GetUnitDirection(Vector) (Variables|Other|GetLocationSecond) (Variables|Other|GetStartLocationSecond))) 0.5)
        (CallFunction|Move)
        (else
          (CallFunction|Zoom)))
      (else
        (CallFunction|Rotate)))
    (CallFunction|CheckDistance)))

(event EventBeginPlay
  (Variables|Other|SetCameraStartRotation (Variables|/Script/Engine.SceneComponent|GetRelativeRotation (Variables|/Game/Blueprints/New/LevelCamera.LevelCamera_C|GetSpringArm (.AsLevel%20Camera (Utilities|Casting|CastToLevelCamera (Components|GetOwner))))))
  (bind _asmy_game_instance (Utilities|Casting|CastToBP_GI (Game|GetGameInstance)))
  (Variables|Settings|SetRotationSpeed (Variables|/Game/Blueprints/SaveGame/BP_SaveGame.BP_SaveGame_C|GetRotationCameraSpeed (Variables|/Game/Blueprints/GI/BP_GI.BP_GI_C|GetSaveGame _asmy_game_instance)))
  (Variables|Settings|SetMoveSpeed (Variables|/Game/Blueprints/SaveGame/BP_SaveGame.BP_SaveGame_C|GetMovingCameraSpeed (Variables|/Game/Blueprints/GI/BP_GI.BP_GI_C|GetSaveGame _asmy_game_instance)))
  (Variables|Settings|SetZoomSpeed (Variables|/Game/Blueprints/SaveGame/BP_SaveGame.BP_SaveGame_C|GetZoomingCameraSpeed (Variables|/Game/Blueprints/GI/BP_GI.BP_GI_C|GetSaveGame _asmy_game_instance))))

(fn Pressed
  (params (Location :type Vector) (FingerIndex :type ETouchIndex%20Enum :default "Touch1"))
  (switch Utilities|FlowControl|Switch|SwitchonETouchIndex FingerIndex
    (:Touch1
      (bind _output_get (Variables|Other|SetStartLocationFirst Location))
      (Variables|Other|SetLocationFirst _output_get))
    (:Touch2
      (bind _output_get_2 (Variables|Other|SetStartLocationSecond Location))
      (Variables|Other|SetLocationSecond _output_get_2)
      (Variables|Default|SetSecondFinger? true))))

(fn Released
  (params (FingerIndex :type ETouchIndex%20Enum :default "Touch1"))
  (switch Utilities|FlowControl|Switch|SwitchonETouchIndex FingerIndex
    (:Touch2
      (Variables|Other|SetStartLocationSecond "0, 0, 0")
      (Variables|Other|SetLocationSecond "0, 0, 0")
      (Variables|Default|SetSecondFinger? false))))

(fn Moved
  (params (Location :type Vector) (FingerIndex :type ETouchIndex%20Enum :default "Touch1"))
  (switch Utilities|FlowControl|Switch|SwitchonETouchIndex FingerIndex
    (:Touch1
      (Variables|Other|SetLocationFirst Location))
    (:Touch2
      (Variables|Other|SetLocationSecond Location))))

(fn Calculate
  (LocalVariables|SettmpDirectionFirst (- (Variables|Other|GetStartLocationFirst) (Variables|Other|GetLocationFirst)))
  (LocalVariables|SettmpDirectionSecond (- (Variables|Other|GetStartLocationSecond) (Variables|Other|GetLocationSecond)))
  (Variables|Other|SetModificatorFirst (Math|Vector|VectorLength (LocalVariables|GettmpDirectionFirst)))
  (LocalVariables|SettmpModificatorFirst (Math|Vector|VectorLength (LocalVariables|GettmpDirectionFirst)))
  (LocalVariables|SettmpModificatorSecond (Math|Vector|VectorLength (LocalVariables|GettmpDirectionSecond)))
  (Variables|Other|SetCurrentPitch (.pitch (Variables|/Script/Engine.SceneComponent|GetRelativeRotation (Variables|/Game/Blueprints/New/LevelCamera.LevelCamera_C|GetSpringArm (.AsLevel%20Camera (Utilities|Casting|CastToLevelCamera (Components|GetOwner)))))))
  (Utilities|FlowControl|Sequence
    (:then_0
      (CallFunction|CalculateFirstTouchLocation (LocalVariables|GettmpModificatorFirst)))
    (:then_1
      (CallFunction|CalculateSecondTouchLocation (LocalVariables|GettmpModificatorSecond)))))

(fn Rotate
  (bind _returnvalue (Components|GetOwner))
  (bind _returnvalue_2 (Components|GetOwner))
  (bind _returnvalue_3 (Components|GetOwner))
  (bind _rotator (Variables|Other|GetRotator))
  (bind _returnvalue_4 (Actor|GetComponentbyClass _returnvalue "/Script/CinematicCamera.CineCameraComponent"))
  (bind _aslevel_camera (Utilities|Casting|CastToLevelCamera _returnvalue_2))
  (bind _aslevel_camera_2 (Utilities|Casting|CastToLevelCamera _returnvalue_3))
  (bind _returnvalue_5 (Transformation|GetWorldLocation _returnvalue_4))
  (if (and (Math|Vector|Equal(Vector) (Variables|Other|GetStartLocationSecond) "0, 0, 0" 0.0001) (Math|Vector|NotEqual(Vector) (Variables|Other|GetLocationFirst) "0, 0, 0" 0.0001))
    (Utilities|FlowControl|Sequence
      (:then_0
        (CallFunction|CalculateRotation))
      (:then_2
        (CallFunction|CalculatePitchLimit))
      (:then_3
        (CallFunction|CalculateYawLimit))
      (:then_4
        (bind (_outhit _returnvalue_6) (Collision|LineTraceForObjects _returnvalue_5 (+ _returnvalue_5 (* (Math|Vector|GetForwardVector _returnvalue_4) -2000)) (Utilities|Array|MakeArray "ObjectTypeQuery8") false 0 "None"))
        (if _returnvalue_6
          (if (<= (.Distance (Collision|BreakHitResult _outhit)) (Variables|Default|GetDistanceCameraAndBlockWall))
            (Variables|Default|SetDistanceCameraAndBlockWall (.Distance (Collision|BreakHitResult _outhit)))
            (if (<= (Variables|/Game/Blueprints/New/LevelCamera.LevelCamera_C|GetMultiplyMovingCamera _aslevel_camera) 0.01)
              (Variables|/Game/Blueprints/New/LevelCamera.LevelCamera_C|SetMultiplyMovingCamera _aslevel_camera 0.01)
              (else
                (Variables|/Game/Blueprints/New/LevelCamera.LevelCamera_C|SetMultiplyMovingCamera _aslevel_camera (- (Variables|/Game/Blueprints/New/LevelCamera.LevelCamera_C|GetMultiplyMovingCamera _aslevel_camera) 0.04))))
            (else
              (Variables|Default|SetDistanceCameraAndBlockWall (.Distance (Collision|BreakHitResult _outhit)))
              (if (>= (Variables|/Game/Blueprints/New/LevelCamera.LevelCamera_C|GetMultiplyMovingCamera (.AsLevel%20Camera (Utilities|Casting|CastToLevelCamera (Components|GetOwner)))) 1.0)
                (Variables|/Game/Blueprints/New/LevelCamera.LevelCamera_C|SetMultiplyMovingCamera (.AsLevel%20Camera (Utilities|Casting|CastToLevelCamera (Components|GetOwner))) 1.0)
                (else
                  (Variables|/Game/Blueprints/New/LevelCamera.LevelCamera_C|SetMultiplyMovingCamera _aslevel_camera_2 (+ (Variables|/Game/Blueprints/New/LevelCamera.LevelCamera_C|GetMultiplyMovingCamera _aslevel_camera_2) 0.04))))))
          (else
            (Variables|/Game/Blueprints/New/LevelCamera.LevelCamera_C|SetMultiplyMovingCamera (.AsLevel%20Camera (Utilities|Casting|CastToLevelCamera (Components|GetOwner))) 1.0)))
        (Transformation|AddRelativeRotation (Variables|/Game/Blueprints/New/LevelCamera.LevelCamera_C|GetSpringArm (.AsLevel%20Camera (Utilities|Casting|CastToLevelCamera (Components|GetOwner)))) (Math|Rotator|MakeRotator 0.0 (* (.pitch _rotator) (Variables|/Game/Blueprints/New/LevelCamera.LevelCamera_C|GetMultiplyMovingCamera (.AsLevel%20Camera (Utilities|Casting|CastToLevelCamera (Components|GetOwner))))) (* (.yaw _rotator) (Variables|/Game/Blueprints/New/LevelCamera.LevelCamera_C|GetMultiplyMovingCamera (.AsLevel%20Camera (Utilities|Casting|CastToLevelCamera (Components|GetOwner)))))) false false)))))

(fn Move
  (bind _returnvalue (Components|GetOwner))
  (bind _moveoffset (Variables|Other|GetMoveOffset))
  (bind _moveoffset_2 (Variables|Other|GetMoveOffset))
  (bind _aslevel_camera (Utilities|Casting|CastToLevelCamera _returnvalue))
  (bind _cinecamera (Variables|/Game/Blueprints/New/LevelCamera.LevelCamera_C|GetCineCamera _aslevel_camera))
  (if (and (Math|Vector|NotEqual(Vector) (Variables|Other|GetStartLocationFirst) "0, 0, 0" 0.0001) (Math|Vector|NotEqual(Vector) (Variables|Other|GetStartLocationSecond) "0, 0, 0" 0.0001))
    (Utilities|FlowControl|Sequence
      (:then_0
        (CallFunction|CalculateMoveOffset))
      (:then_1
        (if (Math|Vector|NotEqual(Vector) (Variables|Other|GetMoveOffset) "0, 0, 0" 1.0)
          (Utilities|FlowControl|Sequence
            (:then_0
              (Math|Float|CompareFloat (.x _moveoffset) 0.0
                (:>
                  (Variables|Default|SetStateCameraMoving "NewEnumerator3")
                  (if (not (Utilities|Enum|Equal(Enum) (Variables|Default|GetStopCameraMoving) "NewEnumerator3"))
                    (bind _sweephitresult (Transformation|AddWorldOffset (Variables|/Script/Engine.Actor|GetRootComponent (Components|GetOwner)) (+ (* (* (Math|Vector|GetUpVector _cinecamera) (.y _moveoffset_2)) -1.0) (* (Math|Vector|GetRightVector _cinecamera) (.x _moveoffset_2))) true false :!label _label))
                    (Utilities|FlowControl|Sequence
                      (:then_0
                        (if (.bBlockingHit (Collision|BreakHitResult _sweephitresult))
                          (if (Utilities|Enum|Equal(Enum) (Variables|Default|GetStateCameraMoving) "NewEnumerator3")
                            (Variables|Default|SetStopCameraMoving "NewEnumerator3")
                            (else
                              (Variables|Default|SetStopCameraMoving "NewEnumerator2")))
                          (else
                            (Variables|Default|SetStopCameraMoving "NewEnumerator4"))))
                      (:then_1
                        (if (.bBlockingHit (Collision|BreakHitResult _sweephitresult))
                          (if (Utilities|Enum|Equal(Enum) (Variables|Default|GetStateCameraMoving) "NewEnumerator0")
                            (Variables|Default|SetStopCameraMoving "NewEnumerator0")
                            (else
                              (Variables|Default|SetStopCameraMoving "NewEnumerator1")))
                          (else
                            (Variables|Default|SetStopCameraMoving "NewEnumerator4")))))))
                (:<
                  (Variables|Default|SetStateCameraMoving "NewEnumerator2")
                  (if (not (Utilities|Enum|Equal(Enum) (Variables|Default|GetStopCameraMoving) "NewEnumerator2"))
                    (goto _label)))))
            (:then_1
              (Math|Float|CompareFloat (.y _moveoffset) 0.0
                (:>
                  (Variables|Default|SetStateCameraMoving "NewEnumerator1")
                  (if (not (Utilities|Enum|Equal(Enum) (Variables|Default|GetStopCameraMoving) "NewEnumerator1"))
                    (goto _label)))
                (:<
                  (Variables|Default|SetStateCameraMoving "NewEnumerator0")
                  (if (not (Utilities|Enum|Equal(Enum) (Variables|Default|GetStopCameraMoving) "NewEnumerator0"))
                    (goto _label)))))))))))

(fn Zoom
  (bind _returnvalue (Components|GetOwner))
  (bind _returnvalue_2 (Components|GetOwner))
  (bind _returnvalue_3 (Components|GetOwner))
  (bind _locationfirst (Variables|Other|GetLocationFirst))
  (bind _aslevel_camera (Utilities|Casting|CastToLevelCamera _returnvalue))
  (bind _aslevel_camera_2 (Utilities|Casting|CastToLevelCamera _returnvalue_2))
  (bind _aslevel_camera_3 (Utilities|Casting|CastToLevelCamera _returnvalue_3))
  (bind _cinecamera (Variables|/Game/Blueprints/New/LevelCamera.LevelCamera_C|GetCineCamera _aslevel_camera))
  (bind _returnvalue_4 (Transformation|GetWorldLocation _cinecamera))
  (if (not (Math|Float|NearlyEqual(Float) (Math|Vector|Distance(Vector) (Variables|Other|GetLocationFirst) (Variables|Other|GetStartLocationFirst)) 0.0 1.0))
    (bind _returnvalue_5 (Collision|LineTraceForObjects _returnvalue_4 (+ _returnvalue_4 (* (Math|Vector|GetForwardVector (Variables|/Game/Blueprints/New/LevelCamera.LevelCamera_C|GetCineCamera _aslevel_camera)) -3000)) (Utilities|Array|MakeArray "ObjectTypeQuery8") false 0 "None"))
    (if _returnvalue_5
      (if (<= (Variables|/Game/Blueprints/New/LevelCamera.LevelCamera_C|GetMultiplyMovingCamera _aslevel_camera_2) 0.0)
        (Variables|/Game/Blueprints/New/LevelCamera.LevelCamera_C|SetMultiplyMovingCamera _aslevel_camera_2 0.0)
        (else
          (Variables|/Game/Blueprints/New/LevelCamera.LevelCamera_C|SetMultiplyMovingCamera _aslevel_camera_2 (- (Variables|/Game/Blueprints/New/LevelCamera.LevelCamera_C|GetMultiplyMovingCamera _aslevel_camera_2) 0.01))))
      (elif (>= (Variables|/Game/Blueprints/New/LevelCamera.LevelCamera_C|GetMultiplyMovingCamera (.AsLevel%20Camera (Utilities|Casting|CastToLevelCamera (Components|GetOwner)))) 1.0)
        (Variables|/Game/Blueprints/New/LevelCamera.LevelCamera_C|SetMultiplyMovingCamera _aslevel_camera_3 1.0)
        (else
          (Variables|/Game/Blueprints/New/LevelCamera.LevelCamera_C|SetMultiplyMovingCamera (.AsLevel%20Camera (Utilities|Casting|CastToLevelCamera (Components|GetOwner))) (+ (Variables|/Game/Blueprints/New/LevelCamera.LevelCamera_C|GetMultiplyMovingCamera _aslevel_camera_3) 0.01)))))
    (Development|PrintString (Utilities|String|ToString(Float) (Variables|/Script/Engine.SpringArmComponent|GetTargetArmLength (LocalVariables|GettmpSpringArm))))
    (LocalVariables|SettmpSpringArm (Actor|GetComponentbyClass (Components|GetOwner) "/Script/Engine.SpringArmComponent"))
    (Utilities|FlowControl|Sequence
      (:then_0
        (LocalVariables|SetStartLocDistanceTmp (Math|Vector|Distance(Vector) (Variables|Other|GetStartLocationFirst) (Variables|Other|GetStartLocationSecond)))
        (LocalVariables|SetLocDistanceTmp (Math|Vector|Distance(Vector) _locationfirst (Variables|Other|GetLocationSecond)))
        (if (> (LocalVariables|GetStartLocDistanceTmp) (+ (LocalVariables|GetLocDistanceTmp) 0.3))
          (Variables|/Script/Engine.SpringArmComponent|SetTargetArmLength (LocalVariables|GettmpSpringArm) (Math|Float|Clamp(Float) (+ (Variables|/Script/Engine.SpringArmComponent|GetTargetArmLength (LocalVariables|GettmpSpringArm)) (* (Variables|/Game/Blueprints/New/LevelCamera.LevelCamera_C|GetMultiplyMovingCamera (.AsLevel%20Camera (Utilities|Casting|CastToLevelCamera (Components|GetOwner)))) (* (Variables|Settings|GetZoomSpeed) (Math|Vector|Distance(Vector) (Variables|Other|GetStartLocationFirst) _locationfirst)))) (Variables|Settings|GetZoomMin) (Variables|Settings|GetZoomMax)))
          (elif (< (LocalVariables|GetStartLocDistanceTmp) (- (LocalVariables|GetLocDistanceTmp) 0.3))
            (Variables|/Script/Engine.SpringArmComponent|SetTargetArmLength (LocalVariables|GettmpSpringArm) (Math|Float|Clamp(Float) (- (Variables|/Script/Engine.SpringArmComponent|GetTargetArmLength (LocalVariables|GettmpSpringArm)) (* (* (Variables|Settings|GetZoomSpeed) (Math|Vector|Distance(Vector) (Variables|Other|GetStartLocationFirst) _locationfirst)) (Variables|/Game/Blueprints/New/LevelCamera.LevelCamera_C|GetMultiplyMovingCamera (.AsLevel%20Camera (Utilities|Casting|CastToLevelCamera (Components|GetOwner)))))) (Variables|Settings|GetZoomMin) (Variables|Settings|GetZoomMax)))
            (if (> (Variables|/Script/Engine.SpringArmComponent|GetTargetArmLength (LocalVariables|GettmpSpringArm)) (+ (Math|Vector|Distance(Vector) (Transformation|GetWorldLocation (LocalVariables|GettmpSpringArm)) (Transformation|GetWorldLocation (Actor|GetComponentbyClass (Components|GetOwner) "/Script/CinematicCamera.CineCameraComponent"))) -3e+01))
              (Variables|/Script/Engine.SpringArmComponent|SetTargetArmLength (LocalVariables|GettmpSpringArm) (Math|Float|Clamp(Float) (+ (Math|Vector|Distance(Vector) (Transformation|GetWorldLocation (LocalVariables|GettmpSpringArm)) (Transformation|GetWorldLocation (Actor|GetComponentbyClass (Components|GetOwner) "/Script/CinematicCamera.CineCameraComponent"))) -3e+01) (Variables|Settings|GetZoomMin) (Variables|Settings|GetZoomMax)))))))
      (:then_1
        (Variables|Other|SetStartLocationFirst (Variables|Other|GetLocationFirst))
        (Variables|Other|SetStartLocationSecond (Variables|Other|GetLocationSecond))))))

(fn CalculateRotation
  (bind _locationfirst (Variables|Other|GetLocationFirst))
  (bind _startlocationfirst (Variables|Other|GetStartLocationFirst))
  (bind _modificatorfirst (Variables|Other|GetModificatorFirst))
  (bind _rotationspeed (Variables|Settings|GetRotationSpeed))
  (bind _returnvalue (Math|Vector|GetUnitDirection(Vector) _locationfirst _startlocationfirst))
  (bind _returnvalue_2 (* _modificatorfirst _rotationspeed))
  (bind _returnvalue_3 (* _returnvalue _returnvalue_2))
  (Variables|Other|SetRotator (Math|Rotator|MakeRotator 0.0 (.y _returnvalue_3) (* (.x _returnvalue_3) -1.0))))

(fn CalculatePitchLimit
  (if (or (>= (+ (Variables|Other|GetCurrentPitch) (.pitch (Variables|Other|GetRotator))) (Variables|Settings|GetPitchMinAngle)) (<= (- (Variables|Other|GetCurrentPitch) (* (.pitch (Variables|Other|GetRotator)) -1.0)) (Variables|Settings|GetPitchMaxAngle)))
    (Variables|Other|SetRotator (Math|Rotator|MakeRotator 0.0 0.0 (.yaw (Variables|Other|GetRotator))))))

(fn CalculateYawLimit
  (bind _returnvalue (Components|GetOwner))
  (bind _camerastartrotation (Variables|Other|GetCameraStartRotation))
  (bind _aslevel_camera (Utilities|Casting|CastToLevelCamera _returnvalue))
  (bind _springarm (Variables|/Game/Blueprints/New/LevelCamera.LevelCamera_C|GetSpringArm _aslevel_camera))
  (bind _relativerotation (Variables|/Script/Engine.SceneComponent|GetRelativeRotation _springarm))
  (bind _returnvalue_2 (Math|Rotator|Delta(Rotator) _camerastartrotation _relativerotation))
  (if (and (or (<= (.yaw _returnvalue_2) (+ (* (Variables|Settings|GetYawLimit) -1.0) (.yaw (Variables|Other|GetRotator)))) (>= (.yaw _returnvalue_2) (+ (Variables|Settings|GetYawLimit) (.yaw (Variables|Other|GetRotator))))) (Variables|Settings|GetbUseLimits))
    (Variables|Other|SetRotator (Math|Rotator|MakeRotator 0.0 (.pitch (Variables|Other|GetRotator)) 0.0))))

(fn CalculateMoveOffset
  (bind _locationfirst (Variables|Other|GetLocationFirst))
  (bind _startlocationfirst (Variables|Other|GetStartLocationFirst))
  (bind _modificatorfirst (Variables|Other|GetModificatorFirst))
  (bind _movespeed (Variables|Settings|GetMoveSpeed))
  (bind _returnvalue (Math|Vector|GetUnitDirection(Vector) _locationfirst _startlocationfirst))
  (bind _returnvalue_2 (* _modificatorfirst _movespeed))
  (bind _returnvalue_3 (* _returnvalue _returnvalue_2))
  (Variables|Other|SetMoveOffset (Math|Vector|MakeVector (.x _returnvalue_3) (.y _returnvalue_3) 0.0)))

(fn CalculateFirstTouchLocation
  (params (Modificator :type Float%20%28single-precision%29))
  (if (> Modificator 0.5)
    (Variables|Other|SetStartLocationFirst (+ (* (Math|Vector|GetUnitDirection(Vector) (Variables|Other|GetStartLocationFirst) (Variables|Other|GetLocationFirst)) (* Modificator (Variables|Settings|GetInertion))) (Variables|Other|GetStartLocationFirst)))
    (elif (Math|Vector|Equal(Vector) (Variables|Other|GetStartLocationFirst) (Variables|Other|GetLocationFirst) 1.0)
      (Variables|Other|SetStartLocationFirst (Variables|Other|GetLocationFirst)))))

(fn CalculateSecondTouchLocation
  (params (Modificator :type Float%20%28single-precision%29))
  (if (> Modificator 0.5)
    (Variables|Other|SetStartLocationSecond (+ (* (Math|Vector|GetUnitDirection(Vector) (Variables|Other|GetStartLocationSecond) (Variables|Other|GetLocationSecond)) (* Modificator (Variables|Settings|GetInertion))) (Variables|Other|GetStartLocationSecond)))
    (elif (Math|Vector|Equal(Vector) (Variables|Other|GetStartLocationSecond) (Variables|Other|GetLocationSecond) 1.0)
      (Variables|Other|SetStartLocationSecond (Variables|Other|GetLocationSecond)))))

(fn ClearFirstLocation
  (Variables|Other|SetStartLocationFirst "0, 0, 0")
  (Variables|Other|SetLocationFirst "0, 0, 0"))

(fn CheckDistance
  (Utilities|FlowControl|Sequence
    (:then_0
      (if (== (Variables|Default|GetTouchDistance) 0.0)
        (Variables|Default|SetTouchDistance (Math|Vector|Distance(Vector) (Variables|Other|GetLocationSecond) (Variables|Other|GetLocationFirst)))))
    (:then_1
      (if (or (> (Math|Vector|Distance(Vector) (Variables|Other|GetLocationSecond) (Variables|Other|GetLocationFirst)) (+ (Variables|Default|GetTouchDistance) 3.0)) (< (Math|Vector|Distance(Vector) (Variables|Other|GetLocationSecond) (Variables|Other|GetLocationFirst)) (- (Variables|Default|GetTouchDistance) 3.0)))
        (Variables|Default|SetbBlockMove true)
        (else
          (Variables|Default|SetbBlockMove false))))
    (:then_2
      (Variables|Default|SetTouchDistance (Math|Vector|Distance(Vector) (Variables|Other|GetLocationSecond) (Variables|Other|GetLocationFirst))))))