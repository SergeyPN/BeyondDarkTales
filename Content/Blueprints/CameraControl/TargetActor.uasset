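; TargetActor is a move-to point marker that plays an animation on its Point2Move component when spawned and can play a reverse one through PlayAnimRevers.
; It caches the first BP_CharMax as Player, then a fast looping timer sphere-traces for pawns from the marker, opposite the player's facing.
; A hit calls Close on the player through a DoOnce that resets when the trace finds nothing.
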(event Custom|TargetClose
  (bind _returnvalue (Transformation|GetActorLocation))
  (bind _returnvalue_2 (Collision|SphereTraceForObjects _returnvalue (+ _returnvalue (* (Math|Vector|GetForwardVector (Transformation|GetActorRotation (Variables|Default|GetPlayer))) -5e+01)) 5e+01 (Utilities|Array|MakeArray "ObjectTypeQuery3") false 0 "None"))
  (if _returnvalue_2
    (Utilities|FlowControl|DoOnce false :!label _label
      (:Completed
        (Default|Close (Variables|Default|GetPlayer))))
    (else
      (goto _label Reset))))

(event Custom|PlayAnimRevers
  (Components|Animation|PlayAnimation (Variables|Default|GetPoint2Move) "/Game/Assets/Objects/Point2Move/Point2Move_AnimBack.Point2Move_AnimBack" false))

(event EventBeginPlay
  (Utilities|FlowControl|Sequence
    (:then_0
      (Components|Animation|PlayAnimation (Variables|Default|GetPoint2Move) "/Game/Assets/Objects/Point2Move/Point2Move_Anim.Point2Move_Anim" false))
    (:then_1
      (bind _outactors (Actor|GetAllActorsOfClass "/Game/Assets/Heroes/Max/BP_CharMax.BP_CharMax_C"))
      (Variables|Default|SetPlayer (Utilities|Array|Get(acopy) _outactors)))
    (:then_2
      (Utilities|Time|SetTimerbyEvent (delegate Custom|TargetClose) 0.01 true))))

(fn ConstructionScript)