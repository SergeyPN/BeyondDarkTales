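; Blueprint function library of shared game helpers for audio, UI, haptics, camera, saving and animation.
; It restarts looping ambience at random offsets, gates vibration on a saved setting, and toggles camera blocking volumes matched by component tag.
; MakeCheckpoint unlocks still-locked checkpoints in both GameInstance and SaveGame season/act data, logging analytics, showing a saving indicator and writing the slot.
; Other helpers fetch shared objects, show continue widgets and reset the character's animation Blueprint.
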(fn PlayRandomStartSoundAtmosphere
  (params (AmbSoundWithLoop :type Array%20of%20Sound%20Base%20Object%20References) (AmbSoundWithoutLoop :type Array%20of%20Sound%20Base%20Object%20References))
  (bind _asmy_game_instance (Utilities|Casting|CastToMyGameInstance (Game|GetGameInstance (LocalVariables|Get__WorldContext))))
  (LocalVariables|SetGameInstance _asmy_game_instance)
  (for _array_element (Variables|/Game/Blueprints/MyGameInstance.MyGameInstance_C|GetRefAudionOnLvls (LocalVariables|GetGameInstance))
    (Utilities|IsValid _array_element
      (:Is%20Valid
        (Components|DestroyComponent _array_element))))
  (Utilities|Array|Clear (Variables|/Game/Blueprints/MyGameInstance.MyGameInstance_C|GetRefAudionOnLvls (LocalVariables|GetGameInstance)))
  (for (_array_element_2 _array_index) AmbSoundWithLoop
    (bind _returnvalue (Audio|SpawnSound2D (Game|GetGameInstance (LocalVariables|Get__WorldContext)) _array_element_2 1.0 1.0 (Math|Random|RandomFloatinRange 0.0 (Variables|/Script/Engine.SoundBase|GetDuration (Utilities|Array|Get(acopy) AmbSoundWithoutLoop _array_index))) 0))
    (Utilities|Array|Add (Variables|/Game/Blueprints/MyGameInstance.MyGameInstance_C|GetRefAudionOnLvls (LocalVariables|GetGameInstance)) _returnvalue)))

(fn GetMainInterfaceWidget
  (bind _foundwidgets (Widget|GetAllWidgetsOfClass (LocalVariables|Get__WorldContext) "/Game/Widgets/New/MainInterface_W.MainInterface_W_C" false))
  (return (Utilities|Array|Get(acopy) _foundwidgets)))

(fn GetMyGameInstance
  (bind _asmy_game_instance (Utilities|Casting|CastToMyGameInstance (Game|GetGameInstance (LocalVariables|Get__WorldContext))))
  (return _asmy_game_instance))

(fn PlayVibro
  (params (FeedBackEffect :type Force%20Feedback%20Effect%20Object%20Reference))
  (bind _asmy_game_instance (Utilities|Casting|CastToMyGameInstance (Game|GetGameInstance (LocalVariables|Get__WorldContext))))
  (if (Variables|/Game/Blueprints/SaveGame/BP_SaveGame.BP_SaveGame_C|GetVibroStatus (Variables|/Game/Blueprints/MyGameInstance.MyGameInstance_C|GetSaveGame _asmy_game_instance))
    (Game|Feedback|ClientPlayForceFeedback (Game|GetPlayerController (LocalVariables|Get__WorldContext)) FeedBackEffect "None" false false false)))

(fn ToggleCollisionBlockCameraVolumes
  (params (LevelCamera :type Level%20Camera%20Object%20Reference) (ON/OFF :type Boolean))
  (for _array_element (Variables|/Game/Blueprints/New/LevelCamera.LevelCamera_C|GetCameraBlockingVolume LevelCamera)
    (bind _outactors (Actor|GetAllActorsOfClass (LocalVariables|Get__WorldContext) "/Script/Engine.CameraBlockingVolume"))
    (bind _array_element_2 (Utilities|Array|ForEachLoopwithBreak _outactors :!label _label)
      (:LoopBody
        (if (> (Utilities|Array|Length (Variables|/Script/Engine.ActorComponent|GetComponentTags (Variables|/Script/Engine.Brush|GetBrushComponent _array_element_2))) 0)
          (if (Utilities|Name|Equal(Name) (Utilities|Array|Get(acopy) (Variables|/Script/Engine.ActorComponent|GetComponentTags (Variables|/Script/Engine.Brush|GetBrushComponent _array_element_2))) (Utilities|String|StringToName (Utilities|String|ToString(Integer) _array_element)))
            (if ON/OFF
              (Collision|SetCollisionEnabled (Variables|/Script/Engine.Brush|GetBrushComponent _array_element_2) "QueryOnly")
              (goto _label Break)
              (else
                (Collision|SetCollisionEnabled (Variables|/Script/Engine.Brush|GetBrushComponent _array_element_2) "NoCollision")
                (goto _label Break))))))))
  (return))

(fn MakeCheckpoint
  (params (AvailableCheckPoint :type Struct%20Check%20Point%20Structure))
  (bind ___worldcontext (LocalVariables|Get__WorldContext))
  (bind ___worldcontext_2 (LocalVariables|Get__WorldContext))
  (bind ___worldcontext_3 (LocalVariables|Get__WorldContext))
  (bind _mygameinstance (CallFunction|GetMyGameInstance ___worldcontext))
  (bind _mygameinstance_2 (CallFunction|GetMyGameInstance ___worldcontext_2))
  (bind _mygameinstance_3 (CallFunction|GetMyGameInstance ___worldcontext_3))
  (bind _season (Variables|/Game/Blueprints/MyGameInstance.MyGameInstance_C|GetSeason _mygameinstance))
  (bind _currentnumseason (Variables|/Game/Blueprints/MyGameInstance.MyGameInstance_C|GetCurrentNumSeason _mygameinstance))
  (bind _currentnumact (Variables|/Game/Blueprints/MyGameInstance.MyGameInstance_C|GetCurrentNumAct _mygameinstance))
  (bind _savegame (Variables|/Game/Blueprints/MyGameInstance.MyGameInstance_C|GetSaveGame _mygameinstance_3))
  (bind _currentnumseason_2 (Variables|/Game/Blueprints/MyGameInstance.MyGameInstance_C|GetCurrentNumSeason _mygameinstance_3))
  (bind _currentnumact_2 (Variables|/Game/Blueprints/MyGameInstance.MyGameInstance_C|GetCurrentNumAct _mygameinstance_3))
  (bind _output (Utilities|Array|Get(acopy) _season _currentnumseason))
  (bind _season_2 (Variables|/Game/Blueprints/SaveGame/BP_SaveGame.BP_SaveGame_C|GetSeason _savegame))
  (bind _acts (Utilities|Struct|BreakStruct_Season _output))
  (bind _output_2 (Utilities|Array|Get(acopy) _season_2 _currentnumseason_2))
  (bind _acts_2 (Utilities|Struct|BreakStruct_Season _output_2))
  (bind _output_3 (Utilities|Array|Get(acopy) _acts _currentnumact))
  (bind _chekpoint (Utilities|Struct|BreakStruct_Act _output_3))
  (bind _output_4 (Utilities|Array|Get(acopy) _acts_2 _currentnumact_2))
  (bind _chekpoint_2 (Utilities|Struct|BreakStruct_Act _output_4))
  ;[1 1 1] CheckSave
  (bind _output_get (LocalVariables|SetLAvailableCheckPoint AvailableCheckPoint))
  (if (!= (.numcheckpoint _output_get) 0)
    (if (not (.Access? (Utilities|Struct|BreakStruct_CheckPoint (Utilities|Array|Get(acopy) (.Chekpoint (Utilities|Struct|BreakStruct_Act (Utilities|Array|Get(acopy) (.Acts (Utilities|Struct|BreakStruct_Season (Utilities|Array|Get(acopy) (Variables|/Game/Blueprints/MyGameInstance.MyGameInstance_C|GetSeason _mygameinstance_2) (Variables|/Game/Blueprints/MyGameInstance.MyGameInstance_C|GetCurrentNumSeason _mygameinstance_2)))) (Variables|/Game/Blueprints/MyGameInstance.MyGameInstance_C|GetCurrentNumAct _mygameinstance_2)))) (- (.NumCheckPoint (Utilities|Struct|BreakStruct_CheckPoint (LocalVariables|GetLAvailableCheckPoint))) 1)))))
      ;[1 1 1] Save CheckPoint
      (Default|SavingGifon (Variables|/Game/Widgets/New/WBP_SavingGif.WBP_SavingGif_C|GetWBP_ImageSaving (Variables|/Game/Widgets/New/MainInterface_W.MainInterface_W_C|GetWBP_SavingGif (CallFunction|GetMainInterfaceWidget (LocalVariables|Get__WorldContext)))))
      (bind _returnvalue (Game|GetCurrentLevelName (LocalVariables|Get__WorldContext)))
      (Class|FirebaseAnalyticsSubsystem|PutString (LocalVariables|GetLBundle) _returnvalue (Utilities|String|ToString(Integer) (.NumCheckPoint (Utilities|Struct|BreakStruct_CheckPoint (LocalVariables|GetLAvailableCheckPoint)))))
      (Class|FirebaseAnalyticsSubsystem|LogEventwithParameters "Save_CheckPoint" (LocalVariables|GetLBundle))
      (Utilities|Array|SetArrayElem _chekpoint (- (.NumCheckPoint (Utilities|Struct|BreakStruct_CheckPoint (Utilities|Array|Get(acopy) _chekpoint (- (.NumCheckPoint (Utilities|Struct|BreakStruct_CheckPoint (LocalVariables|GetLAvailableCheckPoint))) 1)))) 1) (Utilities|Struct|MakeStruct_CheckPoint (.NumCheckPoint (Utilities|Struct|BreakStruct_CheckPoint (Utilities|Array|Get(acopy) _chekpoint (- (.NumCheckPoint (Utilities|Struct|BreakStruct_CheckPoint (LocalVariables|GetLAvailableCheckPoint))) 1)))) (.Access? (Utilities|Struct|BreakStruct_CheckPoint (LocalVariables|GetLAvailableCheckPoint)))))
      (Utilities|Array|SetArrayElem _chekpoint_2 (- (.NumCheckPoint (Utilities|Struct|BreakStruct_CheckPoint (Utilities|Array|Get(acopy) _chekpoint_2 (- (.NumCheckPoint (Utilities|Struct|BreakStruct_CheckPoint (LocalVariables|GetLAvailableCheckPoint))) 1)))) 1) (Utilities|Struct|MakeStruct_CheckPoint (.NumCheckPoint (Utilities|Struct|BreakStruct_CheckPoint (Utilities|Array|Get(acopy) _chekpoint_2 (- (.NumCheckPoint (Utilities|Struct|BreakStruct_CheckPoint (LocalVariables|GetLAvailableCheckPoint))) 1)))) (.Access? (Utilities|Struct|BreakStruct_CheckPoint (LocalVariables|GetLAvailableCheckPoint)))))
      (SaveGame|SaveGametoSlot (Variables|/Game/Blueprints/MyGameInstance.MyGameInstance_C|GetSaveGame (CallFunction|GetMyGameInstance (LocalVariables|Get__WorldContext))) "1"))))

(fn ShowContinueWidget
  (params (PreviosWidget :type User%20Widget%20Object%20Reference) (TargetWidget :type WBP%20Base%20Widget%20Object%20Reference) (WithRemovePreviosWidget :type Boolean))
  (bind _output_get (Variables|/Game/Widgets/MainMenu/WBP_BaseWidget.WBP_BaseWidget_C|SetPreviosWidget TargetWidget PreviosWidget))
  (bind _output_get_2 (LocalVariables|SetLPreviosWidget _output_get))
  (if WithRemovePreviosWidget
    (Widget|RemovefromParent _output_get_2))
  (Class|BPIWidgets|UpdateLocalization(Message) TargetWidget)
  (UserInterface|Viewport|AddtoViewport TargetWidget 0)
  (Class|BPIWidgets|ShowWindow(Message) TargetWidget))

(fn ResetABP
  (bind _ascamera_pc_test (Utilities|Casting|CastToCamera_PC_test (Game|Player|GetPlayerPawn (LocalVariables|Get__WorldContext))))
  (Components|Animation|SetAnimationMode (Variables|/Script/Engine.Character|GetMesh (Variables|/Game/Blueprints/Transfered/Blueprints1/ToTransfer/CameraControl/Camera_PC_test.Camera_PC_test_C|GetCharacterMax _ascamera_pc_test)) "AnimationCustomMode")
  (Components|Animation|SetAnimationMode (Variables|/Script/Engine.Character|GetMesh (Variables|/Game/Blueprints/Transfered/Blueprints1/ToTransfer/CameraControl/Camera_PC_test.Camera_PC_test_C|GetCharacterMax _ascamera_pc_test)) "AnimationBlueprint"))