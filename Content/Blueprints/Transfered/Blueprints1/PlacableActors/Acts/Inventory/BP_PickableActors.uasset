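; BP_PickableActors is a pickable inventory actor that appears to serve as a base for specific items.
; On construction it sets the Interaction component's relative Z from the actor's world-space bounds origin, then calls SetInvName.
; InteractMaterialOn and InteractMaterialOff swap the static mesh's first material between OnMat and OffMat.
; View and SetInvName are empty here.
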(fn ConstructionScript
  (Transformation|SetRelativeLocation (Variables|Default|GetInteraction) (Math|Vector|MakeVector 0.0 0.0 (.z (.Origin (Collision|GetActorBounds false false)))) false false)
  (CallFunction|SetInvName))

(fn View
  (params (Selection :type Byte :default 0)))

(fn InteractMaterialOff
  (Rendering|Material|SetMaterial (Variables|Default|GetStaticMesh) 0 (LocalVariables|GetOffMat)))

(fn InteractMaterialon
  (Rendering|Material|SetMaterial (Variables|Default|GetStaticMesh) 0 (LocalVariables|GetOnMat)))

(fn SetInvName)