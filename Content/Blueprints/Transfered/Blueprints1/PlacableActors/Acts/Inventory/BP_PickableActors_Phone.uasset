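; Pickable phone item that the player can collect into their inventory.
; The construction script sets its Russian and English display names before running the parent's construction logic.
; On widget interaction it calls the pickable-actor clicked notification, then casts the first player controller to PlayerControllereee and passes itself and its InventoryItem to AddItemToInventory.
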(event EventBeginPlay
  (|CallParentFunction) ; This node is disabled and will not be called.\nDrag off pins to build functionality.
)

(event Collision|EventActorBeginOverlap
  (params (OtherActor :type Actor%20Object%20Reference))
  (|CallParentFunction OtherActor) ; This node is disabled and will not be called.\nDrag off pins to build functionality.
)

(event EventTick
  (params (DeltaSeconds :type Float%20%28single-precision%29))
  (|CallParentFunction DeltaSeconds) ; This node is disabled and will not be called.\nDrag off pins to build functionality.
)

(event EventInteractwithWidget
  (Default|CallPickableActorClicked self)
  (bind _asplayer_controllereee (Utilities|Casting|CastToPlayerControllereee (Game|GetPlayerController 0)))
  (Default|AddItemtoInventory _asplayer_controllereee self (Variables|Default|GetInventoryItem)))

(fn ConstructionScript
  (Variables|Default|SetRusName "Телефон")
  (Variables|Default|SetEngName "Phone")
  (|CallParentFunction))