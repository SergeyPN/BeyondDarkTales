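; BP_StaticActors is a placeable static actor that appears to serve as a base for interactable world objects.
; Its construction script sets the relative height of the Interaction and Drop components from the actor's bounds origin, placing Drop slightly higher.
; InteractMaterialOn and InteractMaterialOff toggle interaction feedback by swapping the mesh's first material between OnMat and OffMat.
; View and SetInvName are empty stubs.
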(fn ConstructionScript
  (bind _origin (Collision|GetActorBounds false false))
  (Transformation|SetRelativeLocation (Variables|Default|GetInteraction) (Math|Vector|MakeVector 0.0 0.0 (.z _origin)) false false)
  (Transformation|SetRelativeLocation (Variables|Default|GetDrop) (Math|Vector|MakeVector 0.0 0.0 (+ (.z _origin) 1e+01)) false false))

(fn View
  (params (Selection :type Byte :default 0)))

(fn InteractMaterialon
  (Rendering|Material|SetMaterial (Variables|Default|GetStaticMesh) 0 (LocalVariables|GetOnMat)))

(fn InteractMaterialOff
  (Rendering|Material|SetMaterial (Variables|Default|GetStaticMesh) 0 (LocalVariables|GetOffMat)))

(fn SetInvName)