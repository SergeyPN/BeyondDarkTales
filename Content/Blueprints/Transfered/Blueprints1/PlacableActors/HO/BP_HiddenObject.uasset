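; Placeable hidden-object actor for a hidden-object mechanic, highlighted on demand and reporting clicks through HOClicked when AbleToSee is set.
; ShowInteract and HideInteract swap the mesh material and toggle the PDeadMansLoot effect.
; Hiding can also reverse a timeline-driven flipbook icon on the interaction widget, whose height the construction script sets from actor bounds.
; Much older logic is disconnected, including widget setup, localized naming, pickup counting and the icon's start trigger.
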(event OnComponentBeginOverlap(Box)
  (params (OverlappedComponent :type Primitive%20Component%20Object%20Reference) (OtherActor :type Actor%20Object%20Reference) (OtherComp :type Primitive%20Component%20Object%20Reference) (OtherBodyIndex :type Integer) (bFromSweep :type Boolean) (SweepResult :type Hit%20Result%20Structure%20%28by%20ref%29))
  (if (== OtherActor 0)
    (if (Variables|Default|GetAbleToSee)
      _)))

(event OnComponentEndOverlap(Box)
  (params (OverlappedComponent :type Primitive%20Component%20Object%20Reference) (OtherActor :type Actor%20Object%20Reference) (OtherComp :type Primitive%20Component%20Object%20Reference) (OtherBodyIndex :type Integer))
  (if (== 0 OtherActor)
    (if (Variables|Default|GetInteractSection)
      (Variables|Default|SetInteractSection false)
      (if (Audio|Components|Audio|IsPlaying (Variables|Default|GetLooping))
        (Audio|PlaySound2D 0 1.0 1.0 0.0 0 0 :!label _label)
        (bind (_direction _alpha) (Timeline|St/End Reverse)
          (:Update
            (Class|BPInteractive|UpdIconWidget(Message) (Variables|Default|GetWidgetInterac) (Utilities|Array|Get(acopy) (Variables|Default|GetStartEndFrames) (Math|Float|Round (Math|Float|Lerp 0.0 (Math|Conversions|ToFloat(Integer) (Utilities|Array|LastIndex (Variables|Default|GetStartEndFrames))) _alpha))) (Variables|Default|GetIconText) (Variables|Default|GetStartFlipbook) (Variables|Default|GetLoopFlipbook) 0 0 false self 0 false "" false 0 "NewEnumerator3" "NewEnumerator0"))
          (:Finished
            (switch Utilities|FlowControl|Switch|SwitchonETimelineDirection _direction
              (:Forward
                (bind (_direction_2 _alpha_2) (Timeline|Looping Play)
                  (:Update
                    (if (Variables|Default|GetInteractSection)
                      (Class|BPInteractive|UpdIconWidget(Message) (Variables|Default|GetWidgetInterac) (Utilities|Array|Get(acopy) (Variables|Default|GetLoopFrames) (Math|Float|Round (Math|Float|Lerp 0.0 (Math|Conversions|ToFloat(Integer) (Utilities|Array|LastIndex (Variables|Default|GetLoopFrames))) _alpha_2))) (Variables|Default|GetIconText) (Variables|Default|GetStartFlipbook) (Variables|Default|GetLoopFlipbook) 0 0 false self 0 false (Variables|Default|GetVisText) false 0 "NewEnumerator3" "NewEnumerator0")
                      (else
                        (Utilities|FlowControl|Sequence
                          (:then_0
                            (Timeline|Looping Stop))
                          (:then_1
                            (goto _label))))))
                  (:Finished
                    (switch Utilities|FlowControl|Switch|SwitchonETimelineDirection _direction_2
                      (:Forward
                        (if (Variables|Default|GetInteractSection)
                          (Timeline|Looping PlayFromStart)))))))
              (:Backward
                (Class|BPInteractive|UpdIconWidget(Message) (Variables|Default|GetWidgetInterac) 0 "" 0 0 0 0 false 0 0 false "" false 0 "NewEnumerator3" "NewEnumerator0")))))))))

(event Custom|CustomEvent_0)

(event Custom|ShowInteract
  (CallFunction|InteractMaterialon)
  (Components|Activation|Activate (Variables|Default|GetP_DeadMans_Loot) false))

(event Custom|HideInteract
  (Components|Activation|Deactivate (Variables|Default|GetP_DeadMans_Loot))
  (CallFunction|InteractMaterialOff)
  (Variables|Default|SetInteractSection false)
  (if (Audio|Components|Audio|IsPlaying (Variables|Default|GetLooping))
    (Audio|PlaySound2D 0 1.0 1.0 0.0 0 0 :!label _label)
    (bind (_direction _alpha) (Timeline|St/End Reverse)
      (:Update
        (Class|BPInteractive|UpdIconWidget(Message) (Variables|Default|GetWidgetInterac) (Utilities|Array|Get(acopy) (Variables|Default|GetStartEndFrames) (Math|Float|Round (Math|Float|Lerp 0.0 (Math|Conversions|ToFloat(Integer) (Utilities|Array|LastIndex (Variables|Default|GetStartEndFrames))) _alpha))) (Variables|Default|GetIconText) (Variables|Default|GetStartFlipbook) (Variables|Default|GetLoopFlipbook) 0 0 false self 0 false "" false 0 "NewEnumerator3" "NewEnumerator0"))
      (:Finished
        (switch Utilities|FlowControl|Switch|SwitchonETimelineDirection _direction
          (:Forward
            (bind (_direction_2 _alpha_2) (Timeline|Looping Play)
              (:Update
                (if (Variables|Default|GetInteractSection)
                  (Class|BPInteractive|UpdIconWidget(Message) (Variables|Default|GetWidgetInterac) (Utilities|Array|Get(acopy) (Variables|Default|GetLoopFrames) (Math|Float|Round (Math|Float|Lerp 0.0 (Math|Conversions|ToFloat(Integer) (Utilities|Array|LastIndex (Variables|Default|GetLoopFrames))) _alpha_2))) (Variables|Default|GetIconText) (Variables|Default|GetStartFlipbook) (Variables|Default|GetLoopFlipbook) 0 0 false self 0 false (Variables|Default|GetVisText) false 0 "NewEnumerator3" "NewEnumerator0")
                  (else
                    (Utilities|FlowControl|Sequence
                      (:then_0
                        (Timeline|Looping Stop))
                      (:then_1
                        (goto _label))))))
              (:Finished
                (switch Utilities|FlowControl|Switch|SwitchonETimelineDirection _direction_2
                  (:Forward
                    (if (Variables|Default|GetInteractSection)
                      (Timeline|Looping PlayFromStart)))))))
          (:Backward
            (Class|BPInteractive|UpdIconWidget(Message) (Variables|Default|GetWidgetInterac) 0 "" 0 0 0 0 false 0 0 false "" false 0 "NewEnumerator3" "NewEnumerator0")))))))

(event EventBeginPlay)

(event Collision|EventActorBeginOverlap
  (params (OtherActor :type Actor%20Object%20Reference)))

(event EventTick
  (params (DeltaSeconds :type Float%20%28single-precision%29)))

(event EventInteractwithWidget
  (if (Variables|Default|GetAbleToSee)
    (Default|CallHOClicked)))

(fn ConstructionScript
  (Transformation|SetRelativeLocation (Variables|Default|GetInteraction) (Math|Vector|MakeVector 0.0 0.0 (.z (.Origin (Collision|GetActorBounds false false)))) false false))

(fn View
  (params (Selection :type Byte :default 0))
  (switch Utilities|FlowControl|Switch|Switchon Selection
    (:NewEnumerator0)
    (:NewEnumerator1
      (Variables|Default|SetSwitcher 0))
    (:NewEnumerator2)))

(fn InteractMaterialon
  (Rendering|Material|SetMaterial (Variables|Default|GetStaticMesh) 0 (LocalVariables|GetOnMat)))

(fn InteractMaterialOff
  (Rendering|Material|SetMaterial (Variables|Default|GetStaticMesh) 0 (LocalVariables|GetOffMat)))

(fn SetInvName
  (switch Utilities|FlowControl|Switch|SwitchonGameLanguage (Variables|/Game/Blueprints/MyGameInstance.MyGameInstance_C|GetLanguage (.AsMy%20Game%20Instance (Utilities|Casting|CastToMyGameInstance (Game|GetGameInstance))))
    (:NewEnumerator0
      (Variables|Default|SetVisText (Variables|Default|GetRusName)))
    (:NewEnumerator1
      (Variables|Default|SetVisText (Variables|Default|GetEngName)))))