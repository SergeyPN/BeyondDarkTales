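; Parkour interaction point that shows an animated widget prompt and, on interaction, sends the player (MaxCharTest) to ArrowToUp for a jump/fall move.
; Tick fades and scales the prompt button by player distance.
; TriggerToUp overlap drives intro, loop and reversed-outro icon frames through two timelines, with Russian or English text.
; CheckForJumpType returns a jump type from the JumpFall flag or a forward trace distance; the down-side prompt is unwired.
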(event OnComponentEndOverlap(TriggerToUp)
  (params (OverlappedComponent :type Primitive%20Component%20Object%20Reference) (OtherActor :type Actor%20Object%20Reference) (OtherComp :type Primitive%20Component%20Object%20Reference) (OtherBodyIndex :type Integer))
  (if (== (Variables|Default|GetPlayer) OtherActor)
    (Variables|Default|SetInteractSection false)
    (if (Audio|Components|Audio|IsPlaying (Variables|Default|GetTimeline_1))
      (Audio|PlaySound2D 0 1.0 1.0 0.0 0 0 :!label _label)
      (bind (_direction _alpha) (Timeline|Timeline_0 Reverse)
        (:Update
          (Class|BPInteractive|UpdIconWidget(Message) (Variables|Default|GetWidgetInteracUP) (Utilities|Array|Get(acopy) (Variables|Default|GetStartEndFrames) (Math|Float|Round (Math|Float|Lerp 0.0 (Math|Conversions|ToFloat(Integer) (Utilities|Array|LastIndex (Variables|Default|GetStartEndFrames))) _alpha))) (Variables|Default|GetIconText) (Variables|Default|GetStartFlipbook) (Variables|Default|GetLoopFlipbook) 0 0 false self 0 false "" false))
        (:Finished
          (switch Utilities|FlowControl|Switch|SwitchonETimelineDirection _direction
            (:Forward
              (bind (_direction_2 _alpha_2) (Timeline|Timeline_1 Play)
                (:Update
                  (if (Variables|Default|GetInteractSection)
                    (Class|BPInteractive|UpdIconWidget(Message) (Variables|Default|GetWidgetInteracUP) (Utilities|Array|Get(acopy) (Variables|Default|GetLoopFrames) (Math|Float|Round (Math|Float|Lerp 0.0 (Math|Conversions|ToFloat(Integer) (Utilities|Array|LastIndex (Variables|Default|GetLoopFrames))) _alpha_2))) (Variables|Default|GetIconText) (Variables|Default|GetStartFlipbook) (Variables|Default|GetLoopFlipbook) 0 0 false self 0 false (Variables|Default|GetVisText) false)
                    (else
                      (Utilities|FlowControl|Sequence
                        (:then_0
                          (Timeline|Timeline_1 Stop))
                        (:then_1
                          (goto _label))))))
                (:Finished
                  (switch Utilities|FlowControl|Switch|SwitchonETimelineDirection _direction_2
                    (:Forward
                      (if (Variables|Default|GetInteractSection)
                        (Timeline|Timeline_1 PlayFromStart)
                        (else
                          (goto _label))))))))
            (:Backward
              (Class|BPInteractive|UpdIconWidget(Message) (Variables|Default|GetWidgetInteracUP) 0 "" 0 0 0 0 false 0 0 false "" false))))))))

(event OnComponentBeginOverlap(TriggerToUp)
  (params (OverlappedComponent :type Primitive%20Component%20Object%20Reference) (OtherActor :type Actor%20Object%20Reference) (OtherComp :type Primitive%20Component%20Object%20Reference) (OtherBodyIndex :type Integer) (bFromSweep :type Boolean) (SweepResult :type Hit%20Result%20Structure%20%28by%20ref%29))
  (if (== OtherActor (Variables|Default|GetPlayer))
    (CallFunction|SetInvUpName)
    (Variables|Default|SetInteractSection true)
    (if (Class|TimelineComponent|IsReversing (Variables|Default|GetTimeline_0))
      (Audio|PlaySound2D 0 1.0 1.0 0.0 0 0 :!label _label)
      (Widget|Transform|SetRenderScale (Variables|/Game/Widgets/Assets/tmp/Widget/InteractionWidget.InteractionWidget_C|GetButton_817 (Variables|Default|GetWidgetInteracUP)) "(X=1.000000,Y=1.000000)")
      (bind (_direction _alpha) (Timeline|Timeline_0 Play)
        (:Update
          (Class|BPInteractive|UpdIconWidget(Message) (Variables|Default|GetWidgetInteracUP) (Utilities|Array|Get(acopy) (Variables|Default|GetStartEndFrames) (Math|Float|Round (Math|Float|Lerp 0.0 (Math|Conversions|ToFloat(Integer) (Utilities|Array|LastIndex (Variables|Default|GetStartEndFrames))) _alpha))) (Variables|Default|GetIconText) (Variables|Default|GetStartFlipbook) (Variables|Default|GetLoopFlipbook) 0 0 false self 0 false "" false))
        (:Finished
          (switch Utilities|FlowControl|Switch|SwitchonETimelineDirection _direction
            (:Forward
              (bind (_direction_2 _alpha_2) (Timeline|Timeline_1 Play)
                (:Update
                  (if (Variables|Default|GetInteractSection)
                    (Class|BPInteractive|UpdIconWidget(Message) (Variables|Default|GetWidgetInteracUP) (Utilities|Array|Get(acopy) (Variables|Default|GetLoopFrames) (Math|Float|Round (Math|Float|Lerp 0.0 (Math|Conversions|ToFloat(Integer) (Utilities|Array|LastIndex (Variables|Default|GetLoopFrames))) _alpha_2))) (Variables|Default|GetIconText) (Variables|Default|GetStartFlipbook) (Variables|Default|GetLoopFlipbook) 0 0 false self 0 false (Variables|Default|GetVisText) false)
                    (else
                      (Utilities|FlowControl|Sequence
                        (:then_0
                          (Timeline|Timeline_1 Stop))
                        (:then_1
                          (Audio|PlaySound2D 0 1.0 1.0 0.0 0 0 :!label _label_2)
                          (Timeline|Timeline_0 Reverse))))))
                (:Finished
                  (switch Utilities|FlowControl|Switch|SwitchonETimelineDirection _direction_2
                    (:Forward
                      (if (Variables|Default|GetInteractSection)
                        (Timeline|Timeline_1 PlayFromStart)
                        (else
                          (goto _label_2))))))))
            (:Backward
              (Class|BPInteractive|UpdIconWidget(Message) (Variables|Default|GetWidgetInteracUP) 0 "" 0 0 0 0 false 0 0 false "" false)))))
      (elif (not (Audio|Components|Audio|IsPlaying (Variables|Default|GetTimeline_0)))
        (if (not (Audio|Components|Audio|IsPlaying (Variables|Default|GetTimeline_1)))
          (goto _label))))))

(event Custom|CloseWidgetUP
  (Variables|Default|SetInteractSection false)
  (if (Audio|Components|Audio|IsPlaying (Variables|Default|GetTimeline_1))
    (Audio|PlaySound2D 0 1.0 1.0 0.0 0 0 :!label _label)
    (bind (_direction _alpha) (Timeline|Timeline_0 Reverse)
      (:Update
        (Class|BPInteractive|UpdIconWidget(Message) (Variables|Default|GetWidgetInteracUP) (Utilities|Array|Get(acopy) (Variables|Default|GetStartEndFrames) (Math|Float|Round (Math|Float|Lerp 0.0 (Math|Conversions|ToFloat(Integer) (Utilities|Array|LastIndex (Variables|Default|GetStartEndFrames))) _alpha))) (Variables|Default|GetIconText) (Variables|Default|GetStartFlipbook) (Variables|Default|GetLoopFlipbook) 0 0 false self 0 false "" false))
      (:Finished
        (switch Utilities|FlowControl|Switch|SwitchonETimelineDirection _direction
          (:Forward
            (bind (_direction_2 _alpha_2) (Timeline|Timeline_1 Play)
              (:Update
                (if (Variables|Default|GetInteractSection)
                  (Class|BPInteractive|UpdIconWidget(Message) (Variables|Default|GetWidgetInteracUP) (Utilities|Array|Get(acopy) (Variables|Default|GetLoopFrames) (Math|Float|Round (Math|Float|Lerp 0.0 (Math|Conversions|ToFloat(Integer) (Utilities|Array|LastIndex (Variables|Default|GetLoopFrames))) _alpha_2))) (Variables|Default|GetIconText) (Variables|Default|GetStartFlipbook) (Variables|Default|GetLoopFlipbook) 0 0 false self 0 false (Variables|Default|GetVisText) false)
                  (else
                    (Utilities|FlowControl|Sequence
                      (:then_0
                        (Timeline|Timeline_1 Stop))
                      (:then_1
                        (goto _label))))))
              (:Finished
                (switch Utilities|FlowControl|Switch|SwitchonETimelineDirection _direction_2
                  (:Forward
                    (if (Variables|Default|GetInteractSection)
                      (Timeline|Timeline_1 PlayFromStart)
                      (else
                        (goto _label))))))))
          (:Backward
            (Class|BPInteractive|UpdIconWidget(Message) (Variables|Default|GetWidgetInteracUP) 0 "" 0 0 0 0 false 0 0 false "" false)))))))

(event EventBeginPlay
  (Utilities|FlowControl|Delay 2.0)
  (bind _outactors (Actor|GetAllActorsOfClass "/Game/Assets/Heroes/Max/MaxCharTest.MaxCharTest_C"))
  (Variables|Default|SetPlayer (Utilities|Array|Get(acopy) _outactors))
  (bind _asinteraction_widget (Utilities|Casting|CastToInteractionWidget (UserInterface|GetUserWidgetObject (Variables|Default|GetInteractionUP))))
  (Variables|Default|SetWidgetInteracUP _asinteraction_widget))

(event Collision|EventActorBeginOverlap
  (params (OtherActor :type Actor%20Object%20Reference)))

(event EventTick
  (params (DeltaSeconds :type Float%20%28single-precision%29))
  (bind _returnvalue (Transformation|GetActorLocation))
  (bind _player (Variables|Default|GetPlayer))
  (bind _widgetinteracup (Variables|Default|GetWidgetInteracUP))
  (bind _returnvalue_2 (Transformation|GetActorLocation _player))
  (bind _button_817 (Variables|/Game/Widgets/Assets/tmp/Widget/InteractionWidget.InteractionWidget_C|GetButton_817 _widgetinteracup))
  (bind _returnvalue_3 (Math|Vector|Distance(Vector) _returnvalue _returnvalue_2))
  (bind _backgroundcolor (Variables|/Script/UMG.Button|GetBackgroundColor _button_817))
  (bind _returnvalue_4 (Math|Float|Clamp(Float) _returnvalue_3 1e+02 5e+02))
  (bind _returnvalue_5 (Math|Float|MapRangeClamped _returnvalue_4 1e+02 5e+02 1.0 0.0))
  (bind _returnvalue_6 (Math|Float|MapRangeClamped _returnvalue_5 0.0 1.0 0.5 1.25))
  (Class|Button|SetBackgroundColor _button_817 (Utilities|Struct|MakeLinearColor (.r _backgroundcolor) (.g _backgroundcolor) (.b _backgroundcolor) _returnvalue_5))
  (Widget|Transform|SetRenderScale _button_817 (Math|Vector2D|MakeVector2D _returnvalue_6 _returnvalue_6)))

(event EventInteractwithWidget
  (Development|PrintString "Hello")
  (Variables|Default|SetNewVar_2 false)
  (CallFunction|CloseWidgetUP)
  (Variables|Default|SetNewVar_3 (Transformation|GetActorLocation (Variables|Default|GetPlayer)))
  (Default|MovePLayer (Variables|Default|GetPlayer) 0 (Transformation|GetWorldLocation (Variables|Default|GetArrowToUp)) false (Transformation|GetWorldRotation (Variables|Default|GetArrowToUp)) 0 (Variables|Default|GetStartUpState) 0 "0, 0, 0" 0 false 0 self true))

(fn ConstructionScript)

(fn SetInvUpName
  (switch Utilities|FlowControl|Switch|SwitchonGameLanguage (Variables|/Game/Blueprints/Transfered/Blueprints1/MyGameInstance.MyGameInstance_C|GetLanguage (.AsMy%20Game%20Instance (Utilities|Casting|CastToMyGameInstance (Game|GetGameInstance))))
    (:NewEnumerator0
      (Variables|Default|SetVisText (Variables|Default|GetRusUpName)))
    (:NewEnumerator1
      (Variables|Default|SetVisText (Variables|Default|GetEngUPName)))))

(fn SetInvDownName
  (switch Utilities|FlowControl|Switch|SwitchonGameLanguage (Variables|/Game/Blueprints/Transfered/Blueprints1/MyGameInstance.MyGameInstance_C|GetLanguage (.AsMy%20Game%20Instance (Utilities|Casting|CastToMyGameInstance (Game|GetGameInstance))))
    (:NewEnumerator0
      (Variables|Default|SetVisText (Variables|Default|GetRusDownName)))
    (:NewEnumerator1
      (Variables|Default|SetVisText (Variables|Default|GetEngDownName)))))

(fn CheckforJumpType
  (bind _arrowtoup (Variables|Default|GetArrowToUp))
  (bind _returnvalue (Transformation|GetWorldLocation _arrowtoup))
  (if (Variables|Default|GetJumpFall)
    (return "NewEnumerator0")
    (else
      (bind _outhit (Collision|LineTraceByChannel (- _returnvalue "0, 0,20.000000") (- (+ _returnvalue (* (Math|Vector|GetForwardVector _arrowtoup) 3e+02)) "0, 0,20.000000") "TraceTypeQuery1" false (Variables|Default|GetActorsToIgnore) "None"))
      (Development|PrintString (Utilities|String|ToString(Float) (.Distance (Collision|BreakHitResult _outhit))))
      (if (and (.bBlockingHit (Collision|BreakHitResult _outhit)) (Math|Float|InRange(Float) (.Distance (Collision|BreakHitResult _outhit)) 185.0 275.0))
        (if (Math|Float|InRange(Float) (.Distance (Collision|BreakHitResult _outhit)) 185.0 225.0)
          (return "NewEnumerator2")
          (elif (Math|Float|InRange(Float) (.Distance (Collision|BreakHitResult _outhit)) 225.0 245.0 false)
            (return "NewEnumerator3")
            (elif (Math|Float|InRange(Float) (.Distance (Collision|BreakHitResult _outhit)) 2.6e+02 275.0)
              (return "NewEnumerator4")
              (else
                (return "NewEnumerator1")))))
        (else
          (return "NewEnumerator0"))))))