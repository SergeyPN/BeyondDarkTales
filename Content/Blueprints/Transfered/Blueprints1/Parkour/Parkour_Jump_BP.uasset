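; Parkour jump point that offers the player a prompt to jump up onto a linked mesh (MeshToJumpOn).
; The construction script derives the nearest top edge from the mesh's rotated bounds to place movement arrows (ArrowToDown only when not manual) and set MeshHeight.
; TriggerToUp shows a localized, timeline-animated flipbook widget, whose button Tick adjusts by distance.
; Interacting passes ArrowToUp's transform to the player's MovePLayer; the down prompt has only close logic.
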(event OnComponentEndOverlap(TriggerToUp)
  (params (OverlappedComponent :type Primitive%20Component%20Object%20Reference) (OtherActor :type Actor%20Object%20Reference) (OtherComp :type Primitive%20Component%20Object%20Reference) (OtherBodyIndex :type Integer))
  (Development|PrintString "dssd" true true "(R=1.000000,G=0.905393,B=0.000000,A=1.000000)")
  (if (== (Variables|Default|GetPlayer) OtherActor)
    (Variables|Default|SetInteractSection false)
    (if (Audio|Components|Audio|IsPlaying (Variables|Default|GetTimeline_1))
      (Audio|PlaySound2D 0 1.0 1.0 0.0 0 0 :!label _label)
      (bind (_direction _alpha) (Timeline|Timeline_0 Reverse)
        (:Update
          (Class|BPInteractive|UpdIconWidget(Message) (Variables|Default|GetWidgetInteracUP) (Utilities|Array|Get(acopy) (Variables|Default|GetStartEndFrames) (Math|Float|Round (Math|Float|Lerp 0.0 (Math|Conversions|ToFloat(Integer) (Utilities|Array|LastIndex (Variables|Default|GetStartEndFrames))) _alpha))) (Variables|Default|GetIconText) (Variables|Default|GetStartFlipbook) (Variables|Default|GetLoopFlipbook) 0 0 false self 0 false "" false 0 "NewEnumerator3" "NewEnumerator0"))
        (:Finished
          (switch Utilities|FlowControl|Switch|SwitchonETimelineDirection _direction
            (:Forward
              (bind (_direction_2 _alpha_2) (Timeline|Timeline_1 Play)
                (:Update
                  (if (Variables|Default|GetInteractSection)
                    (Class|BPInteractive|UpdIconWidget(Message) (Variables|Default|GetWidgetInteracUP) (Utilities|Array|Get(acopy) (Variables|Default|GetLoopFrames) (Math|Float|Round (Math|Float|Lerp 0.0 (Math|Conversions|ToFloat(Integer) (Utilities|Array|LastIndex (Variables|Default|GetLoopFrames))) _alpha_2))) (Variables|Default|GetIconText) (Variables|Default|GetStartFlipbook) (Variables|Default|GetLoopFlipbook) 0 0 false self 0 false (Variables|Default|GetVisText) false 0 "NewEnumerator3" "NewEnumerator0")
                    (else
                      (Utilities|FlowControl|Sequence
                        (:then_0
                          (Timeline|Timeline_1 Stop))
                        (:then_1
                          (goto _label))))))
                (:Finished
                  (switch Utilities|FlowControl|Switch|SwitchonETimelineDirection _direction_2
                    (:Forward
                      (if (Variables|Default|GetInteractSection)
                        (Timeline|Timeline_1 PlayFromStart)
                        (else
                          (goto _label))))))))
            (:Backward
              (Class|BPInteractive|UpdIconWidget(Message) (Variables|Default|GetWidgetInteracUP) "/Game/Assets/UI/Icons/Hint_Circle.Hint_Circle" "" 0 0 0 0 false 0 0 false "" false 0 "NewEnumerator3" "NewEnumerator0"))))))))

(event OnComponentBeginOverlap(TriggerToUp)
  (params (OverlappedComponent :type Primitive%20Component%20Object%20Reference) (OtherActor :type Actor%20Object%20Reference) (OtherComp :type Primitive%20Component%20Object%20Reference) (OtherBodyIndex :type Integer) (bFromSweep :type Boolean) (SweepResult :type Hit%20Result%20Structure%20%28by%20ref%29))
  (Development|PrintString "dssd" true true "(R=1.000000,G=0.063851,B=0.000000,A=1.000000)")
  (if (== OtherActor (Variables|Default|GetPlayer))
    (Variables|/Game/Widgets/Assets/tmp/Widget/InteractionWidget.InteractionWidget_C|SetPlayer (Variables|Default|GetWidgetInteracUP) (Variables|Default|GetPlayer))
    (CallFunction|SetInvUpName)
    (Variables|Default|SetInteractSection true)
    (if (Class|TimelineComponent|IsReversing (Variables|Default|GetTimeline_0))
      (Audio|PlaySound2D 0 1.0 1.0 0.0 0 0 :!label _label)
      (Widget|Transform|SetRenderScale (Variables|/Game/Widgets/Assets/tmp/Widget/InteractionWidget.InteractionWidget_C|GetButton_817 (Variables|Default|GetWidgetInteracUP)) "(X=1.000000,Y=1.000000)")
      (bind (_direction _alpha) (Timeline|Timeline_0 Play)
        (:Update
          (Class|BPInteractive|UpdIconWidget(Message) (Variables|Default|GetWidgetInteracUP) (Utilities|Array|Get(acopy) (Variables|Default|GetStartEndFrames) (Math|Float|Round (Math|Float|Lerp 0.0 (Math|Conversions|ToFloat(Integer) (Utilities|Array|LastIndex (Variables|Default|GetStartEndFrames))) _alpha))) (Variables|Default|GetIconText) (Variables|Default|GetStartFlipbook) (Variables|Default|GetLoopFlipbook) 0 0 false self 0 false "" false 0 "NewEnumerator3" "NewEnumerator0"))
        (:Finished
          (switch Utilities|FlowControl|Switch|SwitchonETimelineDirection _direction
            (:Forward
              (bind (_direction_2 _alpha_2) (Timeline|Timeline_1 Play)
                (:Update
                  (if (Variables|Default|GetInteractSection)
                    (Class|BPInteractive|UpdIconWidget(Message) (Variables|Default|GetWidgetInteracUP) (Utilities|Array|Get(acopy) (Variables|Default|GetLoopFrames) (Math|Float|Round (Math|Float|Lerp 0.0 (Math|Conversions|ToFloat(Integer) (Utilities|Array|LastIndex (Variables|Default|GetLoopFrames))) _alpha_2))) (Variables|Default|GetIconText) (Variables|Default|GetStartFlipbook) (Variables|Default|GetLoopFlipbook) 0 0 false self 0 false (Variables|Default|GetVisText) false 0 "NewEnumerator3" "NewEnumerator0")
                    (else
                      (Utilities|FlowControl|Sequence
                        (:then_0
                          (Timeline|Timeline_1 Stop))
                        (:then_1
                          (Audio|PlaySound2D 0 1.0 1.0 0.0 0 0 :!label _label_2)
                          (Timeline|Timeline_0 Reverse))))))
                (:Finished
                  (switch Utilities|FlowControl|Switch|SwitchonETimelineDirection _direction_2
                    (:Forward
                      (if (Variables|Default|GetInteractSection)
                        (Timeline|Timeline_1 PlayFromStart)
                        (else
                          (goto _label_2))))))))
            (:Backward
              (Class|BPInteractive|UpdIconWidget(Message) (Variables|Default|GetWidgetInteracUP) "/Game/Assets/UI/Icons/Hint_Circle.Hint_Circle" "" 0 0 0 0 false 0 0 false "" false 0 "NewEnumerator3" "NewEnumerator0")))))
      (elif (not (Audio|Components|Audio|IsPlaying (Variables|Default|GetTimeline_0)))
        (if (Audio|Components|Audio|IsPlaying (Variables|Default|GetTimeline_1))
          (goto _label)
          (else
            (goto _label)))))))

(event Custom|CloseWidgetDown
  (Variables|Default|SetInteractSection false)
  (if (Audio|Components|Audio|IsPlaying (Variables|Default|GetTimeline_1))
    (Audio|PlaySound2D 0 1.0 1.0 0.0 0 0 :!label _label)
    (bind (_direction _alpha) (Timeline|Timeline_2 Reverse)
      (:Update
        (Class|BPInteractive|UpdIconWidget(Message) (Variables|Default|GetWidgetInteracDown) (Utilities|Array|Get(acopy) (Variables|Default|GetStartEndFrames) (Math|Float|Round (Math|Float|Lerp 0.0 (Math|Conversions|ToFloat(Integer) (Utilities|Array|LastIndex (Variables|Default|GetStartEndFrames))) _alpha))) (Variables|Default|GetIconText) (Variables|Default|GetStartFlipbook) (Variables|Default|GetLoopFlipbook) 0 0 false self 0 false "" false 0 "NewEnumerator3" "NewEnumerator0"))
      (:Finished
        (switch Utilities|FlowControl|Switch|SwitchonETimelineDirection _direction
          (:Forward
            (bind (_direction_2 _alpha_2) (Timeline|Timeline_3 Play)
              (:Update
                (if (Variables|Default|GetInteractSection)
                  (Class|BPInteractive|UpdIconWidget(Message) (Variables|Default|GetWidgetInteracDown) (Utilities|Array|Get(acopy) (Variables|Default|GetLoopFrames) (Math|Float|Round (Math|Float|Lerp 0.0 (Math|Conversions|ToFloat(Integer) (Utilities|Array|LastIndex (Variables|Default|GetLoopFrames))) _alpha_2))) (Variables|Default|GetIconText) (Variables|Default|GetStartFlipbook) (Variables|Default|GetLoopFlipbook) 0 0 false self 0 false (Variables|Default|GetVisText) false 0 "NewEnumerator3" "NewEnumerator0")
                  (else
                    (Utilities|FlowControl|Sequence
                      (:then_0
                        (Timeline|Timeline_3 Stop))
                      (:then_1
                        (goto _label))))))
              (:Finished
                (switch Utilities|FlowControl|Switch|SwitchonETimelineDirection _direction_2
                  (:Forward
                    (if (Variables|Default|GetInteractSection)
                      (Timeline|Timeline_3 PlayFromStart)
                      (else
                        (goto _label)))))))))))))

(event Custom|CloseWidgetUP
  (Variables|Default|SetInteractSection false)
  (if (Audio|Components|Audio|IsPlaying (Variables|Default|GetTimeline_1))
    (Audio|PlaySound2D 0 1.0 1.0 0.0 0 0 :!label _label)
    (bind (_direction _alpha) (Timeline|Timeline_0 Reverse)
      (:Update
        (Class|BPInteractive|UpdIconWidget(Message) (Variables|Default|GetWidgetInteracUP) (Utilities|Array|Get(acopy) (Variables|Default|GetStartEndFrames) (Math|Float|Round (Math|Float|Lerp 0.0 (Math|Conversions|ToFloat(Integer) (Utilities|Array|LastIndex (Variables|Default|GetStartEndFrames))) _alpha))) (Variables|Default|GetIconText) (Variables|Default|GetStartFlipbook) (Variables|Default|GetLoopFlipbook) 0 0 false self 0 false "" false 0 "NewEnumerator3" "NewEnumerator0"))
      (:Finished
        (switch Utilities|FlowControl|Switch|SwitchonETimelineDirection _direction
          (:Forward
            (bind (_direction_2 _alpha_2) (Timeline|Timeline_1 Play)
              (:Update
                (if (Variables|Default|GetInteractSection)
                  (Class|BPInteractive|UpdIconWidget(Message) (Variables|Default|GetWidgetInteracUP) (Utilities|Array|Get(acopy) (Variables|Default|GetLoopFrames) (Math|Float|Round (Math|Float|Lerp 0.0 (Math|Conversions|ToFloat(Integer) (Utilities|Array|LastIndex (Variables|Default|GetLoopFrames))) _alpha_2))) (Variables|Default|GetIconText) (Variables|Default|GetStartFlipbook) (Variables|Default|GetLoopFlipbook) 0 0 false self 0 false (Variables|Default|GetVisText) false 0 "NewEnumerator3" "NewEnumerator0")
                  (else
                    (Utilities|FlowControl|Sequence
                      (:then_0
                        (Timeline|Timeline_1 Stop))
                      (:then_1
                        (goto _label))))))
              (:Finished
                (switch Utilities|FlowControl|Switch|SwitchonETimelineDirection _direction_2
                  (:Forward
                    (if (Variables|Default|GetInteractSection)
                      (Timeline|Timeline_1 PlayFromStart)
                      (else
                        (goto _label))))))))
          (:Backward
            (Class|BPInteractive|UpdIconWidget(Message) (Variables|Default|GetWidgetInteracUP) "/Game/Assets/UI/Icons/Hint_Circle.Hint_Circle" "" 0 0 0 0 false 0 0 false "" false 0 "NewEnumerator3" "NewEnumerator0")))))))

(event EventBeginPlay
  (Utilities|FlowControl|Delay 2.0)
  (bind _outactors (Actor|GetAllActorsOfClass "/Game/Assets/Heroes/Max/BP_CharMax.BP_CharMax_C"))
  (Variables|Default|SetPlayer (Utilities|Array|Get(acopy) _outactors))
  (bind _asinteraction_widget (Utilities|Casting|CastToInteractionWidget (UserInterface|GetUserWidgetObject (Variables|Default|GetInteractionUP))))
  (Variables|Default|SetWidgetInteracUP _asinteraction_widget)
  (bind _asinteraction_widget_2 (Utilities|Casting|CastToInteractionWidget (UserInterface|GetUserWidgetObject (Variables|Default|GetInteractionDown))))
  (Variables|Default|SetWidgetInteracDown _asinteraction_widget_2)
  (Class|BPInteractive|UpdIconWidget(Message) (Variables|Default|GetWidgetInteracUP) 0 "" 0 0 0 0 false 0 0 false "" false 0 "NewEnumerator3" "NewEnumerator0"))

(event Collision|EventActorBeginOverlap
  (params (OtherActor :type Actor%20Object%20Reference)))

(event EventTick
  (params (DeltaSeconds :type Float%20%28single-precision%29))
  (bind _returnvalue (Transformation|GetActorLocation))
  (bind _player (Variables|Default|GetPlayer))
  (bind _widgetinteracup (Variables|Default|GetWidgetInteracUP))
  (bind _returnvalue_2 (Transformation|GetActorLocation _player))
  (bind _button_817 (Variables|/Game/Widgets/Assets/tmp/Widget/InteractionWidget.InteractionWidget_C|GetButton_817 _widgetinteracup))
  (bind _returnvalue_3 (Math|Vector|Distance(Vector) _returnvalue _returnvalue_2))
  (bind _backgroundcolor (Variables|/Script/UMG.Button|GetBackgroundColor _button_817))
  (bind _returnvalue_4 (Math|Float|Clamp(Float) _returnvalue_3 1e+02 5e+02))
  (bind _returnvalue_5 (Math|Float|MapRangeClamped _returnvalue_4 1e+02 5e+02 1.0 0.0))
  (bind _returnvalue_6 (Math|Float|MapRangeClamped _returnvalue_5 0.0 1.0 0.5 1.25))
  (Class|Button|SetBackgroundColor _button_817 (Utilities|Struct|MakeLinearColor (.r _backgroundcolor) (.g _backgroundcolor) (.b _backgroundcolor) _returnvalue_5))
  (Widget|Transform|SetRenderScale _button_817 (Math|Vector2D|MakeVector2D _returnvalue_6 _returnvalue_6)))

(event EventInteractwithWidget
  (Variables|/Game/Assets/Heroes/Max/BP_CharMax.BP_CharMax_C|SetParkourState (Variables|Default|GetPlayer) "NewEnumerator1")
  (switch Utilities|FlowControl|Switch|SwitchonParkourState (Variables|/Game/Assets/Heroes/Max/BP_CharMax.BP_CharMax_C|GetParkourState (Variables|Default|GetPlayer))
    (:NewEnumerator1
      (Variables|/Game/Assets/Heroes/Max/BP_CharMax.BP_CharMax_C|SetParkourState (Variables|Default|GetPlayer) "NewEnumerator0")
      (Variables|/Game/Assets/Heroes/Max/BP_CharMax.BP_CharMax_C|SetOnParcour (Variables|Default|GetPlayer) true)
      (Variables|Default|SetBool2 false)
      (CallFunction|CloseWidgetUP)
      (Variables|Default|SetVet (Transformation|GetActorLocation (Variables|Default|GetPlayer)))
      (Default|MovePLayer (Variables|Default|GetPlayer) 0 (Transformation|GetWorldLocation (Variables|Default|GetArrowToUp)) true (Transformation|GetWorldRotation (Variables|Default|GetArrowToUp)) self (Variables|Default|GetStartUpState) 0 "0, 0, 0" 0 false 0 false))))

(fn ConstructionScript
  (bind _arrowtoup (Variables|Default|GetArrowToUp))
  (bind _newparam (CallFunction|GetPoins))
  (if (Variables|Default|GetIsManual?)
    (Transformation|SetRelativeLocation _arrowtoup (Math|Vector|MakeVector 73.0 0.0 (- (+ (.Z (Math|Vector|BreakVector (Transformation|GetActorLocation))) 1e+01) (.Z (Math|Vector|BreakVector (.Location (Math|Transform|BreakTransform _newparam)))))) false false)
    (Variables|Default|SetMeshHeight (- (.Z (Math|Vector|BreakVector (.Location (Math|Transform|BreakTransform _newparam)))) (Variables|Default|GetMeshHeightMid)))
    (else
      (Transformation|SetWorldTransform (Variables|Default|GetArrowToDown) _newparam false false)
      (Transformation|SetRelativeLocation _arrowtoup (Math|Vector|MakeVector 73.0 0.0 (- (+ (.Z (Math|Vector|BreakVector (Transformation|GetActorLocation))) 1e+01) (.Z (Math|Vector|BreakVector (.Location (Math|Transform|BreakTransform _newparam)))))) false false)
      (Variables|Default|SetMeshHeight (- (.Z (Math|Vector|BreakVector (.Location (Math|Transform|BreakTransform _newparam)))) (Variables|Default|GetJumpDistance))))))

(fn SetInvUpName
  (switch Utilities|FlowControl|Switch|SwitchonGameLanguage (Variables|/Game/Blueprints/Transfered/Blueprints1/MyGameInstance.MyGameInstance_C|GetLanguage (.AsMy%20Game%20Instance (Utilities|Casting|CastToMyGameInstance (Game|GetGameInstance))))
    (:NewEnumerator0
      (Variables|Default|SetVisText (Variables|Default|GetRusUpName)))
    (:NewEnumerator1
      (Variables|Default|SetVisText (Variables|Default|GetEngUPName)))))

(fn SetInvDownName
  (switch Utilities|FlowControl|Switch|SwitchonGameLanguage (Variables|/Game/Blueprints/Transfered/Blueprints1/MyGameInstance.MyGameInstance_C|GetLanguage (.AsMy%20Game%20Instance (Utilities|Casting|CastToMyGameInstance (Game|GetGameInstance))))
    (:NewEnumerator0
      (Variables|Default|SetVisText (Variables|Default|GetRusDownName)))
    (:NewEnumerator1
      (Variables|Default|SetVisText (Variables|Default|GetEngDownName)))))

(fn GetPoins
  (bind (_array _array2) (Utilities|Toppoints))
  (bind (_array3 _array4) (Utilities|Midpoints))
  (LocalVariables|SetVecMids _array3)
  (LocalVariables|SetMidspo _array4)
  (LocalVariables|SetNewLocalVar_0 _array2)
  (LocalVariables|SetVecAr _array)
  (LocalVariables|Setpoint1 (Utilities|Array|Get(acopy) (LocalVariables|GetVecAr) (.IndexOfMinValue (Math|Float|MinOfFloatArray (LocalVariables|GetNewLocalVar_0)))))
  (Utilities|Array|SetArrayElem (LocalVariables|GetNewLocalVar_0) (.IndexOfMinValue (Math|Float|MinOfFloatArray (LocalVariables|GetNewLocalVar_0))) (+ (.MaxValue (Math|Float|MaxOfFloatArray (LocalVariables|GetNewLocalVar_0))) 1e+02))
  (LocalVariables|Setpoint2 (Utilities|Array|Get(acopy) (LocalVariables|GetVecAr) (.IndexOfMinValue (Math|Float|MinOfFloatArray (LocalVariables|GetNewLocalVar_0)))))
  (return (Math|Transform|MakeTransform (Math|Vector|FindClosestPointonSegment (Transformation|GetActorLocation) (LocalVariables|Getpoint1) (LocalVariables|Getpoint2)) (Math|Rotator|MakeRotator 0.0 0.0 (+ (.Yaw (Math|Rotator|BreakRotator (Transformation|GetActorRotation (Variables|Default|GetMeshToJumpOn)))) (.Yaw (Math|Rotator|BreakRotator (Utilities|Array|Get(acopy) (Utilities|Array|MakeArray "0, 0, 0" "0,180.000000, 0" "0,-90.000000, 0" "0,90.000000, 0") (.IndexOfMinValue (Math|Float|MinOfFloatArray (LocalVariables|GetMidspo))))))))) (.IndexOfMinValue (Math|Float|MinOfFloatArray (LocalVariables|GetMidspo)))))