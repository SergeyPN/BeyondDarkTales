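; Interactable actor that shows an animated icon widget when the player enters its overlap sphere.
; Construction script picks icon frames and Box or Sphere shape, and places the widget above a linked actor.
; StartEnd and Loop timelines step through frame textures as a flipbook, with appear and disappear sounds.
; Enabling swaps the linked mesh to a shine material, and interacting with a trigger actor enables other BP_ActorMain instances, chaining interactions.
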(event OnComponentBeginOverlap(Sphere)
  (params (OverlappedComponent :type Primitive%20Component%20Object%20Reference) (OtherActor :type Actor%20Object%20Reference) (OtherComp :type Primitive%20Component%20Object%20Reference) (OtherBodyIndex :type Integer) (bFromSweep :type Boolean) (SweepResult :type Hit%20Result%20Structure%20%28by%20ref%29))
  (if (== OtherActor (Variables|Default|GetPlayer))
    (if (Variables|Default|GetAbleToInteract)
      (Variables|Default|SetIsInteracting true)
      (if (Class|TimelineComponent|IsReversing (Variables|Default|GetStart/End))
        (Audio|PlaySound2D "/Game/Audio/Snd/FX/ButtonAppear.ButtonAppear" 1.0 1.0 0.0 0 0 :!label _label)
        (Widget|Transform|SetRenderScale (Variables|/Game/Widgets/Assets/tmp/Widget/InteractionWidget.InteractionWidget_C|GetButton_817 (Variables|Default|GetIntW)) "(X=1.000000,Y=1.000000)")
        (bind (_direction _alpha) (Timeline|Start/End Play)
          (:Update
            (Default|UpdIconWidget (Variables|Default|GetIntW) (Utilities|Array|Get(acopy) (Variables|Default|GetStart/EndFrames) (Math|Float|Round (Math|Float|Lerp 0.0 (Math|Conversions|ToFloat(Integer) (Utilities|Array|LastIndex (Variables|Default|GetStart/EndFrames))) _alpha))) "" 0 0 0 0 false self 0 false "" false))
          (:Finished
            (switch Utilities|FlowControl|Switch|SwitchonETimelineDirection _direction
              (:Forward
                (bind (_direction_2 _alpha_2) (Timeline|Loop Play)
                  (:Update
                    (Default|UpdIconWidget (Variables|Default|GetIntW) (Utilities|Array|Get(acopy) (Variables|Default|GetLoopFrames) (Math|Float|Round (Math|Float|Lerp 0.0 (Math|Conversions|ToFloat(Integer) (Utilities|Array|LastIndex (Variables|Default|GetLoopFrames))) _alpha_2))) "" 0 0 0 0 false self 0 false "" false))
                  (:Finished
                    (switch Utilities|FlowControl|Switch|SwitchonETimelineDirection _direction_2
                      (:Forward
                        (if (Variables|Default|GetIsInteracting)
                          (Timeline|Loop PlayFromStart))))))))))
        (elif (not (Audio|Components|Audio|IsPlaying (Variables|Default|GetStart/End)))
          (if (not (Audio|Components|Audio|IsPlaying (Variables|Default|GetLoop)))
            (goto _label)))))))

(event OnComponentEndOverlap(InteractionWidget)
  (params (OverlappedComponent :type Primitive%20Component%20Object%20Reference) (OtherActor :type Actor%20Object%20Reference) (OtherComp :type Primitive%20Component%20Object%20Reference) (OtherBodyIndex :type Integer))
  (if (== OtherActor (Variables|Default|GetPlayer))
    (if (Variables|Default|GetIsInteracting)
      (Variables|Default|SetIsInteracting false)
      (if (Audio|Components|Audio|IsPlaying (Variables|Default|GetLoop))
        (Audio|Components|Audio|Stop (Variables|Default|GetLoop)))
      (Audio|PlaySound2D "/Game/Audio/Snd/FX/ButtonDisappear.ButtonDisappear" 1.0 1.0 0.0 0 0)
      (bind (_direction _alpha) (Timeline|Start/End Reverse)
        (:Update
          (Default|UpdIconWidget (Variables|Default|GetIntW) (Utilities|Array|Get(acopy) (Variables|Default|GetStart/EndFrames) (Math|Float|Round (Math|Float|Lerp 0.0 (Math|Conversions|ToFloat(Integer) (Utilities|Array|LastIndex (Variables|Default|GetStart/EndFrames))) _alpha))) "" 0 0 0 0 false self 0 false "" false))
        (:Finished
          (switch Utilities|FlowControl|Switch|SwitchonETimelineDirection _direction
            (:Forward
              (bind (_direction_2 _alpha_2) (Timeline|Loop Play)
                (:Update
                  (Default|UpdIconWidget (Variables|Default|GetIntW) (Utilities|Array|Get(acopy) (Variables|Default|GetLoopFrames) (Math|Float|Round (Math|Float|Lerp 0.0 (Math|Conversions|ToFloat(Integer) (Utilities|Array|LastIndex (Variables|Default|GetLoopFrames))) _alpha_2))) "" 0 0 0 0 false self 0 false "" false))
                (:Finished
                  (switch Utilities|FlowControl|Switch|SwitchonETimelineDirection _direction_2
                    (:Forward
                      (if (Variables|Default|GetIsInteracting)
                        (Timeline|Loop PlayFromStart)))))))))))))

(event Custom|ShowInteract
  (Variables|Default|SetIsInteracting true)
  (if (Class|TimelineComponent|IsReversing (Variables|Default|GetStart/End))
    (Audio|PlaySound2D "/Game/Audio/Snd/FX/ButtonAppear.ButtonAppear" 1.0 1.0 0.0 0 0 :!label _label)
    (Widget|Transform|SetRenderScale (Variables|/Game/Widgets/Assets/tmp/Widget/InteractionWidget.InteractionWidget_C|GetButton_817 (Variables|Default|GetIntW)) "(X=1.000000,Y=1.000000)")
    (bind (_direction _alpha) (Timeline|Start/End Play)
      (:Update
        (Default|UpdIconWidget (Variables|Default|GetIntW) (Utilities|Array|Get(acopy) (Variables|Default|GetStart/EndFrames) (Math|Float|Round (Math|Float|Lerp 0.0 (Math|Conversions|ToFloat(Integer) (Utilities|Array|LastIndex (Variables|Default|GetStart/EndFrames))) _alpha))) "" 0 0 0 0 false self 0 false "" false))
      (:Finished
        (switch Utilities|FlowControl|Switch|SwitchonETimelineDirection _direction
          (:Forward
            (bind (_direction_2 _alpha_2) (Timeline|Loop Play)
              (:Update
                (Default|UpdIconWidget (Variables|Default|GetIntW) (Utilities|Array|Get(acopy) (Variables|Default|GetLoopFrames) (Math|Float|Round (Math|Float|Lerp 0.0 (Math|Conversions|ToFloat(Integer) (Utilities|Array|LastIndex (Variables|Default|GetLoopFrames))) _alpha_2))) "" 0 0 0 0 false self 0 false "" false))
              (:Finished
                (switch Utilities|FlowControl|Switch|SwitchonETimelineDirection _direction_2
                  (:Forward
                    (if (Variables|Default|GetIsInteracting)
                      (Timeline|Loop PlayFromStart))))))))))
    (elif (not (Audio|Components|Audio|IsPlaying (Variables|Default|GetStart/End)))
      (if (not (Audio|Components|Audio|IsPlaying (Variables|Default|GetLoop)))
        (goto _label)))))

(event Custom|HideInteract
  (Variables|Default|SetIsInteracting false)
  (if (Audio|Components|Audio|IsPlaying (Variables|Default|GetLoop))
    (Audio|Components|Audio|Stop (Variables|Default|GetLoop)))
  (Audio|PlaySound2D "/Game/Audio/Snd/FX/ButtonDisappear.ButtonDisappear" 1.0 1.0 0.0 0 0)
  (bind (_direction _alpha) (Timeline|Start/End Reverse)
    (:Update
      (Default|UpdIconWidget (Variables|Default|GetIntW) (Utilities|Array|Get(acopy) (Variables|Default|GetStart/EndFrames) (Math|Float|Round (Math|Float|Lerp 0.0 (Math|Conversions|ToFloat(Integer) (Utilities|Array|LastIndex (Variables|Default|GetStart/EndFrames))) _alpha))) "" 0 0 0 0 false self 0 false "" false))
    (:Finished
      (switch Utilities|FlowControl|Switch|SwitchonETimelineDirection _direction
        (:Forward
          (bind (_direction_2 _alpha_2) (Timeline|Loop Play)
            (:Update
              (Default|UpdIconWidget (Variables|Default|GetIntW) (Utilities|Array|Get(acopy) (Variables|Default|GetLoopFrames) (Math|Float|Round (Math|Float|Lerp 0.0 (Math|Conversions|ToFloat(Integer) (Utilities|Array|LastIndex (Variables|Default|GetLoopFrames))) _alpha_2))) "" 0 0 0 0 false self 0 false "" false))
            (:Finished
              (switch Utilities|FlowControl|Switch|SwitchonETimelineDirection _direction_2
                (:Forward
                  (if (Variables|Default|GetIsInteracting)
                    (Timeline|Loop PlayFromStart)))))))))))

(event EventBeginPlay
  (bind _outactors (Actor|GetAllActorsOfClass "/Game/Assets/Heroes/Max/MaxCharTest.MaxCharTest_C"))
  (Variables|Default|SetPlayer (Utilities|Array|Get(acopy) _outactors))
  (bind _asinteraction_widget (Utilities|Casting|CastToInteractionWidget (UserInterface|GetUserWidgetObject (Variables|Default|GetInteractionWidget))))
  (Variables|Default|SetIntW _asinteraction_widget)
  (if (Variables|Default|GetStartEnabled?)
    (Default|SetEnabled (Variables|Default|GetIntW) (Variables|Default|GetPlayer) self)))

(event EventInteractwithWidget
  (CallFunction|TriggerActors))

(fn ConstructionScript
  (bind _overlapradius (Variables|Default|GetOverlapRadius))
  (bind _actortousewith (Variables|Default|GetActorToUseWith))
  (bind _origin (Collision|GetActorBounds _actortousewith false false))
  (CallFunction|SetIcons (Variables|Default|GetIconsToUse))
  (if (Variables|Default|GetBoxOrSphereCollision)
    (Collision|SetCollisionEnabled (Variables|Default|GetSphere) "NoCollision")
    (Rendering|SetVisibility (Variables|Default|GetSphere) false false)
    (Rendering|SetVisibility (Variables|Default|GetBox) true false)
    (Collision|SetCollisionEnabled (Variables|Default|GetBox) "QueryOnly")
    (Components|Box|SetBoxExtent (Variables|Default|GetBox) (Math|Vector|MakeVector _overlapradius _overlapradius 32.0) true)
    (else
      (Collision|SetCollisionEnabled (Variables|Default|GetBox) "NoCollision")
      (Rendering|SetVisibility (Variables|Default|GetBox) false false)
      (Rendering|SetVisibility (Variables|Default|GetSphere) true false)
      (Collision|SetCollisionEnabled (Variables|Default|GetSphere) "QueryOnly")
      (Components|Sphere|SetSphereRadius (Variables|Default|GetSphere) (Variables|Default|GetOverlapRadius) true)))
  (if (!= (Variables|Default|GetActorToUseWith) 0)
    (Transformation|SetWorldLocation (Variables|Default|GetSphere1) (Math|Vector|MakeVector (.x _origin) (.y _origin) (+ (.z _origin) 2.5e+02)) false false)
    (CallFunction|Enable/DisableActor (Variables|Default|GetStartEnabled?))))

(fn Enable/DisableActor
  (params (IsOn? :type Boolean))
  (bind _actortousewith (Variables|Default|GetActorToUseWith))
  (bind _asstatic_mesh_actor (Utilities|Casting|CastToStaticMeshActor _actortousewith))
  (bind _staticmeshcomponent (Variables|/Script/Engine.StaticMeshActor|GetStaticMeshComponent _asstatic_mesh_actor))
  (if IsOn?
    (Variables|Default|SetAbleToInteract true)
    (Rendering|Material|SetMaterial _staticmeshcomponent 0 "/Game/Assets/Maps/UniversalMats/M_ShineFX_Inst.M_ShineFX_Inst")
    (Utilities|IsValid (Variables|Default|GetPlayer)
      (:Is%20Valid
        (Default|SetEnabled (Variables|Default|GetIntW) (Variables|Default|GetPlayer) self)))
    (else
      (Variables|Default|SetAbleToInteract false)
      (Rendering|Material|SetMaterial _staticmeshcomponent 0 "/Game/Assets/Heroes/Max/Mats/MI_Max.MI_Max")
      (Default|SetDisabled (Variables|Default|GetIntW)))))

(fn SetIcons
  (params (Selection :type IconsTypes%20Enum :default "NewEnumerator5"))
  (switch Utilities|FlowControl|Switch|SwitchonIconsTypes Selection
    (:NewEnumerator5
      (|EmptyIcons))
    (:NewEnumerator0
      (|CommentIcons))
    (:NewEnumerator1
      (|DoorIcons))
    (:NewEnumerator2
      (|GrabIcons))
    (:NewEnumerator3
      (|HOIcons))
    (:NewEnumerator4
      (|PzzleIcons))))

(fn TriggerActors
  (if (Variables|Trigger|GetIsTrigger?)
    (for _array_element (Variables|Trigger|GetActorToTrigger)
      (bind _asbp_actor_main (Utilities|Casting|CastToBP_ActorMain _array_element))
      (CallFunction|Enable/DisableActor _asbp_actor_main true))))