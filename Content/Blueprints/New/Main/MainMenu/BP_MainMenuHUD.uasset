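; BP_MainMenuHUD creates and stores the game's menu and popup widgets on BeginPlay, from main menu and pause to tutorial and credits.
; It shows the loading screen outside the intro level and optionally adds a shipping debug overlay.
; IconFly uses a timeline to slide a widget between two points, then notifies its owner.
; HideTutorialOpenInterface unpauses, restores the player controller's main interface and shows the first quest from the GameInstance.
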(event Custom|HideTutorialOpenInterface
  (Game|SetGamePaused false)
  (bind _as01cm_pc (Utilities|Casting|CastTo01CM_PC (Game|GetPlayerController 0)))
  (UserInterface|Viewport|AddtoViewport (Variables|/Game/Blueprints/New/Main/01CaveMain/01CM_PC.01CM_PC_C|GetMainInterface_W _as01cm_pc) 0)
  (UserInterface|Animation|PlayAnimation (Variables|/Game/Blueprints/New/Main/01CaveMain/01CM_PC.01CM_PC_C|GetMainInterface_W _as01cm_pc) (Variables|/Game/Widgets/New/MainInterface_W.MainInterface_W_C|GetShowInterfaceWithPauseAndHideBackPack (Variables|/Game/Blueprints/New/Main/01CaveMain/01CM_PC.01CM_PC_C|GetMainInterface_W _as01cm_pc)) 0.0 1 "Forward" 4.0 false)
  (bind _asmy_game_instance (Utilities|Casting|CastToMyGameInstance (Game|GetGameInstance)))
  (bind _keys (Utilities|Map|Keys (Variables|/Game/Blueprints/Transfered/Blueprints1/MyGameInstance.MyGameInstance_C|GetQuestsStatus _asmy_game_instance)))
  (Default|ShowQuest (Variables|/Game/Blueprints/New/Main/01CaveMain/01CM_PC.01CM_PC_C|GetMainInterface_W _as01cm_pc) (Utilities|String|StringToName (Utilities|String|EnumtoString (Utilities|Array|Get(acopy) _keys)))))

(event Custom|IconFly
  (params (MOvedW :type Widget%20Object%20Reference) (Target :type Canvas%20Panel%20Slot%20Object%20Reference) (Start :type Vector%202D%20Structure) (End :type Vector%202D%20Structure) (OwnerW :type W%20Inventory%20Item%20Object%20Reference))
  (bind (_x _y) (Math|Vector2D|BreakVector2D Start))
  (bind (_x_2 _y_2) (Math|Vector2D|BreakVector2D End))
  (Audio|PlaySound2D "/Game/Audio/Snd/FX/InvReturn.InvReturn" 1.0 1.0 0.0 0 0)
  (bind _alpha (Timeline|TimelineFlyIcon PlayFromStart)
    (:Update
      (Class|CanvasPanelSlot|SetPosition Target (Math|Vector2D|MakeVector2D (.x (Math|Vector|Lerp(Vector) (Math|Vector|MakeVector _x _y 0.0) (Math|Vector|MakeVector _x_2 _y_2 0.0) _alpha)) (.y (Math|Vector|Lerp(Vector) (Math|Vector|MakeVector _x _y 0.0) (Math|Vector|MakeVector _x_2 _y_2 0.0) _alpha)))))
    (:Finished
      (Default|IconFlyEnd OwnerW MOvedW))))

(event EventBeginPlay
  (bind _returnvalue (UserInterface|CreateWidget "/Game/Widgets/LoadingScreen/WB_LoadingScreen.WB_LoadingScreen_C"))
  (bind _output_get (Variables|Default|SetLoadingScreenWidget _returnvalue))
  (bind _returnvalue_2 (Game|GetCurrentLevelName true))
  (if (Utilities|Enum|Equal(Enum) _returnvalue_2 "01_IntroBegin")
    _
    (else
      (UserInterface|Viewport|AddtoViewport _output_get 0)))
  (bind _returnvalue_3 (UserInterface|CreateWidget "/Game/Widgets/MainMenu/WB_MainMenuSeason.WB_MainMenuSeason_C"))
  (Variables|Default|SetMainMenuSeasonWidget _returnvalue_3)
  (bind _returnvalue_4 (UserInterface|CreateWidget "/Game/Widgets/MainMenu/WB_MainMenuActs.WB_MainMenuActs_C"))
  (Variables|Default|SetMainMenuActsWidget _returnvalue_4)
  (bind _returnvalue_5 (UserInterface|CreateWidget "/Game/Widgets/MainMenu/WB_Options.WB_Options_C"))
  (Variables|Default|SetOptionsWidget _returnvalue_5)
  (bind _returnvalue_6 (UserInterface|CreateWidget "/Game/Widgets/PauseMenu/WBP_PauseMenu.WBP_PauseMenu_C"))
  (Variables|Default|SetPauseMenuWidget _returnvalue_6)
  (Utilities|FlowControl|Sequence
    (:then_0
      (bind _returnvalue_7 (UserInterface|CreateWidget "/Game/Widgets/Tutorial/WB_Tutorial.WB_Tutorial_C"))
      (Variables|Default|SetTutorialWidget _returnvalue_7)
      (bind _returnvalue_8 (UserInterface|CreateWidget "/Game/Widgets/PauseMenu/WBP_Confirm.WBP_Confirm_C"))
      (Variables|Default|SetConfirmWidget _returnvalue_8)
      (bind _returnvalue_9 (UserInterface|CreateWidget "/Game/Widgets/MainMenu/WBP_ShareMenu.WBP_ShareMenu_C"))
      (Variables|Default|SetShareMenuWidget _returnvalue_9)
      (bind _returnvalue_10 (UserInterface|CreateWidget "/Game/Widgets/Inventory/WB_GetItem.WB_GetItem_C"))
      (Variables|Default|SetGetItemWidget _returnvalue_10)
      (bind _returnvalue_11 (UserInterface|CreateWidget "/Game/Widgets/MainMenu/Skins/WBP_Skins.WBP_Skins_C"))
      (Variables|Default|SetSkinsWidget _returnvalue_11)
      (if (Variables|Develop|GetActivateShippingDebugMessages)
        (bind _returnvalue_12 (UserInterface|CreateWidget "/Game/Widgets/ForDevelopAndTesting/WBP_DebugMessageShipping.WBP_DebugMessageShipping_C"))
        (bind _output_get_2 (Variables|Default|SetDebugMessageShippingWidget _returnvalue_12))
        (UserInterface|Viewport|AddtoViewport _output_get_2 2))
      (bind _returnvalue_13 (UserInterface|CreateWidget "/Game/Widgets/MainMenu/WBP_Credits.WBP_Credits_C"))
      (Variables|Default|SetCreditsWidget _returnvalue_13)
      (bind _returnvalue_14 (UserInterface|CreateWidget "/Game/Widgets/MainMenu/WBP_CheckPointsMenu.WBP_CheckPointsMenu_C"))
      (Variables|Default|SetCheckPointsMenuWidget _returnvalue_14))))

(fn ConstructionScript)