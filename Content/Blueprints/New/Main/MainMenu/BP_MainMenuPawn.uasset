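; Main menu pawn that drives the menu camera and handles touch gestures.
; Timelines lerp it to and from target transforms, slide it sideways between act points, and ping-pong a yaw wobble.
; Horizontal drags over 50 pixels swipe the season or act widgets, while dragging with the skins widget open rotates CharMax.
; On BeginPlay it caches controller, HUD and character, then adjusts cine camera focal length for the viewport aspect ratio.
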(event Custom|MoveCameraInStartPosition
  (params (Forward/Back :type Boolean) (TargetMoving :type Vector) (ReturnMoving :type Vector) (TargetRotation :type Rotator) (ReturnRotation :type Rotator) (ON/OFFWobbleCamera :type Boolean))
  (if Forward/Back
    (Variables|Default|SetStartTransform (Transformation|GetActorTransform))
    (CallFunction|ON/OFFWobbleCamera ON/OFFWobbleCamera)
    (bind _alpha (Timeline|StartPositionTimeline PlayFromStart)
      (:Update
        (if Forward/Back
          (Transformation|SetActorLocation (Math|Vector|Lerp(Vector) (Transformation|GetActorLocation) TargetMoving _alpha) false false)
          (Transformation|SetActorRotation (Math|Rotator|Lerp(Rotator) (Transformation|GetActorRotation) TargetRotation _alpha))
          (else
            (Transformation|SetActorLocation (Math|Vector|Lerp(Vector) ReturnMoving (Transformation|GetActorLocation) _alpha) false false)
            (Transformation|SetActorRotation (Math|Rotator|Lerp(Rotator) ReturnRotation (Transformation|GetActorRotation) _alpha))))))
    (else
      (CallFunction|ON/OFFWobbleCamera ON/OFFWobbleCamera)
      (Timeline|StartPositionTimeline ReverseFromEnd))))

(event Custom|MoveCameraLeft/Right
  (params (TargetAct :type Integer))
  (bind _returnvalue (Transformation|GetActorLocation))
  (Utilities|FlowControl|Sequence
    (:then_0
      (bind _alpha (Timeline|StartPositionTimeline Stop)
        (:Update
          (if (stale Custom|MoveCameraInStartPosition Forward/Back)
            (Transformation|SetActorLocation (Math|Vector|Lerp(Vector) (Transformation|GetActorLocation) (stale Custom|MoveCameraInStartPosition TargetMoving) _alpha) false false)
            (Transformation|SetActorRotation (Math|Rotator|Lerp(Rotator) (Transformation|GetActorRotation) (stale Custom|MoveCameraInStartPosition TargetRotation) _alpha))
            (else
              (Transformation|SetActorLocation (Math|Vector|Lerp(Vector) (stale Custom|MoveCameraInStartPosition ReturnMoving) (Transformation|GetActorLocation) _alpha) false false)
              (Transformation|SetActorRotation (Math|Rotator|Lerp(Rotator) (stale Custom|MoveCameraInStartPosition ReturnRotation) (Transformation|GetActorRotation) _alpha)))))))
    (:then_1
      (bind _alpha_2 (Timeline|Left/RightCameraTimeline PlayFromStart)
        (:Update
          (Transformation|SetActorLocation (Math|Vector|Lerp(Vector) (Transformation|GetActorLocation) (Math|Vector|MakeVector (.x _returnvalue) (.y (Transformation|GetActorLocation (Utilities|Array|Get(acopy) (Variables|/Game/Blueprints/New/Main/MainMenu/BP_MainMenuPC.BP_MainMenuPC_C|GetPointActs (Variables|Default|GetPlayerController)) TargetAct))) (.z _returnvalue)) _alpha_2) false false))))))

(event Custom|ON/OFFWobbleCamera
  (params (ON/OFF :type Boolean))
  (bind _scene (Variables|Default|GetScene))
  (bind _relativerotation (Variables|/Script/Engine.SceneComponent|GetRelativeRotation _scene))
  (if ON/OFF
    (Components|Timeline|SetPlayRate (Variables|Default|GetWobbleTimeline) 0.3)
    (bind _zrotation (Timeline|WobbleTimeline PlayFromStart)
      (:Update
        (Transformation|SetRelativeRotation (Variables|Default|GetScene) (Math|Rotator|MakeRotator (.roll _relativerotation) (.pitch _relativerotation) (+ _zrotation (.yaw _relativerotation))) false false))
      (:Finished
        (Utilities|FlowControl|FlipFlop
          (:A
            (Timeline|WobbleTimeline ReverseFromEnd))
          (:B
            (Timeline|WobbleTimeline PlayFromStart)))))
    (else
      (Utilities|FlowControl|Sequence
        (:then_0
          (Timeline|WobbleTimeline Stop))
        (:then_1
          (bind _zrotation_2 (Timeline|ReturnRotationSprinArmTimeline PlayFromStart)
            (:Update
              (Transformation|SetRelativeRotation (Variables|Default|GetScene) (Math|Rotator|Lerp(Rotator) (Variables|/Script/Engine.SceneComponent|GetRelativeRotation (Variables|Default|GetScene)) "0, 0, 0" _zrotation_2) false false))))))))

(event EventBeginPlay
  (bind _returnvalue (Viewport|GetViewportSize))
  (bind _asbp_main_menu_pc (Utilities|Casting|CastToBP_MainMenuPC (Game|GetPlayerController 0)))
  (Variables|Default|SetPlayerController _asbp_main_menu_pc)
  (bind _returnvalue_2 (Actor|GetActorOfClass "/Game/Assets/Heroes/Max/BP_CharMax.BP_CharMax_C"))
  (Variables|Default|SetCharMax _returnvalue_2)
  (bind _asbp_main_menu_hud (Utilities|Casting|CastToBP_MainMenuHUD (HUD|GetHUD (Game|GetPlayerController 0))))
  (Variables|Default|SetHUD _asbp_main_menu_hud)
  (Utilities|FlowControl|Delay 0.5)
  (Variables|/Script/CinematicCamera.CineCameraComponent|SetCurrentFocalLength (Variables|Default|GetCineCamera) (- (Variables|Default|GetDefaultFOV) (* (- (/ (.x _returnvalue) (.y _returnvalue)) (Variables|Default|GetDefaultRatio)) 48.0))))

(event EventTick
  (params (DeltaSeconds :type Float%20%28single-precision%29)))

(event Input|TouchEvents|InputTouch
  (params (Location :type Vector) (FingerIndex :type ETouchIndex%20Enum))
  (bind (_x _y) (Math|Vector|BreakVector Location))
  (bind _hud (Variables|Default|GetHUD))
  (bind _hud_2 (Variables|Default|GetHUD))
  (bind _mainmenuseasonwidget (Variables|/Game/Blueprints/New/Main/MainMenu/BP_MainMenuHUD.BP_MainMenuHUD_C|GetMainMenuSeasonWidget _hud_2))
  (bind _mainmenuactswidget (Variables|/Game/Blueprints/New/Main/MainMenu/BP_MainMenuHUD.BP_MainMenuHUD_C|GetMainMenuActsWidget _hud))
  (:Pressed
    (bind _output_get (Variables|Default|SetStartTap (Math|Vector2D|MakeVector2D _x _y)))
    (Variables|Default|SetEndTap _output_get))
  (:Released
    (goto _label Reset))
  (:Moved
    (Utilities|RotateSkin _x
      (:SkinsWindowOut
        (Variables|Default|SetEndTap (Math|Vector2D|MakeVector2D _x _y))
        (if (> (Math|Float|Absolute(Float) (.x (- (Variables|Default|GetEndTap) (Variables|Default|GetStartTap)))) 5e+01)
          (Utilities|FlowControl|DoOnce false :!label _label
            (:Completed
              (if (UserInterface|Viewport|IsinViewport (Variables|/Game/Blueprints/New/Main/MainMenu/BP_MainMenuHUD.BP_MainMenuHUD_C|GetMainMenuSeasonWidget (Variables|Default|GetHUD)))
                (if (> (.x (Variables|Default|GetStartTap)) (.x (Variables|Default|GetEndTap)))
                  (if (Widget|IsVisible (Variables|/Game/Widgets/MainMenu/WB_MainMenuSeason.WB_MainMenuSeason_C|GetButtonRightArrow (Variables|/Game/Blueprints/New/Main/MainMenu/BP_MainMenuHUD.BP_MainMenuHUD_C|GetMainMenuSeasonWidget (Variables|Default|GetHUD))))
                    (Default|SwipeLeft _mainmenuseasonwidget))
                  (elif (Widget|IsVisible (Variables|/Game/Widgets/MainMenu/WB_MainMenuSeason.WB_MainMenuSeason_C|GetButtonLeftArrow (Variables|/Game/Blueprints/New/Main/MainMenu/BP_MainMenuHUD.BP_MainMenuHUD_C|GetMainMenuSeasonWidget (Variables|Default|GetHUD))))
                    (Default|SwipeRight _mainmenuseasonwidget)))
                (elif (UserInterface|Viewport|IsinViewport (Variables|/Game/Blueprints/New/Main/MainMenu/BP_MainMenuHUD.BP_MainMenuHUD_C|GetMainMenuActsWidget (Variables|Default|GetHUD)))
                  (if (> (.x (Variables|Default|GetStartTap)) (.x (Variables|Default|GetEndTap)))
                    (if (Widget|IsVisible (Variables|/Game/Widgets/MainMenu/WB_MainMenuActs.WB_MainMenuActs_C|GetButtonRightArrow (Variables|/Game/Blueprints/New/Main/MainMenu/BP_MainMenuHUD.BP_MainMenuHUD_C|GetMainMenuActsWidget (Variables|Default|GetHUD))))
                      (Default|LeftSwipe _mainmenuactswidget))
                    (elif (Widget|IsVisible (Variables|/Game/Widgets/MainMenu/WB_MainMenuActs.WB_MainMenuActs_C|GetButtonLeftArrow (Variables|/Game/Blueprints/New/Main/MainMenu/BP_MainMenuHUD.BP_MainMenuHUD_C|GetMainMenuActsWidget (Variables|Default|GetHUD))))
                      (Default|RightSwap _mainmenuactswidget))))))))))))

(fn ConstructionScript)