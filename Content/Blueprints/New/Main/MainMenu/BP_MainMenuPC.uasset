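; BP_MainMenuPC is the main menu player controller that runs the opening presentation of the menu on BeginPlay.
; It caches the BP_SeasonCard actor and BP_MainMenuHUD, then after a short delay fades the camera in and removes the HUD's loading screen.
; It then starts the card's intro montage at reduced speed and adds the main menu widget without waiting for the animation to finish.
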(event EventBeginPlay
  (bind _returnvalue (Actor|GetActorOfClass "/Game/Blueprints/New/Main/MainMenu/SeasonCard/BP_SeasonCard.BP_SeasonCard_C"))
  (Variables|Default|SetSeasonCard _returnvalue)
  (bind _asbp_main_menu_hud (Utilities|Casting|CastToBP_MainMenuHUD (HUD|GetHUD)))
  (Variables|Default|SetMainMenuHUD _asbp_main_menu_hud)
  (Utilities|FlowControl|Delay 1.0)
  (CameraFades|StartCameraFade :self (Variables|Default|GetPlayerCameraManager) :FromAlpha 1.0 :ToAlpha 0.0 :Duration 1.0)
  (Widget|RemovefromParent (Variables|/Game/Blueprints/New/Main/MainMenu/BP_MainMenuHUD.BP_MainMenuHUD_C|GetLoadingScreenWidget (Variables|Default|GetMainMenuHUD)))
  (Utilities|FlowControl|Delay 0.2)
  (Animation|Montage|PlayMontage (Variables|/Game/Blueprints/New/Main/MainMenu/SeasonCard/BP_SeasonCard.BP_SeasonCard_C|GetSkeletalMesh (Variables|Default|GetSeasonCard)) "/Game/Assets/UI/MainMenu/Seasons/Meshes/Anims/AM_CardStart.AM_CardStart" 0.5
    (:then
      (UserInterface|Viewport|AddtoViewport (Variables|/Game/Blueprints/New/Main/MainMenu/BP_MainMenuHUD.BP_MainMenuHUD_C|GetMainMenuWidget (Variables|Default|GetMainMenuHUD)) 0))))

(fn ConstructionScript)