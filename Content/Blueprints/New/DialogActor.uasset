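; Dialog manager actor that plays row-numbered conversations from a DataTable in the dialog widget.
; OpenDialog hides gameplay UI and disables pawn input, then shows each line with localized Russian or English text, speaker icon and optional sound.
; NextDialog/EndDialog reads the next row's status to continue, present answer choices or end.
; CancelDialog restores input and UI, re-enables an optional door and notifies the caller.
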(event EventBeginPlay
  (bind _asmy_game_instance (Utilities|Casting|CastToMyGameInstance (Game|GetGameInstance)))
  (Variables|Default|SetLanguage (Variables|/Game/Blueprints/Transfered/Blueprints1/MyGameInstance.MyGameInstance_C|GetLanguage _asmy_game_instance)))

(fn ConstructionScript)

(fn OpenDialog
  (params (DialogRow :type Integer) (DialogCaller :type Actor%20Object%20Reference) (DoorAfterLoc :type BP%20Doors%20Object%20Reference))
  (Variables|Default|SetDialogCaller DialogCaller)
  (CallFunction|HideGamePlayWidgets)
  (Utilities|IsValid DoorAfterLoc
    (:Is%20Valid
      (Variables|Default|SetDoorAfterLoc DoorAfterLoc))
    (:Is%20Not%20Valid
      _))
  (CallFunction|Enable/DisableInput false)
  (Variables|/Game/Widgets/Dialog/W_Dialog.W_Dialog_C|SetIsOnDialog? (Variables|Default|GetDialog_W) true)
  (Variables|Default|SetCurrentDialogNum DialogRow)
  (CallFunction|ChangeDialogIconandText (Variables|Default|GetDataTableToUse) (Utilities|String|StringToName (Utilities|String|ToString(Integer) DialogRow)) true)
  (Default|ShowUp (Variables|Default|GetDialog_W) true)
  (Widget|SetVisibility (Variables|Default|GetMainInterface_W) "Visible"))

(fn ChangeDialogIconandText
  (params (DataTable :type Data%20Table%20Object%20Reference) (RowName :type Name) (OpenDialog :type Boolean))
  (bind _returnvalue (Utilities|GetDataTableRow DataTable RowName)
    (:then
      (switch Utilities|FlowControl|Switch|SwitchonGameLanguage (Variables|Default|GetLanguage)
        (:NewEnumerator0
          (LocalVariables|SetLocalText (.DialogTextRus (Utilities|Struct|BreakDialog_Struct _returnvalue))))
        (:NewEnumerator1
          (LocalVariables|SetLocalText (.DialogTextEng (Utilities|Struct|BreakDialog_Struct _returnvalue)))))
      (Default|UpdIconWidget (Variables|Default|GetDialog_W) 0 (LocalVariables|GetLocalText) 0 0 (.DialogIcon (Utilities|Struct|BreakDialog_Struct _returnvalue)) 0 false 0 0 (and (Utilities|Enum|NotEqual(Enum) (.CharName (Utilities|Struct|BreakDialog_Struct _returnvalue)) "NewEnumerator3") (== (Variables|Default|GetCharTalk) (.CharName (Utilities|Struct|BreakDialog_Struct _returnvalue)))) "" OpenDialog (.DialogSize (Utilities|Struct|BreakDialog_Struct _returnvalue)) (.CharName (Utilities|Struct|BreakDialog_Struct _returnvalue)) "NewEnumerator0")
      (Variables|Default|SetCharTalk (.CharName (Utilities|Struct|BreakDialog_Struct _returnvalue)))
      (Utilities|IsValid (.DialogSound (Utilities|Struct|BreakDialog_Struct _returnvalue))
        (:Is%20Valid
          (Audio|PlaySound2D (.DialogSound (Utilities|Struct|BreakDialog_Struct _returnvalue)) 1.0 1.0 0.0 0 0))))))

(fn NextDialog/EndDialog
  (bind _returnvalue (Utilities|GetDataTableRow (Variables|Default|GetDataTableToUse) (Utilities|String|StringToName (Utilities|String|ToString(Integer) (+ (Variables|Default|GetCurrentDialogNum) 1))))
    (:then
      (switch Utilities|FlowControl|Switch|SwitchonDialogEnum (.DialogStatus (Utilities|Struct|BreakDialog_Struct _returnvalue))
        (:NewEnumerator0
          (Variables|/Game/Widgets/New/MainInterface_W.MainInterface_W_C|SetAnswer? (Variables|Default|GetMainInterface_W) false)
          (Math|Integer|IncrementInt (Variables|Default|GetCurrentDialogNum)
            (:%20%20
              (CallFunction|ChangeDialogIconandText (Variables|Default|GetDataTableToUse) (Utilities|String|StringToName (Utilities|String|ToString(Integer) (Variables|Default|GetCurrentDialogNum))) false))))
        (:NewEnumerator5
          (Widget|SetVisibility (Variables|/Game/Widgets/Dialog/W_Dialog.W_Dialog_C|GetDialogEndImage (Variables|/Game/Widgets/New/MainInterface_W.MainInterface_W_C|GetW_Dialog (Variables|Default|GetMainInterface_W))) "Hidden")
          (Variables|/Game/Widgets/New/MainInterface_W.MainInterface_W_C|SetAnswer? (Variables|Default|GetMainInterface_W) true)
          (Default|InitAnswers (Variables|/Game/Widgets/Dialog/W_Dialog.W_Dialog_C|GetWB_Answer (Variables|/Game/Widgets/New/MainInterface_W.MainInterface_W_C|GetW_Dialog (Variables|Default|GetMainInterface_W))) (+ (Variables|Default|GetCurrentDialogNum) 1)))
        (:NewEnumerator4
          (Variables|Default|SetCharTalk "NewEnumerator3")
          (Variables|/Game/Widgets/New/MainInterface_W.MainInterface_W_C|SetAnswer? (Variables|Default|GetMainInterface_W) false)
          (CallFunction|CancelDialog))))))

(fn CancelDialog
  (Widget|SetVisibility (Variables|Default|GetMainInterface_W) "SelfHitTestInvisible")
  (Default|ShowUp (Variables|Default|GetDialog_W) false)
  (Variables|/Game/Widgets/Dialog/W_Dialog.W_Dialog_C|SetIsOnDialog? (Variables|Default|GetDialog_W) false)
  (CallFunction|Enable/DisableInput true)
  (Utilities|IsValid (Variables|Default|GetDoorAfterLoc)
    (:Is%20Valid
      (Variables|/Game/Blueprints/New/InteractiveBPs/BP_ActorMain.BP_ActorMain_C|SetAbleToInteract (Variables|Default|GetDoorAfterLoc) true)
      (Variables|Default|SetDoorAfterLoc 0))
    (:Is%20Not%20Valid
      _))
  (CallFunction|ReturnVisibilityGamePlayWidgets)
  (Class|DialogInterface|DialogEnded(Message) (Variables|Default|GetDialogCaller) (Variables|Default|GetCurrentDialogNum)))

(fn Enable/DisableInput
  (params (Condition :type Boolean))
  (bind _returnvalue (Game|GetPlayerController 0))
  (bind _returnvalue_2 (Game|GetPlayerController 0))
  (if Condition
    (Input|EnableInput (Pawn|GetControlledPawn _returnvalue) _returnvalue)
    (else
      (Input|DisableInput (Pawn|GetControlledPawn _returnvalue_2) _returnvalue_2))))

(fn ReturnVisibilityGamePlayWidgets
  (bind _maininterface_w (Variables|Default|GetMainInterface_W))
  (bind _returnvalue (Game|GetCurrentLevelName true))
  (if (Utilities|Enum|NotEqual(Enum) _returnvalue "01_IntroBegin")
    (UserInterface|Animation|PlayAnimation _maininterface_w (Variables|/Game/Widgets/New/MainInterface_W.MainInterface_W_C|GetShowInterface _maininterface_w) 0.0 1 "Forward" 1.0 false)))

(fn HideGamePlayWidgets
  (bind _maininterface_w (Variables|Default|GetMainInterface_W))
  (if (not (== (.a (Variables|/Script/UMG.Button|GetBackgroundColor (Variables|/Game/Widgets/New/MainInterface_W.MainInterface_W_C|GetButtonInventory (Variables|Default|GetMainInterface_W)))) 0.0))
    (UserInterface|Animation|PlayAnimation _maininterface_w (Variables|/Game/Widgets/New/MainInterface_W.MainInterface_W_C|GetShowInterface _maininterface_w) 0.0 1 "Reverse" 1.0 false)))

(fn InteractwithWidget
  (return))