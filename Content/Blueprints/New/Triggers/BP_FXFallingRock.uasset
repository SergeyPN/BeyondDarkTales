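; BP_FXFallingRock is an effect Blueprint that, judging by its name, plays falling rock particles when triggered.
; Its ActivateParticle event waits a short random delay, then activates the ParticleSystem component with reset, so the start time varies.
; An unconnected chain of timestamp debug prints also leads into the activation but never runs, and the construction script is empty.
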(event Custom|ActivateParticle
  (Utilities|FlowControl|Delay (Math|Random|RandomFloatinRange 0.0 2.5))
  (Components|Activation|Activate (Variables|Default|GetParticleSystem) true))

(fn ConstructionScript)