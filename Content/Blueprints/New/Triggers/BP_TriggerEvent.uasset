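; BP_TriggerEvent is a one-shot box trigger that briefly takes control from the player to play a lose animation on BP_CharMax.
; The first overlap by any actor disables player input, then casts that actor to BP_CharMax, stops its movement and plays AM_Lose slowed down.
; Input returns only when the montage completes, so a failed cast leaves it disabled.
; A collapse camera shake node is present but unconnected.
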(event OnComponentBeginOverlap(Box)
  (params (OverlappedComponent :type Primitive%20Component%20Object%20Reference) (OtherActor :type Actor%20Object%20Reference) (OtherComp :type Primitive%20Component%20Object%20Reference) (OtherBodyIndex :type Integer) (bFromSweep :type Boolean) (SweepResult :type Hit%20Result%20Structure%20%28by%20ref%29))
  (bind _returnvalue (Game|GetPlayerController 0))
  (bind _returnvalue_2 (Game|GetPlayerController 0))
  (Utilities|FlowControl|DoOnce false
    (:Completed
      (Input|DisableInput (Pawn|GetControlledPawn _returnvalue) _returnvalue)
      (bind _asbp_char_max (Utilities|Casting|CastToBP_CharMax OtherActor))
      (Default|StopMovement _asbp_char_max)
      (Animation|Montage|PlayMontage (Variables|/Script/Engine.Character|GetMesh _asbp_char_max) "/Game/Assets/Heroes/Max/Anim/AM_Lose.AM_Lose" 0.7
        (:OnCompleted
          (Input|EnableInput (Pawn|GetControlledPawn _returnvalue_2) _returnvalue_2))))))

(event EventBeginPlay
  (|CallParentFunction) ; This node is disabled and will not be called.\nDrag off pins to build functionality.
)

(event Collision|EventActorBeginOverlap
  (params (OtherActor :type Actor%20Object%20Reference))
  (|CallParentFunction OtherActor) ; This node is disabled and will not be called.\nDrag off pins to build functionality.
)

(event EventTick
  (params (DeltaSeconds :type Float%20%28single-precision%29))
  (|CallParentFunction DeltaSeconds) ; This node is disabled and will not be called.\nDrag off pins to build functionality.
)

(fn ConstructionScript
  (|CallParentFunction))