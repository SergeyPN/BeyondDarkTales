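; BP_Trigger_Learning is a box trigger that shows a learning screen when the player enters it.
; On BeginPlay it caches the first BP_CharMax as the player.
; When that character overlaps the box, it stops the player's movement and calls LearningShow on the 01CM_PC controller's main interface widget, passing its LearningToUse value.
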(event OnComponentBeginOverlap(Box)
  (params (OverlappedComponent :type Primitive%20Component%20Object%20Reference) (OtherActor :type Actor%20Object%20Reference) (OtherComp :type Primitive%20Component%20Object%20Reference) (OtherBodyIndex :type Integer) (bFromSweep :type Boolean) (SweepResult :type Hit%20Result%20Structure%20%28by%20ref%29))
  (if (== OtherActor (Variables|Default|GetPlayer))
    (Default|StopMovement (Variables|Default|GetPlayer))
    (Default|LearningShow (Variables|/Game/Blueprints/New/Main/01CaveMain/01CM_PC.01CM_PC_C|GetMainInterface_W (.As01CM%20PC (Utilities|Casting|CastTo01CM_PC (Game|GetPlayerController 0)))) (Variables|Default|GetLearningToUse))))

(event EventBeginPlay
  (bind _outactors (Actor|GetAllActorsOfClass "/Game/Assets/Heroes/Max/BP_CharMax.BP_CharMax_C"))
  (Variables|Default|SetPlayer (Utilities|Array|Get(acopy) _outactors)))

(fn ConstructionScript
  (|CallParentFunction))