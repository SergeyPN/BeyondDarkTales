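; Death zone trigger that shows the death screen and handles restarting the attempt.
; A once-gated box overlap hides the interface, disables input, passes itself to the HUD's death screen, then moves BP_CharMax to a hardcoded location.
; NewAttempt resets all sequence triggers and level sequences, restores character and camera start transforms, removes the loading screen, fades in, restores interface and input, and re-arms the zone.
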(event OnComponentBeginOverlap(Box)
  (params (OverlappedComponent :type Primitive%20Component%20Object%20Reference) (OtherActor :type Actor%20Object%20Reference) (OtherComp :type Primitive%20Component%20Object%20Reference) (OtherBodyIndex :type Integer) (bFromSweep :type Boolean) (SweepResult :type Hit%20Result%20Structure%20%28by%20ref%29))
  (bind _maininterfacewidget (CallFunction|GetMainInterfaceWidget))
  (Utilities|FlowControl|DoOnce false
    (:Completed
      (UserInterface|Animation|PlayAnimation _maininterfacewidget (Variables|/Game/Widgets/New/MainInterface_W.MainInterface_W_C|GetShowInterfaceWithPause _maininterfacewidget) 0.0 1 "Reverse" 4.0 false)
      (Input|DisableInput (Game|Player|GetPlayerPawn 0) (Game|GetPlayerController 0))
      (bind _asbp_main_menu_hud (Utilities|Casting|CastToBP_MainMenuHUD (HUD|GetHUD (Game|GetPlayerController 0))))
      (UserInterface|Viewport|AddtoViewport (Variables|/Game/Blueprints/New/Main/MainMenu/BP_MainMenuHUD.BP_MainMenuHUD_C|GetDieScreenWidget _asbp_main_menu_hud) 3)
      (Variables|/Game/Widgets/DieScreen/WBP_DieScreen.WBP_DieScreen_C|SetActorCreatorWidget (Variables|/Game/Blueprints/New/Main/MainMenu/BP_MainMenuHUD.BP_MainMenuHUD_C|GetDieScreenWidget _asbp_main_menu_hud) self)
      (bind _asbp_char_max (Utilities|Casting|CastToBP_CharMax OtherActor))
      (bind _output_get (Variables|Default|SetCharMax _asbp_char_max))
      (Transformation|SetActorTransform _output_get (Math|Transform|MakeTransform "20.000000,150.000000,-820.000000" "0, 0, 0" "1,1,1")))))

(event Custom|ResetDeathZone
  (bind _maininterfacewidget (CallFunction|GetMainInterfaceWidget))
  (Utilities|FlowControl|DoOnce false) ; enters at Reset
)

(event EventBeginPlay
  (|CallParentFunction) ; This node is disabled and will not be called.\nDrag off pins to build functionality.
)

(event Collision|EventActorBeginOverlap
  (params (OtherActor :type Actor%20Object%20Reference))
  (|CallParentFunction OtherActor) ; This node is disabled and will not be called.\nDrag off pins to build functionality.
)

(event EventTick
  (params (DeltaSeconds :type Float%20%28single-precision%29))
  (|CallParentFunction DeltaSeconds) ; This node is disabled and will not be called.\nDrag off pins to build functionality.
)

(event EventNewAttempt
  (bind _maininterfacewidget (CallFunction|GetMainInterfaceWidget))
  (bind _outactors (Actor|GetAllActorsOfClass "/Game/Blueprints/New/Triggers/BP_TriggerSequence.BP_TriggerSequence_C"))
  (for _array_element _outactors
    (Default|ResetTrigger _array_element))
  (bind _outactors_2 (Actor|GetAllActorsOfClass "/Script/LevelSequence.LevelSequenceActor"))
  (for _array_element_2 _outactors_2
    (Class|MovieSceneSequencePlayer|JumptoFrame (Variables|/Script/LevelSequence.LevelSequenceActor|GetSequencePlayer _array_element_2)))
  (Transformation|SetActorTransform (Variables|Default|GetCharMax) (Variables|Default|GetStartPositionForChar))
  (Utilities|FlowControl|Delay 2.0)
  (bind _ascamera_pc_test (Utilities|Casting|CastToCamera_PC_test (Game|Player|GetPlayerPawn 0)))
  (Transformation|SetActorTransform (Variables|/Game/Blueprints/Transfered/Blueprints1/ToTransfer/CameraControl/Camera_PC_test.Camera_PC_test_C|GetLevelCamera _ascamera_pc_test) (Variables|Default|GetStartPositionForCamera))
  (bind _foundwidgets (Widget|GetAllWidgetsOfClass "/Game/Widgets/LoadingScreen/WB_LoadingScreen.WB_LoadingScreen_C" true))
  (Widget|RemovefromParent (Utilities|Array|Get(acopy) _foundwidgets))
  (CameraFades|StartCameraFade :self (Variables|/Script/Engine.PlayerController|GetPlayerCameraManager (Game|GetPlayerController 0)) :FromAlpha 1.0 :Duration 1.0)
  (UserInterface|Animation|PlayAnimation _maininterfacewidget (Variables|/Game/Widgets/New/MainInterface_W.MainInterface_W_C|GetShowInterfaceWithPause _maininterfacewidget) 0.0 1 "Forward" 4.0 false)
  (Utilities|FlowControl|Delay 1.5)
  (Input|EnableInput (Game|Player|GetPlayerPawn 0) (Game|GetPlayerController 0))
  (Variables|/Game/Widgets/DieScreen/WBP_DieScreen.WBP_DieScreen_C|SetDoOnce (Variables|/Game/Blueprints/New/Main/MainMenu/BP_MainMenuHUD.BP_MainMenuHUD_C|GetDieScreenWidget (.AsBP%20Main%20Menu%20HUD (Utilities|Casting|CastToBP_MainMenuHUD (HUD|GetHUD (Game|GetPlayerController 0))))) false)
  (CallFunction|ResetDeathZone))

(fn ConstructionScript
  (|CallParentFunction))