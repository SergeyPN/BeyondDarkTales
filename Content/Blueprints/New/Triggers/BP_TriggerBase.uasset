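; BP_TriggerBase is a base trigger actor with a configurable box or sphere collision shape.
; Its construction script uses the BoxCollision flag to keep and size one shape from exposed variables, destroying the other component.
; On BeginPlay it finds and caches the level's BP_SequenceManager.
; The file itself implements no overlap response.
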(event EventBeginPlay
  (bind _returnvalue (Actor|GetActorOfClass "/Game/Blueprints/New/Managers/SequenceManager/BP_SequenceManager.BP_SequenceManager_C"))
  (Variables|Default|SetSequenceManager _returnvalue))

(event Collision|EventActorBeginOverlap
  (params (OtherActor :type Actor%20Object%20Reference)))

(event EventTick
  (params (DeltaSeconds :type Float%20%28single-precision%29)))

(fn ConstructionScript
  (if (Variables|Construct|GetBoxCollision?)
    (Components|DestroyComponent (Variables|Default|GetSphere))
    (Components|Box|SetBoxExtent (Variables|Default|GetBox) (Math|Vector|MakeVector (Variables|Construct|GetX) (Variables|Construct|GetY) (Variables|Construct|GetZ)) true)
    (else
      (Components|DestroyComponent (Variables|Default|GetBox))
      (Components|Sphere|SetSphereRadius (Variables|Default|GetSphere) (Variables|Construct|GetSphereRadius) true))))