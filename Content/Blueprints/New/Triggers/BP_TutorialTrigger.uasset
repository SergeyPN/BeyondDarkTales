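; Tutorial trigger actor that opens a numbered tutorial in the main menu HUD's message widget when overlapped while enabled.
; ActivateActor enables it, and it passes itself as caller so CloseTutorial can run on dismissal.
; Closing notifies the HUD, activates a quest via BP_QuestManager, starts any BPC_InteractiveBase component on itself, then destroys the actor.
; The overlap does not filter which actor entered.
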(event EventActivateActor
  (Variables|Default|SetEnabled? true))

(event Collision|EventActorBeginOverlap
  (params (OtherActor :type Actor%20Object%20Reference))
  (if (Variables|Default|GetEnabled?)
    (bind _mainmenuhud (Class|BPIHUD|GetMainMenuHUD(Message) (HUD|GetHUD (Game|GetPlayerController 0))))
    (Default|OpenTutorial _mainmenuhud (Variables|Default|GetNumTutorial) self)))

(event EventCloseTutorial
  (bind _returnvalue (Actor|GetComponentbyClass "/Game/Blueprints/General/BPC_InteractiveBase.BPC_InteractiveBase_C"))
  (Class|BPIHUD|ClosingTutorial(Message) (HUD|GetHUD (Game|GetPlayerController 0)))
  (bind _returnvalue_2 (Actor|GetActorOfClass "/Game/Blueprints/QuestSystem/BP_QuestManager.BP_QuestManager_C"))
  (Default|ActivateQuest _returnvalue_2 "(TagName=\"BackPackAndExit.Trisigns\")")
  (Utilities|IsValid _returnvalue
    (:Is%20Valid
      (Default|StartInteractive _returnvalue)
      (Actor|DestroyActor))
    (:Is%20Not%20Valid
      (Actor|DestroyActor))))

(fn ConstructionScript
  (|CallParentFunction))