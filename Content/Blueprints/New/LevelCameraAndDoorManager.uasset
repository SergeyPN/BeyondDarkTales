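; Manager actor that moves the player between door-linked locations, switching level cameras and streamed levels.
; SwapCamera plays transition audio, disables input, blends to the indexed camera and shows the target level.
; Once shown, it teleports the princess if requested, moves the player to the destination door, hides the old level and resets the previous camera to hardcoded transforms.
; It then opens a follow-up dialog or restores input and door interaction.
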(event Custom|SwapCamera
  (params (CamIndex :type Integer) (DoorIndex :type Integer) (LevelToUnload :type Name) (LevelToLoad :type Name) (WithDialogAfter? :type Boolean) (DialogCaller :type Actor%20Object%20Reference) (DialogRow :type Integer) (PrincessTeleport :type Transform))
  (bind _returnvalue (Game|GetPlayerController 0))
  (bind _returnvalue_2 (Class|GameplayStatics|GetStreamingLevel LevelToLoad))
  (bind _asbp_doors (Utilities|Casting|CastToBP_Doors DialogCaller))
  (bind _asbp_actor_main (Utilities|Casting|CastToBP_ActorMain DialogCaller)
    (:then
      (Variables|Default|SetActorMain _asbp_actor_main))
    (:CastFailed
      _))
  (Audio|PlaySound2D "/Game/Audio/Snd/FX/LocationSwitch.LocationSwitch" 1.0 1.0 0.0 0 0)
  (CallFunction|PlayRandomStartSoundAtmosphere (Variables|/Game/Blueprints/New/InteractiveBPs/BP_Doors.BP_Doors_C|GetAmbSoundForLoc _asbp_doors) (Variables|/Game/Blueprints/New/InteractiveBPs/BP_Doors.BP_Doors_C|GetAmbSoundForLocWithoutLoop _asbp_doors))
  (Input|DisableInput (Pawn|GetControlledPawn _returnvalue) _returnvalue)
  (bind _cameratoswitchlocal1 (CallFunction|GetCamera CamIndex))
  (Game|Player|SetViewTargetwithBlend (Game|GetPlayerController 0) _cameratoswitchlocal1 1.0 "VTBlend_Linear" 0.0 false)
  (Variables|/Script/Engine.LevelStreaming|SetbShouldBeVisible _returnvalue_2 true)
  (EventDispatchers|BindEventtoOnLevelShown _returnvalue_2 (delegate Custom|CustomEvent_0)))

(event Custom|CustomEvent_0
  (bind _returnvalue (Game|GetPlayerController 0))
  (bind _playerpawn (Variables|Default|GetPlayerPawn))
  (bind _currentplayercontroller (Variables|/Game/Blueprints/Transfered/Blueprints1/ToTransfer/Camera_PC_test.Camera_PC_test_C|GetCurrentPlayerController _playerpawn))
  (bind _maininterface_w (Variables|/Game/Blueprints/New/Main/01CaveMain/01CM_PC.01CM_PC_C|GetMainInterface_W _currentplayercontroller))
  (EventDispatchers|UnbindallEventsfromOnLevelShown (Class|GameplayStatics|GetStreamingLevel (stale Custom|SwapCamera LevelToLoad)))
  (if (Math|Vector|Equal(Vector) (.Location (Math|Transform|BreakTransform (stale Custom|SwapCamera PrincessTeleport))) "0, 0, 0" 0.1)
    _
    (else
      (CallFunction|TeleportPrincess (stale Custom|SwapCamera PrincessTeleport))))
  (Utilities|FlowControl|Delay 0.5)
  (bind _newparam (CallFunction|GetDoorLoc (stale Custom|SwapCamera DoorIndex) (stale Custom|SwapCamera WithDialogAfter?)))
  (Transformation|SetActorTransform (Variables|Default|GetPlayer) _newparam)
  (Utilities|FlowControl|Delay 0.5)
  (Variables|/Script/Engine.LevelStreaming|SetbShouldBeVisible (Class|GameplayStatics|GetStreamingLevel (stale Custom|SwapCamera LevelToUnload)) false)
  (CallFunction|ReturnTransformLastCamera (stale Custom|SwapCamera LevelToLoad))
  (Default|SetLevelCamera (.As01CM%20PC (Utilities|Casting|CastTo01CM_PC (Game|GetPlayerController 0))) (stale Custom|SwapCamera _cameratoswitchlocal1))
  (if (stale Custom|SwapCamera WithDialogAfter?)
    (UserInterface|Animation|PlayAnimation _maininterface_w (Variables|/Game/Widgets/New/MainInterface_W.MainInterface_W_C|GetShowInterface _maininterface_w) 0.0 1 "Reverse" 4.0 false)
    (Default|OpenDialog (Variables|Default|GetDialogActor) (stale Custom|SwapCamera DialogRow) (stale Custom|SwapCamera DialogCaller) (Variables|Default|GetDoorTo))
    (Utilities|IsValid (Variables|Default|GetDoorTo)
      (:Is%20Valid
        (Variables|Default|SetDoorTo 0)))
    (else
      (Input|EnableInput (Pawn|GetControlledPawn _returnvalue) _returnvalue)
      (Utilities|IsValid (Variables|Default|GetDoorTo)
        (:Is%20Valid
          (if (Variables|/Game/Blueprints/New/InteractiveBPs/BP_ActorMain.BP_ActorMain_C|GetStartEnabled? (Variables|Default|GetDoorTo))
            (Variables|/Game/Blueprints/New/InteractiveBPs/BP_ActorMain.BP_ActorMain_C|SetAbleToInteract (Variables|Default|GetDoorTo) true))
          (Variables|Default|SetDoorTo 0))))))

(event EventBeginPlay
  (bind _outactors (Actor|GetAllActorsOfClass "/Game/Assets/Heroes/Max/BP_CharMax.BP_CharMax_C"))
  (Variables|Default|SetPlayer (Utilities|Array|Get(acopy) _outactors))
  (bind _outactors_2 (Actor|GetAllActorsOfClass "/Game/Blueprints/New/DialogActor.DialogActor_C"))
  (Variables|Default|SetDialogActor (Utilities|Array|Get(acopy) _outactors_2))
  (bind _ascamera_pc_test (Utilities|Casting|CastToCamera_PC_test (Game|Player|GetPlayerPawn 0)))
  (Variables|Default|SetPlayerPawn _ascamera_pc_test))

(fn ConstructionScript)

(fn GetCamera
  (params (CamIndex :type Integer))
  (bind _outactors (Actor|GetAllActorsOfClass "/Game/Blueprints/New/LevelCamera.LevelCamera_C"))
  (for _array_element _outactors
    (if (== (Variables|/Game/Blueprints/New/LevelCamera.LevelCamera_C|GetCameraIndex _array_element) CamIndex)
      (LocalVariables|SetCameraToSwitchLocal _array_element)))
  (return (LocalVariables|GetCameraToSwitchLocal)))

(fn GetDoorLoc
  (params (DoorIndex :type Integer) (IsWithDialog? :type Boolean))
  (bind _outactors (Actor|GetAllActorsOfClass "/Game/Blueprints/New/InteractiveBPs/BP_Doors.BP_Doors_C"))
  (for _array_element _outactors
    (if (== (Variables|/Game/Blueprints/New/InteractiveBPs/BP_Doors.BP_Doors_C|GetSelfNum _array_element) DoorIndex)
      (LocalVariables|SetNewLocalVar_0 (Transformation|GetActorTransform _array_element))
      (Variables|Default|SetDoorTo _array_element)))
  (if IsWithDialog?
    (Variables|/Game/Blueprints/New/InteractiveBPs/BP_ActorMain.BP_ActorMain_C|SetAbleToInteract (Variables|Default|GetDoorTo) false))
  (return (LocalVariables|GetNewLocalVar_0)))

(fn ReturnTransformLastCamera
  (params (LoadLevel :type Name))
  (LocalVariables|SetLLoadLevel LoadLevel)
  (switch string (Utilities|GetDisplayName (Variables|/Game/Blueprints/Transfered/Blueprints1/ToTransfer/Camera_PC_test.Camera_PC_test_C|GetLevelCamera (Variables|Default|GetPlayerPawn)))
    (:Camera1
      (Transformation|SetActorTransform (Variables|/Game/Blueprints/Transfered/Blueprints1/ToTransfer/Camera_PC_test.Camera_PC_test_C|GetLevelCamera (Variables|Default|GetPlayerPawn)) (Math|Transform|MakeTransform "457.207001,-278.095001,95.271004" "-29.335203,-52.622993, 0" "1,1,1"))
      (Variables|/Script/Engine.SpringArmComponent|SetTargetArmLength (Variables|/Game/Blueprints/New/LevelCamera.LevelCamera_C|GetSpringArm (Variables|/Game/Blueprints/Transfered/Blueprints1/ToTransfer/Camera_PC_test.Camera_PC_test_C|GetLevelCamera (Variables|Default|GetPlayerPawn))) 3.63e+03))
    (:Camera2
      (if (Utilities|Name|Equal(Name) (LocalVariables|GetLLoadLevel) "Cave01Loc1")
        (Transformation|SetActorTransform (Variables|/Game/Blueprints/Transfered/Blueprints1/ToTransfer/Camera_PC_test.Camera_PC_test_C|GetLevelCamera (Variables|Default|GetPlayerPawn)) (Math|Transform|MakeTransform "3897.981934,54.923000,185.903000" "-30.603275,-53.400219, 0" "1,1,1"))
        (Variables|/Script/Engine.SpringArmComponent|SetTargetArmLength (Variables|/Game/Blueprints/New/LevelCamera.LevelCamera_C|GetSpringArm (Variables|/Game/Blueprints/Transfered/Blueprints1/ToTransfer/Camera_PC_test.Camera_PC_test_C|GetLevelCamera (Variables|Default|GetPlayerPawn))) 3535.967285)
        (elif (Utilities|Name|Equal(Name) (LocalVariables|GetLLoadLevel) "Cave01Loc3")
          (Transformation|SetActorTransform (Variables|/Game/Blueprints/Transfered/Blueprints1/ToTransfer/Camera_PC_test.Camera_PC_test_C|GetLevelCamera (Variables|Default|GetPlayerPawn)) (Math|Transform|MakeTransform "5351.542969,72.220001,456.132996" "-35.473351,-125.789268, 0" "1,1,1"))
          (Variables|/Script/Engine.SpringArmComponent|SetTargetArmLength (Variables|/Game/Blueprints/New/LevelCamera.LevelCamera_C|GetSpringArm (Variables|/Game/Blueprints/Transfered/Blueprints1/ToTransfer/Camera_PC_test.Camera_PC_test_C|GetLevelCamera (Variables|Default|GetPlayerPawn))) 3085.967285))))
    (:Camera3
      (if (Utilities|Name|Equal(Name) (LocalVariables|GetLLoadLevel) "Cave01Loc2")
        (Transformation|SetActorTransform (Variables|/Game/Blueprints/Transfered/Blueprints1/ToTransfer/Camera_PC_test.Camera_PC_test_C|GetLevelCamera (Variables|Default|GetPlayerPawn)) (Math|Transform|MakeTransform "-61.915001,3090.000977,129.022003" "-27.822693,42.606373, 0" "1,1,1"))
        (Variables|/Script/Engine.SpringArmComponent|SetTargetArmLength (Variables|/Game/Blueprints/New/LevelCamera.LevelCamera_C|GetSpringArm (Variables|/Game/Blueprints/Transfered/Blueprints1/ToTransfer/Camera_PC_test.Camera_PC_test_C|GetLevelCamera (Variables|Default|GetPlayerPawn))) 3185.930908)
        (elif (Utilities|Name|Equal(Name) (LocalVariables|GetLLoadLevel) "Cave01Loc4")
          (Transformation|SetActorTransform (Variables|/Game/Blueprints/Transfered/Blueprints1/ToTransfer/Camera_PC_test.Camera_PC_test_C|GetLevelCamera (Variables|Default|GetPlayerPawn)) (Math|Transform|MakeTransform "-464.808014,3697.364990,346.213013" "-27.822693,42.606373, 0" "1,1,1"))
          (Variables|/Script/Engine.SpringArmComponent|SetTargetArmLength (Variables|/Game/Blueprints/New/LevelCamera.LevelCamera_C|GetSpringArm (Variables|/Game/Blueprints/Transfered/Blueprints1/ToTransfer/Camera_PC_test.Camera_PC_test_C|GetLevelCamera (Variables|Default|GetPlayerPawn))) 3185.930908))))
    (:Camera4
      (if (Utilities|Name|Equal(Name) (LocalVariables|GetLLoadLevel) "Cave01Loc3")
        (Transformation|SetActorTransform (Variables|/Game/Blueprints/Transfered/Blueprints1/ToTransfer/Camera_PC_test.Camera_PC_test_C|GetLevelCamera (Variables|Default|GetPlayerPawn)) (Math|Transform|MakeTransform "3722.750000,4158.953125,423.127991" "-29.178129,-20.401731, 0" "1,1,1"))
        (Variables|/Script/Engine.SpringArmComponent|SetTargetArmLength (Variables|/Game/Blueprints/New/LevelCamera.LevelCamera_C|GetSpringArm (Variables|/Game/Blueprints/Transfered/Blueprints1/ToTransfer/Camera_PC_test.Camera_PC_test_C|GetLevelCamera (Variables|Default|GetPlayerPawn))) 3542.871826)
        (elif (Utilities|Name|Equal(Name) (LocalVariables|GetLLoadLevel) "Cave01Loc5")
          (Transformation|SetActorTransform (Variables|/Game/Blueprints/Transfered/Blueprints1/ToTransfer/Camera_PC_test.Camera_PC_test_C|GetLevelCamera (Variables|Default|GetPlayerPawn)) (Math|Transform|MakeTransform "3818.956055,3924.533936,708.187012" "-29.598780,-14.529560, 0" "1,1,1"))
          (Variables|/Script/Engine.SpringArmComponent|SetTargetArmLength (Variables|/Game/Blueprints/New/LevelCamera.LevelCamera_C|GetSpringArm (Variables|/Game/Blueprints/Transfered/Blueprints1/ToTransfer/Camera_PC_test.Camera_PC_test_C|GetLevelCamera (Variables|Default|GetPlayerPawn))) 3152.871826)
          (elif (Utilities|Name|Equal(Name) (LocalVariables|GetLLoadLevel) "Cave01Loc6")
            (Transformation|SetActorTransform (Variables|/Game/Blueprints/Transfered/Blueprints1/ToTransfer/Camera_PC_test.Camera_PC_test_C|GetLevelCamera (Variables|Default|GetPlayerPawn)) (Math|Transform|MakeTransform "3918.120117,3708.931885,663.497009" "-27.846249,24.775307, 0" "1,1,1"))
            (Variables|/Script/Engine.SpringArmComponent|SetTargetArmLength (Variables|/Game/Blueprints/New/LevelCamera.LevelCamera_C|GetSpringArm (Variables|/Game/Blueprints/Transfered/Blueprints1/ToTransfer/Camera_PC_test.Camera_PC_test_C|GetLevelCamera (Variables|Default|GetPlayerPawn))) 3152.871826)))))))

(fn HideLastDoor
  (Audio|Components|Audio|Stop (Variables|/Game/Blueprints/New/InteractiveBPs/BP_ActorMain.BP_ActorMain_C|GetTimeline_0 (Variables|Default|GetActorMain)))
  (Default|UpdIconWidget (Variables|/Game/Blueprints/New/InteractiveBPs/BP_ActorMain.BP_ActorMain_C|GetIntW (Variables|Default|GetActorMain)) (Utilities|Array|Get(acopy) (Variables|/Game/Blueprints/New/InteractiveBPs/BP_ActorMain.BP_ActorMain_C|GetStart/EndFrames (Variables|Default|GetActorMain)) 6) "" 0 0 0 0 false (Variables|Default|GetActorMain) 0 false "" false 0 "NewEnumerator3" "NewEnumerator0")
  (Widget|SetVisibility (Variables|/Game/Blueprints/New/InteractiveBPs/BP_ActorMain.BP_ActorMain_C|GetIntW (Variables|Default|GetActorMain)) "Collapsed")
  (Default|SetEnabled/Disabled (Variables|/Game/Blueprints/New/InteractiveBPs/BP_ActorMain.BP_ActorMain_C|GetPreInteract_W (Variables|Default|GetActorMain)) true (Variables|Default|GetPlayer) (Variables|Default|GetActorMain)))

(fn TeleportPrincess
  (params (TeleportTransform :type Transform))
  (bind _outactors (Actor|GetAllActorsOfClass "/Game/Assets/Heroes/FPrincess/BP_CharPrincess.BP_CharPrincess_C"))
  (bind _array_element (Utilities|Array|ForEachLoopwithBreak _outactors :!label _label)
    (:LoopBody
      (if (Utilities|Enum|Equal(Enum) (Utilities|GetObjectName _array_element) "BP_CharPrincess2")
        (Transformation|SetActorTransform _array_element TeleportTransform false true)
        (Rendering|SetActorHiddenInGame _array_element false)
        (Development|SetHiddeninGame (Variables|/Script/Engine.Character|GetMesh _array_element) false false)
        (goto _label Break)))
    (:Completed
      (return))))