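; LevelCamera is a placeable camera actor that can act as a level's starting camera.
; On BeginPlay, if flagged as the start camera, it registers itself with the 01CM_PC player controller, then with the controlled Camera_PC_test pawn.
; The construction script applies its arm length to the spring arm and places a sphere component at a fixed world-space height above the actor.
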(event EventBeginPlay
  (bind _returnvalue (Game|GetPlayerController 0))
  (if (Variables|Default|GetIsStartCam?)
    (bind _as01cm_pc (Utilities|Casting|CastTo01CM_PC _returnvalue))
    (Variables|/Game/Blueprints/New/Main/01CaveMain/01CM_PC.01CM_PC_C|SetNewVar_0 _as01cm_pc self)
    (bind _ascamera_pc_test (Utilities|Casting|CastToCamera_PC_test (Pawn|GetControlledPawn _returnvalue)))
    (Variables|/Game/Blueprints/Transfered/Blueprints1/ToTransfer/Camera_PC_test.Camera_PC_test_C|SetLevelCamera _ascamera_pc_test self)))

(event Collision|EventActorBeginOverlap
  (params (OtherActor :type Actor%20Object%20Reference)))

(event EventTick
  (params (DeltaSeconds :type Float%20%28single-precision%29)))

(fn ConstructionScript
  (Variables|/Script/Engine.SpringArmComponent|SetTargetArmLength (Variables|Default|GetSpringArm) (Variables|Default|GetArmLength))
  (Transformation|SetWorldLocation (Variables|Default|GetSphere1) (+ (Transformation|GetActorLocation) "0, 0,300.000000") false false))