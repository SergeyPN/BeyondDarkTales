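; Sequence manager that plays level sequences from an interaction actor or a trigger, optionally locking input to UI.
; During playback it switches the BP_CharPrincess2 mesh, found by object name, to custom animation mode, then restores its Animation Blueprint.
; With input locked, finish callbacks can open follow-up dialogs.
; They also update another actor's dialog and the sequence variant row, or for triggers handle camera fade and view target.
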(event Custom|ShowSequence
  (params (ActorMain :type BP%20Actor%20Main%20Object%20Reference) (DialogCaller :type Actor%20Object%20Reference) (TriggerSequence :type BP%20Trigger%20Sequence%20Object%20Reference) (WithDisableInput? :type Boolean))
  (Variables|Default|SetActorMain ActorMain)
  (Variables|Default|SetTriggerSequence TriggerSequence)
  (if WithDisableInput?
    (Input|SetInputModeUIOnly (Game|GetPlayerController 0) (CallFunction|GetMainInterfaceWidget) "DoNotLock")
    (CallFunction|SetAnimPrincessMode "AnimationCustomMode")
    (Utilities|IsValid (Variables|Default|GetActorMain)
      (:Is%20Valid
        (Sequencer|Player|Play (Variables|/Script/LevelSequence.LevelSequenceActor|GetSequencePlayer (Variables|/Game/Blueprints/New/InteractiveBPs/BP_ActorMain.BP_ActorMain_C|GetSequence (Variables|Default|GetActorMain))) :!class /Script/MovieScene.MovieSceneSequencePlayer)
        (EventDispatchers|BindEventtoOnFinished (Variables|/Script/LevelSequence.LevelSequenceActor|GetSequencePlayer (Variables|/Game/Blueprints/New/InteractiveBPs/BP_ActorMain.BP_ActorMain_C|GetSequence (Variables|Default|GetActorMain))) (delegate Custom|FinishSequence)))
      (:Is%20Not%20Valid
        ;[1 1 1] For Trigger
        (Sequencer|Player|Play (Variables|/Script/LevelSequence.LevelSequenceActor|GetSequencePlayer (Variables|/Game/Blueprints/New/Triggers/BP_TriggerSequence.BP_TriggerSequence_C|GetSequence (Variables|Default|GetTriggerSequence))) :!class /Script/MovieScene.MovieSceneSequencePlayer)
        (EventDispatchers|BindEventtoOnFinished (Variables|/Script/LevelSequence.LevelSequenceActor|GetSequencePlayer (Variables|/Game/Blueprints/New/Triggers/BP_TriggerSequence.BP_TriggerSequence_C|GetSequence (Variables|Default|GetTriggerSequence))) (delegate Custom|FinishSequenceTrigger))))
    (else
      (CallFunction|SetAnimPrincessMode "AnimationCustomMode")
      (Utilities|IsValid (Variables|Default|GetActorMain)
        (:Is%20Valid
          (Sequencer|Player|Play (Variables|/Script/LevelSequence.LevelSequenceActor|GetSequencePlayer (Variables|/Game/Blueprints/New/InteractiveBPs/BP_ActorMain.BP_ActorMain_C|GetSequence (Variables|Default|GetActorMain))) :!class /Script/MovieScene.MovieSceneSequencePlayer)
          (EventDispatchers|BindEventtoOnFinished (Variables|/Script/LevelSequence.LevelSequenceActor|GetSequencePlayer (Variables|/Game/Blueprints/New/InteractiveBPs/BP_ActorMain.BP_ActorMain_C|GetSequence (Variables|Default|GetActorMain))) (delegate Custom|FinishSequenceWithoutDisableInputActorMain)))
        (:Is%20Not%20Valid
          (Sequencer|Player|Play (Variables|/Script/LevelSequence.LevelSequenceActor|GetSequencePlayer (Variables|/Game/Blueprints/New/Triggers/BP_TriggerSequence.BP_TriggerSequence_C|GetSequence (Variables|Default|GetTriggerSequence))) :!class /Script/MovieScene.MovieSceneSequencePlayer)
          (EventDispatchers|BindEventtoOnFinished (Variables|/Script/LevelSequence.LevelSequenceActor|GetSequencePlayer (Variables|/Game/Blueprints/New/Triggers/BP_TriggerSequence.BP_TriggerSequence_C|GetSequence (Variables|Default|GetTriggerSequence))) (delegate Custom|FinishSequenceWithoutDisableInputTrigger)))))))

(event Custom|FinishSequenceWithoutDisableInputActorMain
  (EventDispatchers|UnbindallEventsfromOnFinished (Variables|/Script/LevelSequence.LevelSequenceActor|GetSequencePlayer (Variables|/Game/Blueprints/New/InteractiveBPs/BP_ActorMain.BP_ActorMain_C|GetSequence (Variables|Default|GetActorMain))))
  (CallFunction|SetAnimPrincessMode "AnimationBlueprint"))

(event Custom|FinishSequenceWithoutDisableInputTrigger
  (EventDispatchers|UnbindallEventsfromOnFinished (Variables|/Script/LevelSequence.LevelSequenceActor|GetSequencePlayer (Variables|/Game/Blueprints/New/Triggers/BP_TriggerSequence.BP_TriggerSequence_C|GetSequence (Variables|Default|GetTriggerSequence))))
  (CallFunction|SetAnimPrincessMode "AnimationBlueprint"))

(event Custom|FinishSequenceTrigger
  ;[1 1 1] For Trigger
  (EventDispatchers|UnbindEventfromOnFinished (Variables|/Script/LevelSequence.LevelSequenceActor|GetSequencePlayer (Variables|/Game/Blueprints/New/Triggers/BP_TriggerSequence.BP_TriggerSequence_C|GetSequence (Variables|Default|GetTriggerSequence))) (delegate Custom|FinishSequenceTrigger))
  (CallFunction|ResetABP)
  (CallFunction|SetAnimPrincessMode "AnimationBlueprint")
  (switch Utilities|FlowControl|Switch|SwitchonE_TypeFadeOut (Variables|/Game/Blueprints/New/Triggers/BP_TriggerSequence.BP_TriggerSequence_C|GetTypeFadeOut (Variables|Default|GetTriggerSequence))
    (:NewEnumerator0
      _)
    (:NewEnumerator1
      (CameraFades|StartCameraFade :self (Variables|/Script/Engine.PlayerController|GetPlayerCameraManager (Game|GetPlayerController 0)) :FromAlpha 1.0 :Duration 1.0 :bHoldWhenFinished true)))
  (Utilities|IsValid (Variables|/Game/Blueprints/New/Triggers/BP_TriggerSequence.BP_TriggerSequence_C|GetCameraInteractiveObj (Variables|Default|GetTriggerSequence))
    (:Is%20Valid
      (Game|Player|SetViewTargetwithBlend (Game|GetPlayerController 0) (Variables|/Game/Blueprints/New/Triggers/BP_TriggerSequence.BP_TriggerSequence_C|GetCameraInteractiveObj (Variables|Default|GetTriggerSequence)) 0.0 "VTBlend_Linear" 0.0 false))
    (:Is%20Not%20Valid
      _))
  (Utilities|FlowControl|Delay 1.0)
  (if (!= (Variables|/Game/Blueprints/New/Triggers/BP_TriggerSequence.BP_TriggerSequence_C|GetNumDialogAfterSequence (Variables|Default|GetTriggerSequence)) 0)
    (Default|OpenDialog (Variables|Default|GetDialogActor) (Variables|/Game/Blueprints/New/Triggers/BP_TriggerSequence.BP_TriggerSequence_C|GetNumDialogAfterSequence (Variables|Default|GetTriggerSequence)) (stale Custom|ShowSequence DialogCaller))
    (Input|SetInputModeGameandUI (Game|GetPlayerController 0) (CallFunction|GetMainInterfaceWidget) "DoNotLock" false)
    (else
      (Class|DialogInterface|DialogEnded(Message) (stale Custom|ShowSequence DialogCaller)))))

(event Custom|FinishSequence
  (bind _actormain (Variables|Default|GetActorMain))
  (bind _actorforinteraction (Variables|/Game/Blueprints/New/InteractiveBPs/BP_ActorMain.BP_ActorMain_C|GetActorForInteraction _actormain))
  (bind (_actorforinteraction_2 _changedialogforhim) (Utilities|Struct|BreakStruct_InteractionWithActors _actorforinteraction))
  ;[1 1 1] Dialog after sequence
  (EventDispatchers|UnbindEventfromOnFinished (Variables|/Script/LevelSequence.LevelSequenceActor|GetSequencePlayer (Variables|/Game/Blueprints/New/InteractiveBPs/BP_ActorMain.BP_ActorMain_C|GetSequence (Variables|Default|GetActorMain))) (delegate Custom|FinishSequence))
  (CallFunction|ResetABP)
  (Input|SetInputModeGameandUI (Game|GetPlayerController 0) (CallFunction|GetMainInterfaceWidget) "DoNotLock" false)
  (CallFunction|SetAnimPrincessMode "AnimationBlueprint")
  (if (!= (Variables|/Game/Blueprints/New/InteractiveBPs/BP_ActorMain.BP_ActorMain_C|GetDialogAfterSequence (Variables|Default|GetActorMain)) 0)
    (Default|OpenDialog (Variables|Default|GetDialogActor) (Variables|/Game/Blueprints/New/InteractiveBPs/BP_ActorMain.BP_ActorMain_C|GetDialogAfterSequence (Variables|Default|GetActorMain)) (stale Custom|ShowSequence DialogCaller)))
  ;[1 1 1] Change dialog another actor
  (Utilities|IsValid _actorforinteraction_2
    (:Is%20Valid
      (Class|BPIInteractive|InteractwithObject(Message) _actorforinteraction_2 _changedialogforhim "0, 0, 0"))
    (:Is%20Not%20Valid
      _))
  ;[1 1 1] 2 dialogs
  (if (Utilities|Name|Equal(Name) (.RowName (Utilities|Struct|BreakDataTableRowHandle (Variables|/Game/Blueprints/New/InteractiveBPs/BP_ActorMain.BP_ActorMain_C|GetWithSequence? (Variables|Default|GetActorMain)))) "After")
    (Utilities|Struct|SetmembersinDataTableRowHandle (Variables|/Game/Blueprints/New/InteractiveBPs/BP_ActorMain.BP_ActorMain_C|GetWithSequence? (Variables|Default|GetActorMain)) "/Game/GameData/VariantPlayerSequence/DT_VariantSequence.DT_VariantSequence" "Not")))

(event EventBeginPlay
  (bind _returnvalue (Actor|GetActorOfClass "/Game/Blueprints/New/Managers/DialogActor.DialogActor_C"))
  (Variables|Default|SetDialogActor _returnvalue)
  (bind _as01cm_pc (Utilities|Casting|CastTo01CM_PC (Game|GetPlayerController 0)))
  (Variables|Default|SetPlayerController _as01cm_pc))

(event EventTick
  (params (DeltaSeconds :type Float%20%28single-precision%29)))

(fn ConstructionScript)

(fn SetAnimPrincessMode
  (params (AnimMode :type EAnimationMode%20Enum :default "AnimationBlueprint"))
  (bind _outactors (Actor|GetAllActorsOfClass "/Game/Assets/Heroes/FPrincess/BP_CharPrincess.BP_CharPrincess_C"))
  (bind _array_element (Utilities|Array|ForEachLoopwithBreak _outactors :!label _label)
    (:LoopBody
      (if (Utilities|Enum|Equal(Enum) (Utilities|GetObjectName _array_element) "BP_CharPrincess2")
        (Components|Animation|SetAnimationMode (Variables|/Script/Engine.Character|GetMesh _array_element) AnimMode)
        (goto _label Break)))
    (:Completed
      (return))))