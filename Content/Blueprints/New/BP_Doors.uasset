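; BP_Doors is a door Blueprint that builds on a parent class with an interaction widget.
; Its construction script runs the parent's, then raises the InteractionWidget to a fixed height offset when an ActorToUseWith comparison passes.
; The event graph adds no behavior of its own: BeginPlay calls the parent, overlap and Tick are disabled, and a ShowInteract call is never executed.
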(event EventBeginPlay
  (|CallParentFunction))

(event Collision|EventActorBeginOverlap
  (params (OtherActor :type Actor%20Object%20Reference))
  (|CallParentFunction OtherActor) ; This node is disabled and will not be called.\nDrag off pins to build functionality.
)

(event EventTick
  (params (DeltaSeconds :type Float%20%28single-precision%29))
  (|CallParentFunction DeltaSeconds) ; This node is disabled and will not be called.\nDrag off pins to build functionality.
)

(fn ConstructionScript
  (|CallParentFunction)
  (if (== (Variables|Default|GetActorToUseWith) 0)
    (Transformation|SetRelativeLocation (Variables|Default|GetInteractionWidget) "0, 0,250.000000" false false)))