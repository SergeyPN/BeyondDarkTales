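; BP_ActorMain is an interactable hotspot that shows the player an action icon for a linked world actor.
; The construction script picks the icon set, sphere or box trigger, and hint widget position.
; Overlap swaps the PreInteract hint for the shared InteractW, animating icon frames through timelines with a Russian/English label.
; Helpers toggle availability and shine material, chain-activate other actors, and handle pickup or drop, including backpack quest logging.
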(event OnComponentBeginOverlap(Sphere)
  (params (OverlappedComponent :type Primitive%20Component%20Object%20Reference) (OtherActor :type Actor%20Object%20Reference) (OtherComp :type Primitive%20Component%20Object%20Reference) (OtherBodyIndex :type Integer) (bFromSweep :type Boolean) (SweepResult :type Hit%20Result%20Structure%20%28by%20ref%29))
  (if (== OtherActor (Variables|Default|GetPlayer))
    (if (Variables|Default|GetAbleToInteract)
      (Variables|Default|SetIsInteracting true)
      (if (Variables|Default|GetAfterLevelChanged?)
        (Utilities|FlowControl|Delay 0.5))
      (CallFunction|CheckIntW)
      (Default|SetEnabled/Disabled (Variables|Default|GetPreInteract_W) false)
      (Audio|PlaySound2D "/Game/Audio/NEW_SOUNDS/BUTTONS/but_fx_appear.but_fx_appear" 1.0 1.0 0.0 0 0)
      (bind (_direction _alpha) (Timeline|Timeline_0 Play)
        (:Update
          (Default|UpdIconWidget (Variables|Default|GetIntW) (Utilities|Array|Get(acopy) (Variables|Default|GetStart/EndFrames) (Math|Float|Round (Math|Float|Lerp 0.0 (Math|Conversions|ToFloat(Integer) (Utilities|Array|LastIndex (Variables|Default|GetStart/EndFrames))) _alpha))) "" 0 0 0 0 false self 0 false "" false 0 "NewEnumerator3" "NewEnumerator0"))
        (:Finished
          (switch Utilities|FlowControl|Switch|SwitchonETimelineDirection _direction
            (:Forward
              (Default|OnOpenClose (Variables|Default|GetIntW) true)
              (bind (_direction_2 _alpha_2) (Timeline|Timeline_1 Play)
                (:Update
                  (switch Utilities|FlowControl|Switch|SwitchonGameLanguage (Variables|/Game/Blueprints/GI/BP_GI.BP_GI_C|GetLanguage (Variables|Default|GetGameInstance))
                    (:NewEnumerator0
                      (Default|UpdIconWidget (Variables|Default|GetIntW) (Utilities|Array|Get(acopy) (Variables|Default|GetLoopFrames) (Math|Float|Round (Math|Float|Lerp 0.0 (Math|Conversions|ToFloat(Integer) (Utilities|Array|LastIndex (Variables|Default|GetLoopFrames))) _alpha_2))) "" 0 0 0 0 false self 0 false (Variables|Widget|GetRusName) false 0 "NewEnumerator3" "NewEnumerator0"))
                    (:NewEnumerator1
                      (Default|UpdIconWidget (Variables|Default|GetIntW) (Utilities|Array|Get(acopy) (Variables|Default|GetLoopFrames) (Math|Float|Round (Math|Float|Lerp 0.0 (Math|Conversions|ToFloat(Integer) (Utilities|Array|LastIndex (Variables|Default|GetLoopFrames))) _alpha_2))) "" 0 0 0 0 false self 0 false (Variables|Widget|GetEngName) false 0 "NewEnumerator3" "NewEnumerator0"))))
                (:Finished
                  (switch Utilities|FlowControl|Switch|SwitchonETimelineDirection _direction_2
                    (:Forward
                      (if (Variables|Default|GetIsInteracting)
                        (Timeline|Timeline_1 PlayFromStart)))))))
            (:Backward
              (Widget|SetVisibility (Variables|Default|GetIntW) "Collapsed")
              (if (and (Variables|Default|GetDone?) (Variables|Interaction|GetDisableAfterInteract?))
                (CallFunction|Enable/DisableActor false)
                (elif (not (Variables|Default|GetWith%20Hide%20Pre%20Interact?))
                  (CallFunction|Enable/DisableActor true))))))))))

(event OnComponentEndOverlap(Sphere)
  (params (OverlappedComponent :type Primitive%20Component%20Object%20Reference) (OtherActor :type Actor%20Object%20Reference) (OtherComp :type Primitive%20Component%20Object%20Reference) (OtherBodyIndex :type Integer))
  (if (== OtherActor (Variables|Default|GetPlayer))
    (if (Variables|Default|GetIsInteracting)
      (Variables|Default|SetIsInteracting false)
      (Audio|PlaySound2D "/Game/Audio/NEW_SOUNDS/BUTTONS/but_fx_disapear.but_fx_disapear" 1.0 1.0 0.0 0 0)
      (Default|SetEnabled/Disabled (Variables|Default|GetPreInteract_W) true (Variables|Default|GetPlayer) self)
      (Default|OnOpenClose (Variables|Default|GetIntW) false)
      (bind (_direction _alpha) (Timeline|Timeline_0 Reverse)
        (:Update
          (Default|UpdIconWidget (Variables|Default|GetIntW) (Utilities|Array|Get(acopy) (Variables|Default|GetStart/EndFrames) (Math|Float|Round (Math|Float|Lerp 0.0 (Math|Conversions|ToFloat(Integer) (Utilities|Array|LastIndex (Variables|Default|GetStart/EndFrames))) _alpha))) "" 0 0 0 0 false self 0 false "" false 0 "NewEnumerator3" "NewEnumerator0"))
        (:Finished
          (switch Utilities|FlowControl|Switch|SwitchonETimelineDirection _direction
            (:Forward
              (Default|OnOpenClose (Variables|Default|GetIntW) true)
              (bind (_direction_2 _alpha_2) (Timeline|Timeline_1 Play)
                (:Update
                  (switch Utilities|FlowControl|Switch|SwitchonGameLanguage (Variables|/Game/Blueprints/GI/BP_GI.BP_GI_C|GetLanguage (Variables|Default|GetGameInstance))
                    (:NewEnumerator0
                      (Default|UpdIconWidget (Variables|Default|GetIntW) (Utilities|Array|Get(acopy) (Variables|Default|GetLoopFrames) (Math|Float|Round (Math|Float|Lerp 0.0 (Math|Conversions|ToFloat(Integer) (Utilities|Array|LastIndex (Variables|Default|GetLoopFrames))) _alpha_2))) "" 0 0 0 0 false self 0 false (Variables|Widget|GetRusName) false 0 "NewEnumerator3" "NewEnumerator0"))
                    (:NewEnumerator1
                      (Default|UpdIconWidget (Variables|Default|GetIntW) (Utilities|Array|Get(acopy) (Variables|Default|GetLoopFrames) (Math|Float|Round (Math|Float|Lerp 0.0 (Math|Conversions|ToFloat(Integer) (Utilities|Array|LastIndex (Variables|Default|GetLoopFrames))) _alpha_2))) "" 0 0 0 0 false self 0 false (Variables|Widget|GetEngName) false 0 "NewEnumerator3" "NewEnumerator0"))))
                (:Finished
                  (switch Utilities|FlowControl|Switch|SwitchonETimelineDirection _direction_2
                    (:Forward
                      (if (Variables|Default|GetIsInteracting)
                        (Timeline|Timeline_1 PlayFromStart)))))))
            (:Backward
              (Widget|SetVisibility (Variables|Default|GetIntW) "Collapsed")
              (if (and (Variables|Default|GetDone?) (Variables|Interaction|GetDisableAfterInteract?))
                (CallFunction|Enable/DisableActor false)
                (elif (not (Variables|Default|GetWith%20Hide%20Pre%20Interact?))
                  (CallFunction|Enable/DisableActor true))))))))))

(event OnComponentBeginOverlap(Box)
  (params (OverlappedComponent :type Primitive%20Component%20Object%20Reference) (OtherActor :type Actor%20Object%20Reference) (OtherComp :type Primitive%20Component%20Object%20Reference) (OtherBodyIndex :type Integer) (bFromSweep :type Boolean) (SweepResult :type Hit%20Result%20Structure%20%28by%20ref%29))
  (if (== OtherActor (Variables|Default|GetPlayer))
    (if (Variables|Default|GetAbleToInteract)
      (Variables|Default|SetIsInteracting true)
      (if (Variables|Default|GetAfterLevelChanged?)
        (Utilities|FlowControl|Delay 0.5))
      (CallFunction|CheckIntW)
      (Default|SetEnabled/Disabled (Variables|Default|GetPreInteract_W) false)
      (Audio|PlaySound2D "/Game/Audio/NEW_SOUNDS/BUTTONS/but_fx_appear.but_fx_appear" 1.0 1.0 0.0 0 0)
      (bind (_direction _alpha) (Timeline|Timeline_0 Play)
        (:Update
          (Default|UpdIconWidget (Variables|Default|GetIntW) (Utilities|Array|Get(acopy) (Variables|Default|GetStart/EndFrames) (Math|Float|Round (Math|Float|Lerp 0.0 (Math|Conversions|ToFloat(Integer) (Utilities|Array|LastIndex (Variables|Default|GetStart/EndFrames))) _alpha))) "" 0 0 0 0 false self 0 false "" false 0 "NewEnumerator3" "NewEnumerator0"))
        (:Finished
          (switch Utilities|FlowControl|Switch|SwitchonETimelineDirection _direction
            (:Forward
              (Default|OnOpenClose (Variables|Default|GetIntW) true)
              (bind (_direction_2 _alpha_2) (Timeline|Timeline_1 Play)
                (:Update
                  (switch Utilities|FlowControl|Switch|SwitchonGameLanguage (Variables|/Game/Blueprints/GI/BP_GI.BP_GI_C|GetLanguage (Variables|Default|GetGameInstance))
                    (:NewEnumerator0
                      (Default|UpdIconWidget (Variables|Default|GetIntW) (Utilities|Array|Get(acopy) (Variables|Default|GetLoopFrames) (Math|Float|Round (Math|Float|Lerp 0.0 (Math|Conversions|ToFloat(Integer) (Utilities|Array|LastIndex (Variables|Default|GetLoopFrames))) _alpha_2))) "" 0 0 0 0 false self 0 false (Variables|Widget|GetRusName) false 0 "NewEnumerator3" "NewEnumerator0"))
                    (:NewEnumerator1
                      (Default|UpdIconWidget (Variables|Default|GetIntW) (Utilities|Array|Get(acopy) (Variables|Default|GetLoopFrames) (Math|Float|Round (Math|Float|Lerp 0.0 (Math|Conversions|ToFloat(Integer) (Utilities|Array|LastIndex (Variables|Default|GetLoopFrames))) _alpha_2))) "" 0 0 0 0 false self 0 false (Variables|Widget|GetEngName) false 0 "NewEnumerator3" "NewEnumerator0"))))
                (:Finished
                  (switch Utilities|FlowControl|Switch|SwitchonETimelineDirection _direction_2
                    (:Forward
                      (if (Variables|Default|GetIsInteracting)
                        (Timeline|Timeline_1 PlayFromStart)))))))
            (:Backward
              (Widget|SetVisibility (Variables|Default|GetIntW) "Collapsed")
              (if (and (Variables|Default|GetDone?) (Variables|Interaction|GetDisableAfterInteract?))
                (CallFunction|Enable/DisableActor false)
                (elif (not (Variables|Default|GetWith%20Hide%20Pre%20Interact?))
                  (CallFunction|Enable/DisableActor true))))))))))

(event OnComponentEndOverlap(Box)
  (params (OverlappedComponent :type Primitive%20Component%20Object%20Reference) (OtherActor :type Actor%20Object%20Reference) (OtherComp :type Primitive%20Component%20Object%20Reference) (OtherBodyIndex :type Integer))
  (if (== OtherActor (Variables|Default|GetPlayer))
    (if (Variables|Default|GetIsInteracting)
      (Variables|Default|SetIsInteracting false)
      (Audio|PlaySound2D "/Game/Audio/NEW_SOUNDS/BUTTONS/but_fx_disapear.but_fx_disapear" 1.0 1.0 0.0 0 0)
      (Default|SetEnabled/Disabled (Variables|Default|GetPreInteract_W) true (Variables|Default|GetPlayer) self)
      (Default|OnOpenClose (Variables|Default|GetIntW) false)
      (bind (_direction _alpha) (Timeline|Timeline_0 Reverse)
        (:Update
          (Default|UpdIconWidget (Variables|Default|GetIntW) (Utilities|Array|Get(acopy) (Variables|Default|GetStart/EndFrames) (Math|Float|Round (Math|Float|Lerp 0.0 (Math|Conversions|ToFloat(Integer) (Utilities|Array|LastIndex (Variables|Default|GetStart/EndFrames))) _alpha))) "" 0 0 0 0 false self 0 false "" false 0 "NewEnumerator3" "NewEnumerator0"))
        (:Finished
          (switch Utilities|FlowControl|Switch|SwitchonETimelineDirection _direction
            (:Forward
              (Default|OnOpenClose (Variables|Default|GetIntW) true)
              (bind (_direction_2 _alpha_2) (Timeline|Timeline_1 Play)
                (:Update
                  (switch Utilities|FlowControl|Switch|SwitchonGameLanguage (Variables|/Game/Blueprints/GI/BP_GI.BP_GI_C|GetLanguage (Variables|Default|GetGameInstance))
                    (:NewEnumerator0
                      (Default|UpdIconWidget (Variables|Default|GetIntW) (Utilities|Array|Get(acopy) (Variables|Default|GetLoopFrames) (Math|Float|Round (Math|Float|Lerp 0.0 (Math|Conversions|ToFloat(Integer) (Utilities|Array|LastIndex (Variables|Default|GetLoopFrames))) _alpha_2))) "" 0 0 0 0 false self 0 false (Variables|Widget|GetRusName) false 0 "NewEnumerator3" "NewEnumerator0"))
                    (:NewEnumerator1
                      (Default|UpdIconWidget (Variables|Default|GetIntW) (Utilities|Array|Get(acopy) (Variables|Default|GetLoopFrames) (Math|Float|Round (Math|Float|Lerp 0.0 (Math|Conversions|ToFloat(Integer) (Utilities|Array|LastIndex (Variables|Default|GetLoopFrames))) _alpha_2))) "" 0 0 0 0 false self 0 false (Variables|Widget|GetEngName) false 0 "NewEnumerator3" "NewEnumerator0"))))
                (:Finished
                  (switch Utilities|FlowControl|Switch|SwitchonETimelineDirection _direction_2
                    (:Forward
                      (if (Variables|Default|GetIsInteracting)
                        (Timeline|Timeline_1 PlayFromStart)))))))
            (:Backward
              (Widget|SetVisibility (Variables|Default|GetIntW) "Collapsed")
              (if (and (Variables|Default|GetDone?) (Variables|Interaction|GetDisableAfterInteract?))
                (CallFunction|Enable/DisableActor false)
                (elif (not (Variables|Default|GetWith%20Hide%20Pre%20Interact?))
                  (CallFunction|Enable/DisableActor true))))))))))

(event Custom|ShowInteract
  (if (Variables|Default|GetBoxOrSphereCollision)
    (Variables|Default|SetIsInteracting true)
    (else
      (Variables|Default|SetIsInteracting true)))
  (if (Variables|Default|GetAfterLevelChanged?)
    (Utilities|FlowControl|Delay 0.5))
  (CallFunction|CheckIntW)
  (Default|SetEnabled/Disabled (Variables|Default|GetPreInteract_W) false)
  (Audio|PlaySound2D "/Game/Audio/NEW_SOUNDS/BUTTONS/but_fx_appear.but_fx_appear" 1.0 1.0 0.0 0 0)
  (bind (_direction _alpha) (Timeline|Timeline_0 Play)
    (:Update
      (Default|UpdIconWidget (Variables|Default|GetIntW) (Utilities|Array|Get(acopy) (Variables|Default|GetStart/EndFrames) (Math|Float|Round (Math|Float|Lerp 0.0 (Math|Conversions|ToFloat(Integer) (Utilities|Array|LastIndex (Variables|Default|GetStart/EndFrames))) _alpha))) "" 0 0 0 0 false self 0 false "" false 0 "NewEnumerator3" "NewEnumerator0"))
    (:Finished
      (switch Utilities|FlowControl|Switch|SwitchonETimelineDirection _direction
        (:Forward
          (Default|OnOpenClose (Variables|Default|GetIntW) true)
          (bind (_direction_2 _alpha_2) (Timeline|Timeline_1 Play)
            (:Update
              (switch Utilities|FlowControl|Switch|SwitchonGameLanguage (Variables|/Game/Blueprints/GI/BP_GI.BP_GI_C|GetLanguage (Variables|Default|GetGameInstance))
                (:NewEnumerator0
                  (Default|UpdIconWidget (Variables|Default|GetIntW) (Utilities|Array|Get(acopy) (Variables|Default|GetLoopFrames) (Math|Float|Round (Math|Float|Lerp 0.0 (Math|Conversions|ToFloat(Integer) (Utilities|Array|LastIndex (Variables|Default|GetLoopFrames))) _alpha_2))) "" 0 0 0 0 false self 0 false (Variables|Widget|GetRusName) false 0 "NewEnumerator3" "NewEnumerator0"))
                (:NewEnumerator1
                  (Default|UpdIconWidget (Variables|Default|GetIntW) (Utilities|Array|Get(acopy) (Variables|Default|GetLoopFrames) (Math|Float|Round (Math|Float|Lerp 0.0 (Math|Conversions|ToFloat(Integer) (Utilities|Array|LastIndex (Variables|Default|GetLoopFrames))) _alpha_2))) "" 0 0 0 0 false self 0 false (Variables|Widget|GetEngName) false 0 "NewEnumerator3" "NewEnumerator0"))))
            (:Finished
              (switch Utilities|FlowControl|Switch|SwitchonETimelineDirection _direction_2
                (:Forward
                  (if (Variables|Default|GetIsInteracting)
                    (Timeline|Timeline_1 PlayFromStart)))))))
        (:Backward
          (Widget|SetVisibility (Variables|Default|GetIntW) "Collapsed")
          (if (and (Variables|Default|GetDone?) (Variables|Interaction|GetDisableAfterInteract?))
            (CallFunction|Enable/DisableActor false)
            (elif (not (Variables|Default|GetWith%20Hide%20Pre%20Interact?))
              (CallFunction|Enable/DisableActor true))))))))

(event Custom|HideInteract
  (params (WithHidePreInteract? :type Boolean))
  (Variables|Default|SetWith%20Hide%20Pre%20Interact? WithHidePreInteract?)
  (if (Variables|Default|GetBoxOrSphereCollision)
    (Variables|Default|SetIsInteracting false)
    (Audio|PlaySound2D "/Game/Audio/NEW_SOUNDS/BUTTONS/but_fx_disapear.but_fx_disapear" 1.0 1.0 0.0 0 0)
    (else
      (Variables|Default|SetIsInteracting false)
      (Audio|PlaySound2D "/Game/Audio/NEW_SOUNDS/BUTTONS/but_fx_disapear.but_fx_disapear" 1.0 1.0 0.0 0 0)))
  (Default|SetEnabled/Disabled (Variables|Default|GetPreInteract_W) true (Variables|Default|GetPlayer) self)
  (Default|OnOpenClose (Variables|Default|GetIntW) false)
  (bind (_direction _alpha) (Timeline|Timeline_0 Reverse)
    (:Update
      (Default|UpdIconWidget (Variables|Default|GetIntW) (Utilities|Array|Get(acopy) (Variables|Default|GetStart/EndFrames) (Math|Float|Round (Math|Float|Lerp 0.0 (Math|Conversions|ToFloat(Integer) (Utilities|Array|LastIndex (Variables|Default|GetStart/EndFrames))) _alpha))) "" 0 0 0 0 false self 0 false "" false 0 "NewEnumerator3" "NewEnumerator0"))
    (:Finished
      (switch Utilities|FlowControl|Switch|SwitchonETimelineDirection _direction
        (:Forward
          (Default|OnOpenClose (Variables|Default|GetIntW) true)
          (bind (_direction_2 _alpha_2) (Timeline|Timeline_1 Play)
            (:Update
              (switch Utilities|FlowControl|Switch|SwitchonGameLanguage (Variables|/Game/Blueprints/GI/BP_GI.BP_GI_C|GetLanguage (Variables|Default|GetGameInstance))
                (:NewEnumerator0
                  (Default|UpdIconWidget (Variables|Default|GetIntW) (Utilities|Array|Get(acopy) (Variables|Default|GetLoopFrames) (Math|Float|Round (Math|Float|Lerp 0.0 (Math|Conversions|ToFloat(Integer) (Utilities|Array|LastIndex (Variables|Default|GetLoopFrames))) _alpha_2))) "" 0 0 0 0 false self 0 false (Variables|Widget|GetRusName) false 0 "NewEnumerator3" "NewEnumerator0"))
                (:NewEnumerator1
                  (Default|UpdIconWidget (Variables|Default|GetIntW) (Utilities|Array|Get(acopy) (Variables|Default|GetLoopFrames) (Math|Float|Round (Math|Float|Lerp 0.0 (Math|Conversions|ToFloat(Integer) (Utilities|Array|LastIndex (Variables|Default|GetLoopFrames))) _alpha_2))) "" 0 0 0 0 false self 0 false (Variables|Widget|GetEngName) false 0 "NewEnumerator3" "NewEnumerator0"))))
            (:Finished
              (switch Utilities|FlowControl|Switch|SwitchonETimelineDirection _direction_2
                (:Forward
                  (if (Variables|Default|GetIsInteracting)
                    (Timeline|Timeline_1 PlayFromStart)))))))
        (:Backward
          (Widget|SetVisibility (Variables|Default|GetIntW) "Collapsed")
          (if (and (Variables|Default|GetDone?) (Variables|Interaction|GetDisableAfterInteract?))
            (CallFunction|Enable/DisableActor false)
            (elif (not (Variables|Default|GetWith%20Hide%20Pre%20Interact?))
              (CallFunction|Enable/DisableActor true))))))))

(event EventBeginPlay
  (bind _asbp_gi (Utilities|Casting|CastToBP_GI (Game|GetGameInstance))
    (:then
      (Variables|Default|SetGameInstance _asbp_gi))
    (:CastFailed
      _))
  (bind _returnvalue (Actor|GetActorOfClass "/Game/Blueprints/New/Managers/SequenceManager/BP_SequenceManager.BP_SequenceManager_C"))
  (Variables|Sequence|SetSequenceManager _returnvalue)
  (bind _ascamera_pc_test (Utilities|Casting|CastToCamera_PC_test (Game|Player|GetPlayerPawn 0))
    (:then
      (Variables|Default|SetPlayerPawn _ascamera_pc_test))
    (:CastFailed
      _))
  (bind _outactors (Actor|GetAllActorsOfClass "/Game/Assets/Heroes/Max/BP_CharMax.BP_CharMax_C"))
  (Variables|Default|SetPlayer (Utilities|Array|Get(acopy) _outactors))
  (bind _outactors_2 (Actor|GetAllActorsOfClass "/Game/Blueprints/New/Managers/DialogActor.DialogActor_C"))
  (Variables|Default|SetDialogActor (Utilities|Array|Get(acopy) _outactors_2))
  (bind _asbp_main_menu_hud (Utilities|Casting|CastToBP_MainMenuHUD (HUD|GetHUD (Game|GetPlayerController 0)))
    (:then
      (Variables|Default|SetHUD _asbp_main_menu_hud))
    (:CastFailed
      _))
  (bind _aspre_interact (Utilities|Casting|CastToPreInteract (UserInterface|GetUserWidgetObject (Variables|Default|GetPreInteractionWidget)))
    (:then
      (Variables|Default|SetPreInteract_W _aspre_interact))
    (:CastFailed
      _))
  (if (or (Variables|Default|GetStartEnabled?) (Variables|Default|GetAfterStreamLevelInteraction))
    (if (and (Variables|Default|GetDone?) (Variables|Interaction|GetDisableAfterInteract?))
      (CallFunction|Enable/DisableActor false)
      (else
        (Default|SetEnabled/Disabled (Variables|Default|GetPreInteract_W) true (Variables|Default|GetPlayer) self)))))

(event EventInteractwithObject
  (params (DialogToStart :type Array%20of%20Integers) (MoveTo :type Vector :default "0, 0, 0"))
  (Variables|Dialog|SetDialogToStart DialogToStart))

(fn ConstructionScript
  (bind _overlapradius (Variables|Default|GetOverlapRadius))
  (bind _actortousewith (Variables|Interaction|GetActorToUseWith))
  (bind _origin (Collision|GetActorBounds _actortousewith false false))
  (CallFunction|SetIcons (Variables|Default|GetIconsToUse))
  (if (Variables|Default|GetBoxOrSphereCollision)
    (Components|Box|SetBoxExtent (Variables|Default|GetBox) (Math|Vector|MakeVector _overlapradius _overlapradius 32.0) true)
    (Components|DestroyComponent (Variables|Default|GetSphere))
    (else
      (Components|Sphere|SetSphereRadius (Variables|Default|GetSphere) (Variables|Default|GetOverlapRadius) true)
      (Components|DestroyComponent (Variables|Default|GetBox))))
  (if (!= (Variables|Interaction|GetActorToUseWith) 0)
    (Transformation|SetWorldLocation (Variables|Default|GetSphere1) (Math|Vector|MakeVector (+ (.x _origin) (Variables|Interaction|GetIW_X)) (+ (.y _origin) (Variables|Interaction|GetIW_Y)) (+ (.z _origin) 2.5e+02 (Variables|Interaction|GetIW_Z))) false false)
    (CallFunction|Enable/DisableActor (Variables|Default|GetStartEnabled?))
    (else
      (Transformation|SetRelativeLocation (Variables|Default|GetPreInteractionWidget) (Math|Vector|MakeVector (+ 0.0 (Variables|Interaction|GetIW_X)) (+ 0.0 (Variables|Interaction|GetIW_Y)) (+ 3.5e+02 (Variables|Interaction|GetIW_Z))) false false)
      (CallFunction|Enable/DisableActor (Variables|Default|GetStartEnabled?)))))

(fn Enable/DisableActor
  (params (IsOn? :type Boolean))
  (bind _asstatic_mesh_actor (Utilities|Casting|CastToStaticMeshActor (Variables|Interaction|GetActorToUseWith))
    (:then
      (LocalVariables|SetLMeshActor _asstatic_mesh_actor))
    (:CastFailed
      _))
  (if IsOn?
    (Variables|Default|SetAbleToInteract true)
    (Variables|Default|SetStartEnabled? true)
    (Utilities|IsValid (Variables|Interaction|GetActorToUseWith)
      (:Is%20Valid
        (bind _lmeshactor (LocalVariables|GetLMeshActor)
          (:then
            (Rendering|Material|SetMaterial (Variables|/Script/Engine.StaticMeshActor|GetStaticMeshComponent _lmeshactor) 0 "/Game/Assets/Maps/UniversalMats/MI_ShineFX.MI_ShineFX"))
          (:else
            _)))
      (:Is%20Not%20Valid
        _))
    (Utilities|IsValid (Variables|Default|GetPlayer)
      (:Is%20Valid
        (Default|SetEnabled/Disabled (Variables|Default|GetPreInteract_W) true (Variables|Default|GetPlayer) self)))
    (else
      (Variables|Default|SetAbleToInteract false)
      (Variables|Default|SetStartEnabled? false)
      (Utilities|IsValid (Variables|Interaction|GetActorToUseWith)
        (:Is%20Valid
          (bind _lmeshactor_2 (LocalVariables|GetLMeshActor)
            (:then
              (Rendering|Material|SetMaterial (Variables|/Script/Engine.StaticMeshActor|GetStaticMeshComponent _lmeshactor_2) 0 "/Game/Assets/Maps/UniversalMats/MI_UMat.MI_UMat"))
            (:else
              _)))
        (:Is%20Not%20Valid
          _))
      (Utilities|IsValid (Variables|Default|GetPreInteract_W)
        (:Is%20Valid
          (Default|SetEnabled/Disabled (Variables|Default|GetPreInteract_W) false))))))

(fn SetIcons
  (params (Selection :type IconsTypes%20Enum :default "NewEnumerator5"))
  (switch Utilities|FlowControl|Switch|SwitchonIconsTypes Selection
    (:NewEnumerator5
      (|EmptyIcons))
    (:NewEnumerator0
      (|CommentIcons))
    (:NewEnumerator1
      (|DoorIcons))
    (:NewEnumerator2
      (|GrabIcons))
    (:NewEnumerator3
      (|HOIcons))
    (:NewEnumerator4
      (|PzzleIcons))
    (:NewEnumerator6
      (|JumpIcons))))

(fn TriggerActors
  (if (Variables|Trigger|GetIsTrigger?)
    (Variables|Trigger|SetIsTrigger? false)
    (for _array_element (Variables|Trigger|GetActorToTrigger)
      (bind _asbp_actor_main (Utilities|Casting|CastToBP_ActorMain _array_element)
        (:then
          (CallFunction|Enable/DisableActor _asbp_actor_main true)
          (if (Variables|Trigger|GetWithShowInteractButton)
            (CallFunction|ShowInteract _asbp_actor_main)))
        (:CastFailed
          (Class|BPIActivableActor|ActivateActor(Message) _array_element))))
    (return)
    (else
      (return))))

(fn DestroyActoronPicked
  (bind _actortousewith (Variables|Interaction|GetActorToUseWith))
  (bind _returnvalue (Transformation|GetActorTransform _actortousewith))
  (CallFunction|TriggerActors)
  (Effects|SpawnEmitteratLocation "/Game/Assets/Particles/P_HO.P_HO" (.location _returnvalue) (.rotation _returnvalue))
  (bind _actortousewith_2 (Variables|Interaction|GetActorToUseWith)
    (:then
      (if (Utilities|Enum|Equal(Enum) (Utilities|GetObjectName _actortousewith_2) "BP_Backpack_2")
        (Utilities|Map|Add (Variables|/Game/Blueprints/GI/BP_GI.BP_GI_C|GetQuestsStatus (Variables|Default|GetGameInstance)) "NewEnumerator0" true)
        (bind _keys (Utilities|Map|Keys (Variables|/Game/Blueprints/GI/BP_GI.BP_GI_C|GetQuestsStatus (Variables|Default|GetGameInstance))))
        (Class|FirebaseAnalyticsSubsystem|PutString (LocalVariables|GetLBundle) "quest" (Utilities|String|EnumtoString (Utilities|Array|Get(acopy) _keys)))
        (Class|FirebaseAnalyticsSubsystem|LogEventwithParameters "QuestSolved" (LocalVariables|GetLBundle))
        (Development|SetHiddeninGame (Variables|/Game/Assets/Heroes/Max/BP_CharMax.BP_CharMax_C|GetBackPack (Variables|Default|GetPlayer)) false false)))
    (:else
      _))
  (Rendering|SetActorHiddenInGame self true)
  (Collision|SetActorEnableCollision self false)
  (Actor|DestroyActor (Variables|Interaction|GetActorToUseWith)))

(fn DropActorSimple
  (bind _actortousewith (Variables|Interaction|GetActorToUseWith))
  (bind _actortousewith_2 (Variables|Interaction|GetActorToUseWith))
  (bind _returnvalue (Transformation|GetActorTransform _actortousewith_2))
  (bind _returnvalue_2 (Actor|GetComponentbyClass _actortousewith "/Script/Engine.ParticleSystemComponent"))
  (CallFunction|TriggerActors)
  (Effects|SpawnEmitteratLocation "/Game/Assets/Particles/P_HO.P_HO" (.location _returnvalue) (.rotation _returnvalue))
  (Rendering|SetActorHiddenInGame (Variables|Interaction|GetActorToUseWith) false)
  (if (Utilities|IsValid _returnvalue_2)
    (Components|Activation|Activate _returnvalue_2 false))
  (CallFunction|Enable/DisableActor false))

(fn CheckIntW
  (Utilities|IsValid (Variables|Default|GetIntW)
    (:Is%20Valid
      _)
    (:Is%20Not%20Valid
      (bind _foundwidgets (Widget|GetAllWidgetsOfClass "/Game/Widgets/New/MainInterface_W.MainInterface_W_C" true))
      (Variables|Default|SetIntW (Variables|/Game/Widgets/New/MainInterface_W.MainInterface_W_C|GetInteract_W (Utilities|Array|Get(acopy) _foundwidgets)))))
  (Widget|SetVisibility (Variables|Default|GetIntW) "Visible")
  (if (not (== self (Variables|/Game/Widgets/New/Interact_W.Interact_W_C|GetActorToInteract (Variables|Default|GetIntW))))
    (Variables|/Game/Widgets/New/Interact_W.Interact_W_C|SetActorToInteract (Variables|Default|GetIntW) self)))

(fn InteractwithWidget
  (return))