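; Interactable static Blueprint that plays a one-time video with subtitles and media sound, then opens a dialog or triggers linked actors.
; Interaction disables input and hides the UI; a data table row decides whether a vision sequence runs first.
; That sequence blends to CCamVision, AI-moves and turns the player, then swaps BP_TreeRune's visuals before the video or dialog.
; Dialog end triggers actors and restores UI and input.
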(event Custom|FinishSequenceVision
  (bind _asbp_tree_rune (Utilities|Casting|CastToBP_TreeRune (Variables|Default|GetActorToUseWith)))
  (Rendering|SetVisibility (Variables|/Game/Assets/Maps/01_Caves/Meshes/BP_TreeRune.BP_TreeRune_C|GetTreeActive _asbp_tree_rune) false false)
  (Rendering|SetVisibility (Variables|/Game/Assets/Maps/01_Caves/Meshes/BP_TreeRune.BP_TreeRune_C|GetTreeDisactived _asbp_tree_rune) true false)
  (CallFunction|ShowVideoorDialog)
  (Utilities|FlowControl|Delay 1.0)
  (Game|Player|SetViewTargetwithBlend (Game|GetPlayerController 0) (Variables|/Game/Blueprints/CameraControl/Camera_PC_test.Camera_PC_test_C|GetLevelCamera (Variables|Default|GetPlayerPawn)) 1.0 "VTBlend_Cubic" 0.0 false)
  (Audio|PlaySound2D "/Game/Audio/NEW_SOUNDS/SFX/fx_camera_move_close.fx_camera_move_close" 1.0 1.0 0.0 0 0))

(event EventBeginPlay
  (|CallParentFunction) ; This node is disabled and will not be called.\nDrag off pins to build functionality.
)

(event Collision|EventActorBeginOverlap
  (params (OtherActor :type Actor%20Object%20Reference))
  (|CallParentFunction OtherActor) ; This node is disabled and will not be called.\nDrag off pins to build functionality.
)

(event EventTick
  (params (DeltaSeconds :type Float%20%28single-precision%29))
  (|CallParentFunction DeltaSeconds) ; This node is disabled and will not be called.\nDrag off pins to build functionality.
)

(event EventInteractwithWidget
  (bind _sequence (Variables|Default|GetSequence))
  (bind _playerpawn (Variables|Default|GetPlayerPawn))
  (bind _sequenceplayer (Variables|/Script/LevelSequence.LevelSequenceActor|GetSequencePlayer _sequence))
  (bind _currentplayercontroller (Variables|/Game/Blueprints/CameraControl/Camera_PC_test.Camera_PC_test_C|GetCurrentPlayerController _playerpawn))
  (bind _maininterface_w (Variables|/Game/Blueprints/New/Main/01CaveMain/01CM_PC.01CM_PC_C|GetMainInterface_W _currentplayercontroller))
  (Input|DisableInput (Game|Player|GetPlayerPawn 0) (Game|GetPlayerController 0))
  (CallFunction|HideInteract false)
  (UserInterface|Animation|PlayAnimation _maininterface_w (Variables|/Game/Widgets/New/MainInterface_W.MainInterface_W_C|GetShowInterface _maininterface_w) 0.0 1 "Reverse" 4.0 false)
  (switch name (.RowName (Utilities|Struct|BreakDataTableRowHandle (Variables|Default|GetWithSequence?)))
    (:Not
      (CallFunction|ShowVideoorDialog))
    (:Before
      (bind _outactors (Actor|GetAllActorsOfClass "/Script/CinematicCamera.CineCameraActor"))
      (bind _array_element (Utilities|Array|ForEachLoopwithBreak _outactors :!label _label)
        (:LoopBody
          (if (Utilities|Enum|Equal(Enum) (Utilities|GetDisplayName _array_element) "CCamVision")
            (Game|Player|SetViewTargetwithBlend (Game|GetPlayerController 0) _array_element 1.0 "VTBlend_Cubic" 0.0 false)
            (Audio|PlaySound2D "/Game/Audio/NEW_SOUNDS/SFX/fx_camera_move_far.fx_camera_move_far" 1.0 1.0 0.0 0 0)
            (bind _returnvalue (Actor|GetActorOfClass "/Script/Engine.TargetPoint"))
            (AI|AIMoveTo (Variables|Default|GetPlayer) "0, 0, 0" _returnvalue 2.0 false
              (:then
                (goto _label Break))
              (:OnSuccess
                (bind _alpha (Timeline|RotateCharacter PlayFromStart)
                  (:Update
                    (Transformation|SetActorRotation (Variables|Default|GetPlayer) (Math|Rotator|Lerp(Rotator) (Transformation|GetActorRotation (Variables|Default|GetPlayer)) "0, 0, 0" _alpha))))))))
        (:Completed
          (|SetBy-RefVar (Variables|Default|GetWithSequence?) (Utilities|Struct|MakeDataTableRowHandle "/Game/GameData/VariantPlayerSequence/DT_VariantSequence.DT_VariantSequence" "Not"))
          (Sequencer|Player|Play _sequenceplayer :!class /Script/MovieScene.MovieSceneSequencePlayer)
          (EventDispatchers|BindEventtoOnFinished _sequenceplayer (delegate Custom|FinishSequenceVision)))))))

(event EventDialogEnded
  (params (CurrentDialogNum :type Integer))
  (bind _playerpawn (Variables|Default|GetPlayerPawn))
  (bind _currentplayercontroller (Variables|/Game/Blueprints/CameraControl/Camera_PC_test.Camera_PC_test_C|GetCurrentPlayerController _playerpawn))
  (bind _maininterface_w (Variables|/Game/Blueprints/New/Main/01CaveMain/01CM_PC.01CM_PC_C|GetMainInterface_W _currentplayercontroller))
  (CallFunction|TriggerActors)
  (UserInterface|Animation|PlayAnimation _maininterface_w (Variables|/Game/Widgets/New/MainInterface_W.MainInterface_W_C|GetShowInterface _maininterface_w) 0.0 1 "Forward" 4.0 false)
  (Utilities|FlowControl|Delay 1.0)
  (Input|EnableInput (Game|Player|GetPlayerPawn 0) (Game|GetPlayerController 0)))

(event EventVideoEnded
  (Widget|RemovefromParent (Variables|Default|GetVideoWidget))
  (Widget|RemovefromParent (Variables|Default|GetSubtitle))
  (if (Variables|Default|GetIsWithDialog?)
    (Default|OpenDialog (Variables|Default|GetDialogActor) (Utilities|Array|Get(acopy) (Variables|Default|GetDialogToStart)) self)
    (else
      (CallFunction|TriggerActors))))

(fn ConstructionScript
  (|CallParentFunction))

(fn ShowVideoorDialog
  (if (Variables|Default|GetIsPlayedOnce?)
    (Variables|Default|SetIsPlayedOnce? false)
    (bind _returnvalue (UserInterface|CreateWidget "/Game/Widgets/New/Video_W.Video_W_C" (Game|GetPlayerController 0) (Variables|Default|GetVideoToPlay) self))
    (UserInterface|Viewport|AddtoViewport _returnvalue 0)
    (Variables|Default|SetVideoWidget _returnvalue)
    (Default|Enable/DisableInput (Variables|Default|GetDialogActor) false)
    (CameraShake|Start (Variables|Default|GetMediaSound))
    (bind _returnvalue_2 (UserInterface|CreateWidget "/Game/Widgets/Subtitles/WBP_Subtitles.WBP_Subtitles_C"))
    (bind _output_get (Variables|Default|SetSubtitle _returnvalue_2))
    (UserInterface|Viewport|AddtoViewport _output_get 0)
    (elif (Variables|Default|GetIsWithDialog?)
      (Default|OpenDialog (Variables|Default|GetDialogActor) (Utilities|Array|Get(acopy) (Variables|Default|GetDialogToStart)) self)
      (else
        (CallFunction|TriggerActors)))))