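; BP_Pickable_Simple is an interactive pickup that plays a camera, dialog or sequence flow before the player picks the item up.
; Interacting hides the UI, fills the item widget, then either hands off to the sequence manager or blends to the object's camera and runs DialogPickItem.
; DialogEnded first triggers the pickup and adds the item to inventory except for one item type; later calls restore the interface.
; A cast to its tutorial subclass hides that variant's widget.
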(event EventBeginPlay
  (|CallParentFunction))

(event Collision|EventActorBeginOverlap
  (params (OtherActor :type Actor%20Object%20Reference))
  (|CallParentFunction OtherActor) ; This node is disabled and will not be called.\nDrag off pins to build functionality.
)

(event EventTick
  (params (DeltaSeconds :type Float%20%28single-precision%29))
  (|CallParentFunction DeltaSeconds))

(event EventInteractwithWidget
  (bind _self self)
  (bind _playerpawn (Variables|Default|GetPlayerPawn))
  (bind _inventoryitem (Variables|Default|GetInventoryItem))
  (bind _currentplayercontroller (Variables|/Game/Blueprints/Transfered/Blueprints1/ToTransfer/Camera_PC_test.Camera_PC_test_C|GetCurrentPlayerController _playerpawn))
  (bind _maininterface_w (Variables|/Game/Blueprints/New/Main/01CaveMain/01CM_PC.01CM_PC_C|GetMainInterface_W _currentplayercontroller))
  (CallFunction|HideInteract)
  (UserInterface|Animation|PlayAnimation _maininterface_w (Variables|/Game/Widgets/New/MainInterface_W.MainInterface_W_C|GetShowInterface _maininterface_w) 0.0 1 "Reverse" 4.0 false)
  (bind _asbp_pickable_simple_tutorial (Utilities|Casting|CastToBP_Pickable_Simple_Tutorial self)
    (:then
      (Development|SetHiddeninGame (Variables|/Game/Blueprints/New/InteractiveBPs/BP_Pickable_Simple_Tutorial.BP_Pickable_Simple_Tutorial_C|GetTutorialWidget _asbp_pickable_simple_tutorial) true false))
    (:CastFailed
      _))
  (bind _returnvalue (Actor|GetActorOfClass "/Game/Blueprints/New/BP_SequenceManager.BP_SequenceManager_C"))
  (Variables|/Game/Blueprints/New/BP_SequenceManager.BP_SequenceManager_C|SetCurrentSequence _returnvalue (Variables|Default|GetSequence))
  (Default|SetDataforWidget (Variables|/Game/Blueprints/New/Main/01CaveMain/01CM_PC.01CM_PC_C|GetGetItemWidget (Variables|/Game/Blueprints/Transfered/Blueprints1/ToTransfer/Camera_PC_test.Camera_PC_test_C|GetCurrentPlayerController (Variables|Default|GetPlayerPawn))) (.icon _inventoryitem) (Utilities|String|StringToName (.name _inventoryitem)))
  (switch name (.RowName (Utilities|Struct|BreakDataTableRowHandle (Variables|Default|GetWithSequence?)))
    (:Not
      (Game|Player|SetViewTargetwithBlend (Variables|/Game/Blueprints/Transfered/Blueprints1/ToTransfer/Camera_PC_test.Camera_PC_test_C|GetCurrentPlayerController (Variables|Default|GetPlayerPawn)) (Variables|Default|GetCameraInteractiveObj) 1.0 "VTBlend_Linear" 0.0 false :!label _label)
      (Audio|PlaySound2D "/Game/Audio/Snd/FX/CameraMoveFar.CameraMoveFar" 1.0 1.0 0.0 0 0)
      (Utilities|FlowControl|Delay 1.0)
      (CallFunction|Dialog/PickItem))
    (:Before
      (Default|ShowSequence (Variables|Default|GetSequenceManager) _self _self))
    (:After
      (goto _label))))

(event EventDialogEnded
  (params (CurrentDialogNum :type Integer))
  (bind _playerpawn (Variables|Default|GetPlayerPawn))
  (bind _currentplayercontroller (Variables|/Game/Blueprints/Transfered/Blueprints1/ToTransfer/Camera_PC_test.Camera_PC_test_C|GetCurrentPlayerController _playerpawn))
  (bind _maininterface_w (Variables|/Game/Blueprints/New/Main/01CaveMain/01CM_PC.01CM_PC_C|GetMainInterface_W _currentplayercontroller))
  (if (Variables|Default|GetDone?)
    (UserInterface|Animation|PlayAnimation _maininterface_w (Variables|/Game/Widgets/New/MainInterface_W.MainInterface_W_C|GetShowInterface _maininterface_w) 0.0 1 "Forward" 4.0 false)
    (else
      (Variables|Default|SetDone? true)
      (Default|PickItem (Variables|Default|GetPlayer) self (Variables|Default|GetActorToUseWith))
      (if (not (Utilities|Enum|Equal(Enum) (.type (Variables|Default|GetInventoryItem)) "NewEnumerator4"))
        (Default|AddItemtoInventory (Variables|Default|GetGameInstance) (Variables|Default|GetInventoryItem))))))

(fn ConstructionScript
  (|CallParentFunction))

(fn Dialog/PickItem
  (if (Variables|Default|GetIsWithDialog?)
    (Default|OpenDialog (Variables|Default|GetDialogActor) (Variables|Default|GetDialogToStart) self)
    (elif (not (Variables|Default|GetDone?))
      (Variables|Default|SetDone? true)
      (Default|PickItem (Variables|Default|GetPlayer) self (Variables|Default|GetActorToUseWith)))))