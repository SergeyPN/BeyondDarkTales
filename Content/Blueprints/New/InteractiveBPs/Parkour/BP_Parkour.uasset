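; BP_Parkour is an interactive parkour point that launches a jump or fall move on the player when used.
; It hides the prompt, walks the player to an arrow via AIMoveTo, aligns them, then branches on ParkourType.
; Jump Up plays a montage in Flying mode, then restores Walking.
; Other types pass settings to the player and enable Flying, except forward death jumps, which flag Max_Anim instead.
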(event EventBeginPlay
  (|CallParentFunction) ; This node is disabled and will not be called.\nDrag off pins to build functionality.
)

(event Collision|EventActorBeginOverlap
  (params (OtherActor :type Actor%20Object%20Reference))
  (|CallParentFunction OtherActor))

(event EventTick
  (params (DeltaSeconds :type Float%20%28single-precision%29))
  (|CallParentFunction DeltaSeconds))

(event EventInteractwithWidget
  (bind _arrow_0 (Variables|Default|GetArrow_0))
  (bind _arrow_0_2 (Variables|Default|GetArrow_0))
  (bind _arrow_0_3 (Variables|Default|GetArrow_0))
  (bind _returnvalue (Transformation|GetWorldLocation _arrow_0))
  (bind _returnvalue_2 (Transformation|GetWorldTransform _arrow_0_2))
  (bind _returnvalue_3 (Transformation|GetWorldTransform _arrow_0_3))
  (CallFunction|HideInteract)
  (AI|AIMoveTo (Variables|Default|GetPlayer) (Math|Vector|MakeVector (.x _returnvalue) (.y _returnvalue) (.z (Transformation|GetActorLocation (Variables|Default|GetPlayer)))) 0 1.0 false
    (:OnSuccess
      (Transformation|SetActorRotation (Variables|Default|GetPlayer) (Transformation|GetWorldRotation (Variables|Default|GetArrow_0)))
      (Default|StopMovement (Variables|Default|GetPlayer))
      (switch Utilities|FlowControl|Switch|SwitchonParkourTypes (Variables|Default|GetParkourType)
        (:NewEnumerator0
          (Variables|/Game/Assets/Heroes/Max/BP_CharMax.BP_CharMax_C|SetJumpHeight (Variables|Default|GetPlayer) (Variables|Default|GetPlusForJumpUp))
          (Variables|/Game/Assets/Heroes/Max/BP_CharMax.BP_CharMax_C|SetOnParcour (Variables|Default|GetPlayer) true)
          (Pawn|Components|CharacterMovement|SetMovementMode (Variables|/Script/Engine.Character|GetCharacterMovement (Variables|Default|GetPlayer)) "MOVE_Flying" 0)
          (Animation|Montage|PlayMontage (Variables|/Script/Engine.Character|GetMesh (Variables|Default|GetPlayer)) "/Game/Assets/Heroes/Max/Anim/JumpMidUp_Montage.JumpMidUp_Montage"
            (:OnCompleted
              (Pawn|Components|CharacterMovement|SetMovementMode (Variables|/Script/Engine.Character|GetCharacterMovement (Variables|Default|GetPlayer)) "MOVE_Walking" 0)
              (Variables|/Game/Assets/Heroes/Max/BP_CharMax.BP_CharMax_C|SetOnParcour (Variables|Default|GetPlayer) false))))
        (:NewEnumerator5
          (Variables|/Game/Assets/Heroes/Max/BP_CharMax.BP_CharMax_C|SetPowerOfJumpForward (Variables|Default|GetPlayer) (Variables|Default|GetMultiplyForJumpForward))
          (Variables|/Game/Assets/Heroes/Max/BP_CharMax.BP_CharMax_C|SetParkourTypeEnum (Variables|Default|GetPlayer) "NewEnumerator5")
          (Transformation|SetActorTransform (Variables|Default|GetPlayer) (Math|Transform|MakeTransform (Math|Vector|MakeVector (.x (.location _returnvalue_3)) (.y (.location _returnvalue_3)) (.z (Transformation|GetActorLocation (Variables|Default|GetPlayer)))) (.rotation _returnvalue_3) "1,1,1") :!label _label)
          (Variables|/Game/Assets/Heroes/Max/BP_CharMax.BP_CharMax_C|SetOnParcour (Variables|Default|GetPlayer) true)
          (if (Variables|Default|GetDeathJump)
            (bind _asmax_anim (Utilities|Casting|CastToMax_Anim (Components|SkeletalMesh|GetAnimInstance (Variables|/Script/Engine.Character|GetMesh (Variables|Default|GetPlayer)))))
            (Variables|/Game/Assets/Heroes/Max/Anim/Max_Anim.Max_Anim_C|SetDeathJump _asmax_anim (Variables|Default|GetDeathJump))
            (else
              (Pawn|Components|CharacterMovement|SetMovementMode (Variables|/Script/Engine.Character|GetCharacterMovement (Variables|Default|GetPlayer)) "MOVE_Flying" 0))))
        (:NewEnumerator4
          (Variables|/Game/Assets/Heroes/Max/BP_CharMax.BP_CharMax_C|SetPowerOfJumpForward (Variables|Default|GetPlayer) (Variables|Default|GetMultiplyForJumpForward))
          (Variables|/Game/Assets/Heroes/Max/BP_CharMax.BP_CharMax_C|SetParkourTypeEnum (Variables|Default|GetPlayer) "NewEnumerator4")
          (goto _label))
        (:NewEnumerator8
          (Variables|/Game/Assets/Heroes/Max/BP_CharMax.BP_CharMax_C|SetPowerOfJumpForward (Variables|Default|GetPlayer) (Variables|Default|GetMultiplyForJumpForward))
          (Variables|/Game/Assets/Heroes/Max/BP_CharMax.BP_CharMax_C|SetParkourTypeEnum (Variables|Default|GetPlayer) "NewEnumerator8")
          (goto _label))
        (:NewEnumerator7
          (Variables|/Game/Assets/Heroes/Max/BP_CharMax.BP_CharMax_C|SetParkourTypeEnum (Variables|Default|GetPlayer) "NewEnumerator7")
          (Transformation|SetActorTransform (Variables|Default|GetPlayer) (Math|Transform|MakeTransform (Math|Vector|MakeVector (.x (.location _returnvalue_2)) (.y (.location _returnvalue_2)) (.z (Transformation|GetActorLocation (Variables|Default|GetPlayer)))) (.rotation _returnvalue_2) "1,1,1"))
          (Variables|/Game/Assets/Heroes/Max/BP_CharMax.BP_CharMax_C|SetOnParcour (Variables|Default|GetPlayer) true)
          (Pawn|Components|CharacterMovement|SetMovementMode (Variables|/Script/Engine.Character|GetCharacterMovement (Variables|Default|GetPlayer)) "MOVE_Flying" 0))))))

(fn ConstructionScript
  (|CallParentFunction))