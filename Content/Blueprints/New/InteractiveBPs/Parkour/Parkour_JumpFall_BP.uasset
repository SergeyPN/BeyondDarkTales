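; Interactive parkour point that sets the player up for a jump-fall move when they use its interact widget.
; It hides the prompt and AI-moves the player to Arrow0's horizontal position, keeping the player's own height.
; On success it snaps the player to the arrow's position and rotation, sets the jump type, flags parkour as active and switches movement to Flying.
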(event EventBeginPlay
  (|CallParentFunction))

(event Collision|EventActorBeginOverlap
  (params (OtherActor :type Actor%20Object%20Reference))
  (|CallParentFunction OtherActor))

(event EventTick
  (params (DeltaSeconds :type Float%20%28single-precision%29))
  (|CallParentFunction DeltaSeconds))

(event EventInteractwithWidget
  (bind _arrow_0 (Variables|Default|GetArrow_0))
  (bind _arrow_0_2 (Variables|Default|GetArrow_0))
  (bind _returnvalue (Transformation|GetWorldLocation _arrow_0))
  (bind _returnvalue_2 (Transformation|GetWorldTransform _arrow_0_2))
  (CallFunction|HideInteract)
  (AI|AIMoveTo (Variables|Default|GetPlayer) (Math|Vector|MakeVector (.x _returnvalue) (.y _returnvalue) (.z (Transformation|GetActorLocation (Variables|Default|GetPlayer)))) 0 1.0 false
    (:OnSuccess
      (Transformation|SetActorRotation (Variables|Default|GetPlayer) (Transformation|GetWorldRotation (Variables|Default|GetArrow_0)))
      (Variables|/Game/Assets/Heroes/Max/BP_CharMax.BP_CharMax_C|SetJumpTypeEnum (Variables|Default|GetPlayer) "NewEnumerator1")
      (Transformation|SetActorTransform (Variables|Default|GetPlayer) (Math|Transform|MakeTransform (Math|Vector|MakeVector (.x (.location _returnvalue_2)) (.y (.location _returnvalue_2)) (.z (Transformation|GetActorLocation (Variables|Default|GetPlayer)))) (.rotation _returnvalue_2) "1,1,1"))
      (Variables|/Game/Assets/Heroes/Max/BP_CharMax.BP_CharMax_C|SetOnParcour (Variables|Default|GetPlayer) true)
      (Pawn|Components|CharacterMovement|SetMovementMode (Variables|/Script/Engine.Character|GetCharacterMovement (Variables|Default|GetPlayer)) "MOVE_Flying" 0))))

(fn ConstructionScript
  (|CallParentFunction))