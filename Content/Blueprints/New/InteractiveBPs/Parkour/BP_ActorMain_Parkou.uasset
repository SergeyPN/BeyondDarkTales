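; Interactable parkour actor that makes the player perform a jump-up montage from a fixed start point.
; On widget interaction it hides the prompt and uses AI MoveTo to walk the player to Arrow0, keeping the player's height.
; On arrival it matches the arrow's rotation, sets OnParcour and switches movement to Flying for the montage.
; When the montage completes, it restores Walking and clears the flag.
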(event EventBeginPlay
  (|CallParentFunction) ; This node is disabled and will not be called.\nDrag off pins to build functionality.
)

(event Collision|EventActorBeginOverlap
  (params (OtherActor :type Actor%20Object%20Reference))
  (|CallParentFunction OtherActor))

(event EventTick
  (params (DeltaSeconds :type Float%20%28single-precision%29))
  (|CallParentFunction DeltaSeconds))

(event EventInteractwithWidget
  (bind _arrow_0 (Variables|Default|GetArrow_0))
  (bind _returnvalue (Transformation|GetWorldLocation _arrow_0))
  (CallFunction|HideInteract)
  (AI|AIMoveTo (Variables|Default|GetPlayer) (Math|Vector|MakeVector (.x _returnvalue) (.y _returnvalue) (.z (Transformation|GetActorLocation (Variables|Default|GetPlayer)))) 0 1.0 false
    (:OnSuccess
      (Transformation|SetActorRotation (Variables|Default|GetPlayer) (Transformation|GetWorldRotation (Variables|Default|GetArrow_0)))
      (Variables|/Game/Assets/Heroes/Max/BP_CharMax.BP_CharMax_C|SetOnParcour (Variables|Default|GetPlayer) true)
      (Pawn|Components|CharacterMovement|SetMovementMode (Variables|/Script/Engine.Character|GetCharacterMovement (Variables|Default|GetPlayer)) "MOVE_Flying" 0)
      (Animation|Montage|PlayMontage (Variables|/Script/Engine.Character|GetMesh (Variables|Default|GetPlayer)) "/Game/Assets/Heroes/Max/Anim/JumpMidUp_Montage.JumpMidUp_Montage"
        (:OnCompleted
          (Pawn|Components|CharacterMovement|SetMovementMode (Variables|/Script/Engine.Character|GetCharacterMovement (Variables|Default|GetPlayer)) "MOVE_Walking" 0)
          (Variables|/Game/Assets/Heroes/Max/BP_CharMax.BP_CharMax_C|SetOnParcour (Variables|Default|GetPlayer) false))))))

(fn ConstructionScript
  (|CallParentFunction))