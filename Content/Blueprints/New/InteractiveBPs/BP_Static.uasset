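; BP_Static is an interactive object that, when used, opens dialog or triggers linked actors.
; Interaction disables player input, hides the HUD and optionally blends to an object camera.
; It cycles through dialog keys, also advancing other BP_Static instances whose current key matches.
; When dialog ends, it triggers actors, disables or re-shows itself, then either starts a sequence or restores HUD, level camera and input.
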(event Custom|EnableInteractWidget
  (CallFunction|Enable/DisableActor true)
  (CallFunction|ShowInteract))

(event EventBeginPlay
  (|CallParentFunction)
  (if (!= (Variables|Default|GetLevelCameraIndex) 0)
    (bind _outactors (Actor|GetAllActorsOfClass "/Game/Blueprints/New/LevelCamera.LevelCamera_C"))
    (bind _array_element (Utilities|Array|ForEachLoopwithBreak _outactors :!label _label)
      (:LoopBody
        (if (== (Variables|/Game/Blueprints/New/LevelCamera.LevelCamera_C|GetCameraIndex _array_element) (Variables|Default|GetLevelCameraIndex))
          (Variables|Default|SetLevelCamera _array_element)
          (goto _label Break))))))

(event Collision|EventActorBeginOverlap
  (params (OtherActor :type Actor%20Object%20Reference))
  (|CallParentFunction OtherActor) ; This node is disabled and will not be called.\nDrag off pins to build functionality.
)

(event EventTick
  (params (DeltaSeconds :type Float%20%28single-precision%29))
  (|CallParentFunction DeltaSeconds) ; This node is disabled and will not be called.\nDrag off pins to build functionality.
)

(event EventInteractwithWidget
  (bind _playerpawn (Variables|Default|GetPlayerPawn))
  (bind _playerpawn_2 (Variables|Default|GetPlayerPawn))
  (bind _currentplayercontroller (Variables|/Game/Blueprints/CameraControl/Camera_PC_test.Camera_PC_test_C|GetCurrentPlayerController _playerpawn))
  (bind _currentplayercontroller_2 (Variables|/Game/Blueprints/CameraControl/Camera_PC_test.Camera_PC_test_C|GetCurrentPlayerController _playerpawn_2))
  (bind _maininterface_w (Variables|/Game/Blueprints/New/Main/01CaveMain/01CM_PC.01CM_PC_C|GetMainInterface_W _currentplayercontroller))
  (bind _maininterface_w_2 (Variables|/Game/Blueprints/New/Main/01CaveMain/01CM_PC.01CM_PC_C|GetMainInterface_W _currentplayercontroller_2))
  (Input|DisableInput (Game|Player|GetPlayerPawn 0) (Game|GetPlayerController 0))
  (CallFunction|HideInteract false)
  (Utilities|MaxHavingBackpack
    (:true
      (UserInterface|Animation|PlayAnimation _maininterface_w (Variables|/Game/Widgets/New/MainInterface_W.MainInterface_W_C|GetShowInterface _maininterface_w) 0.0 1 "Reverse" 4.0 false))
    (:false
      (UserInterface|Animation|PlayAnimation _maininterface_w_2 (Variables|/Game/Widgets/New/MainInterface_W.MainInterface_W_C|GetShowInterfaceWithoutBackPack _maininterface_w_2) 0.0 1 "Reverse" 4.0 false)))
  (Utilities|IsValid (Variables|Default|GetCameraInteractiveObj)
    (:Is%20Valid
      (Game|Player|SetViewTargetwithBlend (Variables|/Game/Blueprints/CameraControl/Camera_PC_test.Camera_PC_test_C|GetCurrentPlayerController (Variables|Default|GetPlayerPawn)) (Variables|Default|GetCameraInteractiveObj) 1.0 "VTBlend_Linear" 0.0 false)
      (Audio|PlaySound2D "/Game/Audio/NEW_SOUNDS/SFX/fx_camera_move_far.fx_camera_move_far" 1.0 1.0 0.0 0 0)
      (Utilities|FlowControl|Delay 1.0))
    (:Is%20Not%20Valid
      _))
  (if (Variables|Default|GetIsWithDialog?)
    (if (> (Utilities|Array|Length (Variables|Default|GetDialogToStart)) 0)
      (Default|OpenDialog (Variables|Default|GetDialogActor) (Utilities|Array|Get(acopy) (Variables|Default|GetDialogToStart) (Variables|Default|GetCurrentNumDialogToStart)) self)
      (bind _outactors (Actor|GetAllActorsOfClass "BP_Static_C"))
      (for _array_element _outactors
        (if (not (== _array_element self))
          (if (== (Utilities|Array|Get(acopy) (Variables|/Game/Blueprints/New/InteractiveBPs/BP_ActorMain.BP_ActorMain_C|GetDialogToStart _array_element) (Variables|/Game/Blueprints/New/InteractiveBPs/BP_ActorMain.BP_ActorMain_C|GetCurrentNumDialogToStart _array_element)) (Utilities|Array|Get(acopy) (Variables|Default|GetDialogToStart) (Variables|Default|GetCurrentNumDialogToStart)))
            (if (== (Variables|/Game/Blueprints/New/InteractiveBPs/BP_ActorMain.BP_ActorMain_C|GetCurrentNumDialogToStart _array_element) (- (Utilities|Array|Length (Variables|/Game/Blueprints/New/InteractiveBPs/BP_ActorMain.BP_ActorMain_C|GetDialogToStart _array_element)) 1))
              (Variables|/Game/Blueprints/New/InteractiveBPs/BP_ActorMain.BP_ActorMain_C|SetCurrentNumDialogToStart _array_element 0)
              (else
                (Math|Integer|IncrementInt (Variables|/Game/Blueprints/New/InteractiveBPs/BP_ActorMain.BP_ActorMain_C|GetCurrentNumDialogToStart _array_element)))))))
      (if (== (Variables|Default|GetCurrentNumDialogToStart) (- (Utilities|Array|Length (Variables|Default|GetDialogToStart)) 1))
        (Variables|Default|SetCurrentNumDialogToStart 0)
        (else
          (Math|Integer|IncrementInt (Variables|Default|GetCurrentNumDialogToStart))))
      (else
        (Default|OpenDialog (Variables|Default|GetDialogActor) (Utilities|Array|Get(acopy) (Variables|Default|GetDialogToStart)) self)))
    (else
      (CallFunction|TriggerActors))))

(event EventDialogEnded
  (params (CurrentDialogNum :type Integer))
  (bind _playerpawn (Variables|Default|GetPlayerPawn))
  (bind _actorforinteraction (Variables|Default|GetActorForInteraction))
  (bind _playerpawn_2 (Variables|Default|GetPlayerPawn))
  (bind _currentplayercontroller (Variables|/Game/Blueprints/CameraControl/Camera_PC_test.Camera_PC_test_C|GetCurrentPlayerController _playerpawn))
  (bind _currentplayercontroller_2 (Variables|/Game/Blueprints/CameraControl/Camera_PC_test.Camera_PC_test_C|GetCurrentPlayerController _playerpawn_2))
  (bind _maininterface_w (Variables|/Game/Blueprints/New/Main/01CaveMain/01CM_PC.01CM_PC_C|GetMainInterface_W _currentplayercontroller))
  (bind _maininterface_w_2 (Variables|/Game/Blueprints/New/Main/01CaveMain/01CM_PC.01CM_PC_C|GetMainInterface_W _currentplayercontroller_2))
  (CallFunction|TriggerActors)
  (if (Variables|Default|GetDisableAfterInteract?)
    (CallFunction|Enable/DisableActor false)
    (else
      (Variables|Default|SetAfterStreamLevelInteraction true)
      (CallFunction|ShowInteract)))
  (if (Utilities|Name|Equal(Name) (.RowName (Utilities|Struct|BreakDataTableRowHandle (Variables|Default|GetWithSequence?))) "After")
    (Utilities|FlowControl|Delay 1.5)
    (Default|ShowSequence (Variables|Default|GetSequenceManager) self self 0 true)
    (else
      (Utilities|MaxHavingBackpack
        (:true
          (UserInterface|Animation|PlayAnimation _maininterface_w_2 (Variables|/Game/Widgets/New/MainInterface_W.MainInterface_W_C|GetShowInterface _maininterface_w_2) 0.0 1 "Forward" 4.0 false))
        (:false
          (UserInterface|Animation|PlayAnimation _maininterface_w (Variables|/Game/Widgets/New/MainInterface_W.MainInterface_W_C|GetShowInterfaceWithoutBackPack _maininterface_w) 0.0 1 "Forward" 4.0 false)))
      (Utilities|FlowControl|Sequence
        (:then_0
          (Utilities|IsValid (Variables|Default|GetCameraInteractiveObj)
            (:Is%20Valid
              (Game|Player|SetViewTargetwithBlend (Game|GetPlayerController 0) (Variables|Default|GetLevelCamera) 1.0 "VTBlend_Linear" 0.0 false)
              (Audio|PlaySound2D "/Game/Audio/NEW_SOUNDS/SFX/fx_camera_move_close.fx_camera_move_close" 1.0 1.0 0.0 0 0)
              (bind _asbp_char_princess (Utilities|Casting|CastToBP_CharPrincess (.actorforinteraction _actorforinteraction)))
              (Class|BPIInteractive|InteractwithObject(Message) _asbp_char_princess (.changedialogforhim _actorforinteraction) (Variables|Default|GetMoveTo)))))
        (:then_1
          (Utilities|FlowControl|Delay 1.0)
          (Input|EnableInput (Game|Player|GetPlayerPawn 0) (Game|GetPlayerController 0)))))))

(fn ConstructionScript
  (|CallParentFunction))