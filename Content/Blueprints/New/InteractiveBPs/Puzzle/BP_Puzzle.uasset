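; Interactable puzzle actor that takes the player into a puzzle sublevel and plays a sequence once it is solved.
; Interacting disables the actor, fades the screen, switches to the puzzle camera from LevelCameraAndDoorManager and makes the streaming level visible.
; When the level is shown, it binds completion on every BP_PuzzleCell.
; Completion or Return hides the level and restores camera and interface; Return also re-enables interaction.
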(event Custom|LoadedPuzzleLevel
  (bind _maininterfacewidget (CallFunction|GetMainInterfaceWidget))
  (bind _outactors (Actor|GetAllActorsOfClass "/Game/Blueprints/New/InteractiveBPs/OtherActors/Puzzle/BP_PuzzleCell.BP_PuzzleCell_C"))
  (for _array_element _outactors
    (EventDispatchers|BindEventtoCompletePuzzle _array_element (delegate Custom|CompletePuzzle)))
  (CameraFades|StartCameraFade :self (Variables|/Script/Engine.PlayerController|GetPlayerCameraManager (Game|GetPlayerController 0)) :FromAlpha 1.0 :Duration 1.0 :bHoldWhenFinished true)
  (UserInterface|Animation|PlayAnimation _maininterfacewidget (Variables|/Game/Widgets/New/MainInterface_W.MainInterface_W_C|GetShowButtonCloseAndResetPuzzle _maininterfacewidget) 0.0 1 "Forward" 4.0 false))

(event Custom|Return
  (Utilities|ReturnCameraandInterface)
  (Variables|Default|SetDisableAfterInteract? false)
  (CallFunction|Enable/DisableActor true)
  (CallFunction|ShowInteract))

(event Custom|CompletePuzzle
  (Utilities|ReturnCameraandInterface)
  (Sequencer|Player|Play (Variables|/Script/LevelSequence.LevelSequenceActor|GetSequencePlayer (Variables|Default|GetSequence)) :!class /Script/MovieScene.MovieSceneSequencePlayer))

(event EventBeginPlay
  (|CallParentFunction) ; This node is disabled and will not be called.\nDrag off pins to build functionality.
)

(event EventInteractwithWidget
  (bind _maininterfacewidget (CallFunction|GetMainInterfaceWidget))
  (bind _streaminglvl (Variables|Default|GetStreamingLvl))
  (bind _returnvalue (Class|GameplayStatics|GetStreamingLevel _streaminglvl))
  (Variables|/Game/Blueprints/New/InteractiveBPs/BP_ActorMain.BP_ActorMain_C|SetDisableAfterInteract? self true)
  (CallFunction|HideInteract false)
  (CallFunction|Enable/DisableActor false)
  (Variables|/Game/Widgets/New/MainInterface_W.MainInterface_W_C|SetInteractActor (CallFunction|GetMainInterfaceWidget) self)
  (CameraFades|StartCameraFade :self (Variables|/Script/Engine.PlayerController|GetPlayerCameraManager (Game|GetPlayerController 0)) :ToAlpha 1.0 :Duration 1.0 :bHoldWhenFinished true)
  (UserInterface|Animation|PlayAnimation _maininterfacewidget (Variables|/Game/Widgets/New/MainInterface_W.MainInterface_W_C|GetShowInterfaceWithPause _maininterfacewidget) 0.0 1 "Reverse" 4.0 false)
  (Utilities|FlowControl|Delay 1.0)
  (bind _returnvalue_2 (Actor|GetActorOfClass "/Game/Blueprints/New/LevelCameraAndDoorManager.LevelCameraAndDoorManager_C"))
  (bind _cameratoswitchlocal1 (Default|GetCamera _returnvalue_2 (Variables|Default|GetLoadNumLevelCamera)))
  (Game|Player|SetViewTargetwithBlend (Game|GetPlayerController 0) _cameratoswitchlocal1 0.0 "VTBlend_Linear" 0.0 false)
  (Variables|/Script/Engine.LevelStreaming|SetbShouldBeVisible _returnvalue true)
  (EventDispatchers|BindEventtoOnLevelShown _returnvalue (delegate Custom|LoadedPuzzleLevel)))

(fn ConstructionScript
  (|CallParentFunction))