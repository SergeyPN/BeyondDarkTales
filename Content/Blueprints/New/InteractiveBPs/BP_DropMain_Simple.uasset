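; BP_DropMain_Simple is an interactive object where the player uses the inventory on a world-space drop widget, placed at a hidden linked actor.
; Interaction disables pawn input, optionally runs dialog, then blends to the object's camera and opens inventory and drop UI.
; DropEnded restores buttons and starts a SequenceManager sequence.
; DialogEnded, branching on Done, either opens the drop or restores control and saves any higher checkpoint.
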(event Custom|OpenDrop
  (if (Utilities|Enum|Equal(Enum) (Widget|GetVisibility (Variables|/Game/Widgets/New/MainInterface_W.MainInterface_W_C|GetWB_Inventory (CallFunction|GetMainInterfaceWidget))) "Collapsed")
    (Default|PushButtonInventory (CallFunction|GetMainInterfaceWidget)))
  (Variables|/Game/Widgets/New/MainInterface_W.MainInterface_W_C|SetDropActor (CallFunction|GetMainInterfaceWidget) self)
  (bind _asw_drop (Utilities|Casting|CastToW_Drop (UserInterface|GetUserWidgetObject (Variables|Default|GetWidgetDrop))))
  (bind _output_get (Variables|/Game/Widgets/New/MainInterface_W.MainInterface_W_C|SetW_Drop (CallFunction|GetMainInterfaceWidget) _asw_drop))
  (Class|BPInteractive|UpdIconWidget(Message) _output_get (Variables|Default|GetDropWStart) "" 0 0 0 0 false 0 0 false "" false 0 "NewEnumerator3" "NewEnumerator0" self))

(event Custom|BeginDrop
  (bind _maininterfacewidget (CallFunction|GetMainInterfaceWidget))
  (bind _maininterfacewidget_2 (CallFunction|GetMainInterfaceWidget))
  (UserInterface|Animation|PlayAnimation _maininterfacewidget_2 (Variables|/Game/Widgets/New/MainInterface_W.MainInterface_W_C|GetShowPauseButton _maininterfacewidget_2) 0.0 1 "Reverse" 4.0 false)
  (UserInterface|Animation|PlayAnimation _maininterfacewidget (Variables|/Game/Widgets/New/MainInterface_W.MainInterface_W_C|GetShowButtonCloseDropAndInventory _maininterfacewidget) 0.0 1 "Forward" 4.0 false)
  (Game|Player|SetViewTargetwithBlend (Game|GetPlayerController 0) (Variables|Default|GetCameraInteractiveObj) 1.0 "VTBlend_Linear" 0.0 false)
  (Utilities|FlowControl|Delay 1.0)
  (CallFunction|OpenDrop))

(event Custom|FinishLeftButtonAnim
  (bind _maininterfacewidget (CallFunction|GetMainInterfaceWidget))
  (bind _maininterfacewidget_2 (CallFunction|GetMainInterfaceWidget))
  (bind _self self)
  (Class|UserWidget|UnbindfromAnimationFinished _maininterfacewidget_2 (Variables|/Game/Widgets/New/MainInterface_W.MainInterface_W_C|GetShowLeftDownButtons _maininterfacewidget_2) (delegate Custom|FinishLeftButtonAnim))
  (UserInterface|Animation|PlayAnimation _maininterfacewidget (Variables|/Game/Widgets/New/MainInterface_W.MainInterface_W_C|GetShowInterface _maininterfacewidget) 0.0 1 "Reverse" 4.0 false)
  (Default|ShowSequence (Variables|Default|GetSequenceManager) _self _self))

(event EventBeginPlay
  (|CallParentFunction))

(event Collision|EventActorBeginOverlap
  (params (OtherActor :type Actor%20Object%20Reference))
  (|CallParentFunction OtherActor) ; This node is disabled and will not be called.\nDrag off pins to build functionality.
)

(event EventTick
  (params (DeltaSeconds :type Float%20%28single-precision%29))
  (|CallParentFunction DeltaSeconds) ; This node is disabled and will not be called.\nDrag off pins to build functionality.
)

(event EventInteractwithWidget
  (bind _returnvalue (Game|GetPlayerController 0))
  (bind _playerpawn (Variables|Default|GetPlayerPawn))
  (bind _currentplayercontroller (Variables|/Game/Blueprints/Transfered/Blueprints1/ToTransfer/CameraControl/Camera_PC_test.Camera_PC_test_C|GetCurrentPlayerController _playerpawn))
  (bind _maininterface_w (Variables|/Game/Blueprints/New/Main/01CaveMain/01CM_PC.01CM_PC_C|GetMainInterface_W _currentplayercontroller))
  (Input|DisableInput (Game|Player|GetPlayerPawn 0) (Game|GetPlayerController 0))
  (CallFunction|HideInteract)
  (Input|DisableInput (Pawn|GetControlledPawn _returnvalue) _returnvalue)
  (UserInterface|Animation|PlayAnimation _maininterface_w (Variables|/Game/Widgets/New/MainInterface_W.MainInterface_W_C|GetShowInterface _maininterface_w) 0.0 1 "Reverse" 4.0 false)
  (if (Variables|Default|GetIsWithDialog?)
    (Default|OpenDialog (Variables|Default|GetDialogActor) (Utilities|Array|Get(acopy) (Variables|Default|GetDialogToStart)) self)
    (elif (not (Variables|Default|GetDone?))
      (Variables|Default|SetDone? true)
      (CallFunction|BeginDrop))))

(event EventDialogEnded
  (params (CurrentDialogNum :type Integer))
  (bind _maininterfacewidget (CallFunction|GetMainInterfaceWidget))
  (bind _maininterfacewidget_2 (CallFunction|GetMainInterfaceWidget))
  (bind _returnvalue (Game|GetPlayerController 0))
  (bind _gameinstance (Variables|Default|GetGameInstance))
  (bind _gameinstance_2 (Variables|Default|GetGameInstance))
  (bind _gameinstance_3 (Variables|Default|GetGameInstance))
  (bind _gameinstance_4 (Variables|Default|GetGameInstance))
  (bind _season (Variables|/Game/Blueprints/Transfered/Blueprints1/MyGameInstance.MyGameInstance_C|GetSeason _gameinstance))
  (bind _currentnumseason (Variables|/Game/Blueprints/Transfered/Blueprints1/MyGameInstance.MyGameInstance_C|GetCurrentNumSeason _gameinstance))
  (bind _currentnumact (Variables|/Game/Blueprints/Transfered/Blueprints1/MyGameInstance.MyGameInstance_C|GetCurrentNumAct _gameinstance))
  (bind _savegame (Variables|/Game/Blueprints/Transfered/Blueprints1/MyGameInstance.MyGameInstance_C|GetSaveGame _gameinstance_2))
  (bind _currentnumseason_2 (Variables|/Game/Blueprints/Transfered/Blueprints1/MyGameInstance.MyGameInstance_C|GetCurrentNumSeason _gameinstance_4))
  (bind _currentnumact_2 (Variables|/Game/Blueprints/Transfered/Blueprints1/MyGameInstance.MyGameInstance_C|GetCurrentNumAct _gameinstance_4))
  (bind _output (Utilities|Array|Get(acopy) _season _currentnumseason))
  (bind _season_2 (Variables|/Game/Blueprints/SaveGame/BP_SaveGame.BP_SaveGame_C|GetSeason _savegame))
  (bind _acts (Utilities|Struct|BreakStruct_Season _output))
  (bind _output_2 (Utilities|Array|Get(acopy) _season_2 _currentnumseason_2))
  (bind _acts_2 (Utilities|Struct|BreakStruct_Season _output_2))
  (bind _output_3 (Utilities|Array|Get(acopy) _acts _currentnumact))
  (bind (_access_ _counttrisigns) (Utilities|Struct|BreakStruct_Act _output_3))
  (bind _output_4 (Utilities|Array|Get(acopy) _acts_2 _currentnumact_2))
  (bind (_access__2 _counttrisigns_2) (Utilities|Struct|BreakStruct_Act _output_4))
  (if (Variables|Default|GetDone?)
    (bind _foundwidgets (Widget|GetAllWidgetsOfClass "/Game/Widgets/New/MainInterface_W.MainInterface_W_C" true))
    (UserInterface|Animation|PlayAnimation (Utilities|Array|Get(acopy) _foundwidgets) (Variables|/Game/Widgets/New/MainInterface_W.MainInterface_W_C|GetShowInterface (Utilities|Array|Get(acopy) _foundwidgets)) 0.0 1 "Forward" 4.0 false)
    (Utilities|FlowControl|Delay 1.0)
    (Input|EnableInput (Pawn|GetControlledPawn _returnvalue) _returnvalue)
    (if (and (!= (Variables|Default|GetNumAccessCheckPoint) 0) (> (Variables|Default|GetNumAccessCheckPoint) (.CountAccessChekpoints (Utilities|Struct|BreakStruct_Act (Utilities|Array|Get(acopy) (.Acts (Utilities|Struct|BreakStruct_Season (Utilities|Array|Get(acopy) (Variables|/Game/Blueprints/Transfered/Blueprints1/MyGameInstance.MyGameInstance_C|GetSeason _gameinstance_3) (Variables|/Game/Blueprints/Transfered/Blueprints1/MyGameInstance.MyGameInstance_C|GetCurrentNumSeason _gameinstance_3)))) (Variables|/Game/Blueprints/Transfered/Blueprints1/MyGameInstance.MyGameInstance_C|GetCurrentNumAct _gameinstance_3))))))
      ;[1 1 1] Save CheckPoint
      (Default|SavingGifon (Variables|/Game/Widgets/New/WBP_SavingGif.WBP_SavingGif_C|GetWBP_ImageSaving (Variables|/Game/Widgets/New/MainInterface_W.MainInterface_W_C|GetWBP_SavingGif (CallFunction|GetMainInterfaceWidget))))
      (Utilities|Array|SetArrayElem _acts (Variables|/Game/Blueprints/Transfered/Blueprints1/MyGameInstance.MyGameInstance_C|GetCurrentNumAct _gameinstance) (Utilities|Struct|MakeStruct_Act _access_ _counttrisigns (Variables|Default|GetNumAccessCheckPoint)))
      (Utilities|Array|SetArrayElem _acts_2 (Variables|/Game/Blueprints/Transfered/Blueprints1/MyGameInstance.MyGameInstance_C|GetCurrentNumAct _gameinstance_4) (Utilities|Struct|MakeStruct_Act _access__2 _counttrisigns_2 (Variables|Default|GetNumAccessCheckPoint)))
      (SaveGame|SaveGametoSlot (Variables|/Game/Blueprints/Transfered/Blueprints1/MyGameInstance.MyGameInstance_C|GetSaveGame (Variables|Default|GetGameInstance)) "1"))
    (else
      (Variables|Default|SetDone? true)
      (UserInterface|Animation|PlayAnimation _maininterfacewidget_2 (Variables|/Game/Widgets/New/MainInterface_W.MainInterface_W_C|GetShowPauseButton _maininterfacewidget_2) 0.0 1 "Reverse" 4.0 false)
      (UserInterface|Animation|PlayAnimation _maininterfacewidget (Variables|/Game/Widgets/New/MainInterface_W.MainInterface_W_C|GetShowButtonCloseDropAndInventory _maininterfacewidget) 0.0 1 "Forward" 4.0 false)
      (Game|Player|SetViewTargetwithBlend (Game|GetPlayerController 0) (Variables|Default|GetCameraInteractiveObj) 1.0 "VTBlend_Linear" 0.0 false)
      (Utilities|FlowControl|Delay 1.0)
      (CallFunction|OpenDrop))))

(event EventDropEnded
  (bind _maininterfacewidget (CallFunction|GetMainInterfaceWidget))
  (bind _maininterfacewidget_2 (CallFunction|GetMainInterfaceWidget))
  (UserInterface|Animation|PlayAnimation _maininterfacewidget (Variables|/Game/Widgets/New/MainInterface_W.MainInterface_W_C|GetShowPauseButton _maininterfacewidget) 0.0 1 "Forward" 4.0 false)
  (Class|UserWidget|BindtoAnimationFinished _maininterfacewidget_2 (Variables|/Game/Widgets/New/MainInterface_W.MainInterface_W_C|GetShowLeftDownButtons _maininterfacewidget_2) (delegate Custom|FinishLeftButtonAnim)))

(fn ConstructionScript
  (|CallParentFunction)
  (Rendering|SetActorHiddenInGame (Variables|Default|GetActorToUseWith) true)
  (Utilities|IsValid (Variables|Default|GetActorToUseWith)
    (:Is%20Valid
      (Transformation|SetWorldLocation (Variables|Default|GetWidgetDrop) (Transformation|GetActorLocation (Variables|Default|GetActorToUseWith)) false false))))