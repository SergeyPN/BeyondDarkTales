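; Cave floor brick trap that, when flagged as a killing brick, breaks under BP_CharMax and kills him.
; Overlap freezes character and input, then a timer swaps the whole brick for seven physics-simulated pieces.
; A timeline shrinks pieces and character mesh during the fall, then shows the death screen, passing itself along.
; NewAttempt restores pieces from construction-script transforms, resets character, camera and UI, and re-arms the trap, using hardcoded level positions.
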(event OnComponentBeginOverlap(Box)
  (params (OverlappedComponent :type Primitive%20Component%20Object%20Reference) (OtherActor :type Actor%20Object%20Reference) (OtherComp :type Primitive%20Component%20Object%20Reference) (OtherBodyIndex :type Integer) (bFromSweep :type Boolean) (SweepResult :type Hit%20Result%20Structure%20%28by%20ref%29))
  (if (Variables|Default|GetKillingBrick)
    (Utilities|FlowControl|Delay 0.5)
    (Utilities|FlowControl|DoOnce false
      (:Completed
        (bind _returnvalue (Utilities|Time|SetTimerbyEvent (delegate Custom|StopShake) 0.5))
        (Variables|Default|SetTimerShake _returnvalue)
        (bind _asbp_char_max (Utilities|Casting|CastToBP_CharMax OtherActor))
        (bind _output_get (Variables|Default|SetCharMax _asbp_char_max))
        (Default|StopMovement _output_get)
        (Pawn|Components|CharacterMovement|DisableMovement (Variables|/Script/Engine.Character|GetCharacterMovement _output_get))
        (Input|DisableInput (Game|Player|GetPlayerPawn 0) (Game|GetPlayerController 0))))))

(event Custom|StopShake
  (bind _maininterfacewidget (CallFunction|GetMainInterfaceWidget))
  (bind _cavebrickfloor_broken_part_1 (Variables|Default|GetCaveBrickFloor_Broken_Part_1))
  (bind _cavebrickfloor_broken_part_1_2 (Variables|Default|GetCaveBrickFloor_Broken_Part_1))
  (bind _asmax_anim (Utilities|Casting|CastToMax_Anim (Components|SkeletalMesh|GetAnimInstance (Variables|/Script/Engine.Character|GetMesh (Variables|Default|GetCharMax)))))
  (Variables|/Game/Assets/Heroes/Max/Anim/Max_Anim.Max_Anim_C|SetDangerAndFalling _asmax_anim true)
  (Components|Activation|Activate (Variables|Default|GetP_DustBurst) false)
  (Utilities|Time|ClearandInvalidateTimerbyHandle (Variables|Default|GetTimerShake))
  (Development|SetHiddeninGame (Variables|Default|GetWholeBrick) true false)
  (Development|SetHiddeninGame (Variables|Default|GetCaveBrickFloor_Broken_Part_2) false false)
  (Utilities|FlowControl|Delay 0.5)
  (Collision|SetCollisionEnabled _cavebrickfloor_broken_part_1_2 "PhysicsOnly")
  (Physics|SetSimulatePhysics _cavebrickfloor_broken_part_1_2 true)
  (Pawn|Components|CharacterMovement|SetMovementMode (Variables|/Script/Engine.Character|GetCharacterMovement (Variables|Default|GetCharMax)) "MOVE_Walking" 0)
  (Collision|SetCollisionEnabled (Variables|Default|GetWholeBrick) "NoCollision")
  (bind (_direction _scale _scalebrick7 _scalebrick5) (Timeline|TimelineDecSize PlayFromStart)
    (:Update
      (Transformation|SetRelativeScale3D (Variables|Default|GetCaveBrickFloor_Broken_Part_2) _scale)
      (Transformation|SetRelativeScale3D (Variables|Default|GetCaveBrickFloor_Broken_Part_7) _scalebrick7)
      (Transformation|SetRelativeScale3D (Variables|Default|GetCaveBrickFloor_Broken_Part_5) _scalebrick5)
      (Transformation|SetRelativeScale3D (Variables|/Script/Engine.Character|GetMesh (Variables|Default|GetCharMax)) _scale))
    (:Finished
      (UserInterface|Animation|PlayAnimation _maininterfacewidget (Variables|/Game/Widgets/New/MainInterface_W.MainInterface_W_C|GetShowInterfaceWithPause _maininterfacewidget) 0.0 1 "Reverse" 4.0 false)
      (Utilities|FlowControl|Sequence
        (:then_0
          (Physics|SetSimulatePhysics _cavebrickfloor_broken_part_1 false)
          (Collision|SetCollisionEnabled _cavebrickfloor_broken_part_1 "NoCollision")
          (Transformation|SetActorTransform (Variables|Default|GetCharMax) (Math|Transform|MakeTransform "20.000000,150.000000,-820.000000" "0, 0, 0" "1,1,1")))
        (:then_1
          (bind _asbp_main_menu_hud (Utilities|Casting|CastToBP_MainMenuHUD (HUD|GetHUD (Game|GetPlayerController 0))))
          (UserInterface|Viewport|AddtoViewport (Variables|/Game/Blueprints/New/Main/MainMenu/BP_MainMenuHUD.BP_MainMenuHUD_C|GetDieScreenWidget _asbp_main_menu_hud) 3)
          (Variables|/Game/Widgets/DieScreen/WBP_DieScreen.WBP_DieScreen_C|SetActorCreatorWidget (Variables|/Game/Blueprints/New/Main/MainMenu/BP_MainMenuHUD.BP_MainMenuHUD_C|GetDieScreenWidget _asbp_main_menu_hud) self))))))

(event Custom|NewAttempt
  (bind _maininterfacewidget (CallFunction|GetMainInterfaceWidget))
  (CallFunction|HandleReset)
  (Utilities|FlowControl|Delay 2.0)
  (bind _ascamera_pc_test (Utilities|Casting|CastToCamera_PC_test (Game|Player|GetPlayerPawn 0)))
  (Transformation|SetActorTransform (Variables|/Game/Blueprints/Transfered/Blueprints1/ToTransfer/CameraControl/Camera_PC_test.Camera_PC_test_C|GetLevelCamera _ascamera_pc_test) (Math|Transform|MakeTransform "11964.000000,734.000000,393.000000" "-44.000000,-43.000000, 0" "1,1,1"))
  (bind _foundwidgets (Widget|GetAllWidgetsOfClass "/Game/Widgets/LoadingScreen/WB_LoadingScreen.WB_LoadingScreen_C" true))
  (Widget|RemovefromParent (Utilities|Array|Get(acopy) _foundwidgets))
  (CameraFades|StartCameraFade :self (Variables|/Script/Engine.PlayerController|GetPlayerCameraManager (Game|GetPlayerController 0)) :FromAlpha 1.0 :Duration 1.0)
  (UserInterface|Animation|PlayAnimation _maininterfacewidget (Variables|/Game/Widgets/New/MainInterface_W.MainInterface_W_C|GetShowInterfaceWithPause _maininterfacewidget) 0.0 1 "Forward" 4.0 false)
  (Utilities|FlowControl|Delay 1.5)
  (CallFunction|ResetBrick)
  (Input|EnableInput (Game|Player|GetPlayerPawn 0) (Game|GetPlayerController 0))
  (Variables|/Game/Widgets/DieScreen/WBP_DieScreen.WBP_DieScreen_C|SetDoOnce (Variables|/Game/Blueprints/New/Main/MainMenu/BP_MainMenuHUD.BP_MainMenuHUD_C|GetDieScreenWidget (.AsBP%20Main%20Menu%20HUD (Utilities|Casting|CastToBP_MainMenuHUD (HUD|GetHUD (Game|GetPlayerController 0))))) false))

(event Custom|ResetBrick
  (Utilities|FlowControl|DoOnce false) ; enters at Reset
)

(event EventTick
  (params (DeltaSeconds :type Float%20%28single-precision%29)))

(fn ConstructionScript
  (Variables|Default|SetStartTransform (Utilities|Array|MakeArray (Transformation|GetWorldTransform (Variables|Default|GetCaveBrickFloor_Broken_Part_1)) (Transformation|GetWorldTransform (Variables|Default|GetCaveBrickFloor_Broken_Part_2)) (Transformation|GetWorldTransform (Variables|Default|GetCaveBrickFloor_Broken_Part_4)) (Transformation|GetWorldTransform (Variables|Default|GetCaveBrickFloor_Broken_Part_6)) (Transformation|GetWorldTransform (Variables|Default|GetCaveBrickFloor_Broken_Part_5)) (Transformation|GetWorldTransform (Variables|Default|GetCaveBrickFloor_Broken_Part_3)) (Transformation|GetWorldTransform (Variables|Default|GetCaveBrickFloor_Broken_Part_7)))))

(fn HandleReset
  (bind _cavebrickfloor_broken_part_4 (Variables|Default|GetCaveBrickFloor_Broken_Part_4))
  (bind _cavebrickfloor_broken_part_6 (Variables|Default|GetCaveBrickFloor_Broken_Part_6))
  (bind _cavebrickfloor_broken_part_5 (Variables|Default|GetCaveBrickFloor_Broken_Part_5))
  (bind _cavebrickfloor_broken_part_3 (Variables|Default|GetCaveBrickFloor_Broken_Part_3))
  (bind _cavebrickfloor_broken_part_7 (Variables|Default|GetCaveBrickFloor_Broken_Part_7))
  (bind _cavebrickfloor_broken_part_2 (Variables|Default|GetCaveBrickFloor_Broken_Part_2))
  (bind _cavebrickfloor_broken_part_1 (Variables|Default|GetCaveBrickFloor_Broken_Part_1))
  ;[1 1 1] Return begin Brick
  (Transformation|SetActorTransform (Variables|Default|GetCharMax) (Math|Transform|MakeTransform "11850.000000,300.000000,-5.000000" "0, 0, 0" "1,1,1"))
  (Transformation|SetRelativeScale3D (Variables|/Script/Engine.Character|GetMesh (Variables|Default|GetCharMax)) "1.000000,1.000000,1.000000")
  (bind _asmax_anim (Utilities|Casting|CastToMax_Anim (Components|SkeletalMesh|GetAnimInstance (Variables|/Script/Engine.Character|GetMesh (Variables|Default|GetCharMax)))))
  (Variables|/Game/Assets/Heroes/Max/Anim/Max_Anim.Max_Anim_C|SetDangerAndFalling _asmax_anim false)
  (Collision|SetCollisionEnabled (Variables|Default|GetWholeBrick) "QueryAndPhysics")
  (Development|SetHiddeninGame (Variables|Default|GetWholeBrick) false false)
  (Utilities|FlowControl|Sequence
    (:then_0
      (Transformation|SetWorldTransform _cavebrickfloor_broken_part_1 (Utilities|Array|Get(acopy) (Variables|Default|GetStartTransform)) false false)
      (Development|SetHiddeninGame _cavebrickfloor_broken_part_1 true false))
    (:then_1
      (Transformation|SetWorldTransform _cavebrickfloor_broken_part_2 (Utilities|Array|Get(acopy) (Variables|Default|GetStartTransform) 1) false false)
      (Development|SetHiddeninGame _cavebrickfloor_broken_part_2 true false))
    (:then_2
      (Transformation|SetWorldTransform _cavebrickfloor_broken_part_4 (Utilities|Array|Get(acopy) (Variables|Default|GetStartTransform) 2) false false)
      (Development|SetHiddeninGame _cavebrickfloor_broken_part_4 true false))
    (:then_3
      (Transformation|SetWorldTransform _cavebrickfloor_broken_part_6 (Utilities|Array|Get(acopy) (Variables|Default|GetStartTransform) 3) false false)
      (Development|SetHiddeninGame _cavebrickfloor_broken_part_6 true false))
    (:then_4
      (Transformation|SetWorldTransform _cavebrickfloor_broken_part_5 (Utilities|Array|Get(acopy) (Variables|Default|GetStartTransform) 4) false false)
      (Development|SetHiddeninGame _cavebrickfloor_broken_part_5 true false))
    (:then_5
      (Transformation|SetWorldTransform _cavebrickfloor_broken_part_3 (Utilities|Array|Get(acopy) (Variables|Default|GetStartTransform) 5) false false)
      (Development|SetHiddeninGame _cavebrickfloor_broken_part_3 true false))
    (:then_6
      (Transformation|SetWorldTransform _cavebrickfloor_broken_part_7 (Utilities|Array|Get(acopy) (Variables|Default|GetStartTransform) 6) false false)
      (Development|SetHiddeninGame _cavebrickfloor_broken_part_7 true false))))