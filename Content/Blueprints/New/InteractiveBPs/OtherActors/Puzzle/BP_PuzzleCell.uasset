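; BP_PuzzleCell is a touch-activated cell in a lights-out style puzzle.
; A touch plays a sound and toggles the cell's lighting mesh visibility, then after a short delay toggles each cell in its RefPuzzleCell array.
; It then scans every BP_PuzzleCell in the level and calls CallCompletePuzzle when all are lit, using mesh visibility itself as the on/off state.
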(event EventBeginPlay)

(event Collision|EventActorBeginOverlap
  (params (OtherActor :type Actor%20Object%20Reference)))

(event EventTick
  (params (DeltaSeconds :type Float%20%28single-precision%29)))

(event EventActorOnInputTouchBegin
  (params (FingerIndex :type ETouchIndex%20Enum :default "Touch1"))
  (Audio|PlaySound2D "/Game/Audio/Snd/FX/Cues/WithoutLooping/Cue_Cells_TurnOn.Cue_Cells_TurnOn" 1.0 1.0 0.0 0 0)
  (if (Rendering|IsVisible (Variables|Default|GetLightingStaticMesh))
    (Rendering|SetVisibility (Variables|Default|GetLightingStaticMesh) false false)
    (else
      (Rendering|SetVisibility (Variables|Default|GetLightingStaticMesh) true false)))
  (Utilities|FlowControl|Delay 0.15)
  (for _array_element (Variables|Default|GetRefPuzzleCell)
    (if (Rendering|IsVisible (Variables|BP_PuzzleCell_C|GetLightingStaticMesh _array_element))
      (Rendering|SetVisibility (Variables|BP_PuzzleCell_C|GetLightingStaticMesh _array_element) false false)
      (else
        (Rendering|SetVisibility (Variables|BP_PuzzleCell_C|GetLightingStaticMesh _array_element) true false))))
  (Variables|Default|SetCompletePuzzle? true)
  (bind _outactors (Actor|GetAllActorsOfClass "BP_PuzzleCell_C"))
  (bind _array_element_2 (Utilities|Array|ForEachLoopwithBreak _outactors :!label _label)
    (:LoopBody
      (if (not (Rendering|IsVisible (Variables|BP_PuzzleCell_C|GetLightingStaticMesh _array_element_2)))
        (Variables|Default|SetCompletePuzzle? false)
        (goto _label Break)))
    (:Completed
      (if (Variables|Default|GetCompletePuzzle?)
        (Default|CallCompletePuzzle)))))

(fn ConstructionScript)