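; BP_LockActivator is a lock panel that lights up when its trigger box is overlapped and drives a gate sequence with sound.
; Default panels must light in NumPanelPriority order, checked across all instances: the last opens the gate, while a wrong order blinks lit panels off and resets them.
; "Not Stable" panels open immediately and enable linked BP_ActorMain actors, reversing both when the box empties while the tagged streaming level should be visible.
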(event OnComponentBeginOverlap(Box)
  (params (OverlappedComponent :type Primitive%20Component%20Object%20Reference) (OtherActor :type Actor%20Object%20Reference) (OtherComp :type Primitive%20Component%20Object%20Reference) (OtherBodyIndex :type Integer) (bFromSweep :type Boolean) (SweepResult :type Hit%20Result%20Structure%20%28by%20ref%29))
  (bind _numpanelpriority (Variables|Default|GetNumPanelPriority))
  (bind _sound (Variables|Default|GetSound))
  (Utilities|FlowControl|DoOnce false
    (:Completed
      (Utilities|IsValid _sound
        (:Is%20Valid
          (Audio|Components|Audio|Stop _sound))
        (:Is%20Not%20Valid
          _))
      (Rendering|SetVisibility (Variables|Default|GetLockActSign) true false)
      (Audio|PlaySound2D "/Game/Audio/NEW_SOUNDS/CUES/CuesFX/WithoutLooping/Cue_Cells_TurnOn.Cue_Cells_TurnOn" 1.0 1.0 0.0 0 0)
      (Components|Activation|Activate (Variables|Default|GetP_Correct) false)
      (switch name (.rowname (Variables|Default|GetTypeCell))
        (:Default
          (bind _outactors (Actor|GetAllActorsOfClass "BP_LockActivator_C"))
          (bind _array_element (Utilities|Array|ForEachLoopwithBreak _outactors :!label _label)
            (:LoopBody
              (if (== (- _numpanelpriority 1) (Variables|BP_LockActivator_C|GetNumPanelPriority _array_element))
                (if (Variables|/Script/Engine.SceneComponent|GetbVisible (Variables|BP_LockActivator_C|GetLockActSign _array_element))
                  (if (== (Utilities|Array|Length _outactors) _numpanelpriority)
                    (CallFunction|PlaySequence false)
                    (goto _label Break))
                  (else
                    (Utilities|FlowControl|Sequence
                      (:then_0
                        (bind _outactors_2 (Actor|GetAllActorsOfClass "BP_LockActivator_C"))
                        (for _array_element_2 _outactors_2
                          (if (Variables|/Script/Engine.SceneComponent|GetbVisible (Variables|BP_LockActivator_C|GetLockActSign _array_element_2))
                            (CallFunction|StartBlinking _array_element_2))))
                      (:then_1
                        (goto _label Break)))))))))
        (:NotStable
          (bind _asbp_drag_actor (Utilities|Casting|CastToBP_DragActor (Utilities|Array|Get(acopy) (Collision|GetOverlappingActors (Variables|Default|GetBox) "/Game/Blueprints/New/DraggableActors/BP_DragActor.BP_DragActor_C" :!class /Script/Engine.PrimitiveComponent)))
            (:then
              (Rendering|Material|SetScalarParameterValue (Variables|/Game/Blueprints/New/DraggableActors/BP_DragActor.BP_DragActor_C|GetDynMat _asbp_drag_actor) "SignOpacity" 1.0 :!class /Script/Engine.MaterialInstanceDynamic))
            (:CastFailed
              _))
          (CallFunction|PlaySequence false)
          (for _array_element_3 (Variables|Default|GetActivateActor)
            (bind _asbp_actor_main (Utilities|Casting|CastToBP_ActorMain _array_element_3))
            (Default|Enable/DisableActor _asbp_actor_main true)))))))

(event OnComponentEndOverlap(Box)
  (params (OverlappedComponent :type Primitive%20Component%20Object%20Reference) (OtherActor :type Actor%20Object%20Reference) (OtherComp :type Primitive%20Component%20Object%20Reference) (OtherBodyIndex :type Integer))
  (if (!= (Utilities|Array|Length (Variables|Actor|GetTags)) 0)
    (if (Variables|/Script/Engine.LevelStreaming|GetbShouldBeVisible (Class|GameplayStatics|GetStreamingLevel (Utilities|Array|Get(acopy) (Variables|Actor|GetTags))))
      (switch name (.rowname (Variables|Default|GetTypeCell))
        (:NotStable
          (if (<= (Utilities|Array|Length (Collision|GetOverlappingActors (Variables|Default|GetBox) "/Script/Engine.Actor" :!class /Script/Engine.PrimitiveComponent)) 0)
            (bind _asbp_drag_actor (Utilities|Casting|CastToBP_DragActor OtherActor)
              (:then
                (Rendering|Material|SetScalarParameterValue (Variables|/Game/Blueprints/New/DraggableActors/BP_DragActor.BP_DragActor_C|GetDynMat _asbp_drag_actor) "SignOpacity" 0.0 :!class /Script/Engine.MaterialInstanceDynamic))
              (:CastFailed
                _))
            (CallFunction|StartBlinking)
            (CallFunction|PlaySequence true)
            (for _array_element (Variables|Default|GetActivateActor)
              (bind _asbp_actor_main (Utilities|Casting|CastToBP_ActorMain _array_element))
              (Default|Enable/DisableActor _asbp_actor_main false))))))))

(event Custom|StartBlinking
  (bind _returnvalue (Utilities|Time|SetTimerbyEvent (delegate Custom|TogglePowerPanel) 0.08 true))
  (Variables|Default|SetTimerBlinking _returnvalue))

(event Custom|TogglePowerPanel
  (Math|Integer|IncrementInt (Variables|Default|GetCounterTimerPowerPanel)
    (:%20%20
      (Utilities|FlowControl|FlipFlop
        (:A
          (Rendering|SetVisibility (Variables|Default|GetLockActSign) false false))
        (:B
          (Rendering|SetVisibility (Variables|Default|GetLockActSign) true false)))
      (if (>= (Variables|Default|GetCounterTimerPowerPanel) 6)
        (Variables|Default|SetCounterTimerPowerPanel 0)
        (Utilities|Time|ClearandInvalidateTimerbyHandle (Variables|Default|GetTimerBlinking))
        (Rendering|SetVisibility (Variables|Default|GetLockActSign) false false)
        (Audio|PlaySound2D "/Game/Audio/NEW_SOUNDS/CUES/CuesFX/WithoutLooping/Cue_Cells_TurnOff.Cue_Cells_TurnOff" 1.0 1.0 0.0 0 0)
        (CallFunction|ResetPanel)))))

(event Custom|ResetPanel
  (bind _numpanelpriority (Variables|Default|GetNumPanelPriority))
  (bind _sound (Variables|Default|GetSound))
  (Utilities|FlowControl|DoOnce false) ; enters at Reset
)

(event Custom|Finishseq
  (Audio|Components|Audio|Stop (Variables|Default|GetSound)))

(fn ConstructionScript)

(fn PlaySequence
  (params (bReverse? :type Boolean))
  (bind _gatesfx (Variables|Default|GetGateSFX))
  (bind _sequence (Variables|Default|GetSequence))
  (bind _sequenceplayer (Variables|/Script/LevelSequence.LevelSequenceActor|GetSequencePlayer _sequence))
  (EventDispatchers|BindEventtoOnFinished _sequenceplayer (EventDispatchers|CreateEvent :!event Custom|Finishseq))
  (if bReverse?
    (Class|MovieSceneSequencePlayer|PlayReverse _sequenceplayer)
    (bind _returnvalue (Audio|SpawnSound2D _gatesfx 1.0 1.0 0.0 0 false false))
    (bind _output_get (Variables|Default|SetSound _returnvalue))
    (Audio|Components|Audio|FadeIn _output_get 0.2 1.0 0.0 "SCurve" :!class /Script/Engine.AudioComponent)
    (else
      (Sequencer|Player|Play _sequenceplayer :!class /Script/MovieScene.MovieSceneSequencePlayer)
      (bind _returnvalue_2 (Audio|SpawnSound2D _gatesfx 1.0 1.0 0.0 0 false false))
      (bind _output_get_2 (Variables|Default|SetSound _returnvalue_2))
      (Audio|Components|Audio|FadeIn _output_get_2 0.2 1.0 0.0 "SCurve" :!class /Script/Engine.AudioComponent)))
  (return))