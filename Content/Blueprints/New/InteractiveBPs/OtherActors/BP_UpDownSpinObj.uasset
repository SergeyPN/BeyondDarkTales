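; BP_UpDownSpinObj is an actor that moves a configurable static mesh vertically between a high and a bottom value.
; The construction script applies the selected mesh to the component.
; On BeginPlay, a timeline runs at a configurable play rate, and its track lerps the mesh's relative Z location.
; Despite the Spin in its name, the graphs contain no rotation logic.
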(event EventBeginPlay
  (Components|Timeline|SetPlayRate (Variables|Default|GetTimeline_UpDown) (Variables|Default|GetTimeScale))
  (bind _updowntrack (Timeline|Timeline_UpDown Play)
    (:Update
      (Transformation|SetRelativeLocation (Variables|Default|GetStaticMesh) (Math|Vector|MakeVector 0.0 0.0 (Math|Float|Lerp (Variables|Default|GetHigh_Value) (Variables|Default|GetBottom_Value) (/ _updowntrack 1.0))) false false))))

(fn ConstructionScript
  (Components|StaticMesh|SetStaticMesh (Variables|Default|GetStaticMesh) (Variables|Default|GetSelect%20StaticMesh)))