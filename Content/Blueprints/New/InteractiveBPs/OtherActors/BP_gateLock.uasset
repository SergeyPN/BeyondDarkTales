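; Gate lock panel for an ordered activation puzzle: overlapping its box lights its sign once, with sound and effect.
; It finds the BP_LockActivator with the preceding priority; if that is lit and this panel is last, a level sequence plays.
; If the predecessor is unlit, all lit activators start blinking.
; A looping timer toggles the sign briefly, then switches it off and resets the DoOnce for another attempt.
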(event OnComponentBeginOverlap(Box)
  (params (OverlappedComponent :type Primitive%20Component%20Object%20Reference) (OtherActor :type Actor%20Object%20Reference) (OtherComp :type Primitive%20Component%20Object%20Reference) (OtherBodyIndex :type Integer) (bFromSweep :type Boolean) (SweepResult :type Hit%20Result%20Structure%20%28by%20ref%29))
  (bind _numpanelpriority (Variables|Default|GetNumPanelPriority))
  (Utilities|FlowControl|DoOnce false
    (:Completed
      (Rendering|SetVisibility (Variables|Default|GetLockActSign) true false)
      (Audio|PlaySound2D "/Game/Audio/Snd/FX/Cues/WithoutLooping/Cue_Cells_TurnOn.Cue_Cells_TurnOn" 1.0 1.0 0.0 0 0)
      (Components|Activation|Activate (Variables|Default|GetP_Correct) false)
      (bind _outactors (Actor|GetAllActorsOfClass "/Game/Blueprints/New/InteractiveBPs/OtherActors/BP_LockActivator.BP_LockActivator_C"))
      (bind _array_element (Utilities|Array|ForEachLoopwithBreak _outactors :!label _label)
        (:LoopBody
          (if (== (- _numpanelpriority 1) (Variables|/Game/Blueprints/New/InteractiveBPs/OtherActors/BP_LockActivator.BP_LockActivator_C|GetNumPanelPriority _array_element))
            (if (Variables|/Script/Engine.SceneComponent|GetbVisible (Variables|/Game/Blueprints/New/InteractiveBPs/OtherActors/BP_LockActivator.BP_LockActivator_C|GetLockActSign _array_element))
              (if (== (Utilities|Array|Length _outactors) _numpanelpriority)
                (Sequencer|Player|Play (Variables|/Script/LevelSequence.LevelSequenceActor|GetSequencePlayer (Variables|Default|GetSequence)) :!class /Script/MovieScene.MovieSceneSequencePlayer)
                (goto _label Break))
              (else
                (Utilities|FlowControl|Sequence
                  (:then_0
                    (bind _outactors_2 (Actor|GetAllActorsOfClass "/Game/Blueprints/New/InteractiveBPs/OtherActors/BP_LockActivator.BP_LockActivator_C"))
                    (for _array_element_2 _outactors_2
                      (if (Variables|/Script/Engine.SceneComponent|GetbVisible (Variables|/Game/Blueprints/New/InteractiveBPs/OtherActors/BP_LockActivator.BP_LockActivator_C|GetLockActSign _array_element_2))
                        (CallFunction|StartBlinking _array_element_2))))
                  (:then_1
                    (goto _label Break)))))))))))

(event Custom|StartBlinking
  (bind _returnvalue (Utilities|Time|SetTimerbyEvent (delegate Custom|TogglePowerPanel) 0.08 true))
  (Variables|Default|SetTimerBlinking _returnvalue))

(event Custom|ResetPanel
  (bind _numpanelpriority (Variables|Default|GetNumPanelPriority))
  (Utilities|FlowControl|DoOnce false) ; enters at Reset
)

(event Custom|TogglePowerPanel
  (Math|Integer|IncrementInt (Variables|Default|GetCounterTimerPowerPanel)
    (:%20%20
      (Utilities|FlowControl|FlipFlop
        (:A
          (Rendering|SetVisibility (Variables|Default|GetLockActSign) false false))
        (:B
          (Rendering|SetVisibility (Variables|Default|GetLockActSign) true false)))
      (if (>= (Variables|Default|GetCounterTimerPowerPanel) 6)
        (Variables|Default|SetCounterTimerPowerPanel 0)
        (Utilities|Time|ClearandInvalidateTimerbyHandle (Variables|Default|GetTimerBlinking))
        (Rendering|SetVisibility (Variables|Default|GetLockActSign) false false)
        (Audio|PlaySound2D "/Game/Audio/Snd/FX/Cues/WithoutLooping/Cue_Cells_TurnOff.Cue_Cells_TurnOff" 1.0 1.0 0.0 0 0)
        (CallFunction|ResetPanel)))))

(fn ConstructionScript)