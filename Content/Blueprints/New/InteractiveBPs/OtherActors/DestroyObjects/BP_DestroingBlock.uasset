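; Breakable block that, when flagged as a killing brick, collapses under BP_CharMax and triggers the death screen.
; On overlap it freezes movement and input, then swaps MainMesh for physics-simulated child debris with dust and a falling animation.
; Debris transforms are cached at BeginPlay so NewAttempt can rebuild the block.
; NewAttempt also resets trigger sequences, character and camera, then restores the interface and input after a fade.
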(event OnComponentBeginOverlap(Box)
  (params (OverlappedComponent :type Primitive%20Component%20Object%20Reference) (OtherActor :type Actor%20Object%20Reference) (OtherComp :type Primitive%20Component%20Object%20Reference) (OtherBodyIndex :type Integer) (bFromSweep :type Boolean) (SweepResult :type Hit%20Result%20Structure%20%28by%20ref%29))
  (if (Variables|Default|GetKillingBrick)
    (Utilities|FlowControl|Delay 0.5)
    (Utilities|FlowControl|DoOnce false
      (:Completed
        (bind _returnvalue (Utilities|Time|SetTimerbyEvent (delegate Custom|StopShake) 0.5))
        (Variables|Default|SetTimerShake _returnvalue)
        (bind _asbp_char_max (Utilities|Casting|CastToBP_CharMax OtherActor))
        (bind _output_get (Variables|Default|SetCharMax _asbp_char_max))
        (Default|StopMovement _output_get)
        (Pawn|Components|CharacterMovement|DisableMovement (Variables|/Script/Engine.Character|GetCharacterMovement _output_get))
        (Input|DisableInput (Game|Player|GetPlayerPawn 0) (Game|GetPlayerController 0))))))

(event Custom|StopShake
  (bind _maininterfacewidget (CallFunction|GetMainInterfaceWidget))
  (bind _asmax_anim (Utilities|Casting|CastToMax_Anim (Components|SkeletalMesh|GetAnimInstance (Variables|/Script/Engine.Character|GetMesh (Variables|Default|GetCharMax)))))
  (Variables|/Game/Assets/Heroes/Max/Anim/Max_Anim.Max_Anim_C|SetDangerAndFalling _asmax_anim true)
  (Components|Activation|Activate (Variables|Default|GetP_DustBurst) false)
  (Development|SetHiddeninGame (Variables|Default|GetMainMesh) true false)
  (for _array_element (Variables|Default|GetRefDebris)
    (Development|SetHiddeninGame _array_element false false))
  (Utilities|FlowControl|Delay 0.5)
  (Pawn|Components|CharacterMovement|SetMovementMode (Variables|/Script/Engine.Character|GetCharacterMovement (Variables|Default|GetCharMax)) "MOVE_Walking" 0)
  (Collision|SetCollisionEnabled (Variables|Default|GetMainMesh) "NoCollision")
  (Collision|SetCollisionProfileName (Variables|/Script/Engine.Character|GetCapsuleComponent (Variables|Default|GetCharMax)) "OverlapAll" true :!class /Script/Engine.PrimitiveComponent)
  (for _array_element_2 (Variables|Default|GetRefDebris)
    (Collision|SetCollisionEnabled (.AsStatic%20Mesh%20Component (Utilities|Casting|CastToStaticMeshComponent _array_element_2)) "PhysicsOnly")
    (Collision|SetCollisionProfileName (.AsStatic%20Mesh%20Component (Utilities|Casting|CastToStaticMeshComponent _array_element_2)) "BlockAll" true :!class /Script/Engine.PrimitiveComponent)
    (Physics|SetSimulatePhysics (.AsStatic%20Mesh%20Component (Utilities|Casting|CastToStaticMeshComponent _array_element_2)) true))
  (Utilities|FlowControl|Delay 3.0)
  (UserInterface|Animation|PlayAnimation _maininterfacewidget (Variables|/Game/Widgets/New/MainInterface_W.MainInterface_W_C|GetShowInterfaceWithPause _maininterfacewidget) 0.0 1 "Reverse" 4.0 false)
  (Utilities|FlowControl|Sequence
    (:then_0
      (for _array_element_3 (Variables|Default|GetRefDebris)
        (Transformation|AttachComponentToComponent _array_element_3 (Variables|Default|GetMainMesh) "None" "KeepWorld" "KeepWorld" "KeepWorld" true)
        (Physics|SetSimulatePhysics _array_element_3 false)
        (Collision|SetCollisionEnabled _array_element_3 "NoCollision")
        (Collision|SetCollisionProfileName _array_element_3 "NoCollision" true :!class /Script/Engine.PrimitiveComponent))
      (Collision|SetCollisionProfileName (Variables|/Script/Engine.Character|GetCapsuleComponent (Variables|Default|GetCharMax)) "Pawn" true :!class /Script/Engine.PrimitiveComponent)
      (Transformation|SetActorTransform (Variables|Default|GetCharMax) (Math|Transform|MakeTransform "20.000000,150.000000,-820.000000" "0, 0, 0" "1,1,1"))
      (Utilities|Time|ClearandInvalidateTimerbyHandle (Variables|Default|GetTimerShake)))
    (:then_1
      (bind _asbp_main_menu_hud (Utilities|Casting|CastToBP_MainMenuHUD (HUD|GetHUD (Game|GetPlayerController 0))))
      (UserInterface|Viewport|AddtoViewport (Variables|/Game/Blueprints/New/Main/MainMenu/BP_MainMenuHUD.BP_MainMenuHUD_C|GetDieScreenWidget _asbp_main_menu_hud) 3)
      (Variables|/Game/Widgets/DieScreen/WBP_DieScreen.WBP_DieScreen_C|SetActorCreatorWidget (Variables|/Game/Blueprints/New/Main/MainMenu/BP_MainMenuHUD.BP_MainMenuHUD_C|GetDieScreenWidget _asbp_main_menu_hud) self))))

(event Custom|ResetBrick
  (Utilities|FlowControl|DoOnce false) ; enters at Reset
)

(event EventTick
  (params (DeltaSeconds :type Float%20%28single-precision%29)))

(event EventBeginPlay
  (Utilities|Array|Clear (Variables|Default|GetRefDebris))
  (Utilities|Array|Clear (Variables|Default|GetStartTransformBreakingMesh))
  (for _array_element (Components|GetChildrenComponents (Variables|Default|GetMainMesh) false)
    (bind _asstatic_mesh_component (Utilities|Casting|CastToStaticMeshComponent _array_element))
    (Utilities|Array|Add (Variables|Default|GetRefDebris) _asstatic_mesh_component)
    (Utilities|Array|Add (Variables|Default|GetStartTransformBreakingMesh) (Transformation|GetWorldTransform _asstatic_mesh_component))))

(event EventNewAttempt
  (bind _maininterfacewidget (CallFunction|GetMainInterfaceWidget))
  (CallFunction|HandleReset)
  (Utilities|FlowControl|Delay 2.0)
  (bind _ascamera_pc_test (Utilities|Casting|CastToCamera_PC_test (Game|Player|GetPlayerPawn 0)))
  (Transformation|SetActorTransform (Variables|/Game/Blueprints/Transfered/Blueprints1/ToTransfer/CameraControl/Camera_PC_test.Camera_PC_test_C|GetLevelCamera _ascamera_pc_test) (Variables|Default|GetStartPositionForCamera))
  (bind _foundwidgets (Widget|GetAllWidgetsOfClass "/Game/Widgets/LoadingScreen/WB_LoadingScreen.WB_LoadingScreen_C" true))
  (Widget|RemovefromParent (Utilities|Array|Get(acopy) _foundwidgets))
  (CameraFades|StartCameraFade :self (Variables|/Script/Engine.PlayerController|GetPlayerCameraManager (Game|GetPlayerController 0)) :FromAlpha 1.0 :Duration 1.0)
  (UserInterface|Animation|PlayAnimation _maininterfacewidget (Variables|/Game/Widgets/New/MainInterface_W.MainInterface_W_C|GetShowInterfaceWithPause _maininterfacewidget) 0.0 1 "Forward" 4.0 false)
  (Utilities|FlowControl|Delay 1.5)
  (CallFunction|ResetBrick)
  (Input|EnableInput (Game|Player|GetPlayerPawn 0) (Game|GetPlayerController 0))
  (Variables|/Game/Widgets/DieScreen/WBP_DieScreen.WBP_DieScreen_C|SetDoOnce (Variables|/Game/Blueprints/New/Main/MainMenu/BP_MainMenuHUD.BP_MainMenuHUD_C|GetDieScreenWidget (.AsBP%20Main%20Menu%20HUD (Utilities|Casting|CastToBP_MainMenuHUD (HUD|GetHUD (Game|GetPlayerController 0))))) false))

(fn ConstructionScript)

(fn HandleReset
  ;[1 1 1] Return begin Brick
  (bind _outactors (Actor|GetAllActorsOfClass "/Game/Blueprints/New/Triggers/BP_TriggerSequence.BP_TriggerSequence_C"))
  (for _array_element _outactors
    (Default|ResetTrigger _array_element))
  (for _array_element_2 (Variables|Default|GetResetSequences)
    (Components|Timeline|SetPlaybackPosition (Variables|/Script/LevelSequence.LevelSequenceActor|GetSequencePlayer _array_element_2) (Utilities|Struct|MakeMovieSceneSequencePlaybackParams "(FrameNumber=(Value=0),SubFrame=0.000000)" 0.0 "" "Frame" "Play")))
  (Transformation|SetActorTransform (Variables|Default|GetCharMax) (Variables|Default|GetStartPositionForChar))
  (Transformation|SetRelativeScale3D (Variables|/Script/Engine.Character|GetMesh (Variables|Default|GetCharMax)) "1.000000,1.000000,1.000000")
  (bind _asmax_anim (Utilities|Casting|CastToMax_Anim (Components|SkeletalMesh|GetAnimInstance (Variables|/Script/Engine.Character|GetMesh (Variables|Default|GetCharMax)))))
  (Variables|/Game/Assets/Heroes/Max/Anim/Max_Anim.Max_Anim_C|SetDangerAndFalling _asmax_anim false)
  (Collision|SetCollisionEnabled (Variables|Default|GetMainMesh) "QueryAndPhysics")
  (Development|SetHiddeninGame (Variables|Default|GetMainMesh) false false)
  (for (_array_element_3 _array_index) (Variables|Default|GetRefDebris)
    (Transformation|SetWorldTransform _array_element_3 (Utilities|Array|Get(acopy) (Variables|Default|GetStartTransformBreakingMesh) _array_index) false false)
    (Development|SetHiddeninGame _array_element_3 true false))
  (return))