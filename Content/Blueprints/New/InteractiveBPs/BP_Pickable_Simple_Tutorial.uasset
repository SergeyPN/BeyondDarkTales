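; BP_Pickable_Simple_Tutorial is, by its name, a simple pickable with a tutorial widget that turns with the level camera.
; On BeginPlay it caches the player's Camera_PC_test pawn and starts a looping timer at roughly 60 Hz instead of using Tick.
; The timer sets the widget's world yaw to the LevelCamera's yaw, with zero pitch and roll.
; Destroyed clears the timer.
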(event EventBeginPlay
  (|CallParentFunction)
  (bind _ascamera_pc_test (Utilities|Casting|CastToCamera_PC_test (Game|Player|GetPlayerPawn 0)))
  (Variables|Default|SetPlayerPawn _ascamera_pc_test)
  (bind _returnvalue (Utilities|Time|SetTimerbyFunctionName self "RotateWidget" 0.016 true))
  (Variables|Default|SetTimerRotateWidget _returnvalue))

(event Collision|EventActorBeginOverlap
  (params (OtherActor :type Actor%20Object%20Reference))
  (|CallParentFunction OtherActor) ; This node is disabled and will not be called.\nDrag off pins to build functionality.
)

(event EventTick
  (params (DeltaSeconds :type Float%20%28single-precision%29))
  (|CallParentFunction DeltaSeconds) ; This node is disabled and will not be called.\nDrag off pins to build functionality.
)

(event EventDestroyed
  (Utilities|Time|ClearandInvalidateTimerbyHandle (Variables|Default|GetTimerRotateWidget)))

(fn ConstructionScript
  (|CallParentFunction))

(fn RotateWidget
  (Transformation|SetWorldRotation (Variables|Default|GetSceneWidgetTutorial) (Math|Rotator|MakeRotator 0.0 0.0 (.yaw (Transformation|GetActorRotation (Variables|/Game/Blueprints/Transfered/Blueprints1/ToTransfer/Camera_PC_test.Camera_PC_test_C|GetLevelCamera (Variables|Default|GetPlayerPawn))))) false false))