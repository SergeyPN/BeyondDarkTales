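; Interactive door that moves the player between areas by handing camera, door and level streaming indices to the LevelCameraAndDoorManager's SwapCamera.
; On interaction it either swaps immediately, passing along any follow-up dialog, or opens a dialog first and swaps when that ends.
; When dialog ends it restores the main interface, and Discord doors show the Discord UI instead of swapping.
; The Changer camera-blend teleport macros are unused.
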(event EventBeginPlay
  (|CallParentFunction)
  (bind _outactors (Actor|GetAllActorsOfClass "/Game/Blueprints/New/LevelCameraAndDoorManager.LevelCameraAndDoorManager_C"))
  (Variables|Default|SetLvlCam&DoorManager (Utilities|Array|Get(acopy) _outactors)))

(event Collision|EventActorBeginOverlap
  (params (OtherActor :type Actor%20Object%20Reference))
  (|CallParentFunction OtherActor) ; This node is disabled and will not be called.\nDrag off pins to build functionality.
)

(event EventTick
  (params (DeltaSeconds :type Float%20%28single-precision%29))
  (|CallParentFunction DeltaSeconds) ; This node is disabled and will not be called.\nDrag off pins to build functionality.
)

(event EventInteractwithWidget
  (CallFunction|HideInteract)
  (if (Variables|Default|GetIsWithDialog?)
    (if (Variables|Default|GetDialogAfter?)
      (Default|SwapCamera (Variables|Default|GetLvlCam&DoorManager) (Variables|Doors|GetCameraToChange) (Variables|Doors|GetDoorToPlace) (Variables|Doors|GetLevelToUnload) (Variables|Doors|GetLevelToLoad) (Variables|Default|GetDialogAfter?) self (Variables|Default|GetDialogToStart))
      (Variables|Default|SetAfterStreamLevelInteraction true)
      (else
        (Default|OpenDialog (Variables|Default|GetDialogActor) (Variables|Default|GetDialogToStart) self)))
    (else
      (Default|SwapCamera (Variables|Default|GetLvlCam&DoorManager) (Variables|Doors|GetCameraToChange) (Variables|Doors|GetDoorToPlace) (Variables|Doors|GetLevelToUnload) (Variables|Doors|GetLevelToLoad) (Variables|Default|GetDialogAfter?) self (Variables|Default|GetDialogToStart))
      (Variables|Default|SetAfterStreamLevelInteraction true))))

(event EventDialogEnded
  (params (CurrentDialogNum :type Integer))
  (bind _playerpawn (Variables|Default|GetPlayerPawn))
  (bind _currentplayercontroller (Variables|/Game/Blueprints/Transfered/Blueprints1/ToTransfer/Camera_PC_test.Camera_PC_test_C|GetCurrentPlayerController _playerpawn))
  (bind _maininterface_w (Variables|/Game/Blueprints/New/Main/01CaveMain/01CM_PC.01CM_PC_C|GetMainInterface_W _currentplayercontroller))
  (UserInterface|Animation|PlayAnimation _maininterface_w (Variables|/Game/Widgets/New/MainInterface_W.MainInterface_W_C|GetShowInterface _maininterface_w) 0.0 1 "Forward" 4.0 false)
  (if (Variables|Default|GetDiscordDoor?)
    (Default|DiscordShow (Variables|/Game/Blueprints/New/Main/01CaveMain/01CM_PC.01CM_PC_C|GetMainInterface_W (.As01CM%20PC (Utilities|Casting|CastTo01CM_PC (Game|GetPlayerController 0)))))
    (Variables|Default|SetAfterStreamLevelInteraction true)
    (elif (not (Variables|Default|GetDialogAfter?))
      (Default|SwapCamera (Variables|Default|GetLvlCam&DoorManager) (Variables|Doors|GetCameraToChange) (Variables|Doors|GetDoorToPlace) (Variables|Doors|GetLevelToUnload) (Variables|Doors|GetLevelToLoad) (Variables|Default|GetDialogAfter?) self (Variables|Default|GetDialogToStart))
      (Variables|Default|SetAfterStreamLevelInteraction true))))

(fn ConstructionScript
  (|CallParentFunction)
  (Variables|Default|SetRusName "Дверь")
  (Variables|Default|SetEngName "Door")
  (if (== (Variables|Default|GetActorToUseWith) 0)
    (Transformation|SetRelativeLocation (Variables|Default|GetPreInteractionWidget) "0, 0,250.000000" false false)))