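; BP_ActorMain_Parkou is an interactable parkour spot that makes the player perform a jump-up move when triggered.
; On widget interaction it hides the prompt and snaps the player to Arrow0's XY position and rotation, keeping the player's height.
; It then flags OnParcour, switches movement to Flying and plays JumpMidUp_Montage, restoring Walking and clearing the flag on completion.
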(event EventBeginPlay
  (|CallParentFunction) ; This node is disabled and will not be called.\nDrag off pins to build functionality.
)

(event Collision|EventActorBeginOverlap
  (params (OtherActor :type Actor%20Object%20Reference))
  (|CallParentFunction OtherActor))

(event EventTick
  (params (DeltaSeconds :type Float%20%28single-precision%29))
  (|CallParentFunction DeltaSeconds))

(event EventInteractwithWidget
  (bind _player (Variables|Default|GetPlayer))
  (bind _arrow_0 (Variables|Default|GetArrow_0))
  (bind _returnvalue (Transformation|GetWorldTransform _arrow_0))
  (bind _charactermovement (Variables|/Script/Engine.Character|GetCharacterMovement _player))
  (CallFunction|HideInteract)
  (Transformation|SetActorTransform _player (Math|Transform|MakeTransform (Math|Vector|MakeVector (.x (.location _returnvalue)) (.y (.location _returnvalue)) (.z (Transformation|GetActorLocation _player))) (.rotation _returnvalue) "1,1,1"))
  (Variables|/Game/Assets/Heroes/Max/BP_CharMax.BP_CharMax_C|SetOnParcour _player true)
  (Pawn|Components|CharacterMovement|SetMovementMode _charactermovement "MOVE_Flying" 0)
  (Animation|Montage|PlayMontage (Variables|/Script/Engine.Character|GetMesh _player) "/Game/Assets/Heroes/Max/Anim/JumpMidUp_Montage.JumpMidUp_Montage"
    (:OnCompleted
      (Pawn|Components|CharacterMovement|SetMovementMode _charactermovement "MOVE_Walking" 0)
      (Variables|/Game/Assets/Heroes/Max/BP_CharMax.BP_CharMax_C|SetOnParcour _player false))))

(fn ConstructionScript
  (|CallParentFunction))