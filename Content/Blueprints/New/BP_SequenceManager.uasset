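; BP_SequenceManager plays level sequences for an interacting actor or a trigger and opens follow-up dialog when they finish.
; ShowSequence disables player input, plays the valid ActorMain's sequence, otherwise the trigger's, and binds a finish handler.
; The actor handler can also message another actor to change dialog and switches an "After" sequence variant row to "Not".
; The trigger handler unbinds itself and fades the camera before opening dialog.
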(event Custom|ShowSequence
  (params (ActorMain :type BP%20Actor%20Main%20Object%20Reference) (DialogCaller :type Actor%20Object%20Reference) (TriggerSequence :type BP%20Trigger%20Sequence%20Object%20Reference))
  (Variables|Default|SetActorMain ActorMain)
  (Variables|Default|SetTriggerSequence TriggerSequence)
  (Input|DisableInput (Game|Player|GetPlayerPawn 0) (Game|GetPlayerController 0))
  (Utilities|IsValid (Variables|Default|GetActorMain)
    (:Is%20Valid
      (Sequencer|Player|Play (Variables|/Script/LevelSequence.LevelSequenceActor|GetSequencePlayer (Variables|/Game/Blueprints/New/InteractiveBPs/BP_ActorMain.BP_ActorMain_C|GetSequence (Variables|Default|GetActorMain))) :!class /Script/MovieScene.MovieSceneSequencePlayer)
      (EventDispatchers|BindEventtoOnFinished (Variables|/Script/LevelSequence.LevelSequenceActor|GetSequencePlayer (Variables|/Game/Blueprints/New/InteractiveBPs/BP_ActorMain.BP_ActorMain_C|GetSequence (Variables|Default|GetActorMain))) (delegate Custom|FinishSequence)))
    (:Is%20Not%20Valid
      (Sequencer|Player|Play (Variables|/Script/LevelSequence.LevelSequenceActor|GetSequencePlayer (Variables|/Game/Blueprints/New/Triggers/BP_TriggerSequence.BP_TriggerSequence_C|GetSequence (Variables|Default|GetTriggerSequence))) :!class /Script/MovieScene.MovieSceneSequencePlayer)
      (EventDispatchers|BindEventtoOnFinished (Variables|/Script/LevelSequence.LevelSequenceActor|GetSequencePlayer (Variables|/Game/Blueprints/New/Triggers/BP_TriggerSequence.BP_TriggerSequence_C|GetSequence (Variables|Default|GetTriggerSequence))) (delegate Custom|FinishSequenceTrigger)))))

(event Custom|FinishSequenceTrigger
  (EventDispatchers|UnbindEventfromOnFinished (Variables|/Script/LevelSequence.LevelSequenceActor|GetSequencePlayer (Variables|/Game/Blueprints/New/Triggers/BP_TriggerSequence.BP_TriggerSequence_C|GetSequence (Variables|Default|GetTriggerSequence))) (delegate Custom|FinishSequenceTrigger))
  (CameraFades|StartCameraFade :self (Variables|/Script/Engine.PlayerController|GetPlayerCameraManager (Game|GetPlayerController 0)) :FromAlpha 1.0 :Duration 1.0 :bHoldWhenFinished true)
  (Utilities|FlowControl|Delay 1.0)
  (if (!= (Variables|/Game/Blueprints/New/Triggers/BP_TriggerSequence.BP_TriggerSequence_C|GetNumDialogAfterSequence (Variables|Default|GetTriggerSequence)) 0)
    (Default|OpenDialog (Variables|Default|GetDialogActor) (Variables|/Game/Blueprints/New/Triggers/BP_TriggerSequence.BP_TriggerSequence_C|GetNumDialogAfterSequence (Variables|Default|GetTriggerSequence)) (stale Custom|ShowSequence DialogCaller))))

(event Custom|FinishSequence
  (bind _actormain (Variables|Default|GetActorMain))
  (bind _actorforinteraction (Variables|/Game/Blueprints/New/InteractiveBPs/BP_ActorMain.BP_ActorMain_C|GetActorForInteraction _actormain))
  (bind (_actorforinteraction_2 _changedialogforhim) (Utilities|Struct|BreakStruct_InteractionWithActors _actorforinteraction))
  ;[1 1 1] Dialog after sequence
  (if (!= (Variables|/Game/Blueprints/New/InteractiveBPs/BP_ActorMain.BP_ActorMain_C|GetDialogAfterSequence (Variables|Default|GetActorMain)) 0)
    (Default|OpenDialog (Variables|Default|GetDialogActor) (Variables|/Game/Blueprints/New/InteractiveBPs/BP_ActorMain.BP_ActorMain_C|GetDialogAfterSequence (Variables|Default|GetActorMain)) (stale Custom|ShowSequence DialogCaller)))
  ;[1 1 1] Change dialog another actor
  (Utilities|IsValid _actorforinteraction_2
    (:Is%20Valid
      (Class|BPInteractive|InteractwithObject(Message) _actorforinteraction_2 _changedialogforhim "0, 0, 0"))
    (:Is%20Not%20Valid
      _))
  ;[1 1 1] 2 dialogs
  (if (Utilities|Name|Equal(Name) (.RowName (Utilities|Struct|BreakDataTableRowHandle (Variables|/Game/Blueprints/New/InteractiveBPs/BP_ActorMain.BP_ActorMain_C|GetWithSequence? (Variables|Default|GetActorMain)))) "After")
    (Utilities|Struct|SetmembersinDataTableRowHandle (Variables|/Game/Blueprints/New/InteractiveBPs/BP_ActorMain.BP_ActorMain_C|GetWithSequence? (Variables|Default|GetActorMain)) "/Game/GameData/VariantPlayerSequence/DT_VariantSequence.DT_VariantSequence" "Not")))

(event EventBeginPlay
  (bind _returnvalue (Actor|GetActorOfClass "/Game/Blueprints/New/DialogActor.DialogActor_C"))
  (Variables|Default|SetDialogActor _returnvalue)
  (bind _as01cm_pc (Utilities|Casting|CastTo01CM_PC (Game|GetPlayerController 0)))
  (Variables|Default|SetPlayerController _as01cm_pc))

(event EventTick
  (params (DeltaSeconds :type Float%20%28single-precision%29)))

(fn ConstructionScript)