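; BP_DragActor is an interactable object that the player can grab and drag around.
; It places four arrows from the mesh bounds, and interaction sends the player to the nearest one.
; DragW_On attaches the player to the object, disables pawn input, hands itself to the touch interface and shows a close button.
; A looping timer event is started for the drag, and SpawnSFX unpauses the sound only while grab axes show movement.
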(event Custom|DragW_Off
  (bind _widget (Variables|Default|GetWidget))
  (bind _returnvalue (UserInterface|GetUserWidgetObject _widget))
  (bind _aswbp_button_close_drag (Utilities|Casting|CastToWBP_ButtonCloseDrag _returnvalue))
  ;[1 1 1] Intract pressed
  (UserInterface|Animation|PlayAnimation _aswbp_button_close_drag (Variables|/Game/Widgets/New/WBP_ButtonCloseDrag.WBP_ButtonCloseDrag_C|GetShowButtonClose _aswbp_button_close_drag) 0.0 1 "Reverse" 4.0 false)
  (Transformation|DetachFromActor (Variables|Default|GetPlayer) "KeepWorld" "KeepWorld" "KeepWorld")
  (Variables|/Game/Assets/Heroes/Max/BP_CharMax.BP_CharMax_C|SetPushItem? (Variables|Default|GetPlayer) false)
  (Variables|Default|SetStartEnabled? true)
  (Variables|Default|SetWith%20Hide%20Pre%20Interact? false)
  (Utilities|Time|ClearandInvalidateTimerbyHandle (Variables|Default|GetSFX_Spawn_Timer)))

(event Custom|SpawnSFX
  (bind _sfx_spawn (Variables|Default|GetSFX_Spawn))
  ;[1 1 1] Intract pressed
  (if (CallFunction|FCheckMovement)
    (Class|AudioComponent|SetPaused _sfx_spawn false)
    (else
      (Class|AudioComponent|SetPaused _sfx_spawn true))))

(event Custom|DragW_On
  (bind _maininterfacewidget (CallFunction|GetMainInterfaceWidget))
  (bind _widget (Variables|Default|GetWidget))
  (bind _returnvalue (UserInterface|GetUserWidgetObject _widget))
  (bind _aswbp_button_close_drag (Utilities|Casting|CastToWBP_ButtonCloseDrag _returnvalue))
  ;[1 1 1] Intract pressed
  (UserInterface|Animation|PlayAnimation _maininterfacewidget (Variables|/Game/Widgets/New/MainInterface_W.MainInterface_W_C|GetShowPauseButton _maininterfacewidget) 0.0 1 "Reverse" 4.0 false)
  (UserInterface|Animation|PlayAnimation _aswbp_button_close_drag (Variables|/Game/Widgets/New/WBP_ButtonCloseDrag.WBP_ButtonCloseDrag_C|GetShowButtonClose _aswbp_button_close_drag) 0.0 1 "Forward" 4.0 false)
  (Variables|/Game/Widgets/New/TouchInterface/WBP_TouchInterface.WBP_TouchInterface_C|SetDragActor (Variables|/Game/Widgets/New/MainInterface_W.MainInterface_W_C|GetWBP_TouchInterface (CallFunction|GetMainInterfaceWidget)) self)
  (Transformation|AttachActorToActor (Variables|Default|GetPlayer) self "None" "KeepWorld" "KeepWorld" "KeepWorld" true)
  (Input|DisableInput (Game|Player|GetPlayerPawn 0) (Game|GetPlayerController 0))
  (bind _returnvalue_2 (Utilities|Time|SetTimerbyEvent (EventDispatchers|CreateEvent :!event Custom|SpawnSFX) 0.3 true))
  (Variables|Default|SetSFX_Spawn_Timer _returnvalue_2))

(event EventBeginPlay
  (|CallParentFunction)
  (CallFunction|SetArrows)
  (bind _returnvalue (Rendering|Material|CreateDynamicMaterialInstance (Variables|Default|GetSpecificMesh) 0 "/Game/Assets/Maps/01_Caves/Mats/MI_CaveSigns.MI_CaveSigns" "SignOpacity" :!class /Script/Engine.PrimitiveComponent))
  (Variables|Default|SetDynMat _returnvalue)
  (bind _returnvalue_2 (Audio|SpawnSoundatLocation (Variables|Default|GetSFX) (Transformation|GetActorLocation) "0, 0, 0" 1.0 1.0 0.0 0 0))
  (bind _output_get (Variables|Default|SetSFX_Spawn _returnvalue_2))
  (Class|AudioComponent|SetPaused _output_get true))

(event EventInteractwithWidget
  (bind _player (Variables|Default|GetPlayer))
  ;[1 1 1] Intract pressed
  (Variables|/Game/Blueprints/New/InteractiveBPs/BP_ActorMain.BP_ActorMain_C|SetDisableAfterInteract? self true)
  (CallFunction|HideInteract true)
  (CallFunction|Enable/DisableActor false)
  (bind (_arrowtomoveto _newparam) (CallFunction|CheckDistance))
  (Variables|Default|SetNewVar_3 _newparam)
  (Variables|/Game/Assets/Heroes/Max/BP_CharMax.BP_CharMax_C|SetOnParcour _player true)
  (Default|MovePLayer _player 0 (Transformation|GetWorldLocation _arrowtomoveto) false "0, 0, 0" "NewEnumerator6" "0, 0, 0" _arrowtomoveto true self false))

(event EventTick
  (params (DeltaSeconds :type Float%20%28single-precision%29)))

(fn ConstructionScript
  (|CallParentFunction))

(fn SetInvUpName
  (switch Utilities|FlowControl|Switch|SwitchonGameLanguage (Variables|/Game/Blueprints/MyGameInstance.MyGameInstance_C|GetLanguage (Variables|Default|GetGameInstance))
    (:NewEnumerator0
      (Variables|Default|SetVisText (Variables|Default|GetRusUpName)))
    (:NewEnumerator1
      (Variables|Default|SetVisText (Variables|Default|GetEngUPName)))))

(fn CheckDistance
  (Utilities|Array|Add (LocalVariables|GetDistance) (Math|Vector|Distance(Vector) (Transformation|GetActorLocation (Variables|Default|GetPlayer)) (Transformation|GetWorldLocation (Variables|Default|GetArrow))))
  (Utilities|Array|Add (LocalVariables|GetDistance) (Math|Vector|Distance(Vector) (Transformation|GetActorLocation (Variables|Default|GetPlayer)) (Transformation|GetWorldLocation (Variables|Default|GetArrow1))))
  (Utilities|Array|Add (LocalVariables|GetDistance) (Math|Vector|Distance(Vector) (Transformation|GetActorLocation (Variables|Default|GetPlayer)) (Transformation|GetWorldLocation (Variables|Default|GetArrow2))))
  (Utilities|Array|Add (LocalVariables|GetDistance) (Math|Vector|Distance(Vector) (Transformation|GetActorLocation (Variables|Default|GetPlayer)) (Transformation|GetWorldLocation (Variables|Default|GetArrow3))))
  (switch int (.IndexOfMinValue (Math|Float|MinOfFloatArray (LocalVariables|GetDistance)))
    (:0
      (return (Variables|Default|GetArrow) 1))
    (:1
      (return (Variables|Default|GetArrow1) 2))
    (:2
      (return (Variables|Default|GetArrow2) 3))
    (:3
      (return (Variables|Default|GetArrow3) 4))))

(fn SetArrows
  (Transformation|SetRelativeLocation (Variables|Default|GetArrow) (Math|Vector|MakeVector (* (.x (.BoxExtent (Collision|GetComponentBounds (Variables|Default|GetStaticMesh)))) -1.0) 0.0 0.0) false false)
  (Transformation|SetRelativeLocation (Variables|Default|GetArrow1) (Math|Vector|MakeVector (.x (.BoxExtent (Collision|GetComponentBounds (Variables|Default|GetStaticMesh)))) 0.0 0.0) false false)
  (Transformation|SetRelativeLocation (Variables|Default|GetArrow2) (Math|Vector|MakeVector 0.0 (.x (.BoxExtent (Collision|GetComponentBounds (Variables|Default|GetStaticMesh)))) 0.0) false false)
  (Transformation|SetRelativeLocation (Variables|Default|GetArrow3) (Math|Vector|MakeVector 0.0 (* (.y (.BoxExtent (Collision|GetComponentBounds (Variables|Default|GetStaticMesh)))) -1.0) 0.0) false false))

(fn FCheckMovement
  (bind _player (Variables|Default|GetPlayer))
  (return (or (> (Math|Float|Absolute(Float) (Variables|/Game/Assets/Heroes/Max/BP_CharMax.BP_CharMax_C|GetRightGrab _player)) 0.05) (> (Math|Float|Absolute(Float) (Variables|/Game/Assets/Heroes/Max/BP_CharMax.BP_CharMax_C|GetForwardGrab _player)) 0.05))))