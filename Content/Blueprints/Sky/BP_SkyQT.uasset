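; BP_SkyQT is a sky sphere Blueprint that gives a level a configurable sky with color and Fresnel controls.
; Its construction script creates a dynamic instance of M_SkyQT on the sphere mesh and stores it as SkyMaterial.
; It then copies the Blueprint's variables into the material parameters: three colors, a midpoint, an overall color, and Fresnel color, exponent and base reflect fraction.
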(fn ConstructionScript
  (bind _returnvalue (Rendering|Material|CreateDynamicMaterialInstance (Variables|BP_Skydome|GetSkySphereMesh) 0 "/Game/Blueprints/Sky/M_SkyQT.M_SkyQT" "None" :!class /Script/Engine.PrimitiveComponent))
  (bind _output_get (Variables|Default|SetSky%20material _returnvalue))
  (Rendering|Material|SetVectorParameterValue _output_get "Color1" (Variables|Default|GetColor1) :!class /Script/Engine.MaterialInstanceDynamic)
  (Rendering|Material|SetVectorParameterValue _output_get "Color2" (Variables|Default|GetColor2) :!class /Script/Engine.MaterialInstanceDynamic)
  (Rendering|Material|SetVectorParameterValue _output_get "Color3" (Variables|Default|GetColor3) :!class /Script/Engine.MaterialInstanceDynamic)
  (Rendering|Material|SetScalarParameterValue _output_get "MidPoint" (Variables|Default|GetMidPoint) :!class /Script/Engine.MaterialInstanceDynamic)
  (Rendering|Material|SetVectorParameterValue _output_get "OverAllColor" (Variables|Default|GetOverAllColor) :!class /Script/Engine.MaterialInstanceDynamic)
  (Rendering|Material|SetVectorParameterValue _output_get "FresnelColor" (Variables|Default|GetFresnelColor) :!class /Script/Engine.MaterialInstanceDynamic)
  (Rendering|Material|SetScalarParameterValue _output_get "ExponentIn" (Variables|Default|GetExponentIn) :!class /Script/Engine.MaterialInstanceDynamic)
  (Rendering|Material|SetScalarParameterValue _output_get "BaseReflectFractionIn" (Variables|Default|GetBaseReflectFractionIn) :!class /Script/Engine.MaterialInstanceDynamic))