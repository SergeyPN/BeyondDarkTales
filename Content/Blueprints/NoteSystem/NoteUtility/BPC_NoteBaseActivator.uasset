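; BPC_NoteBaseActivator is a component that updates a note's state when its owning BP_InteractiveActor fires the ActivateNote dispatcher.
; On BeginPlay it binds to that dispatcher, doing nothing if the owner is another class.
; When triggered, it unbinds, sets the state for its NoteTag on the level's BP_NoteManager, then destroys itself, making activation one-shot.
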(event Custom|ActivateNote_Event
  (bind _asbp_interactive_actor (Utilities|Casting|CastToBP_InteractiveActor (Components|GetOwner)))
  (EventDispatchers|UnbindEventfromActivateNote _asbp_interactive_actor (delegate Custom|ActivateNote_Event))
  (bind _returnvalue (Actor|GetActorOfClass "/Game/Blueprints/NoteSystem/BP_NoteManager.BP_NoteManager_C"))
  (Default|SetStateNote _returnvalue (Variables|Default|GetNoteTag) "NewEnumerator1")
  (Components|DestroyComponent))

(event EventBeginPlay
  (bind _asbp_interactive_actor (Utilities|Casting|CastToBP_InteractiveActor (Components|GetOwner)))
  (EventDispatchers|AssignActivateNote _asbp_interactive_actor (delegate Custom|ActivateNote_Event)))