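; BP_NoteManager holds the notes for the current level and tracks each note's state.
; On BeginPlay it looks up the DT_Notes row named after the level and copies that row's tag-keyed note map.
; Functions return one note or the whole map, or set a note's state by tag.
; A bulk setter changes states through a type filter, implementing only the found-notes case.
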(event EventBeginPlay
  (bind _returnvalue (Game|GetCurrentLevelName true))
  (bind _returnvalue_2 (Utilities|GetDataTableRow "/Game/Blueprints/NoteSystem/DT_Notes.DT_Notes" (Utilities|String|StringToName _returnvalue))
    (:then
      (Variables|Default|SetNotes (Utilities|Struct|BreakS_SetNotes _returnvalue_2)))))

(fn ConstructionScript)

(fn GetNote
  (params (NoteTag :type Gameplay%20Tag%20Structure))
  (return (.Value (Utilities|Map|Find (Variables|Default|GetNotes) NoteTag))))

(fn SetStateNote
  (params (NoteTag :type Gameplay%20Tag%20Structure) (StateNote :type E_StateNote%20Enum :default "NewEnumerator0"))
  (bind _structout (Utilities|Struct|SetmembersinS_Note (.Value (Utilities|Map|Find (Variables|Default|GetNotes) NoteTag)) StateNote))
  (Utilities|Map|Add (Variables|Default|GetNotes) NoteTag _structout))

(fn GetNotes
  (return (Variables|Default|GetNotes)))

(fn SetStateforAllNote
  (params (StateNote :type E_StateNote%20Enum :default "NewEnumerator0") (TypeFilter :type E_FilterSetStateNote%20Enum :default "NewEnumerator0"))
  (switch Utilities|FlowControl|Switch|SwitchonE_FilterSetStateNote TypeFilter
    (:NewEnumerator1
      (bind _values (Utilities|Map|Values (Variables|Default|GetNotes)))
      (for (_array_element _array_index) _values
        (LocalVariables|SetL_Index _array_index)
        (if (Utilities|Enum|Equal(Enum) (.StateNote (Utilities|Struct|BreakS_Note _array_element)) "NewEnumerator1")
          (bind _structout (Utilities|Struct|SetmembersinS_Note _array_element StateNote))
          (bind _keys (Utilities|Map|Keys (Variables|Default|GetNotes)))
          (Utilities|Map|Add (Variables|Default|GetNotes) (Utilities|Array|Get(acopy) _keys (LocalVariables|GetL_Index)) _structout))))))