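; BP_TrisignManager tracks how many trisigns have been collected at each named location in the current level.
; On BeginPlay it fills its location-to-count map from the DT_TrisignsOnLvl row matching the level name.
; An update function increments a location's count up to three and pushes the new value to the first MainInterface_W widget found.
; A getter returns the count for a given location.
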(event EventBeginPlay
  (bind _returnvalue (Game|GetCurrentLevelName true))
  (bind _returnvalue_2 (Utilities|GetDataTableRow "/Game/Blueprints/Trisign/DT_TrisignsOnLvl.DT_TrisignsOnLvl" (Utilities|String|StringToName _returnvalue))
    (:then
      (Variables|Default|SetCount%20Trisigns%20on%20Lvl (Utilities|Struct|BreakS_TrisignsOnLvls _returnvalue_2)))))

(fn ConstructionScript)

(fn UpdateCountCollectedTrisigns
  (params (CurrentLocName :type Name))
  (bind _count_trisigns_on_lvl (Variables|Default|GetCount%20Trisigns%20on%20Lvl))
  (bind _value (Utilities|Map|Find _count_trisigns_on_lvl CurrentLocName))
  (bind _returnvalue (+ _value 1))
  (if (< _returnvalue 4)
    (LocalVariables|SetL_CurrentCountCollectedTrisign (Math|Integer|Clamp(Integer) _returnvalue 0 3))
    (Utilities|Map|Add (Variables|Default|GetCount%20Trisigns%20on%20Lvl) CurrentLocName (LocalVariables|GetL_CurrentCountCollectedTrisign))
    (bind _foundwidgets (Widget|GetAllWidgetsOfClass "/Game/Widgets/New/MainInterface_W.MainInterface_W_C" true))
    (Default|UpdateTrisignWidget (Utilities|Array|Get(acopy) _foundwidgets) (LocalVariables|GetL_CurrentCountCollectedTrisign))))

(fn GetCountCollectedTrisignonLoc
  (params (KeyNameLoc :type Name%20%28by%20ref%29))
  (return (.Value (Utilities|Map|Find (Variables|Default|GetCount%20Trisigns%20on%20Lvl) KeyNameLoc))))