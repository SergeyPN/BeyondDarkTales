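; Game instance that holds persistent game state: save data, options, skins, season progress, inventory, play-time clock and audio.
; Init loads or creates the save, then applies graphics, sound and language settings.
; It reconciles skins and season/act/checkpoint progress with the save, appending new content and repairing duplicate equipped skins.
; Music helpers chain intros into level themes and use timers to wait for fade-outs before switching tracks.
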(event Custom|TickTime
  (CallFunction|HandlerTimeGame))

(event EventInit
  (bind _returnvalue (Utilities|Time|SetTimerbyEvent (delegate Custom|TickTime) 1.0 true))
  (Variables|Default|SetTimerGameTime _returnvalue)
  (bind _returnvalue_2 (SaveGame|DoesSaveGameExist "1"))
  (if _returnvalue_2
    (bind _returnvalue_3 (SaveGame|LoadGamefromSlot "1"))
    (bind _asbp_save_game (Utilities|Casting|CastToBP_SaveGame _returnvalue_3))
    (bind _output_get (Variables|SaveForSaveGame|SetSaveGame _asbp_save_game))
    (Utilities|FlowControl|Delay 0.2)
    (CallFunction|InitOptions _output_get)
    (CallFunction|InitPurchasesPlayer)
    (CallFunction|InitWalkthrough)
    (else
      (bind _returnvalue_4 (SaveGame|CreateSaveGameObject "/Game/Blueprints/SaveGame/BP_SaveGame.BP_SaveGame_C"))
      (bind _output_get_2 (Variables|SaveForSaveGame|SetSaveGame _returnvalue_4))
      (SaveGame|SaveGametoSlot _output_get_2 "1"))))

(fn InitOptions
  (params (SaveGame :type BP%20Save%20Game%20Object%20Reference))
  (LocalVariables|SetLSaveGame SaveGame)
  ;[1 1 1] AntiAliasing
  (Development|ExecuteConsoleCommand (Utilities|String|Append "r.MobileMSAA" " " (Utilities|String|ToString(Integer) (Variables|/Game/Blueprints/SaveGame/BP_SaveGame.BP_SaveGame_C|GetAntiAliasing (LocalVariables|GetLSaveGame)))) (Game|GetPlayerController 0))
  ;[1 1 1] Material Quality
  (Development|ExecuteConsoleCommand (Utilities|String|Append "r.MaterialQualityLevel" " " (Utilities|String|ToString(Integer) (Variables|/Game/Blueprints/SaveGame/BP_SaveGame.BP_SaveGame_C|GetMaterialQualityLvl (LocalVariables|GetLSaveGame)))) (Game|GetPlayerController 0))
  ;[1 1 1] Sound
  (Audio|SetSoundMixClassOverride "/Game/Audio/SCM_Main_Mix.SCM_Main_Mix" "/Engine/EngineSounds/Master.Master" (Variables|/Game/Blueprints/SaveGame/BP_SaveGame.BP_SaveGame_C|GetAllSoundInGame (LocalVariables|GetLSaveGame)) 1.0 0.0 true)
  (Audio|PushSoundMixModifier "/Game/Audio/SCM_Main_Mix.SCM_Main_Mix")
  (Utilities|FlowControl|Sequence
    (:then_0
      (Audio|SetSoundMixClassOverride "/Game/Audio/SCM_MAX_FS.SCM_Max_FS" "/Game/Audio/SC_MAX_FS.SC_Max_FS" (Variables|/Game/Blueprints/SaveGame/BP_SaveGame.BP_SaveGame_C|GetSoundsValue (Variables|SaveForSaveGame|GetSaveGame)) 1.0 0.0 true)
      (Audio|PushSoundMixModifier "/Game/Audio/SCM_MAX_FS.SCM_Max_FS"))
    (:then_1
      (Audio|SetSoundMixClassOverride "/Game/Audio/SCM_Music.SCM_Music" "/Game/Audio/SC_Music_BUS.SC_Music_BUS" (Variables|/Game/Blueprints/SaveGame/BP_SaveGame.BP_SaveGame_C|GetMusicValue (Variables|SaveForSaveGame|GetSaveGame)) 1.0 0.0 true)
      (Audio|PushSoundMixModifier "/Game/Audio/SCM_Music.SCM_Music")))
  (Variables|SaveForSaveGame|SetLanguageSelectionChosen? (Variables|/Game/Blueprints/SaveGame/BP_SaveGame.BP_SaveGame_C|GetLanguageSelectionChosen? (Variables|SaveForSaveGame|GetSaveGame)))
  (Variables|SaveforSaveGame|SetLanguage (Variables|/Game/Blueprints/SaveGame/BP_SaveGame.BP_SaveGame_C|GetGameLanguage (Variables|SaveForSaveGame|GetSaveGame))))

(fn AddItemtoInventory
  (params (NewItem :type Inventory%20Items%20Structure))
  (LocalVariables|SetLNewItem NewItem)
  (if (Utilities|Array|IsValidIndex (Variables|SaveOnlyGameInstance|GetInventoryItems))
    (bind (_array_element _array_index) (Utilities|Array|ForEachLoopwithBreak (Variables|SaveOnlyGameInstance|GetInventoryItems) :!label _label)
      (:LoopBody
        (if (== (.Type (Utilities|Struct|BreakInventoryItems _array_element)) (.Type (Utilities|Struct|BreakInventoryItems (LocalVariables|GetLNewItem))))
          (LocalVariables|SetLBreak true)
          (Utilities|Array|SetArrayElem (Variables|SaveOnlyGameInstance|GetInventoryItems) _array_index (Utilities|Struct|MakeInventoryItems (.NameRus (Utilities|Struct|BreakInventoryItems _array_element)) (.NameEng (Utilities|Struct|BreakInventoryItems _array_element)) (.Type (Utilities|Struct|BreakInventoryItems _array_element)) (.Icon (Utilities|Struct|BreakInventoryItems _array_element)) (+ (.Amount (Utilities|Struct|BreakInventoryItems _array_element)) 1)))
          (goto _label Break)))
      (:Completed
        (if (LocalVariables|GetLBreak)
          (LocalVariables|SetLBreak false)
          (else
            (Utilities|Array|Add (Variables|SaveOnlyGameInstance|GetInventoryItems) (LocalVariables|GetLNewItem))))
        (LocalVariables|SetLNewItem (Utilities|Struct|MakeInventoryItems "" "" "NewEnumerator4" "/Game/Assets/UI/ItemImages/T_Clear.T_Clear"))))
    (else
      (Utilities|Array|Add (Variables|SaveOnlyGameInstance|GetInventoryItems) (LocalVariables|GetLNewItem)))))

(fn RemoveItemfromInventory
  (params (RemoveIndexItem :type Integer))
  (Utilities|Array|RemoveIndex (Variables|SaveOnlyGameInstance|GetInventoryItems) (- RemoveIndexItem 1))
  (bind _foundwidgets (Widget|GetAllWidgetsOfClass "/Game/Widgets/New/MainInterface_W.MainInterface_W_C" true))
  (Default|UpdateExistingInventort (Variables|/Game/Widgets/New/MainInterface_W.MainInterface_W_C|GetWB_Inventory (Utilities|Array|Get(acopy) _foundwidgets)) RemoveIndexItem))

(fn InitPurchasesPlayer
  (for (_array_element _array_index) (Variables|BDSave|GetSkins)
    (if (and (Utilities|Enum|NotEqual(Enum) (.StatusSkin (Utilities|Struct|BreakStruct_Skins _array_element)) "NewEnumerator2") (Utilities|Enum|Equal(Enum) (.StatusSkin (Utilities|Struct|BreakStruct_Skins (Utilities|Array|Get(acopy) (Variables|/Game/Blueprints/SaveGame/BP_SaveGame.BP_SaveGame_C|GetSkins (Variables|SaveForSaveGame|GetSaveGame)) _array_index))) "NewEnumerator2"))
      (Utilities|Array|SetArrayElem (Variables|/Game/Blueprints/SaveGame/BP_SaveGame.BP_SaveGame_C|GetSkins (Variables|SaveForSaveGame|GetSaveGame)) _array_index _array_element)
      (else
        (Utilities|Array|SetArrayElem (Variables|BDSave|GetSkins) _array_index (Utilities|Array|Get(acopy) (Variables|/Game/Blueprints/SaveGame/BP_SaveGame.BP_SaveGame_C|GetSkins (Variables|SaveForSaveGame|GetSaveGame)) _array_index))))
    ;[1 1 1] Check for bug 2 equip skins
    (if (Utilities|Enum|Equal(Enum) (.StatusSkin (Utilities|Struct|BreakStruct_Skins (Utilities|Array|Get(acopy) (Variables|/Game/Blueprints/SaveGame/BP_SaveGame.BP_SaveGame_C|GetSkins (Variables|SaveForSaveGame|GetSaveGame)) _array_index))) "NewEnumerator0")
      (Math|Integer|IncrementInt (LocalVariables|GetCounterEquipSkins)
        (:%20%20
          (if (> (LocalVariables|GetCounterEquipSkins) 1)
            (Utilities|Array|SetArrayElem (Variables|/Game/Blueprints/SaveGame/BP_SaveGame.BP_SaveGame_C|GetSkins (Variables|SaveForSaveGame|GetSaveGame)) _array_index (Utilities|Struct|MakeStruct_Skins (.ImageEquipNormal (Utilities|Struct|BreakStruct_Skins (Utilities|Array|Get(acopy) (Variables|/Game/Blueprints/SaveGame/BP_SaveGame.BP_SaveGame_C|GetSkins (Variables|SaveForSaveGame|GetSaveGame)) _array_index))) (.ImageEquipPressed (Utilities|Struct|BreakStruct_Skins (Utilities|Array|Get(acopy) (Variables|/Game/Blueprints/SaveGame/BP_SaveGame.BP_SaveGame_C|GetSkins (Variables|SaveForSaveGame|GetSaveGame)) _array_index))) (.ImageBoughtNormal (Utilities|Struct|BreakStruct_Skins (Utilities|Array|Get(acopy) (Variables|/Game/Blueprints/SaveGame/BP_SaveGame.BP_SaveGame_C|GetSkins (Variables|SaveForSaveGame|GetSaveGame)) _array_index))) (.ImageBoughtPressed (Utilities|Struct|BreakStruct_Skins (Utilities|Array|Get(acopy) (Variables|/Game/Blueprints/SaveGame/BP_SaveGame.BP_SaveGame_C|GetSkins (Variables|SaveForSaveGame|GetSaveGame)) _array_index))) (.ImageSaleNormal (Utilities|Struct|BreakStruct_Skins (Utilities|Array|Get(acopy) (Variables|/Game/Blueprints/SaveGame/BP_SaveGame.BP_SaveGame_C|GetSkins (Variables|SaveForSaveGame|GetSaveGame)) _array_index))) (.ImageSalePressed (Utilities|Struct|BreakStruct_Skins (Utilities|Array|Get(acopy) (Variables|/Game/Blueprints/SaveGame/BP_SaveGame.BP_SaveGame_C|GetSkins (Variables|SaveForSaveGame|GetSaveGame)) _array_index))) "NewEnumerator3" (.Mesh (Utilities|Struct|BreakStruct_Skins (Utilities|Array|Get(acopy) (Variables|/Game/Blueprints/SaveGame/BP_SaveGame.BP_SaveGame_C|GetSkins (Variables|SaveForSaveGame|GetSaveGame)) _array_index))) (.ProductIndetifier (Utilities|Struct|BreakStruct_Skins (Utilities|Array|Get(acopy) (Variables|/Game/Blueprints/SaveGame/BP_SaveGame.BP_SaveGame_C|GetSkins (Variables|SaveForSaveGame|GetSaveGame)) _array_index)))))
            (Utilities|Array|SetArrayElem (Variables|BDSave|GetSkins) _array_index (Utilities|Struct|MakeStruct_Skins (.ImageEquipNormal (Utilities|Struct|BreakStruct_Skins (Utilities|Array|Get(acopy) (Variables|BDSave|GetSkins) _array_index))) (.ImageEquipPressed (Utilities|Struct|BreakStruct_Skins (Utilities|Array|Get(acopy) (Variables|BDSave|GetSkins) _array_index))) (.ImageBoughtNormal (Utilities|Struct|BreakStruct_Skins (Utilities|Array|Get(acopy) (Variables|BDSave|GetSkins) _array_index))) (.ImageBoughtPressed (Utilities|Struct|BreakStruct_Skins (Utilities|Array|Get(acopy) (Variables|BDSave|GetSkins) _array_index))) (.ImageSaleNormal (Utilities|Struct|BreakStruct_Skins (Utilities|Array|Get(acopy) (Variables|BDSave|GetSkins) _array_index))) (.ImageSalePressed (Utilities|Struct|BreakStruct_Skins (Utilities|Array|Get(acopy) (Variables|BDSave|GetSkins) _array_index))) "NewEnumerator3" (.Mesh (Utilities|Struct|BreakStruct_Skins (Utilities|Array|Get(acopy) (Variables|BDSave|GetSkins) _array_index))) (.ProductIndetifier (Utilities|Struct|BreakStruct_Skins (Utilities|Array|Get(acopy) (Variables|BDSave|GetSkins) _array_index)))))
            (LocalVariables|SetCounterEquipSkins 1))))))
  (LocalVariables|SetCounterEquipSkins 0)
  (SaveGame|SaveGametoSlot (Variables|SaveForSaveGame|GetSaveGame) "1")
  (return))

(fn InitWalkthrough
  (bind _season (Variables|SaveForSaveGame|GetSeason))
  (bind _savegame (Variables|SaveForSaveGame|GetSaveGame))
  (bind _returnvalue (Utilities|Array|Length _season))
  (bind _season_2 (Variables|/Game/Blueprints/SaveGame/BP_SaveGame.BP_SaveGame_C|GetSeason _savegame))
  (bind _returnvalue_2 (Utilities|Array|Length _season_2))
  ;[1 1 1] Change count Seasons
  (if (> _returnvalue _returnvalue_2)
    (for _index (range 0 (- _returnvalue 1))
      (if (> _index (- _returnvalue_2 1))
        (Utilities|Array|Add (Variables|/Game/Blueprints/SaveGame/BP_SaveGame.BP_SaveGame_C|GetSeason (Variables|SaveForSaveGame|GetSaveGame)) (Utilities|Array|Get(acopy) (Variables|SaveForSaveGame|GetSeason) _index)))))
  ;[1 1 1] Change count Acts
  (for (_array_element _array_index) (Variables|SaveForSaveGame|GetSeason)
    (if (> (Utilities|Array|Length (.Acts (Utilities|Struct|BreakStruct_Season _array_element))) (Utilities|Array|Length (.Acts (Utilities|Struct|BreakStruct_Season (Utilities|Array|Get(acopy) (Variables|/Game/Blueprints/SaveGame/BP_SaveGame.BP_SaveGame_C|GetSeason (Variables|SaveForSaveGame|GetSaveGame)) _array_index)))))
      (for _index_2 (range 0 (- (Utilities|Array|Length (.Acts (Utilities|Struct|BreakStruct_Season _array_element))) 1))
        (if (> _index_2 (- (Utilities|Array|Length (.Acts (Utilities|Struct|BreakStruct_Season (Utilities|Array|Get(acopy) (Variables|/Game/Blueprints/SaveGame/BP_SaveGame.BP_SaveGame_C|GetSeason (Variables|SaveForSaveGame|GetSaveGame)) _array_index)))) 1))
          (Utilities|Array|Add (.Acts (Utilities|Struct|BreakStruct_Season (Utilities|Array|Get(acopy) (Variables|/Game/Blueprints/SaveGame/BP_SaveGame.BP_SaveGame_C|GetSeason (Variables|SaveForSaveGame|GetSaveGame)) _array_index))) (Utilities|Array|Get(acopy) (.Acts (Utilities|Struct|BreakStruct_Season _array_element)) _index_2))))))
  ;[1 1 1] Change count CheckPoints
  (for (_array_element_2 _array_index_2) (Variables|SaveForSaveGame|GetSeason)
    (for (_array_element_3 _array_index_3) (.Acts (Utilities|Struct|BreakStruct_Season _array_element_2))
      (if (> (Utilities|Array|Length (.Chekpoint (Utilities|Struct|BreakStruct_Act _array_element_3))) (Utilities|Array|Length (.Chekpoint (Utilities|Struct|BreakStruct_Act (Utilities|Array|Get(acopy) (.Acts (Utilities|Struct|BreakStruct_Season (Utilities|Array|Get(acopy) (Variables|/Game/Blueprints/SaveGame/BP_SaveGame.BP_SaveGame_C|GetSeason (Variables|SaveForSaveGame|GetSaveGame)) _array_index_2))) _array_index_3)))))
        (for _index_3 (range 0 (- (Utilities|Array|Length (.Chekpoint (Utilities|Struct|BreakStruct_Act _array_element_3))) 1))
          (if (> _index_3 (- (Utilities|Array|Length (.Chekpoint (Utilities|Struct|BreakStruct_Act (Utilities|Array|Get(acopy) (.Acts (Utilities|Struct|BreakStruct_Season (Utilities|Array|Get(acopy) (Variables|/Game/Blueprints/SaveGame/BP_SaveGame.BP_SaveGame_C|GetSeason (Variables|SaveForSaveGame|GetSaveGame)) _array_index_2))) _array_index_3)))) 1))
            (Utilities|Array|Add (.Chekpoint (Utilities|Struct|BreakStruct_Act (Utilities|Array|Get(acopy) (.Acts (Utilities|Struct|BreakStruct_Season (Utilities|Array|Get(acopy) (Variables|/Game/Blueprints/SaveGame/BP_SaveGame.BP_SaveGame_C|GetSeason (Variables|SaveForSaveGame|GetSaveGame)) _array_index_2))) _array_index_3))) (Utilities|Array|Get(acopy) (.Chekpoint (Utilities|Struct|BreakStruct_Act _array_element_3)) _index_3)))))))
  (for (_array_element_4 _array_index_4) (Variables|SaveForSaveGame|GetSeason)
    (LocalVariables|SetLSeasonIndex _array_index_4)
    ;[1 1 1] Change accesss season
    (if (and (Math|Boolean|NotEqual(Boolean) (.Access? (Utilities|Struct|BreakStruct_Season _array_element_4)) false) (Math|Boolean|Equal(Boolean) (.Access? (Utilities|Struct|BreakStruct_Season (Utilities|Array|Get(acopy) (Variables|/Game/Blueprints/SaveGame/BP_SaveGame.BP_SaveGame_C|GetSeason (Variables|SaveForSaveGame|GetSaveGame)) _array_index_4))) false))
      (Utilities|Array|SetArrayElem (Variables|/Game/Blueprints/SaveGame/BP_SaveGame.BP_SaveGame_C|GetSeason (Variables|SaveForSaveGame|GetSaveGame)) _array_index_4 (Utilities|Struct|MakeStruct_Season true (.Acts (Utilities|Struct|BreakStruct_Season _array_element_4))))
      (else
        (Utilities|Array|SetArrayElem (Variables|SaveForSaveGame|GetSeason) _array_index_4 (Utilities|Struct|MakeStruct_Season (.Access? (Utilities|Struct|BreakStruct_Season (Utilities|Array|Get(acopy) (Variables|/Game/Blueprints/SaveGame/BP_SaveGame.BP_SaveGame_C|GetSeason (Variables|SaveForSaveGame|GetSaveGame)) _array_index_4))) (.Acts (Utilities|Struct|BreakStruct_Season (Utilities|Array|Get(acopy) (Variables|SaveForSaveGame|GetSeason) _array_index_4)))))))
    (for (_array_element_5 _array_index_5) (.Acts (Utilities|Struct|BreakStruct_Season _array_element_4))
      ;[1 1 1] Change Access Act
      (LocalVariables|SetLActIndex _array_index_5)
      (LocalVariables|SetLActGameInstance _array_element_5)
      (if (and (Math|Boolean|NotEqual(Boolean) (.Access? (Utilities|Struct|BreakStruct_Act _array_element_5)) false) (Math|Boolean|Equal(Boolean) (.Access? (Utilities|Struct|BreakStruct_Act (Utilities|Array|Get(acopy) (.Acts (Utilities|Struct|BreakStruct_Season (Utilities|Array|Get(acopy) (Variables|/Game/Blueprints/SaveGame/BP_SaveGame.BP_SaveGame_C|GetSeason (Variables|SaveForSaveGame|GetSaveGame)) (LocalVariables|GetLSeasonIndex)))) _array_index_5))) false))
        (Utilities|Array|SetArrayElem (.Acts (Utilities|Struct|BreakStruct_Season (Utilities|Array|Get(acopy) (Variables|/Game/Blueprints/SaveGame/BP_SaveGame.BP_SaveGame_C|GetSeason (Variables|SaveForSaveGame|GetSaveGame)) (LocalVariables|GetLSeasonIndex)))) (LocalVariables|GetLActIndex) (Utilities|Struct|MakeStruct_Act (.Access? (Utilities|Struct|BreakStruct_Act _array_element_5)) (.CountCollectedTriSigns (Utilities|Struct|BreakStruct_Act (Utilities|Array|Get(acopy) (.Acts (Utilities|Struct|BreakStruct_Season (Utilities|Array|Get(acopy) (Variables|/Game/Blueprints/SaveGame/BP_SaveGame.BP_SaveGame_C|GetSeason (Variables|SaveForSaveGame|GetSaveGame)) (LocalVariables|GetLSeasonIndex)))) _array_index_5))) (.Chekpoint (Utilities|Struct|BreakStruct_Act (Utilities|Array|Get(acopy) (.Acts (Utilities|Struct|BreakStruct_Season (Utilities|Array|Get(acopy) (Variables|/Game/Blueprints/SaveGame/BP_SaveGame.BP_SaveGame_C|GetSeason (Variables|SaveForSaveGame|GetSaveGame)) (LocalVariables|GetLSeasonIndex)))) _array_index_5)))))
        (else
          (Utilities|Array|SetArrayElem (.Acts (Utilities|Struct|BreakStruct_Season (Utilities|Array|Get(acopy) (Variables|SaveForSaveGame|GetSeason) (LocalVariables|GetLSeasonIndex)))) (LocalVariables|GetLActIndex) (Utilities|Struct|MakeStruct_Act (.Access? (Utilities|Struct|BreakStruct_Act (Utilities|Array|Get(acopy) (.Acts (Utilities|Struct|BreakStruct_Season (Utilities|Array|Get(acopy) (Variables|/Game/Blueprints/SaveGame/BP_SaveGame.BP_SaveGame_C|GetSeason (Variables|SaveForSaveGame|GetSaveGame)) (LocalVariables|GetLSeasonIndex)))) (LocalVariables|GetLActIndex)))) (.CountCollectedTriSigns (Utilities|Struct|BreakStruct_Act (Utilities|Array|Get(acopy) (.Acts (Utilities|Struct|BreakStruct_Season (Utilities|Array|Get(acopy) (Variables|SaveForSaveGame|GetSeason) (LocalVariables|GetLSeasonIndex)))) (LocalVariables|GetLActIndex)))) (.Chekpoint (Utilities|Struct|BreakStruct_Act (Utilities|Array|Get(acopy) (.Acts (Utilities|Struct|BreakStruct_Season (Utilities|Array|Get(acopy) (Variables|SaveForSaveGame|GetSeason) (LocalVariables|GetLSeasonIndex)))) (LocalVariables|GetLActIndex))))))))
      ;[1 1 1] Change count TriSign
      (if (> (.countcollectedtrisigns (LocalVariables|GetLActGameInstance)) (.CountCollectedTriSigns (Utilities|Struct|BreakStruct_Act (Utilities|Array|Get(acopy) (.Acts (Utilities|Struct|BreakStruct_Season (Utilities|Array|Get(acopy) (Variables|/Game/Blueprints/SaveGame/BP_SaveGame.BP_SaveGame_C|GetSeason (Variables|SaveForSaveGame|GetSaveGame)) (LocalVariables|GetLSeasonIndex)))) (LocalVariables|GetLActIndex)))))
        (Utilities|Array|SetArrayElem (.Acts (Utilities|Struct|BreakStruct_Season (Utilities|Array|Get(acopy) (Variables|/Game/Blueprints/SaveGame/BP_SaveGame.BP_SaveGame_C|GetSeason (Variables|SaveForSaveGame|GetSaveGame)) (LocalVariables|GetLSeasonIndex)))) (LocalVariables|GetLActIndex) (Utilities|Struct|MakeStruct_Act (.Access? (Utilities|Struct|BreakStruct_Act (Utilities|Array|Get(acopy) (.Acts (Utilities|Struct|BreakStruct_Season (Utilities|Array|Get(acopy) (Variables|/Game/Blueprints/SaveGame/BP_SaveGame.BP_SaveGame_C|GetSeason (Variables|SaveForSaveGame|GetSaveGame)) (LocalVariables|GetLSeasonIndex)))) (LocalVariables|GetLActIndex)))) (.countcollectedtrisigns (LocalVariables|GetLActGameInstance)) (.Chekpoint (Utilities|Struct|BreakStruct_Act (Utilities|Array|Get(acopy) (.Acts (Utilities|Struct|BreakStruct_Season (Utilities|Array|Get(acopy) (Variables|/Game/Blueprints/SaveGame/BP_SaveGame.BP_SaveGame_C|GetSeason (Variables|SaveForSaveGame|GetSaveGame)) (LocalVariables|GetLSeasonIndex)))) (LocalVariables|GetLActIndex))))))
        (else
          (Utilities|Array|SetArrayElem (.Acts (Utilities|Struct|BreakStruct_Season (Utilities|Array|Get(acopy) (Variables|SaveForSaveGame|GetSeason) (LocalVariables|GetLSeasonIndex)))) (LocalVariables|GetLActIndex) (Utilities|Struct|MakeStruct_Act (.Access? (Utilities|Struct|BreakStruct_Act (Utilities|Array|Get(acopy) (.Acts (Utilities|Struct|BreakStruct_Season (Utilities|Array|Get(acopy) (Variables|SaveForSaveGame|GetSeason) (LocalVariables|GetLSeasonIndex)))) (LocalVariables|GetLActIndex)))) (.CountCollectedTriSigns (Utilities|Struct|BreakStruct_Act (Utilities|Array|Get(acopy) (.Acts (Utilities|Struct|BreakStruct_Season (Utilities|Array|Get(acopy) (Variables|/Game/Blueprints/SaveGame/BP_SaveGame.BP_SaveGame_C|GetSeason (Variables|SaveForSaveGame|GetSaveGame)) (LocalVariables|GetLSeasonIndex)))) (LocalVariables|GetLActIndex)))) (.Chekpoint (Utilities|Struct|BreakStruct_Act (Utilities|Array|Get(acopy) (.Acts (Utilities|Struct|BreakStruct_Season (Utilities|Array|Get(acopy) (Variables|SaveForSaveGame|GetSeason) (LocalVariables|GetLSeasonIndex)))) (LocalVariables|GetLActIndex))))))))
      ;[1 1 1] Change Count Access checkpoints
      (for (_array_element_6 _array_index_6) (.chekpoint (LocalVariables|GetLActGameInstance))
        (LocalVariables|SetLCheckPointIndex _array_index_6)
        (if (.Access? (Utilities|Struct|BreakStruct_CheckPoint _array_element_6))
          (Utilities|Array|SetArrayElem (.Chekpoint (Utilities|Struct|BreakStruct_Act (Utilities|Array|Get(acopy) (.Acts (Utilities|Struct|BreakStruct_Season (Utilities|Array|Get(acopy) (Variables|/Game/Blueprints/SaveGame/BP_SaveGame.BP_SaveGame_C|GetSeason (Variables|SaveForSaveGame|GetSaveGame)) (LocalVariables|GetLSeasonIndex)))) (LocalVariables|GetLActIndex)))) (LocalVariables|GetLCheckPointIndex) (Utilities|Struct|MakeStruct_CheckPoint (.NumCheckPoint (Utilities|Struct|BreakStruct_CheckPoint (Utilities|Array|Get(acopy) (.chekpoint (LocalVariables|GetLActGameInstance)) (LocalVariables|GetLCheckPointIndex)))) (.Access? (Utilities|Struct|BreakStruct_CheckPoint (Utilities|Array|Get(acopy) (.Chekpoint (Utilities|Struct|BreakStruct_Act (Utilities|Array|Get(acopy) (.Acts (Utilities|Struct|BreakStruct_Season (Utilities|Array|Get(acopy) (Variables|/Game/Blueprints/SaveGame/BP_SaveGame.BP_SaveGame_C|GetSeason (Variables|SaveForSaveGame|GetSaveGame)) (LocalVariables|GetLSeasonIndex)))) (LocalVariables|GetLActIndex)))) (LocalVariables|GetLCheckPointIndex))))))
          (else
            (Utilities|Array|SetArrayElem (.Chekpoint (Utilities|Struct|BreakStruct_Act (Utilities|Array|Get(acopy) (.Acts (Utilities|Struct|BreakStruct_Season (Utilities|Array|Get(acopy) (Variables|SaveForSaveGame|GetSeason) (LocalVariables|GetLSeasonIndex)))) (LocalVariables|GetLActIndex)))) (LocalVariables|GetLCheckPointIndex) (Utilities|Struct|MakeStruct_CheckPoint (.NumCheckPoint (Utilities|Struct|BreakStruct_CheckPoint (Utilities|Array|Get(acopy) (.Chekpoint (Utilities|Struct|BreakStruct_Act (Utilities|Array|Get(acopy) (.Acts (Utilities|Struct|BreakStruct_Season (Utilities|Array|Get(acopy) (Variables|SaveForSaveGame|GetSeason) (LocalVariables|GetLSeasonIndex)))) (LocalVariables|GetLActIndex)))) (LocalVariables|GetLCheckPointIndex)))) (.Access? (Utilities|Struct|BreakStruct_CheckPoint (Utilities|Array|Get(acopy) (.Chekpoint (Utilities|Struct|BreakStruct_Act (Utilities|Array|Get(acopy) (.Acts (Utilities|Struct|BreakStruct_Season (Utilities|Array|Get(acopy) (Variables|/Game/Blueprints/SaveGame/BP_SaveGame.BP_SaveGame_C|GetSeason (Variables|SaveForSaveGame|GetSaveGame)) (LocalVariables|GetLSeasonIndex)))) (LocalVariables|GetLActIndex)))) (LocalVariables|GetLCheckPointIndex)))))))))))
  (return))

(fn HandlerTimeGame
  (bind _output_get (Variables|SaveOnlyGameInstance|SetTimeInGame (Utilities|Struct|MakeStruct_GameTime (.hours (Variables|SaveOnlyGameInstance|GetTimeInGame)) (.minutes (Variables|SaveOnlyGameInstance|GetTimeInGame)) (+ (.seconds (Variables|SaveOnlyGameInstance|GetTimeInGame)) 1))))
  (if (== (.seconds _output_get) 60)
    (bind _output_get_2 (Variables|SaveOnlyGameInstance|SetTimeInGame (Utilities|Struct|MakeStruct_GameTime (.hours (Variables|SaveOnlyGameInstance|GetTimeInGame)) (+ (.minutes (Variables|SaveOnlyGameInstance|GetTimeInGame)) 1) 0)))
    (if (== (.minutes _output_get_2) 60)
      (bind _output_get_3 (Variables|SaveOnlyGameInstance|SetTimeInGame (Utilities|Struct|MakeStruct_GameTime (+ (.hours (Variables|SaveOnlyGameInstance|GetTimeInGame)) 1) 0 0)))
      (if (== (.hours _output_get_3) 24)
        (Variables|SaveOnlyGameInstance|SetTimeInGame (Utilities|Struct|MakeStruct_GameTime 0 0 0))))))

(fn FMusicPlay
  (params (Sound :type Sound%20Base%20Object%20Reference) (FadeInDuration :type Float%20%28single-precision%29) (Type :type MusicType%20Enum :default "NewEnumerator1"))
  (bind _returnvalue (Audio|SpawnSound2D Sound 1.0 1.0 0.0 0 true false))
  (bind _output_get (Variables|Default|SetCurrentMusic _returnvalue))
  (switch Utilities|FlowControl|Switch|SwitchonMusicType Type
    (:NewEnumerator1
      (Audio|Components|Audio|FadeIn (Variables|Default|GetCurrentMusic) FadeInDuration 1.0 0.0 "Linear" :!class /Script/Engine.AudioComponent)
      (return _output_get Sound))
    (:NewEnumerator0
      (return _output_get Sound))))

(fn FMusicStop
  (params (FadeOutDuration :type Float%20%28single-precision%29) (Type :type MusicType%20Enum :default "NewEnumerator1"))
  (bind _currentmusic (Variables|Default|GetCurrentMusic))
  (Utilities|IsValid _currentmusic
    (:Is%20Valid
      (switch Utilities|FlowControl|Switch|SwitchonMusicType Type
        (:NewEnumerator1
          (Audio|Components|Audio|FadeOut _currentmusic FadeOutDuration 0.0 "Sin" :!class /Script/Engine.AudioComponent)
          (Utilities|Time|SetTimerbyFunctionName 0 "F_MusicDestroy" FadeOutDuration))
        (:NewEnumerator0
          (Audio|Components|Audio|Stop _currentmusic)
          (CallFunction|FMusicDestroy)))
      (return))
    (:Is%20Not%20Valid
      (return))))

(fn FMusicDestroy
  (bind _currentmusic (Variables|Default|GetCurrentMusic))
  (Utilities|IsValid _currentmusic
    (:Is%20Valid
      (Components|DestroyComponent _currentmusic))
    (:Is%20Not%20Valid
      _))
  (return))

(fn TMCreateMusic
  (params (HaveIntro? :type Boolean) (IntroSound :type Sound%20Base%20Object%20Reference) (LevelThem :type Sound%20Base%20Object%20Reference))
  (Variables|SoundOnLvls|SetHave%20Intro? HaveIntro?)
  (Variables|SoundOnLvls|SetLevelThem_Intro IntroSound)
  (Variables|SoundOnLvls|SetLevelThem LevelThem)
  (bind _havemusic (CallFunction|TMHavePlayingMusic?))
  (if _havemusic
    (return)
    (else
      (Utilities|IsValid LevelThem
        (:Is%20Valid
          (if HaveIntro?
            (bind _output (CallFunction|FMusicPlay (Variables|SoundOnLvls|GetLevelThem_Intro) 0.0 "NewEnumerator0"))
            (Utilities|Time|SetTimerbyFunctionName 0 "TM_SwitchIntro" (- (Variables|/Script/Engine.SoundBase|GetDuration _output) 0.24))
            (return)
            (else
              (CallFunction|FMusicPlay (Variables|SoundOnLvls|GetLevelThem) 0.0 "NewEnumerator0")
              (return))))
        (:Is%20Not%20Valid
          (return))))))

(fn TMSwitchIntro
  (CallFunction|FMusicPlay (Variables|SoundOnLvls|GetLevelThem) 0.0 "NewEnumerator0")
  (return))

(fn TMHavePlayingMusic?
  (bind _currentmusic (Variables|Default|GetCurrentMusic))
  (Utilities|IsValid _currentmusic
    (:Is%20Valid
      (if (Audio|Components|Audio|IsPlaying _currentmusic)
        (CallFunction|FMusicStop 4.0 "NewEnumerator1")
        (bind _returnvalue (Utilities|Time|SetTimerbyFunctionName 0 "TM_FadeCheck" 0.2 true))
        (Variables|Default|SetFadeTimer _returnvalue)
        (return true)
        (else
          (return false))))
    (:Is%20Not%20Valid
      (return false))))

(fn TMFadeCheck
  (bind _currentmusic (Variables|Default|GetCurrentMusic))
  (Utilities|IsValid _currentmusic
    (:Is%20Valid
      (if (Audio|Components|Audio|IsPlaying _currentmusic)
        (return)
        (else
          _)))
    (:Is%20Not%20Valid
      _))
  (CallFunction|TMCreateMusic (Variables|SoundOnLvls|GetHave%20Intro?) (Variables|SoundOnLvls|GetLevelThem_Intro) (Variables|SoundOnLvls|GetLevelThem))
  (return))

(fn SFXSpawn
  (params (Sound :type Sound%20Base%20Object%20Reference))
  (bind _returnvalue (Audio|SpawnSound2D Sound 1.0 1.0 0.0 0))
  (Variables|Default|SetSFX _returnvalue)
  (return))

(fn DestroySFX
  (Class|AudioComponent|SetPaused (Variables|Default|GetSFX) true)
  (Components|DestroyComponent (Variables|Default|GetSFX))
  (Variables|Default|SetSFX 0)
  (return))